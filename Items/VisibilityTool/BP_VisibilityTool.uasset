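; Held visibility tool that shows or hides nearby pipes, wires and fence foundations.
; Targeting toggles Show/Hide mode, notifying the player and swapping the tool's material, while raw mouse and trigger keys play animations.
; Fire runs an octree query for structures around the pawn and updates those the player can access, or all three types if cheats are allowed.
; Input is enabled after a short BeginPlay delay for the local owner.
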(event Custom|HandleFireEvent
  (params (IsShowMode :type Boolean))
  (CallFunction|HandleToggleVisibility IsShowMode))

(event EventBeginPlay
  (Utilities|FlowControl|Delay 0.2)
  (bind _returnvalue (Class|Actor|GetOwnerController))
  (if (Pawn|IsLocalController _returnvalue)
    (Input|EnableInput _returnvalue)))

(event Input|ActionEvents|InputActionGamepadRightFire
  (:Pressed
    (CallFunction|HandleFireEvent (Variables|Default|GetIsShowMode))))

(event Input|ActionEvents|InputActionGamepadLeftFire
  (bind _mesh1p (Variables|Default|GetMesh1P))
  (:Pressed
    (Variables|Default|SetIsShowMode (not (Variables|Default|GetIsShowMode)))
    (bind _returnvalue (Class|Actor|GetOwnerController))
    (bind _asshooterplayercontroller (Utilities|Casting|CastToShooterPlayerController _returnvalue))
    (Class|ShooterPlayerController|ClientServerNotification _asshooterplayercontroller (Utilities|String|SelectString "Show Mode Enabled" "Hide Mode Enabled" (Variables|Default|GetIsShowMode)) "(R=0.249093,G=0.164050,B=0.965000,A=1.000000)" 1.5 3.0)
    (if (Variables|Default|GetIsShowMode)
      (Rendering|Material|SetMaterial _mesh1p 0 "/Game/PrimalEarth/WeaponGrenade/grenade_Mat_Ins.grenade_Mat_Ins")
      (else
        (Rendering|Material|SetMaterial _mesh1p 0 "/Game/PrimalEarth/Test_Efecto/WaterPipeSystem/WaterPipe_Materials/NM_WaterPipeWatered_MIC.NM_WaterPipeWatered_MIC")))))

(event Input|ActionEvents|InputActionFire
  (:Pressed
    (CallFunction|HandleFireEvent (Variables|Default|GetIsShowMode))))

(event Input|ActionEvents|InputActionTargeting
  (bind _mesh1p (Variables|Default|GetMesh1P))
  (:Pressed
    (Variables|Default|SetIsShowMode (not (Variables|Default|GetIsShowMode)))
    (bind _returnvalue (Class|Actor|GetOwnerController))
    (bind _asshooterplayercontroller (Utilities|Casting|CastToShooterPlayerController _returnvalue))
    (Class|ShooterPlayerController|ClientServerNotification _asshooterplayercontroller (Utilities|String|SelectString "Show Mode Enabled" "Hide Mode Enabled" (Variables|Default|GetIsShowMode)) "(R=0.249093,G=0.164050,B=0.965000,A=1.000000)" 1.5 3.0)
    (if (Variables|Default|GetIsShowMode)
      (Rendering|Material|SetMaterial _mesh1p 0 "/Game/PrimalEarth/WeaponGrenade/grenade_Mat_Ins.grenade_Mat_Ins")
      (else
        (Rendering|Material|SetMaterial _mesh1p 0 "/Game/PrimalEarth/Test_Efecto/WaterPipeSystem/WaterPipe_Materials/NM_WaterPipeWatered_MIC.NM_WaterPipeWatered_MIC")))))

(event Input|GamepadEvents|GamepadRightTrigger
  (:Pressed
    (Class|ShooterWeapon|PlayWeaponAnimation (Variables|Default|GetMeleeAnim) false false false false false false)))

(event Input|GamepadEvents|GamepadLeftTrigger
  (:Pressed
    (Class|ShooterWeapon|PlayWeaponAnimation (Variables|Default|GetReloadAnim) false false false false false false)))

(event Input|MouseEvents|LeftMouseButton
  (:Pressed
    (Class|ShooterWeapon|PlayWeaponAnimation (Variables|Default|GetMeleeAnim) false false false false false false)))

(event Input|MouseEvents|RightMouseButton
  (:Pressed
    (Class|ShooterWeapon|PlayWeaponAnimation (Variables|Default|GetReloadAnim) false false false false false false)))

(fn ConstructionScript)

(fn HandleToggleVisibility
  (params (IsShowMode :type Boolean))
  (bind _returnvalue (not IsShowMode))
  (bind _returnvalue_2 (Class|Actor|GetOwnerController))
  (bind _asshooterplayercontroller (Utilities|Casting|CastToShooterPlayerController _returnvalue_2))
  (bind _asshootergamemode (Utilities|Casting|CastToShooterGameMode (Game|GetGameMode)))
  (bind _returnvalue_3 (Class|ShooterGameMode|IsPlayerAllowedtoCheat _asshootergamemode _asshooterplayercontroller))
  (bind _returnvalue_4 (Class|VictoryCore|ServerOctreeOverlapActorsClass (Class|Actor|GetWorld _returnvalue_2) (Transformation|GetActorLocation (Pawn|GetControlledPawn _returnvalue_2)) 1e+04 "STRUCTURES" "/Script/ShooterGame.PrimalStructure" false))
  (for _array_element _returnvalue_4
    (bind _asprimalstructure (Utilities|Casting|CastToPrimalStructure _array_element))
    (bind _returnvalue_5 (Class|PrimalStructure|AllowStructureAccess _asprimalstructure _returnvalue_2))
    (if (or _returnvalue_5 _returnvalue_3)
      (bind _asbase_pipe_c (Utilities|Casting|CastToBase_Pipe _array_element)
        (:then
          (Default|UpdateSelf _asbase_pipe_c _returnvalue))
        (:CastFailed
          (bind _asbase_wire_c (Utilities|Casting|CastToBase_Wire _array_element)
            (:then
              (Default|UpdateSelf _asbase_wire_c _returnvalue))
            (:CastFailed
              (bind _asbase_fencefoundation_c (Utilities|Casting|CastToBase_FenceFoundation _array_element))
              (Default|UpdateVisibilityEvent _asbase_fencefoundation_c _returnvalue))))))))