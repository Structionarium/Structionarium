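; Held Inventory Assistant item that acts as the player's control for the Structures Plus Inventory Assistant buff.
; After a short BeginPlay delay it enables input for the local controller, while the authority finds or adds the buff on the player character and caches it.
; Fire opens the buff's UI and Targeting toggles its active state via MulticastProperty, with gamepad equivalents and a shared secondary-action animation.
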(event Custom|OpenUIEvent
  (bind _buffref (Variables|Default|GetBuffRef))
  (Utilities|IsValid _buffref
    (:Is%20Valid
      (Default|InitializeUI _buffref self))))

(event Custom|ToggleActivationEvent
  (bind _buffref (Variables|Default|GetBuffRef))
  (Utilities|IsValid _buffref
    (:Is%20Valid
      (Variables|/Game/Mods/StructuresPlusMod/_Buffs/Buff_StructuresPlus_InventoryAssistant.Buff_StructuresPlus_InventoryAssistant_C|SetIsActive _buffref (not (Variables|/Game/Mods/StructuresPlusMod/_Buffs/Buff_StructuresPlus_InventoryAssistant.Buff_StructuresPlus_InventoryAssistant_C|GetIsActive _buffref)) false)
      (Class|Actor|MulticastProperty _buffref "IsActive"))))

(event EventBeginPlay
  (Utilities|FlowControl|Delay 0.2)
  (bind _returnvalue (Class|Actor|GetOwnerController))
  (Utilities|FlowControl|Sequence
    (:then_0
      (if (Pawn|IsLocalController _returnvalue)
        (Input|EnableInput _returnvalue)))
    (:then_1
      (Networking|SwitchHasAuthority
        (:Authority
          (bind _asshooterplayercontroller (Utilities|Casting|CastToShooterPlayerController _returnvalue))
          (bind _returnvalue_2 (Class|PrimalCharacter|GetBuff (Class|ShooterPlayerController|GetPlayerCharacter _asshooterplayercontroller) "/Game/Mods/StructuresPlusMod/_Buffs/Buff_StructuresPlus_InventoryAssistant.Buff_StructuresPlus_InventoryAssistant_C"))
          (Utilities|IsValid _returnvalue_2
            (:Is%20Valid
              (bind _asbuff_structuresplus_inventoryassistant_c (Utilities|Casting|CastToBuff_StructuresPlus_InventoryAssistant _returnvalue_2))
              (Variables|Default|SetBuffRef _asbuff_structuresplus_inventoryassistant_c))
            (:Is%20Not%20Valid
              (bind _returnvalue_3 (Class|PrimalBuff|StaticAddBuff "/Game/Mods/StructuresPlusMod/_Buffs/Buff_StructuresPlus_InventoryAssistant.Buff_StructuresPlus_InventoryAssistant_C" (Class|ShooterPlayerController|GetPlayerCharacter _asshooterplayercontroller) 0 0 false))
              (bind _asbuff_structuresplus_inventoryassistant_c_2 (Utilities|Casting|CastToBuff_StructuresPlus_InventoryAssistant _returnvalue_3))
              (Variables|Default|SetBuffRef _asbuff_structuresplus_inventoryassistant_c_2))))))))

(event Input|ActionEvents|InputActionGamepadRightFire
  (:Pressed
    (CallFunction|OpenUIEvent)
    (Class|ShooterWeapon|PlayWeaponAnimation (Variables|Default|GetSecondaryActionAnim) false false false false false false)))

(event Input|ActionEvents|InputActionGamepadLeftFire
  (:Pressed
    (CallFunction|ToggleActivationEvent)
    (Class|ShooterWeapon|PlayWeaponAnimation (Variables|Default|GetSecondaryActionAnim) false false false false false false)))

(event Input|ActionEvents|InputActionTargeting
  (:Pressed
    (CallFunction|ToggleActivationEvent)
    (Class|ShooterWeapon|PlayWeaponAnimation (Variables|Default|GetSecondaryActionAnim) false false false false false false)))

(event Input|ActionEvents|InputActionFire
  (:Pressed
    (CallFunction|OpenUIEvent)
    (Class|ShooterWeapon|PlayWeaponAnimation (Variables|Default|GetSecondaryActionAnim) false false false false false false)))

(fn ConstructionScript)