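; Handheld underwater tool weapon that edits portholes and side locking on underwater base structures.
; Targeting input cycles five modes (open, close/unfreeze, freeze, lock sides, unlock sides), showing a notification and recoloring the gun's dynamic material.
; Fire line-traces from the muzzle for accessible same-team structure components, then dispatches by mode.
; Porthole handlers map component names to TryMultiUse indices, offset for freezing, while side locking sets and multicasts LockSides.
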(event Custom|ExecuteChangesEvent
  (params (Components :type Array%20of%20Primitive%20Component%20Object%20References) (ChangeType :type Integer))
  (switch int ChangeType
    (:0
      (CallFunction|HandleOpen Components))
    (:1
      (CallFunction|HandleClose Components))
    (:2
      (CallFunction|HandleFreeze Components))
    (:3
      (CallFunction|HandleLockToggle Components true))
    (:4
      (CallFunction|HandleLockToggle Components false))))

(event EventBeginPlay
  (Utilities|FlowControl|Delay 0.2)
  (bind _returnvalue (Class|Actor|GetOwnerController))
  (if (Pawn|IsLocalController _returnvalue)
    (Input|EnableInput _returnvalue)
    (bind _asshooterplayercontroller (Utilities|Casting|CastToShooterPlayerController _returnvalue))
    (Class|ShooterPlayerController|ClientServerNotification _asshooterplayercontroller "Open Mode" "(R=0.249093,G=0.164050,B=0.965000,A=1.000000)" 1.5 3.0)))

(event Input|ActionEvents|InputActionGamepadRightFire
  (:Pressed
    (bind _returnvalue (Class|Actor|GetOwnerController))
    (Utilities|SPIsPlacingStructure _returnvalue
      (:No
        (Utilities|SPIsRadialMenuOpen _returnvalue
          (:No
            (bind _hitcomponents (CallFunction|DoCompartmentTrace))
            (if (> (Utilities|Array|Length _hitcomponents) 0)
              (CallFunction|ExecuteChangesEvent _hitcomponents (Variables|Default|GetGunMode)))))))))

(event Input|ActionEvents|InputActionGamepadLeftFire
  (bind _gunmat (Variables|Default|GetGunMat))
  (bind _gunmode (Variables|Default|GetGunMode))
  (bind _returnvalue (Utilities|Select :Index _gunmode :Option%200 "0.100000,0.100000,0.100000" :Option%201 "0.500000,0.750000,0.250000" :Option%202 "0.250000,0.500000,1.000000" :Option%203 "0.750000,0.250000,0.500000" :Option%204 "0.900000,0.900000,0.900000"))
  (bind _returnvalue_2 (Math|Conversions|ToLinearColor(Vector) _returnvalue))
  (:Pressed
    (CallFunction|CycleGunMode)
    (bind _returnvalue_3 (Class|Actor|GetOwnerController))
    (bind _asshooterplayercontroller (Utilities|Casting|CastToShooterPlayerController _returnvalue_3))
    (Class|ShooterPlayerController|ClientServerNotification _asshooterplayercontroller (Utilities|Select :Index _gunmode :Option%200 "Open Mode" :Option%201 "Close/Unfreeze Mode" :Option%202 "Freeze Mode" :Option%203 "Lock Sides Mode" :Option%204 "Unlock Sides Mode") "(R=0.249093,G=0.164050,B=0.965000,A=1.000000)" 1.5 3.0)
    (Rendering|Material|SetVectorParameterValue _gunmat "Color2" _returnvalue_2 :!class /Script/Engine.MaterialInstanceDynamic)
    (Rendering|Material|SetVectorParameterValue _gunmat "Color4" _returnvalue_2 :!class /Script/Engine.MaterialInstanceDynamic)))

(event Input|ActionEvents|InputActionTargeting
  (bind _gunmat (Variables|Default|GetGunMat))
  (bind _gunmode (Variables|Default|GetGunMode))
  (bind _returnvalue (Utilities|Select :Index _gunmode :Option%200 "0.100000,0.100000,0.100000" :Option%201 "0.500000,0.750000,0.250000" :Option%202 "0.250000,0.500000,1.000000" :Option%203 "0.750000,0.250000,0.500000" :Option%204 "0.900000,0.900000,0.900000"))
  (bind _returnvalue_2 (Math|Conversions|ToLinearColor(Vector) _returnvalue))
  (:Pressed
    (CallFunction|CycleGunMode)
    (bind _returnvalue_3 (Class|Actor|GetOwnerController))
    (bind _asshooterplayercontroller (Utilities|Casting|CastToShooterPlayerController _returnvalue_3))
    (Class|ShooterPlayerController|ClientServerNotification _asshooterplayercontroller (Utilities|Select :Index _gunmode :Option%200 "Open Mode" :Option%201 "Close/Unfreeze Mode" :Option%202 "Freeze Mode" :Option%203 "Lock Sides Mode" :Option%204 "Unlock Sides Mode") "(R=0.249093,G=0.164050,B=0.965000,A=1.000000)" 1.5 3.0)
    (Rendering|Material|SetVectorParameterValue _gunmat "Color2" _returnvalue_2 :!class /Script/Engine.MaterialInstanceDynamic)
    (Rendering|Material|SetVectorParameterValue _gunmat "Color4" _returnvalue_2 :!class /Script/Engine.MaterialInstanceDynamic)))

(event Input|ActionEvents|InputActionFire
  (:Pressed
    (bind _returnvalue (Class|Actor|GetOwnerController))
    (Utilities|SPIsPlacingStructure _returnvalue
      (:No
        (Utilities|SPIsRadialMenuOpen _returnvalue
          (:No
            (bind _hitcomponents (CallFunction|DoCompartmentTrace))
            (if (> (Utilities|Array|Length _hitcomponents) 0)
              (CallFunction|ExecuteChangesEvent _hitcomponents (Variables|Default|GetGunMode)))))))))

(event Input|MouseEvents|RightMouseButton
  (:Pressed
    (Class|ShooterWeapon|PlayWeaponAnimation (Variables|Default|GetReloadAnim) false false false false false false)))

(event Input|MouseEvents|LeftMouseButton
  (:Pressed
    (bind _returnvalue (Class|Actor|GetOwnerController))
    (Utilities|SPIsRadialMenuOpen _returnvalue
      (:No
        (Utilities|SPIsPlacingStructure _returnvalue
          (:No
            (Class|ShooterWeapon|PlayWeaponAnimation (Variables|Default|GetFireAnim) false false false false false false)))))))

(event Input|GamepadEvents|GamepadRightTrigger
  (:Pressed
    (bind _returnvalue (Class|Actor|GetOwnerController))
    (Utilities|SPIsRadialMenuOpen _returnvalue
      (:No
        (Utilities|SPIsPlacingStructure _returnvalue
          (:No
            (Class|ShooterWeapon|PlayWeaponAnimation (Variables|Default|GetFireAnim) false false false false false false)))))))

(event Input|GamepadEvents|GamepadLeftTrigger
  (:Pressed
    (Class|ShooterWeapon|PlayWeaponAnimation (Variables|Default|GetReloadAnim) false false false false false false)))

(fn ConstructionScript
  (bind _gunmode (Variables|Default|GetGunMode))
  (bind _returnvalue (Utilities|Select :Index _gunmode :Option%200 "0.100000,0.100000,0.100000" :Option%201 "0.500000,0.750000,0.250000" :Option%202 "0.250000,0.500000,1.000000"))
  (bind _returnvalue_2 (Math|Conversions|ToLinearColor(Vector) _returnvalue))
  (if (not (Networking|IsDedicatedServer))
    (bind _returnvalue_3 (Rendering|Material|CreateDynamicMaterialInstance "/Game/PrimalEarth/WeaponPistolMachined/PistolMachined_Colorized_MIC.PistolMachined_Colorized_MIC" :!class /Script/Engine.KismetMaterialLibrary))
    (Variables|Default|SetGunMat _returnvalue_3)
    (Rendering|Material|SetMaterial (Variables|Default|GetMesh1P) 0 _returnvalue_3)
    (Rendering|Material|SetVectorParameterValue (Variables|Default|GetGunMat) "Color2" _returnvalue_2 :!class /Script/Engine.MaterialInstanceDynamic)
    (Rendering|Material|SetVectorParameterValue (Variables|Default|GetGunMat) "Color4" _returnvalue_2 :!class /Script/Engine.MaterialInstanceDynamic)))

(fn DoCompartmentTrace
  (bind _returnvalue (Class|ShooterWeapon|GetWeaponMesh))
  (bind _returnvalue_2 (Transformation|GetSocketLocation _returnvalue "MuzzleFlashSocket"))
  (bind _returnvalue_3 (Class|Actor|GetOwnerController))
  (bind (_outhits _returnvalue_4) (Class|KismetSystemLibrary|LineTraceMultiforObjects _returnvalue_2 (+ _returnvalue_2 (* (Math|Vector|GetForwardVector (Pawn|GetBaseAimRotation (Pawn|GetControlledPawn _returnvalue_3))) 1.75e+03)) (Utilities|Array|MakeArray "ObjectTypeQuery9") false (Utilities|Array|MakeArray) "Persistent" true))
  (if _returnvalue_4
    (for _array_element _outhits
      (bind _asprimalstructureunderwaterbase (Utilities|Casting|CastToPrimalStructureUnderwaterBase (.HitActor (Collision|BreakHitResult _array_element))))
      (bind _returnvalue_5 (Class|PrimalStructure|AllowStructureAccess _asprimalstructureunderwaterbase _returnvalue_3))
      (if (and _returnvalue_5 (== (Variables|/Script/Engine.Actor|GetTargetingTeam _returnvalue_3) (Variables|/Script/Engine.Actor|GetTargetingTeam (.HitActor (Collision|BreakHitResult _array_element)))))
        (Utilities|Array|Add (LocalVariables|GetFoundComponents) (.HitComponent (Collision|BreakHitResult _array_element))))))
  (return (LocalVariables|GetFoundComponents)))

(fn CycleGunMode
  (Variables|Default|SetGunMode (Math|Integer|SelectInt 0 (+ (Variables|Default|GetGunMode) 1) (> (+ (Variables|Default|GetGunMode) 1) 4))))

(fn HandleOpen
  (params (Components :type Array%20of%20Primitive%20Component%20Object%20References))
  (bind _array_element (Utilities|Array|ForEachLoopwithBreak Components :!label _label)
    (:LoopBody
      (bind _asprimalstructureunderwaterbase (Utilities|Casting|CastToPrimalStructureUnderwaterBase (Components|GetOwner _array_element)))
      (bind _index (CallFunction|SPPortholeNametoIndex (Utilities|GetDisplayName _array_element)))
      (if (and (not (Utilities|Array|Get(acopy) (Variables|/Script/ShooterGame.PrimalStructureUnderwaterBase|GetPortholeLocked _asprimalstructureunderwaterbase) (- _index 42))) (not (Utilities|Array|Get(acopy) (Variables|/Script/ShooterGame.PrimalStructureUnderwaterBase|GetPortholeOpen _asprimalstructureunderwaterbase) (- _index 42))))
        (bind _returnvalue (Class|Actor|GetOwnerController))
        (Class|Actor|TryMultiUse _asprimalstructureunderwaterbase _returnvalue _index)
        (goto _label Break)))))

(fn HandleClose
  (params (Components :type Array%20of%20Primitive%20Component%20Object%20References))
  (bind _item (Utilities|Array|Get(acopy) Components))
  (if (> (Utilities|Array|Length Components) 0)
    (bind _asprimalstructureunderwaterbase (Utilities|Casting|CastToPrimalStructureUnderwaterBase (Components|GetOwner _item)))
    (bind _index (CallFunction|SPPortholeNametoIndex (Utilities|GetDisplayName _item)))
    (if (or (Utilities|Array|Get(acopy) (Variables|/Script/ShooterGame.PrimalStructureUnderwaterBase|GetPortholeLocked _asprimalstructureunderwaterbase) (- _index 42)) (Utilities|Array|Get(acopy) (Variables|/Script/ShooterGame.PrimalStructureUnderwaterBase|GetPortholeOpen _asprimalstructureunderwaterbase) (- _index 42)))
      (bind _returnvalue (Class|Actor|GetOwnerController))
      (Class|Actor|TryMultiUse _asprimalstructureunderwaterbase _returnvalue (Math|Integer|SelectInt (+ _index 30) _index (Utilities|Array|Get(acopy) (Variables|/Script/ShooterGame.PrimalStructureUnderwaterBase|GetPortholeLocked _asprimalstructureunderwaterbase) (- _index 42)))))))

(fn HandleFreeze
  (params (Components :type Array%20of%20Primitive%20Component%20Object%20References))
  (bind _array_element (Utilities|Array|ForEachLoopwithBreak Components :!label _label)
    (:LoopBody
      (bind _asprimalstructureunderwaterbase (Utilities|Casting|CastToPrimalStructureUnderwaterBase (Components|GetOwner _array_element)))
      (bind _index (CallFunction|SPPortholeNametoIndex (Utilities|GetDisplayName _array_element)))
      (if (and (not (Utilities|Array|Get(acopy) (Variables|/Script/ShooterGame.PrimalStructureUnderwaterBase|GetPortholeLocked _asprimalstructureunderwaterbase) (- _index 42))) (not (Utilities|Array|Get(acopy) (Variables|/Script/ShooterGame.PrimalStructureUnderwaterBase|GetPortholeOpen _asprimalstructureunderwaterbase) (- _index 42))))
        (bind _returnvalue (Class|Actor|GetOwnerController))
        (Class|Actor|TryMultiUse _asprimalstructureunderwaterbase _returnvalue (+ _index 30))
        (goto _label Break)))))

(fn HandleLockToggle
  (params (Components :type Array%20of%20Primitive%20Component%20Object%20References) (DoLock :type Boolean))
  (bind _item (Utilities|Array|Get(acopy) Components))
  (bind _returnvalue (Components|GetOwner _item))
  (if (> (Utilities|Array|Length Components) 0)
    (bind _asbase_underwater_c (Utilities|Casting|CastToBase_Underwater _returnvalue)
      (:then
        (Variables|/Game/Mods/StructuresPlusMod/Structures/Underwater/Base_Underwater.Base_Underwater_C|SetLockSides _asbase_underwater_c DoLock false)
        (Class|Actor|MulticastProperty _asbase_underwater_c "LockSides"))
      (:CastFailed
        (bind _asbp_underwater_cube_sloped_c (Utilities|Casting|CastToBP_Underwater_Cube_Sloped _returnvalue))
        (Variables|/Game/Mods/StructuresPlusMod/Structures/Underwater/Underwater_Cube_Sloped/BP_Underwater_Cube_Sloped.BP_Underwater_Cube_Sloped_C|SetLockSides _asbp_underwater_cube_sloped_c DoLock false)
        (Class|Actor|MulticastProperty _asbp_underwater_cube_sloped_c "LockSides")))))