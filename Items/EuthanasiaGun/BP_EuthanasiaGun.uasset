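; Euthanasia gun weapon that lets players kill their own team's dinos in two steps: mark with targeting, then kill with fire.
; Inputs, enabled for the local owner, line trace for a dino unless placing structures or using the radial menu.
; Marking checks team and tribe Unclaim permission; killing requires the marked dino, same team and Ride permission.
; The kill applies friendly-kill damage exceeding max health; client messages report marking and refusals.
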(event Custom|MarkDinoEvent
  (params (Dino :type Primal%20Dino%20Character%20Object%20Reference))
  (bind _tamedname (Variables|/Script/ShooterGame.PrimalDinoCharacter|GetTamedName Dino))
  (bind _returnvalue (Class|Actor|GetOwnerController))
  (bind _asshooterplayercontroller (Utilities|Casting|CastToShooterPlayerController _returnvalue))
  (bind _returnvalue_2 (Class|ShooterPlayerController|AllowTribeGroupPermission _asshooterplayercontroller "PET_UNCLAIM" Dino))
  (if (and _returnvalue_2 (== (Variables|/Script/Engine.Actor|GetTargetingTeam _returnvalue) (Variables|/Script/Engine.Actor|GetTargetingTeam Dino)))
    (Variables|Default|SetMarkedDino Dino)
    (CallFunction|SPMessageClient _returnvalue (Utilities|String|Append (Utilities|String|SelectString _tamedname (Variables|/Script/ShooterGame.PrimalCharacter|GetDescriptiveName Dino) (> (Utilities|String|Len _tamedname) 0)) " Marked For Death.") "NewEnumerator3")
    (else
      (CallFunction|SPMessageClient _returnvalue "You do not have permission to kill this dino." "NewEnumerator1"))))

(event Custom|KillDinoEvent
  (params (Dino :type Primal%20Dino%20Character%20Object%20Reference))
  (if (== Dino (Variables|Default|GetMarkedDino))
    (CallFunction|HandleDinoKilling)
    (else
      (bind _returnvalue (Class|Actor|GetOwnerController))
      (CallFunction|SPMessageClient _returnvalue "Dino Isn't Marked For Death." "NewEnumerator1"))))

(event EventBeginPlay
  (Utilities|FlowControl|Delay 0.2)
  (bind _returnvalue (Class|Actor|GetOwnerController))
  (if (Pawn|IsLocalController _returnvalue)
    (Input|EnableInput _returnvalue)))

(event Input|ActionEvents|InputActionGamepadRightFire
  (:Pressed
    (bind _returnvalue (Class|Actor|GetOwnerController))
    (Utilities|SPIsPlacingStructure _returnvalue
      (:No
        (Utilities|SPIsRadialMenuOpen _returnvalue
          (:No
            (bind _result (CallFunction|SPDoItemLineTrace _returnvalue self (Utilities|Array|MakeArray "ObjectTypeQuery7" "ObjectTypeQuery16" "ObjectTypeQuery8") false))
            (Utilities|IsValid _result
              (:Is%20Valid
                (bind _asprimaldinocharacter (Utilities|Casting|CastToPrimalDinoCharacter _result))
                (CallFunction|KillDinoEvent _asprimaldinocharacter)))))))))

(event Input|ActionEvents|InputActionGamepadLeftFire
  (:Pressed
    (bind _returnvalue (Class|Actor|GetOwnerController))
    (Utilities|SPIsPlacingStructure _returnvalue
      (:No
        (Utilities|SPIsRadialMenuOpen _returnvalue
          (:No
            (bind _result (CallFunction|SPDoItemLineTrace _returnvalue self (Utilities|Array|MakeArray "ObjectTypeQuery7" "ObjectTypeQuery16" "ObjectTypeQuery8") false))
            (Utilities|IsValid _result
              (:Is%20Valid
                (bind _asprimaldinocharacter (Utilities|Casting|CastToPrimalDinoCharacter _result))
                (CallFunction|MarkDinoEvent _asprimaldinocharacter)))))))))

(event Input|ActionEvents|InputActionTargeting
  (:Pressed
    (bind _returnvalue (Class|Actor|GetOwnerController))
    (Utilities|SPIsPlacingStructure _returnvalue
      (:No
        (Utilities|SPIsRadialMenuOpen _returnvalue
          (:No
            (bind _result (CallFunction|SPDoItemLineTrace _returnvalue self (Utilities|Array|MakeArray "ObjectTypeQuery7" "ObjectTypeQuery16" "ObjectTypeQuery8") false))
            (Utilities|IsValid _result
              (:Is%20Valid
                (bind _asprimaldinocharacter (Utilities|Casting|CastToPrimalDinoCharacter _result))
                (CallFunction|MarkDinoEvent _asprimaldinocharacter)))))))))

(event Input|ActionEvents|InputActionFire
  (:Pressed
    (bind _returnvalue (Class|Actor|GetOwnerController))
    (Utilities|SPIsPlacingStructure _returnvalue
      (:No
        (Utilities|SPIsRadialMenuOpen _returnvalue
          (:No
            (bind _result (CallFunction|SPDoItemLineTrace _returnvalue self (Utilities|Array|MakeArray "ObjectTypeQuery7" "ObjectTypeQuery16" "ObjectTypeQuery8") false))
            (Utilities|IsValid _result
              (:Is%20Valid
                (bind _asprimaldinocharacter (Utilities|Casting|CastToPrimalDinoCharacter _result))
                (CallFunction|KillDinoEvent _asprimaldinocharacter)))))))))

(event Input|MouseEvents|RightMouseButton
  (:Pressed
    (bind _returnvalue (Class|Actor|GetOwnerController))
    (Utilities|SPIsRadialMenuOpen _returnvalue
      (:No
        (Utilities|SPIsPlacingStructure _returnvalue
          (:No
            (Class|ShooterWeapon|PlayWeaponAnimation (Variables|Default|GetFireAnim) false false false false false false)))))))

(event Input|MouseEvents|LeftMouseButton
  (:Pressed
    (bind _returnvalue (Class|Actor|GetOwnerController))
    (Utilities|SPIsRadialMenuOpen _returnvalue
      (:No
        (Utilities|SPIsPlacingStructure _returnvalue
          (:No
            (Class|ShooterWeapon|PlayWeaponAnimation (Variables|Default|GetFireAnim) false false false false false false)))))))

(event Input|GamepadEvents|GamepadRightTrigger
  (:Pressed
    (bind _returnvalue (Class|Actor|GetOwnerController))
    (Utilities|SPIsRadialMenuOpen _returnvalue
      (:No
        (Utilities|SPIsPlacingStructure _returnvalue
          (:No
            (Class|ShooterWeapon|PlayWeaponAnimation (Variables|Default|GetFireAnim) false false false false false false)))))))

(event Input|GamepadEvents|GamepadLeftTrigger
  (:Pressed
    (bind _returnvalue (Class|Actor|GetOwnerController))
    (Utilities|SPIsRadialMenuOpen _returnvalue
      (:No
        (Utilities|SPIsPlacingStructure _returnvalue
          (:No
            (Class|ShooterWeapon|PlayWeaponAnimation (Variables|Default|GetFireAnim) false false false false false false)))))))

(fn ConstructionScript)

(fn HandleDinoKilling
  (bind _markeddino (Variables|Default|GetMarkedDino))
  (bind _markeddino_2 (Variables|Default|GetMarkedDino))
  (bind _returnvalue (Class|Actor|GetOwnerController))
  (bind _asshooterplayercontroller (Utilities|Casting|CastToShooterPlayerController _returnvalue))
  (bind _returnvalue_2 (Class|ShooterPlayerController|AllowTribeGroupPermission _asshooterplayercontroller "PET_RIDE" _markeddino))
  (if (and _returnvalue_2 (== (Variables|/Script/Engine.Actor|GetTargetingTeam _returnvalue) (Variables|/Script/Engine.Actor|GetTargetingTeam _markeddino)))
    (bind _returnvalue_3 (Class|PrimalCharacter|GetCharacterStatusComponent _markeddino_2))
    (Game|Damage|ApplyDamage _markeddino_2 (* (Class|PrimalCharacterStatusComponent|BPGetMaxStatusValue _returnvalue_3 "Health") 1.1) _returnvalue self "/Game/Mods/StructuresPlusMod/Items/EuthanasiaGun/DmgType_FriendlyDinoKill.DmgType_FriendlyDinoKill_C")
    (else
      (CallFunction|SPMessageClient _returnvalue "You do not have permission to kill this dino." "NewEnumerator1"))))