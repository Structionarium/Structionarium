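; Handheld Structures Plus weapon for remotely changing the model of placed structures the player aims at.
; Fire traces past a class blacklist, toggling railing and ramp variants directly; other targets open buff-driven model selection or, as SPlus_IGlass, receive the stored model index.
; Targeting passes the traced structure, or an empty hit, to set that index.
; A lazily added Buff_StructuresPlus_Models holds the state and is removed on EndPlay.
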(event Custom|ExecuteModelSelectEvent
  (params (Target :type Actor%20Object%20Reference))
  (bind _wasnothandled (CallFunction|HandleModelToggles Target))
  (if _wasnothandled
    (Utilities|FlowControl|Sequence
      (:then_0
        (Utilities|IsValid (Variables|Default|GetBuffRef)
          (:Is%20Not%20Valid
            (bind _returnvalue (Class|Actor|GetOwnerController))
            (bind _asshooterplayercontroller (Utilities|Casting|CastToShooterPlayerController _returnvalue))
            (bind _returnvalue_2 (Class|PrimalBuff|StaticAddBuff "/Game/Mods/StructuresPlusMod/_Buffs/Buff_StructuresPlus_Models.Buff_StructuresPlus_Models_C" (Class|ShooterPlayerController|GetPlayerCharacter _asshooterplayercontroller) 0 0 false))
            (bind _asbuff_structuresplus_models_c (Utilities|Casting|CastToBuff_StructuresPlus_Models _returnvalue_2))
            (Variables|Default|SetBuffRef _asbuff_structuresplus_models_c))))
      (:then_1
        (if (== (Variables|/Game/Mods/StructuresPlusMod/_Buffs/Buff_StructuresPlus_Models.Buff_StructuresPlus_Models_C|GetGunModelIndex (Variables|Default|GetBuffRef)) -1)
          (Default|RemoteSelectModelEvent (Variables|Default|GetBuffRef) Target)
          (else
            (bind _asprimalstructure (Utilities|Casting|CastToPrimalStructure Target))
            (bind _assplus_iglass_c (Utilities|Casting|CastToSPlus_IGlass (Class|TargetableInterface|ToUObject _asprimalstructure)))
            (Default|IGlassSetModel _assplus_iglass_c (Variables|/Game/Mods/StructuresPlusMod/_Buffs/Buff_StructuresPlus_Models.Buff_StructuresPlus_Models_C|GetGunModelIndex (Variables|Default|GetBuffRef)))))))))

(event Custom|SetIndexEvent
  (params (Target :type Actor%20Object%20Reference))
  (Utilities|FlowControl|Sequence
    (:then_0
      (Utilities|IsValid (Variables|Default|GetBuffRef)
        (:Is%20Not%20Valid
          (bind _returnvalue (Class|Actor|GetOwnerController))
          (bind _asshooterplayercontroller (Utilities|Casting|CastToShooterPlayerController _returnvalue))
          (bind _returnvalue_2 (Class|PrimalBuff|StaticAddBuff "/Game/Mods/StructuresPlusMod/_Buffs/Buff_StructuresPlus_Models.Buff_StructuresPlus_Models_C" (Class|ShooterPlayerController|GetPlayerCharacter _asshooterplayercontroller) 0 0 false))
          (bind _asbuff_structuresplus_models_c (Utilities|Casting|CastToBuff_StructuresPlus_Models _returnvalue_2))
          (Variables|Default|SetBuffRef _asbuff_structuresplus_models_c))))
    (:then_1
      (Default|HandleGunModelIndexEvent (Variables|Default|GetBuffRef) Target))))

(event EventEndPlay
  (params (EndPlayReason :type EEndPlayReason%20Enum :default "ActorDestroyed"))
  (bind _buffref (Variables|Default|GetBuffRef))
  (Networking|SwitchHasAuthority
    (:Authority
      (Utilities|IsValid _buffref
        (:Is%20Valid
          (Default|RemoveBuffEvent _buffref))))))

(event EventBeginPlay
  (Utilities|FlowControl|Delay 0.2)
  (bind _returnvalue (Class|Actor|GetOwnerController))
  (if (Pawn|IsLocalController _returnvalue)
    (Input|EnableInput _returnvalue)))

(event Input|ActionEvents|InputActionGamepadRightFire
  (:Pressed
    (bind _returnvalue (Class|Actor|GetOwnerController))
    (Utilities|SPIsPlacingStructure _returnvalue
      (:No
        (Utilities|SPIsRadialMenuOpen _returnvalue
          (:No
            (bind _result (CallFunction|SPDoItemLineTrace _returnvalue self (Utilities|Array|MakeArray "ObjectTypeQuery9") false))
            (Utilities|IsValid _result
              (:Is%20Valid
                (if (CallFunction|CheckBlackList _result)
                  (CallFunction|ExecuteModelSelectEvent _result))))))))))

(event Input|ActionEvents|InputActionGamepadLeftFire
  (:Pressed
    (bind _returnvalue (Class|Actor|GetOwnerController))
    (Utilities|SPIsPlacingStructure _returnvalue
      (:No
        (Utilities|SPIsRadialMenuOpen _returnvalue
          (:No
            (bind _result (CallFunction|SPDoItemLineTrace _returnvalue self (Utilities|Array|MakeArray "ObjectTypeQuery9") false))
            (Utilities|IsValid _result
              (:Is%20Valid
                (if (CallFunction|CheckBlackList _result)
                  (CallFunction|SetIndexEvent _result :!label _label)))
              (:Is%20Not%20Valid
                (goto _label)))))))))

(event Input|ActionEvents|InputActionTargeting
  (:Pressed
    (bind _returnvalue (Class|Actor|GetOwnerController))
    (Utilities|SPIsPlacingStructure _returnvalue
      (:No
        (Utilities|SPIsRadialMenuOpen _returnvalue
          (:No
            (bind _result (CallFunction|SPDoItemLineTrace _returnvalue self (Utilities|Array|MakeArray "ObjectTypeQuery9") false))
            (Utilities|IsValid _result
              (:Is%20Valid
                (if (CallFunction|CheckBlackList _result)
                  (CallFunction|SetIndexEvent _result :!label _label)))
              (:Is%20Not%20Valid
                (goto _label)))))))))

(event Input|ActionEvents|InputActionFire
  (:Pressed
    (bind _returnvalue (Class|Actor|GetOwnerController))
    (Utilities|SPIsPlacingStructure _returnvalue
      (:No
        (Utilities|SPIsRadialMenuOpen _returnvalue
          (:No
            (bind _result (CallFunction|SPDoItemLineTrace _returnvalue self (Utilities|Array|MakeArray "ObjectTypeQuery9") false))
            (Utilities|IsValid _result
              (:Is%20Valid
                (if (CallFunction|CheckBlackList _result)
                  (CallFunction|ExecuteModelSelectEvent _result))))))))))

(event Input|MouseEvents|RightMouseButton
  (:Pressed
    (bind _returnvalue (Class|Actor|GetOwnerController))
    (Utilities|SPIsRadialMenuOpen _returnvalue
      (:No
        (Utilities|SPIsPlacingStructure _returnvalue
          (:No
            (Class|ShooterWeapon|PlayWeaponAnimation (Variables|Default|GetFireAnim) false false false false false false)))))))

(event Input|MouseEvents|LeftMouseButton
  (:Pressed
    (bind _returnvalue (Class|Actor|GetOwnerController))
    (Utilities|SPIsRadialMenuOpen _returnvalue
      (:No
        (Utilities|SPIsPlacingStructure _returnvalue
          (:No
            (Class|ShooterWeapon|PlayWeaponAnimation (Variables|Default|GetFireAnim) false false false false false false)))))))

(event Input|GamepadEvents|GamepadRightTrigger
  (:Pressed
    (bind _returnvalue (Class|Actor|GetOwnerController))
    (Utilities|SPIsRadialMenuOpen _returnvalue
      (:No
        (Utilities|SPIsPlacingStructure _returnvalue
          (:No
            (Class|ShooterWeapon|PlayWeaponAnimation (Variables|Default|GetFireAnim) false false false false false false)))))))

(event Input|GamepadEvents|GamepadLeftTrigger
  (:Pressed
    (bind _returnvalue (Class|Actor|GetOwnerController))
    (Utilities|SPIsRadialMenuOpen _returnvalue
      (:No
        (Utilities|SPIsPlacingStructure _returnvalue
          (:No
            (Class|ShooterWeapon|PlayWeaponAnimation (Variables|Default|GetFireAnim) false false false false false false)))))))

(fn ConstructionScript)

(fn CheckBlackList
  (params (Actor :type Actor%20Object%20Reference))
  (bind _array_element (Utilities|Array|ForEachLoopwithBreak (Variables|Default|GetBlackListedClasses) :!label _label)
    (:LoopBody
      (if (>= (Utilities|String|FindSubstring (Utilities|GetClassDisplayName (Utilities|GetClass Actor)) _array_element) 0)
        (LocalVariables|SetIsBlackListed true)
        (goto _label Break)))
    (:Completed
      (return (not (LocalVariables|GetIsBlackListed))))))

(fn HandleModelToggles
  (params (Target :type Actor%20Object%20Reference))
  (Utilities|FlowControl|Sequence
    (:then_0
      (bind _asbase_railing_c (Utilities|Casting|CastToBase_Railing Target)
        (:then
          (Variables|/Game/Mods/StructuresPlusMod/Structures/Railings/Base_Railing.Base_Railing_C|SetIsHalfWall _asbase_railing_c (not (Variables|/Game/Mods/StructuresPlusMod/Structures/Railings/Base_Railing.Base_Railing_C|GetIsHalfWall _asbase_railing_c)) false)
          (Class|Actor|MulticastProperty _asbase_railing_c "IsHalfWall"))
        (:CastFailed
          (bind _asbase_ramp_c (Utilities|Casting|CastToBase_Ramp Target))
          (Variables|/Game/Mods/StructuresPlusMod/Structures/Ramps/Base_Ramp.Base_Ramp_C|SetAreStairs _asbase_ramp_c (not (Variables|/Game/Mods/StructuresPlusMod/Structures/Ramps/Base_Ramp.Base_Ramp_C|GetAreStairs _asbase_ramp_c)) false)
          (Class|Actor|MulticastProperty _asbase_ramp_c "AreStairs")))
      (LocalVariables|SetFoundPriorityEvent true))
    (:then_1
      (return (not (LocalVariables|GetFoundPriorityEvent))))))