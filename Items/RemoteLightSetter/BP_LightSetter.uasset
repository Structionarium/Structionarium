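; Handheld Structures Plus remote that edits and copies light settings on multi-lamps, Tek lights, standing torches and wall torches.
; Fire line-traces a light, then opens its settings UI or applies saved settings; Targeting saves the traced light's settings or clears saved ones.
; Settings live on a lazily added player Buff_StructuresPlus_Lights, removed by authority on EndPlay.
; Local-only input is ignored during structure placement or radial menu use.
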(event Custom|ExecuteLightingEvent
  (params (Target :type Actor%20Object%20Reference))
  (Utilities|FlowControl|Sequence
    (:then_0
      (Utilities|IsValid (Variables|Default|GetBuffRef)
        (:Is%20Not%20Valid
          (bind _returnvalue (Class|Actor|GetOwnerController))
          (bind _asshooterplayercontroller (Utilities|Casting|CastToShooterPlayerController _returnvalue))
          (bind _returnvalue_2 (Class|PrimalBuff|StaticAddBuff "/Game/Mods/StructuresPlusMod/_Buffs/Buff_StructuresPlus_Lights.Buff_StructuresPlus_Lights_C" (Class|ShooterPlayerController|GetPlayerCharacter _asshooterplayercontroller) 0 0 false))
          (bind _asbuff_structuresplus_lights_c (Utilities|Casting|CastToBuff_StructuresPlus_Lights _returnvalue_2))
          (Variables|Default|SetBuffRef _asbuff_structuresplus_lights_c))))
    (:then_1
      (bind _asbp_multilamp_c (Utilities|Casting|CastToBP_MultiLamp Target)
        (:then
          (if (not (Variables|/Game/Mods/StructuresPlusMod/_Buffs/Buff_StructuresPlus_Lights.Buff_StructuresPlus_Lights_C|GetHasSavedSettings (Variables|Default|GetBuffRef)))
            (Default|InitializeLightUI (Variables|Default|GetBuffRef) _asbp_multilamp_c (Variables|/Game/Mods/StructuresPlusMod/Misc/MultiLamp/BP_MultiLamp.BP_MultiLamp_C|GetLightSettings _asbp_multilamp_c))
            (else
              (Default|SetLightingEvent _asbp_multilamp_c (Variables|/Game/Mods/StructuresPlusMod/_Buffs/Buff_StructuresPlus_Lights.Buff_StructuresPlus_Lights_C|GetLightConfig (Variables|Default|GetBuffRef)))
              (bind _returnvalue_3 (Class|Actor|GetOwnerController :!label _label))
              (CallFunction|SPMessageClient _returnvalue_3 "Settings Set." "NewEnumerator3"))))
        (:CastFailed
          (bind _asbp_splusteklight_c (Utilities|Casting|CastToBP_SPlusTekLight Target)
            (:then
              (if (not (Variables|/Game/Mods/StructuresPlusMod/_Buffs/Buff_StructuresPlus_Lights.Buff_StructuresPlus_Lights_C|GetHasSavedSettings (Variables|Default|GetBuffRef)))
                (Default|InitializeLightUI (Variables|Default|GetBuffRef) _asbp_splusteklight_c (Variables|/Game/Mods/StructuresPlusMod/Misc/LightTek/BP_SPlusTekLight.BP_SPlusTekLight_C|GetLightSettings _asbp_splusteklight_c))
                (else
                  (Default|SetLightingEvent _asbp_splusteklight_c (Variables|/Game/Mods/StructuresPlusMod/_Buffs/Buff_StructuresPlus_Lights.Buff_StructuresPlus_Lights_C|GetLightConfig (Variables|Default|GetBuffRef)))
                  (goto _label))))
            (:CastFailed
              (bind _asbp_standingtorchplus_c (Utilities|Casting|CastToBP_StandingTorchPlus Target)
                (:then
                  (if (not (Variables|/Game/Mods/StructuresPlusMod/_Buffs/Buff_StructuresPlus_Lights.Buff_StructuresPlus_Lights_C|GetHasSavedSettings (Variables|Default|GetBuffRef)))
                    (Default|InitializeLightUI (Variables|Default|GetBuffRef) _asbp_standingtorchplus_c (Variables|/Game/Mods/StructuresPlusMod/Misc/TorchStanding/BP_StandingTorchPlus.BP_StandingTorchPlus_C|GetTorchSettings _asbp_standingtorchplus_c))
                    (else
                      (Default|SetLightSettingsEvent _asbp_standingtorchplus_c (Variables|/Game/Mods/StructuresPlusMod/_Buffs/Buff_StructuresPlus_Lights.Buff_StructuresPlus_Lights_C|GetLightConfig (Variables|Default|GetBuffRef)))
                      (goto _label))))
                (:CastFailed
                  (bind _asbp_walltorchplus_c (Utilities|Casting|CastToBP_WallTorchPlus Target))
                  (if (not (Variables|/Game/Mods/StructuresPlusMod/_Buffs/Buff_StructuresPlus_Lights.Buff_StructuresPlus_Lights_C|GetHasSavedSettings (Variables|Default|GetBuffRef)))
                    (Default|InitializeLightUI (Variables|Default|GetBuffRef) _asbp_walltorchplus_c (Variables|/Game/Mods/StructuresPlusMod/Misc/TorchWall/BP_WallTorchPlus.BP_WallTorchPlus_C|GetTorchSettings _asbp_walltorchplus_c))
                    (else
                      (Default|SetLightSettingsEvent _asbp_walltorchplus_c (Variables|/Game/Mods/StructuresPlusMod/_Buffs/Buff_StructuresPlus_Lights.Buff_StructuresPlus_Lights_C|GetLightConfig (Variables|Default|GetBuffRef)))
                      (goto _label))))))))))))

(event Custom|SaveSettingsEvent
  (params (Target :type Actor%20Object%20Reference))
  (bind _returnvalue (Class|Actor|GetOwnerController))
  (if (Variables|/Game/Mods/StructuresPlusMod/_Buffs/Buff_StructuresPlus_Lights.Buff_StructuresPlus_Lights_C|GetHasSavedSettings (Variables|Default|GetBuffRef))
    (Variables|/Game/Mods/StructuresPlusMod/_Buffs/Buff_StructuresPlus_Lights.Buff_StructuresPlus_Lights_C|SetHasSavedSettings (Variables|Default|GetBuffRef) false)
    (CallFunction|SPMessageClient _returnvalue "Settings Cleared." "NewEnumerator3")
    (else
      (Utilities|IsValid Target
        (:Is%20Valid
          (Utilities|FlowControl|Sequence
            (:then_0
              (Utilities|IsValid (Variables|Default|GetBuffRef)
                (:Is%20Not%20Valid
                  (bind _asshooterplayercontroller (Utilities|Casting|CastToShooterPlayerController _returnvalue))
                  (bind _returnvalue_2 (Class|PrimalBuff|StaticAddBuff "/Game/Mods/StructuresPlusMod/_Buffs/Buff_StructuresPlus_Lights.Buff_StructuresPlus_Lights_C" (Class|ShooterPlayerController|GetPlayerCharacter _asshooterplayercontroller) 0 0 false))
                  (bind _asbuff_structuresplus_lights_c (Utilities|Casting|CastToBuff_StructuresPlus_Lights _returnvalue_2))
                  (Variables|Default|SetBuffRef _asbuff_structuresplus_lights_c))))
            (:then_1
              (bind _asbp_multilamp_c (Utilities|Casting|CastToBP_MultiLamp Target)
                (:then
                  (Variables|/Game/Mods/StructuresPlusMod/_Buffs/Buff_StructuresPlus_Lights.Buff_StructuresPlus_Lights_C|SetHasSavedSettings (Variables|Default|GetBuffRef) true)
                  (Variables|/Game/Mods/StructuresPlusMod/_Buffs/Buff_StructuresPlus_Lights.Buff_StructuresPlus_Lights_C|SetLightConfig (Variables|Default|GetBuffRef) (Variables|/Game/Mods/StructuresPlusMod/Misc/MultiLamp/BP_MultiLamp.BP_MultiLamp_C|GetLightSettings _asbp_multilamp_c)))
                (:CastFailed
                  (bind _asbp_standingtorchplus_c (Utilities|Casting|CastToBP_StandingTorchPlus Target)
                    (:then
                      (Variables|/Game/Mods/StructuresPlusMod/_Buffs/Buff_StructuresPlus_Lights.Buff_StructuresPlus_Lights_C|SetHasSavedSettings (Variables|Default|GetBuffRef) true)
                      (Variables|/Game/Mods/StructuresPlusMod/_Buffs/Buff_StructuresPlus_Lights.Buff_StructuresPlus_Lights_C|SetLightConfig (Variables|Default|GetBuffRef) (Variables|/Game/Mods/StructuresPlusMod/Misc/TorchStanding/BP_StandingTorchPlus.BP_StandingTorchPlus_C|GetTorchSettings _asbp_standingtorchplus_c)))
                    (:CastFailed
                      (bind _asbp_walltorchplus_c (Utilities|Casting|CastToBP_WallTorchPlus Target)
                        (:then
                          (Variables|/Game/Mods/StructuresPlusMod/_Buffs/Buff_StructuresPlus_Lights.Buff_StructuresPlus_Lights_C|SetHasSavedSettings (Variables|Default|GetBuffRef) true)
                          (Variables|/Game/Mods/StructuresPlusMod/_Buffs/Buff_StructuresPlus_Lights.Buff_StructuresPlus_Lights_C|SetLightConfig (Variables|Default|GetBuffRef) (Variables|/Game/Mods/StructuresPlusMod/Misc/TorchWall/BP_WallTorchPlus.BP_WallTorchPlus_C|GetTorchSettings _asbp_walltorchplus_c)))
                        (:CastFailed
                          (bind _asbp_splusteklight_c (Utilities|Casting|CastToBP_SPlusTekLight Target))
                          (Variables|/Game/Mods/StructuresPlusMod/_Buffs/Buff_StructuresPlus_Lights.Buff_StructuresPlus_Lights_C|SetHasSavedSettings (Variables|Default|GetBuffRef) true)
                          (Variables|/Game/Mods/StructuresPlusMod/_Buffs/Buff_StructuresPlus_Lights.Buff_StructuresPlus_Lights_C|SetLightConfig (Variables|Default|GetBuffRef) (Variables|/Game/Mods/StructuresPlusMod/Misc/LightTek/BP_SPlusTekLight.BP_SPlusTekLight_C|GetLightSettings _asbp_splusteklight_c))))))))
              (CallFunction|SPMessageClient _returnvalue "Settings Saved." "NewEnumerator3"))))))))

(event EventBeginPlay
  (Utilities|FlowControl|Delay 0.2)
  (bind _returnvalue (Class|Actor|GetOwnerController))
  (if (Pawn|IsLocalController _returnvalue)
    (Input|EnableInput _returnvalue)))

(event EventEndPlay
  (params (EndPlayReason :type EEndPlayReason%20Enum :default "ActorDestroyed"))
  (bind _buffref (Variables|Default|GetBuffRef))
  (Networking|SwitchHasAuthority
    (:Authority
      (Utilities|IsValid _buffref
        (:Is%20Valid
          (Default|RemoveBuffEvent _buffref))))))

(event Input|ActionEvents|InputActionGamepadRightFire
  (:Pressed
    (bind _returnvalue (Class|Actor|GetOwnerController))
    (Utilities|SPIsPlacingStructure _returnvalue
      (:No
        (Utilities|SPIsRadialMenuOpen _returnvalue
          (:No
            (bind _result (CallFunction|SPDoItemLineTrace _returnvalue self (Utilities|Array|MakeArray "ObjectTypeQuery9") false))
            (Utilities|IsValid _result
              (:Is%20Valid
                (CallFunction|ExecuteLightingEvent _result)))))))))

(event Input|ActionEvents|InputActionGamepadLeftFire
  (:Pressed
    (bind _returnvalue (Class|Actor|GetOwnerController))
    (Utilities|SPIsPlacingStructure _returnvalue
      (:No
        (Utilities|SPIsRadialMenuOpen _returnvalue
          (:No
            (bind _result (CallFunction|SPDoItemLineTrace _returnvalue self (Utilities|Array|MakeArray "ObjectTypeQuery9") false))
            (CallFunction|SaveSettingsEvent _result)))))))

(event Input|ActionEvents|InputActionTargeting
  (:Pressed
    (bind _returnvalue (Class|Actor|GetOwnerController))
    (Utilities|SPIsPlacingStructure _returnvalue
      (:No
        (Utilities|SPIsRadialMenuOpen _returnvalue
          (:No
            (bind _result (CallFunction|SPDoItemLineTrace _returnvalue self (Utilities|Array|MakeArray "ObjectTypeQuery9") false))
            (CallFunction|SaveSettingsEvent _result)))))))

(event Input|ActionEvents|InputActionFire
  (:Pressed
    (bind _returnvalue (Class|Actor|GetOwnerController))
    (Utilities|SPIsPlacingStructure _returnvalue
      (:No
        (Utilities|SPIsRadialMenuOpen _returnvalue
          (:No
            (bind _result (CallFunction|SPDoItemLineTrace _returnvalue self (Utilities|Array|MakeArray "ObjectTypeQuery9") false))
            (Utilities|IsValid _result
              (:Is%20Valid
                (CallFunction|ExecuteLightingEvent _result)))))))))

(event Input|MouseEvents|RightMouseButton
  (:Pressed
    (bind _returnvalue (Class|Actor|GetOwnerController))
    (Utilities|SPIsRadialMenuOpen _returnvalue
      (:No
        (Utilities|SPIsPlacingStructure _returnvalue
          (:No
            (Class|ShooterWeapon|PlayWeaponAnimation (Variables|Default|GetFireAnim) false false false false false false)))))))

(event Input|MouseEvents|LeftMouseButton
  (:Pressed
    (bind _returnvalue (Class|Actor|GetOwnerController))
    (Utilities|SPIsRadialMenuOpen _returnvalue
      (:No
        (Utilities|SPIsPlacingStructure _returnvalue
          (:No
            (Class|ShooterWeapon|PlayWeaponAnimation (Variables|Default|GetFireAnim) false false false false false false)))))))

(event Input|GamepadEvents|GamepadRightTrigger
  (:Pressed
    (bind _returnvalue (Class|Actor|GetOwnerController))
    (Utilities|SPIsRadialMenuOpen _returnvalue
      (:No
        (Utilities|SPIsPlacingStructure _returnvalue
          (:No
            (Class|ShooterWeapon|PlayWeaponAnimation (Variables|Default|GetFireAnim) false false false false false false)))))))

(event Input|GamepadEvents|GamepadLeftTrigger
  (:Pressed
    (bind _returnvalue (Class|Actor|GetOwnerController))
    (Utilities|SPIsRadialMenuOpen _returnvalue
      (:No
        (Utilities|SPIsPlacingStructure _returnvalue
          (:No
            (Class|ShooterWeapon|PlayWeaponAnimation (Variables|Default|GetFireAnim) false false false false false false)))))))

(fn ConstructionScript)