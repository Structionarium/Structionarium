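; Handheld Structures Plus tool that configures turrets the player aims at.
; Fire line-traces for a turret, applies the TurretOptions buff, then pastes saved settings or opens the options UI through that buff.
; Targeting toggles between copying and clearing saved settings, using SPlus_ITurret where implemented, otherwise native turret and Tek fields.
; Ammo transfer helpers are defined but never called here, and ToggleActive is empty.
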(event Custom|ExecuteTurretOptionsEvent
  (params (Turret :type Actor%20Object%20Reference))
  (Utilities|FlowControl|Sequence
    (:then_0
      (bind _buff (CallFunction|SPApplyBufffromWeapon self "/Game/Mods/StructuresPlusMod/_Buffs/Buff_StructuresPlus_TurretOptions.Buff_StructuresPlus_TurretOptions_C"))
      (bind _asbuff_structuresplus_turretoptions_c (Utilities|Casting|CastToBuff_StructuresPlus_TurretOptions _buff))
      (Variables|Default|SetBuffRef _asbuff_structuresplus_turretoptions_c))
    (:then_1
      (if (Variables|Default|GetHasSavedSettings)
        (CallFunction|PasteSettings Turret)
        (else
          (bind _asprimalstructureturret (Utilities|Casting|CastToPrimalStructureTurret Turret))
          (Default|InitializeTurretUI (Variables|Default|GetBuffRef) _asprimalstructureturret false))))))

(event Custom|CopySettingsEvent
  (params (Target :type Actor%20Object%20Reference))
  (CallFunction|CopySettings Target))

(event EventBeginPlay
  (Utilities|FlowControl|Delay 0.2)
  (bind _returnvalue (Class|Actor|GetOwnerController))
  (if (Pawn|IsLocalController _returnvalue)
    (Input|EnableInput _returnvalue)))

(event Input|ActionEvents|InputActionGamepadRightFire
  (:Pressed
    (bind _returnvalue (Class|Actor|GetOwnerController))
    (Utilities|SPIsPlacingStructure _returnvalue
      (:No
        (Utilities|SPIsRadialMenuOpen _returnvalue
          (:No
            (bind _result (CallFunction|SPDoItemLineTrace _returnvalue self (Utilities|Array|MakeArray "ObjectTypeQuery9") false))
            (Utilities|IsValid _result
              (:Is%20Valid
                (CallFunction|ExecuteTurretOptionsEvent _result)))))))))

(event Input|ActionEvents|InputActionGamepadLeftFire
  (:Pressed
    (bind _returnvalue (Class|Actor|GetOwnerController))
    (Utilities|SPIsPlacingStructure _returnvalue
      (:No
        (Utilities|SPIsRadialMenuOpen _returnvalue
          (:No
            (bind _result (CallFunction|SPDoItemLineTrace _returnvalue self (Utilities|Array|MakeArray "ObjectTypeQuery9") false))
            (CallFunction|CopySettingsEvent _result)))))))

(event Input|ActionEvents|InputActionTargeting
  (:Pressed
    (bind _returnvalue (Class|Actor|GetOwnerController))
    (Utilities|SPIsPlacingStructure _returnvalue
      (:No
        (Utilities|SPIsRadialMenuOpen _returnvalue
          (:No
            (bind _result (CallFunction|SPDoItemLineTrace _returnvalue self (Utilities|Array|MakeArray "ObjectTypeQuery9") false))
            (CallFunction|CopySettingsEvent _result)))))))

(event Input|ActionEvents|InputActionFire
  (:Pressed
    (bind _returnvalue (Class|Actor|GetOwnerController))
    (Utilities|SPIsPlacingStructure _returnvalue
      (:No
        (Utilities|SPIsRadialMenuOpen _returnvalue
          (:No
            (bind _result (CallFunction|SPDoItemLineTrace _returnvalue self (Utilities|Array|MakeArray "ObjectTypeQuery9") false))
            (Utilities|IsValid _result
              (:Is%20Valid
                (CallFunction|ExecuteTurretOptionsEvent _result)))))))))

(event Input|MouseEvents|RightMouseButton
  (:Pressed
    (bind _returnvalue (Class|Actor|GetOwnerController))
    (Utilities|SPIsRadialMenuOpen _returnvalue
      (:No
        (Utilities|SPIsPlacingStructure _returnvalue
          (:No
            (Class|ShooterWeapon|PlayWeaponAnimation (Variables|Default|GetFireAnim) false false false false false false)))))))

(event Input|MouseEvents|LeftMouseButton
  (:Pressed
    (bind _returnvalue (Class|Actor|GetOwnerController))
    (Utilities|SPIsRadialMenuOpen _returnvalue
      (:No
        (Utilities|SPIsPlacingStructure _returnvalue
          (:No
            (Class|ShooterWeapon|PlayWeaponAnimation (Variables|Default|GetFireAnim) false false false false false false)))))))

(event Input|GamepadEvents|GamepadRightTrigger
  (:Pressed
    (bind _returnvalue (Class|Actor|GetOwnerController))
    (Utilities|SPIsRadialMenuOpen _returnvalue
      (:No
        (Utilities|SPIsPlacingStructure _returnvalue
          (:No
            (Class|ShooterWeapon|PlayWeaponAnimation (Variables|Default|GetFireAnim) false false false false false false)))))))

(event Input|GamepadEvents|GamepadLeftTrigger
  (:Pressed
    (bind _returnvalue (Class|Actor|GetOwnerController))
    (Utilities|SPIsRadialMenuOpen _returnvalue
      (:No
        (Utilities|SPIsPlacingStructure _returnvalue
          (:No
            (Class|ShooterWeapon|PlayWeaponAnimation (Variables|Default|GetFireAnim) false false false false false false)))))))

(fn ConstructionScript)

(fn CopySettings
  (params (Target :type Actor%20Object%20Reference))
  (bind _returnvalue (Class|Actor|GetOwnerController))
  (bind _asshooterplayercontroller (Utilities|Casting|CastToShooterPlayerController _returnvalue))
  (if (not (Variables|Default|GetHasSavedSettings))
    (Variables|Default|SetHasSavedSettings true)
    (bind _asprimalstructureturret (Utilities|Casting|CastToPrimalStructureTurret Target))
    (Utilities|FlowControl|Sequence
      (:then_0
        (bind _assplus_iturret_c (Utilities|Casting|CastToSPlus_ITurret (Class|TargetableInterface|ToUObject _asprimalstructureturret))
          (:then
            (bind _turretoptions (Default|ITurretGetOptions _assplus_iturret_c))
            (Variables|Default|SetSavedSettings _turretoptions))
          (:CastFailed
            (Utilities|Struct|SetmembersinSPTurretOptions (Variables|Default|GetSavedSettings) (Variables|/Script/ShooterGame.PrimalStructureTurret|GetRangeSetting _asprimalstructureturret) (Variables|/Script/ShooterGame.PrimalStructureTurret|GetAISetting _asprimalstructureturret) (Variables|/Script/ShooterGame.PrimalStructureTurret|GetWarningSetting _asprimalstructureturret))
            (bind _asstructureturrettek_c (Utilities|Casting|CastToStructureTurretTek Target)
              (:then
                (Utilities|Struct|SetmembersinSPTurretOptions (Variables|Default|GetSavedSettings) (Variables|/Game/PrimalEarth/Structures/BuildingBases/StructureTurretTek.StructureTurretTek_C|GetMinDinoLevel _asstructureturrettek_c) (Variables|/Game/PrimalEarth/Structures/BuildingBases/StructureTurretTek.StructureTurretTek_C|GetMaxDinoLevel _asstructureturrettek_c) (Variables|/Game/PrimalEarth/Structures/BuildingBases/StructureTurretTek.StructureTurretTek_C|GetDinoClassList _asstructureturrettek_c) (Variables|/Game/PrimalEarth/Structures/BuildingBases/StructureTurretTek.StructureTurretTek_C|GetbIsInclusionList _asstructureturrettek_c)))
              (:CastFailed
                (Utilities|Struct|SetmembersinSPTurretOptions (Variables|Default|GetSavedSettings) 0 0 (Utilities|Array|MakeArray) false))))))
      (:then_1
        (Class|ShooterPlayerController|ClientServerNotification _asshooterplayercontroller "Settings copied." "(R=0.000000,G=1.000000,B=0.061501,A=1.000000)" 1.5 3.0)))
    (else
      (Variables|Default|SetHasSavedSettings false)
      (Class|ShooterPlayerController|ClientServerNotification _asshooterplayercontroller "Settings cleared." "(R=0.000000,G=1.000000,B=0.061501,A=1.000000)" 1.5 3.0))))

(fn PasteSettings
  (params (Target :type Actor%20Object%20Reference))
  (bind _savedsettings (Variables|Default|GetSavedSettings))
  (bind (_mindinolevel _maxdinolevel _dinolist _isinclusionlist) (Utilities|Struct|BreakSPTurretOptions _savedsettings))
  (bind _asprimalstructureturret (Utilities|Casting|CastToPrimalStructureTurret Target))
  (CallFunction|SPSetTurretOptions _asprimalstructureturret _savedsettings)
  (Utilities|FlowControl|Sequence
    (:then_0
      (bind _assplus_iturret_c (Utilities|Casting|CastToSPlus_ITurret (Class|TargetableInterface|ToUObject _asprimalstructureturret))
        (:then
          (Default|ITurretSetOptions _assplus_iturret_c (Variables|Default|GetSavedSettings)))
        (:CastFailed
          (bind _asstructureturrettek_c (Utilities|Casting|CastToStructureTurretTek Target))
          (Variables|/Game/PrimalEarth/Structures/BuildingBases/StructureTurretTek.StructureTurretTek_C|SetMinDinoLevel _asstructureturrettek_c _mindinolevel false)
          (Variables|/Game/PrimalEarth/Structures/BuildingBases/StructureTurretTek.StructureTurretTek_C|SetMaxDinoLevel _asstructureturrettek_c _maxdinolevel false)
          (Variables|/Game/PrimalEarth/Structures/BuildingBases/StructureTurretTek.StructureTurretTek_C|SetDinoClassList _asstructureturrettek_c _dinolist false)
          (Variables|/Game/PrimalEarth/Structures/BuildingBases/StructureTurretTek.StructureTurretTek_C|SetbIsInclusionList _asstructureturrettek_c _isinclusionlist false))))
    (:then_1
      (bind _returnvalue (Class|Actor|GetOwnerController))
      (bind _asshooterplayercontroller (Utilities|Casting|CastToShooterPlayerController _returnvalue))
      (Class|ShooterPlayerController|ClientServerNotification _asshooterplayercontroller "Settings changed." "(R=0.069651,G=0.000000,B=1.000000,A=1.000000)" 1.5 3.0)
      (Networking|ForceNetUpdate _asprimalstructureturret))))

(fn ToggleActive
  (params (Target :type Actor%20Object%20Reference)))

(fn TransferAmmo
  (params (Target :type Actor%20Object%20Reference))
  (bind _asbp_autoturrettek_c (Utilities|Casting|CastToBP_AutoTurretTek Target)
    (:then
      (CallFunction|HandleAmmoTransfer (Variables|/Script/ShooterGame.PrimalStructureItemContainer|GetMyInventoryComponent _asbp_autoturrettek_c) true))
    (:CastFailed
      (bind _asstructureturrettek_c (Utilities|Casting|CastToStructureTurretTek Target)
        (:then
          (CallFunction|HandleAmmoTransfer (Variables|/Script/ShooterGame.PrimalStructureItemContainer|GetMyInventoryComponent _asstructureturrettek_c) true))
        (:CastFailed
          (bind _asprimalstructureturret (Utilities|Casting|CastToPrimalStructureTurret Target))
          (CallFunction|HandleAmmoTransfer (Variables|/Script/ShooterGame.PrimalStructureItemContainer|GetMyInventoryComponent _asprimalstructureturret) false))))))

(fn HandleAmmoTransfer
  (params (Inventory :type Primal%20Inventory%20Component%20Object%20Reference) (IsTek :type Boolean))
  (bind _returnvalue (Class|Actor|GetOwnerController))
  (bind _asshooterplayercontroller (Utilities|Casting|CastToShooterPlayerController _returnvalue))
  (if IsTek
    (bind _returnvalue_2 (Class|PrimalInventoryComponent|GetItemTemplateQuantity (Variables|/Script/ShooterGame.PrimalCharacter|GetMyInventoryComponent (Class|ShooterPlayerController|GetPlayerCharacter _asshooterplayercontroller)) "/Game/PrimalEarth/CoreBlueprints/Resources/PrimalItemResource_ElementShard.PrimalItemResource_ElementShard_C" 0 true false false))
    (if (and (> _returnvalue_2 0) (< (Utilities|Array|Length (Variables|/Script/ShooterGame.PrimalInventoryComponent|GetInventoryItems Inventory)) (Variables|/Script/ShooterGame.PrimalInventoryComponent|GetMaxInventoryItems Inventory)))
      (LocalVariables|SetTransferQty (Math|Integer|SelectInt 50 _returnvalue_2 (> _returnvalue_2 50)))
      (Class|PrimalInventoryComponent|BPIncrementItemTemplateQuantity (Variables|/Script/ShooterGame.PrimalCharacter|GetMyInventoryComponent (Class|ShooterPlayerController|GetPlayerCharacter _asshooterplayercontroller)) "/Game/PrimalEarth/CoreBlueprints/Resources/PrimalItemResource_ElementShard.PrimalItemResource_ElementShard_C" (* (LocalVariables|GetTransferQty) -1) true false false false false false 0 false)
      (Class|PrimalInventoryComponent|BPIncrementItemTemplateQuantity Inventory "/Game/PrimalEarth/CoreBlueprints/Resources/PrimalItemResource_ElementShard.PrimalItemResource_ElementShard_C" (LocalVariables|GetTransferQty) true false false false false false 0 false))
    (else
      (bind _returnvalue_3 (Class|PrimalInventoryComponent|GetItemTemplateQuantity (Variables|/Script/ShooterGame.PrimalCharacter|GetMyInventoryComponent (Class|ShooterPlayerController|GetPlayerCharacter _asshooterplayercontroller)) "/Game/PrimalEarth/CoreBlueprints/Weapons/PrimalItemAmmo_AdvancedRifleBullet.PrimalItemAmmo_AdvancedRifleBullet_C" 0 true false false))
      (if (and (> _returnvalue_3 0) (< (Utilities|Array|Length (Variables|/Script/ShooterGame.PrimalInventoryComponent|GetInventoryItems Inventory)) (Variables|/Script/ShooterGame.PrimalInventoryComponent|GetMaxInventoryItems Inventory)))
        (LocalVariables|SetTransferQty (Math|Integer|SelectInt 50 _returnvalue_3 (> _returnvalue_3 50)))
        (Class|PrimalInventoryComponent|BPIncrementItemTemplateQuantity (Variables|/Script/ShooterGame.PrimalCharacter|GetMyInventoryComponent (Class|ShooterPlayerController|GetPlayerCharacter _asshooterplayercontroller)) "/Game/PrimalEarth/CoreBlueprints/Weapons/PrimalItemAmmo_AdvancedRifleBullet.PrimalItemAmmo_AdvancedRifleBullet_C" (* (LocalVariables|GetTransferQty) -1) true false false false false false 0 false)
        (Class|PrimalInventoryComponent|BPIncrementItemTemplateQuantity Inventory "/Game/PrimalEarth/CoreBlueprints/Weapons/PrimalItemAmmo_AdvancedRifleBullet.PrimalItemAmmo_AdvancedRifleBullet_C" (LocalVariables|GetTransferQty) true false false false false false 0 false)))))