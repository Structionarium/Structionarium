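; Handheld Structures Plus tool that changes glass structure transparency remotely via line trace, ignoring input during placement or radial menus.
; Fire applies the transparency buff's saved settings through SPlus_IGlass, or delegates to the buff when none are saved.
; Targeting hands the traced structure, or an empty hit, to the buff to handle saved settings.
; Valid targets are filtered by class-name substring blacklist, and EndPlay removes the buff on authority.
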(event Custom|ExecuteTransparencyEvent
  (params (Target :type Actor%20Object%20Reference))
  (Utilities|FlowControl|Sequence
    (:then_0
      (bind _buff (CallFunction|SPApplyBufffromWeapon self "/Game/Mods/StructuresPlusMod/_Buffs/Buff_StructuresPlus_Transparency.Buff_StructuresPlus_Transparency_C"))
      (bind _asbuff_structuresplus_transparency_c (Utilities|Casting|CastToBuff_StructuresPlus_Transparency _buff))
      (Variables|Default|SetBuffRef _asbuff_structuresplus_transparency_c))
    (:then_1
      (if (not (Variables|/Game/Mods/StructuresPlusMod/_Buffs/Buff_StructuresPlus_Transparency.Buff_StructuresPlus_Transparency_C|GetHasSavedValues (Variables|Default|GetBuffRef)))
        (Default|RemoteSetTransparencyEvent (Variables|Default|GetBuffRef) Target)
        (else
          (bind _asprimalstructure (Utilities|Casting|CastToPrimalStructure Target))
          (bind _assplus_iglass_c (Utilities|Casting|CastToSPlus_IGlass (Class|TargetableInterface|ToUObject _asprimalstructure)))
          (Default|IGlassSetTransparency _assplus_iglass_c (Utilities|Struct|MakeSPGlassSettings (Variables|/Game/Mods/StructuresPlusMod/_Buffs/Buff_StructuresPlus_Transparency.Buff_StructuresPlus_Transparency_C|GetSavedTransparency (Variables|Default|GetBuffRef)) (Variables|/Game/Mods/StructuresPlusMod/_Buffs/Buff_StructuresPlus_Transparency.Buff_StructuresPlus_Transparency_C|GetSavedOpacity (Variables|Default|GetBuffRef)))))))))

(event Custom|SaveTransparencySettingsEvent
  (params (Target :type Actor%20Object%20Reference))
  (Utilities|FlowControl|Sequence
    (:then_0
      (bind _buff (CallFunction|SPApplyBufffromWeapon self "/Game/Mods/StructuresPlusMod/_Buffs/Buff_StructuresPlus_Transparency.Buff_StructuresPlus_Transparency_C"))
      (bind _asbuff_structuresplus_transparency_c (Utilities|Casting|CastToBuff_StructuresPlus_Transparency _buff))
      (Variables|Default|SetBuffRef _asbuff_structuresplus_transparency_c))
    (:then_1
      (Default|HandleGunTransparencyEvent (Variables|Default|GetBuffRef) Target))))

(event EventBeginPlay
  (Utilities|FlowControl|Delay 0.2)
  (bind _returnvalue (Class|Actor|GetOwnerController))
  (if (Pawn|IsLocalController _returnvalue)
    (Input|EnableInput _returnvalue)))

(event EventEndPlay
  (params (EndPlayReason :type EEndPlayReason%20Enum :default "ActorDestroyed"))
  (bind _buffref (Variables|Default|GetBuffRef))
  (Networking|SwitchHasAuthority
    (:Authority
      (Utilities|IsValid _buffref
        (:Is%20Valid
          (Default|RemoveBuffEvent _buffref))))))

(event Input|ActionEvents|InputActionGamepadRightFire
  (:Pressed
    (bind _returnvalue (Class|Actor|GetOwnerController))
    (Utilities|SPIsPlacingStructure _returnvalue
      (:No
        (Utilities|SPIsRadialMenuOpen _returnvalue
          (:No
            (bind _result (CallFunction|SPDoItemLineTrace _returnvalue self (Utilities|Array|MakeArray "ObjectTypeQuery9") false))
            (Utilities|IsValid _result
              (:Is%20Valid
                (if (CallFunction|CheckBlackList _result)
                  (CallFunction|ExecuteTransparencyEvent _result))))))))))

(event Input|ActionEvents|InputActionGamepadLeftFire
  (:Pressed
    (bind _returnvalue (Class|Actor|GetOwnerController))
    (Utilities|SPIsPlacingStructure _returnvalue
      (:No
        (Utilities|SPIsRadialMenuOpen _returnvalue
          (:No
            (bind _result (CallFunction|SPDoItemLineTrace _returnvalue self (Utilities|Array|MakeArray "ObjectTypeQuery9") false))
            (Utilities|IsValid _result
              (:Is%20Valid
                (if (CallFunction|CheckBlackList _result)
                  (CallFunction|SaveTransparencySettingsEvent _result :!label _label)))
              (:Is%20Not%20Valid
                (goto _label)))))))))

(event Input|ActionEvents|InputActionTargeting
  (:Pressed
    (bind _returnvalue (Class|Actor|GetOwnerController))
    (Utilities|SPIsPlacingStructure _returnvalue
      (:No
        (Utilities|SPIsRadialMenuOpen _returnvalue
          (:No
            (bind _result (CallFunction|SPDoItemLineTrace _returnvalue self (Utilities|Array|MakeArray "ObjectTypeQuery9") false))
            (Utilities|IsValid _result
              (:Is%20Valid
                (if (CallFunction|CheckBlackList _result)
                  (CallFunction|SaveTransparencySettingsEvent _result :!label _label)))
              (:Is%20Not%20Valid
                (goto _label)))))))))

(event Input|ActionEvents|InputActionFire
  (:Pressed
    (bind _returnvalue (Class|Actor|GetOwnerController))
    (Utilities|SPIsPlacingStructure _returnvalue
      (:No
        (Utilities|SPIsRadialMenuOpen _returnvalue
          (:No
            (bind _result (CallFunction|SPDoItemLineTrace _returnvalue self (Utilities|Array|MakeArray "ObjectTypeQuery9") false))
            (Utilities|IsValid _result
              (:Is%20Valid
                (if (CallFunction|CheckBlackList _result)
                  (CallFunction|ExecuteTransparencyEvent _result))))))))))

(event Input|MouseEvents|RightMouseButton
  (:Pressed
    (bind _returnvalue (Class|Actor|GetOwnerController))
    (Utilities|SPIsRadialMenuOpen _returnvalue
      (:No
        (Utilities|SPIsPlacingStructure _returnvalue
          (:No
            (Class|ShooterWeapon|PlayWeaponAnimation (Variables|Default|GetFireAnim) false false false false false false)))))))

(event Input|MouseEvents|LeftMouseButton
  (:Pressed
    (bind _returnvalue (Class|Actor|GetOwnerController))
    (Utilities|SPIsRadialMenuOpen _returnvalue
      (:No
        (Utilities|SPIsPlacingStructure _returnvalue
          (:No
            (Class|ShooterWeapon|PlayWeaponAnimation (Variables|Default|GetFireAnim) false false false false false false)))))))

(event Input|GamepadEvents|GamepadRightTrigger
  (:Pressed
    (bind _returnvalue (Class|Actor|GetOwnerController))
    (Utilities|SPIsRadialMenuOpen _returnvalue
      (:No
        (Utilities|SPIsPlacingStructure _returnvalue
          (:No
            (Class|ShooterWeapon|PlayWeaponAnimation (Variables|Default|GetFireAnim) false false false false false false)))))))

(event Input|GamepadEvents|GamepadLeftTrigger
  (:Pressed
    (bind _returnvalue (Class|Actor|GetOwnerController))
    (Utilities|SPIsRadialMenuOpen _returnvalue
      (:No
        (Utilities|SPIsPlacingStructure _returnvalue
          (:No
            (Class|ShooterWeapon|PlayWeaponAnimation (Variables|Default|GetFireAnim) false false false false false false)))))))

(fn ConstructionScript)

(fn CheckBlackList
  (params (Actor :type Actor%20Object%20Reference))
  (bind _array_element (Utilities|Array|ForEachLoopwithBreak (Variables|Default|GetBlackListedClasses) :!label _label)
    (:LoopBody
      (if (>= (Utilities|String|FindSubstring (Utilities|GetClassDisplayName (Utilities|GetClass Actor)) _array_element) 0)
        (LocalVariables|SetIsBlackListed true)
        (goto _label Break)))
    (:Completed
      (return (not (LocalVariables|GetIsBlackListed))))))