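; Pillarator weapon for editing dynamic pillars, with copy and paste of pillar shape settings.
; Fire line-traces for a pillar and applies a buff, which opens its UI or, if settings are saved, the pillar takes them and replicates.
; Targeting toggles between saving the traced pillar's length, thickness and rotation and clearing them.
; Settings persist in the item's custom data, and the buff is removed on EndPlay.
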(event Custom|ApplyChangesEvent
  (params (Pillar :type Base%20Dynamic%20Pillar%20Object%20Reference))
  (bind (_hassaveddata _data) (CallFunction|GetSavedSettings))
  (Utilities|FlowControl|Sequence
    (:then_0
      (bind _buff (CallFunction|SPApplyBufffromWeapon self "/Game/Mods/StructuresPlusMod/_Buffs/Buff_StructuresPlus_DynamicPillar.Buff_StructuresPlus_DynamicPillar_C"))
      (bind _asbuff_structuresplus_dynamicpillar_c (Utilities|Casting|CastToBuff_StructuresPlus_DynamicPillar _buff))
      (Variables|Default|SetBuffRef _asbuff_structuresplus_dynamicpillar_c))
    (:then_1
      (if (not _hassaveddata)
        (Default|InitializeUI (Variables|Default|GetBuffRef) Pillar)
        (else
          (Variables|/Game/Mods/StructuresPlusMod/Structures/Pillars/Base_DynamicPillar.Base_DynamicPillar_C|SetPillarData Pillar _data false)
          (Class|Actor|MulticastProperty Pillar "PillarData")
          (Default|InitializePillar Pillar))))))

(event Custom|SaveChangesEvent
  (params (Actor :type Actor%20Object%20Reference))
  (bind _returnvalue (Class|Actor|GetOwnerController))
  (if (.HasSavedData (CallFunction|GetSavedSettings))
    (CallFunction|ClearSettings)
    (CallFunction|SPMessageClient _returnvalue "Settings Cleared." "NewEnumerator3")
    (else
      (bind _asbase_dynamicpillar_c (Utilities|Casting|CastToBase_DynamicPillar Actor))
      (CallFunction|SaveSettings (Variables|/Game/Mods/StructuresPlusMod/Structures/Pillars/Base_DynamicPillar.Base_DynamicPillar_C|GetPillarData _asbase_dynamicpillar_c))
      (CallFunction|SPMessageClient _returnvalue "Settings Saved." "NewEnumerator3"))))

(event EventBeginPlay
  (Utilities|FlowControl|Delay 0.2)
  (bind _returnvalue (Class|Actor|GetOwnerController))
  (if (Pawn|IsLocalController _returnvalue)
    (Input|EnableInput _returnvalue)))

(event EventEndPlay
  (params (EndPlayReason :type EEndPlayReason%20Enum :default "ActorDestroyed"))
  (bind _buffref (Variables|Default|GetBuffRef))
  (Networking|SwitchHasAuthority
    (:Authority
      (Utilities|IsValid _buffref
        (:Is%20Valid
          (Default|RemoveBuffEvent _buffref))))))

(event Input|ActionEvents|InputActionGamepadRightFire
  (:Pressed
    (bind _returnvalue (Class|Actor|GetOwnerController))
    (Utilities|SPIsPlacingStructure _returnvalue
      (:No
        (Utilities|SPIsRadialMenuOpen _returnvalue
          (:No
            (bind _result (CallFunction|SPDoItemLineTrace _returnvalue self (Utilities|Array|MakeArray "ObjectTypeQuery9") false))
            (Utilities|IsValid _result
              (:Is%20Valid
                (bind _asbase_dynamicpillar_c (Utilities|Casting|CastToBase_DynamicPillar _result))
                (CallFunction|ApplyChangesEvent _asbase_dynamicpillar_c)))))))))

(event Input|ActionEvents|InputActionGamepadLeftFire
  (:Pressed
    (bind _returnvalue (Class|Actor|GetOwnerController))
    (Utilities|SPIsPlacingStructure _returnvalue
      (:No
        (Utilities|SPIsRadialMenuOpen _returnvalue
          (:No
            (bind _result (CallFunction|SPDoItemLineTrace _returnvalue self (Utilities|Array|MakeArray "ObjectTypeQuery9") false))
            (CallFunction|SaveChangesEvent _result)))))))

(event Input|ActionEvents|InputActionTargeting
  (:Pressed
    (bind _returnvalue (Class|Actor|GetOwnerController))
    (Utilities|SPIsPlacingStructure _returnvalue
      (:No
        (Utilities|SPIsRadialMenuOpen _returnvalue
          (:No
            (bind _result (CallFunction|SPDoItemLineTrace _returnvalue self (Utilities|Array|MakeArray "ObjectTypeQuery9") false))
            (CallFunction|SaveChangesEvent _result)))))))

(event Input|ActionEvents|InputActionFire
  (:Pressed
    (bind _returnvalue (Class|Actor|GetOwnerController))
    (Utilities|SPIsPlacingStructure _returnvalue
      (:No
        (Utilities|SPIsRadialMenuOpen _returnvalue
          (:No
            (bind _result (CallFunction|SPDoItemLineTrace _returnvalue self (Utilities|Array|MakeArray "ObjectTypeQuery9") false))
            (Utilities|IsValid _result
              (:Is%20Valid
                (bind _asbase_dynamicpillar_c (Utilities|Casting|CastToBase_DynamicPillar _result))
                (CallFunction|ApplyChangesEvent _asbase_dynamicpillar_c)))))))))

(event Input|MouseEvents|RightMouseButton
  (:Pressed
    (bind _returnvalue (Class|Actor|GetOwnerController))
    (Utilities|SPIsRadialMenuOpen _returnvalue
      (:No
        (Utilities|SPIsPlacingStructure _returnvalue
          (:No
            (Class|ShooterWeapon|PlayWeaponAnimation (Variables|Default|GetFireAnim) false false false false false false)))))))

(event Input|MouseEvents|LeftMouseButton
  (:Pressed
    (bind _returnvalue (Class|Actor|GetOwnerController))
    (Utilities|SPIsRadialMenuOpen _returnvalue
      (:No
        (Utilities|SPIsPlacingStructure _returnvalue
          (:No
            (Class|ShooterWeapon|PlayWeaponAnimation (Variables|Default|GetFireAnim) false false false false false false)))))))

(event Input|GamepadEvents|GamepadRightTrigger
  (:Pressed
    (bind _returnvalue (Class|Actor|GetOwnerController))
    (Utilities|SPIsRadialMenuOpen _returnvalue
      (:No
        (Utilities|SPIsPlacingStructure _returnvalue
          (:No
            (Class|ShooterWeapon|PlayWeaponAnimation (Variables|Default|GetFireAnim) false false false false false false)))))))

(event Input|GamepadEvents|GamepadLeftTrigger
  (:Pressed
    (bind _returnvalue (Class|Actor|GetOwnerController))
    (Utilities|SPIsRadialMenuOpen _returnvalue
      (:No
        (Utilities|SPIsPlacingStructure _returnvalue
          (:No
            (Class|ShooterWeapon|PlayWeaponAnimation (Variables|Default|GetFireAnim) false false false false false false)))))))

(fn ConstructionScript)

(fn GetSavedSettings
  (bind _associatedprimalitem (Variables|Default|GetAssociatedPrimalItem))
  (Utilities|FlowControl|Sequence
    (:then_0
      (Utilities|IsValid _associatedprimalitem
        (:Is%20Valid
          (bind (_outdata _returnvalue) (Class|PrimalItem|GetCustomItemData _associatedprimalitem "Splus_Pillarator"))
          (if _returnvalue
            (if (>= (Utilities|Array|Length (Utilities|Struct|BreakCustomItemData _outdata)) 4)
              (LocalVariables|SetHasData true)
              (LocalVariables|SetSavedData (Utilities|Struct|MakeSP_DynamicPillarData (Utilities|Array|Get(acopy) (Utilities|Struct|BreakCustomItemData _outdata)) (Utilities|Array|Get(acopy) (Utilities|Struct|BreakCustomItemData _outdata) 1) (Utilities|Array|Get(acopy) (Utilities|Struct|BreakCustomItemData _outdata) 2) (Utilities|Array|Get(acopy) (Utilities|Struct|BreakCustomItemData _outdata) 3))))))))
    (:then_1
      (return (LocalVariables|GetHasData) (LocalVariables|GetSavedData)))))

(fn SaveSettings
  (params (PillarData :type SP%20Dynamic%20Pillar%20Data%20Structure))
  (bind (_length _thickness _rot_x _rot_y) (Utilities|Struct|BreakSP_DynamicPillarData PillarData))
  (bind _associatedprimalitem (Variables|Default|GetAssociatedPrimalItem))
  (Utilities|IsValid _associatedprimalitem
    (:Is%20Valid
      (Class|PrimalItem|SetCustomItemData _associatedprimalitem (Utilities|Struct|MakeCustomItemData "Splus_Pillarator" (Utilities|Array|MakeArray _length _thickness _rot_x _rot_y))))))

(fn ClearSettings
  (bind _associatedprimalitem (Variables|Default|GetAssociatedPrimalItem))
  (Utilities|IsValid _associatedprimalitem
    (:Is%20Valid
      (Class|PrimalItem|RemoveCustomItemData _associatedprimalitem "Splus_Pillarator"))))