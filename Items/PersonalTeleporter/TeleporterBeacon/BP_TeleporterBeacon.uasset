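; BP_TeleporterBeacon is the placed beacon actor of the personal teleporter item, which removes itself after a limited lifespan.
; Shortly after BeginPlay, the server destroys its inventory component and reads the lifespan from a game mode INI option, with a default and an upper cap.
; A one-shot timer then fires DestroySelfEvent to destroy the actor.
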(event Custom|DestroySelfEvent
  (Actor|DestroyActor))

(event EventBeginPlay
  (Utilities|FlowControl|Delay 0.2)
  (Networking|SwitchHasAuthority
    (:Authority
      (Components|DestroyComponent (Variables|Default|GetMyInventoryComponent))
      (bind _value (CallFunction|SPGetFloatIniOption (Game|GetGameMode) "PersonalTeleporterBeaconLifespanInSeconds" 3e+02 3.6e+03))
      (Utilities|Time|SetTimerbyEvent (delegate Custom|DestroySelfEvent) _value))))

(fn ConstructionScript
  (|CallParentFunction))