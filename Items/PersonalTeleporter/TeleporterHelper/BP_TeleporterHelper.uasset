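; Short-lived helper actor for the personal teleporter that lets a player fast travel to a Tek Teleporter.
; A teleport request opens the local player's spawn UI, reusing bed fast travel filtered to TekTeleporter, with team and activation checks.
; Choosing a destination moves the pawn with sound and VFX at both ends, scaling effects by dino drag weight.
; The helper destroys itself after travel, or on a server-side timeout if unused.
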(event Custom|DoTeleportOutVFX
  (params (EffectScale :type Float%20%28single-precision%29) (EffectLoc :type Vector) (EffectRot :type Rotator))
  (if (not (Networking|IsDedicatedServer))
    (bind _returnvalue (Effects|SpawnEmitteratLocation (Variables|Default|GetTeleportOutEmitter) EffectLoc EffectRot true true 1.5e+03))
    (Transformation|SetWorldScale3D _returnvalue (Math|Conversions|ToVector(Float) EffectScale))))

(event Custom|DoPlayTeleportOutSound
  (Audio|PlaySoundatLocation (Variables|Default|GetTeleportOutSound) (Transformation|GetActorLocation)))

(event Custom|TeleportRequestEvent
  (params (PC :type Player%20Controller%20Object%20Reference))
  (CallFunction|ShowSpawnUIEvent PC))

(event Custom|ShowSpawnUIEvent
  (params (PC :type Player%20Controller%20Object%20Reference))
  (if (not (Networking|IsDedicatedServer))
    (if (== PC (Game|GetPlayerController 0))
      (bind _asshooterhud (Utilities|Casting|CastToShooterHUD (HUD|GetHUD PC)))
      (Class|ShooterHUD|ShowSpawnUI _asshooterhud self))))

(event Custom|DestroyActorEvent
  (Utilities|FlowControl|Delay 0.2)
  (Actor|DestroyActor))

(event EventBeginPlay
  (Networking|SwitchHasAuthority
    (:Authority
      (Utilities|Time|SetTimerbyEvent (delegate Custom|DestroyActorEvent) 9e+01))))

(fn ConstructionScript
  (|CallParentFunction))

(fn DoTeleport
  (params (ToTeleporter :type Tek%20Teleporter%20Object%20Reference) (SPC :type Shooter%20Player%20Controller%20Object%20Reference))
  (bind _returnvalue (Class|ShooterPlayerController|GetPlayerCharacter SPC))
  (bind _returnvalue_2 (Pawn|GetControlledPawn SPC))
  (bind _returnvalue_3 (Transformation|GetActorTransform ToTeleporter))
  (bind (_location _rotation) (Math|Transform|BreakTransform _returnvalue_3))
  (bind _outscale (CallFunction|GetTeleportEffectScale _returnvalue))
  (Utilities|IsValid ToTeleporter
    (:Is%20Valid
      (CallFunction|DoPlayTeleportOutSound)
      (Default|DoPlayTeleportinSound ToTeleporter)
      (CallFunction|DoTeleportOutVFX _outscale (Transformation|GetActorLocation SPC) (Transformation|GetActorRotation SPC))
      (Transformation|Teleport _returnvalue_2 (+ _location "-50.000000, 0,50.000000") _rotation)
      (Networking|ForceNetUpdate SPC)
      (Default|DoTeleportinVFX ToTeleporter _outscale (Transformation|GetActorLocation _returnvalue_2) (Transformation|GetActorRotation _returnvalue_2)))))

(fn BPHandleBedFastTravel
  (params (ForPC :type Shooter%20Player%20Controller%20Object%20Reference) (ToBed :type Primal%20Structure%20Object%20Reference))
  (bind _astekteleporter_c (Utilities|Casting|CastToTekTeleporter ToBed))
  (CallFunction|DoTeleport _astekteleporter_c ForPC)
  (CallFunction|DestroyActorEvent)
  (return true))

(fn GetBedFilterClass
  (return "/Game/PrimalEarth/Structures/TekTier/TekTeleporter.TekTeleporter_C"))

(fn GetTeleportEffectScale
  (params (ForCharacter :type Primal%20Character%20Object%20Reference))
  (bind _teleporteffectscaledinomindrag (Variables|Default|GetTeleportEffectScaleDinoMinDrag))
  (bind _teleporteffectscaledinomaxdrag (Variables|Default|GetTeleportEffectScaleDinoMaxDrag))
  (Utilities|FlowControl|Sequence
    (:then_0
      (Utilities|Casting|CastToShooterCharacter ForCharacter
        (:then
          (LocalVariables|SetretVal (Variables|Default|GetElementCostPlayer)))
        (:CastFailed
          (bind _asprimaldinocharacter (Utilities|Casting|CastToPrimalDinoCharacter ForCharacter))
          (LocalVariables|SetretVal (Class|KismetMathLibrary|MapRange (Math|Float|Clamp(Float) (Variables|/Script/ShooterGame.PrimalCharacter|GetDragWeight _asprimaldinocharacter) _teleporteffectscaledinomindrag _teleporteffectscaledinomaxdrag) _teleporteffectscaledinomindrag _teleporteffectscaledinomaxdrag (Variables|Default|GetTeleportEffectScaleDinoMinScale) (Variables|Default|GetTeleportEffectScaleDinoMaxScale))))))
    (:then_1
      (return (LocalVariables|GetretVal)))))

(fn BPPreventSpawnforPlayer
  (params (PC :type Shooter%20Player%20Controller%20Object%20Reference) (bCheckCooldownTime :type Boolean) (FromStructure :type Primal%20Structure%20Object%20Reference))
  (return (or (!= (Variables|/Script/Engine.Actor|GetTargetingTeam PC) (Variables|Default|GetTargetingTeam)) (not (Variables|Default|GetbContainerActivated)))))