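; Handheld personal teleporter weapon that lets a player request teleports and place a personal beacon.
; Fire spawns a BP_TeleporterHelper that handles the request, unless the player is mounted.
; Targeting spends loaded element shards to replace the player's existing beacon, after checking for nearby enemy structures and boss arenas.
; Game mode options, read on the authority, can disable beacons or allow placement inside boss arenas.
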(event Custom|TryPlaceBeaconEvent
  (bind _returnvalue (Components|GetOwner))
  (bind _associatedprimalitem (Variables|Default|GetAssociatedPrimalItem))
  (if (not (Variables|Default|GetDisablePersonalBeacon))
    (bind _returnvalue_2 (Class|Actor|GetOwnerController))
    (bind _asshooterplayercontroller (Utilities|Casting|CastToShooterPlayerController _returnvalue_2))
    (bind _isallowed (CallFunction|IsAllowedtoPlaceBeacon _asshooterplayercontroller))
    (if _isallowed
      (bind _returnvalue_3 (Class|PrimalItem|GetWeaponClipAmmo _associatedprimalitem))
      (Class|PrimalInventoryComponent|UpdateNetWeaponClipAmmo (Variables|/Script/ShooterGame.PrimalCharacter|GetMyInventoryComponent (Class|ShooterPlayerController|GetPlayerCharacter _asshooterplayercontroller)) _associatedprimalitem (- _returnvalue_3 10))
      (CallFunction|DestroyExistingBeacon)
      (bind _returnvalue_4 (Class|ShooterPlayerController|GetPlayerCharacterName _asshooterplayercontroller))
      (bind _returnvalue_5 (Game|SpawnActorfromClass "/Game/Mods/StructuresPlusMod/Items/PersonalTeleporter/TeleporterBeacon/BP_TeleporterBeacon.BP_TeleporterBeacon_C" (Math|Transform|MakeTransform (+ (Transformation|GetActorLocation _returnvalue) "0, 0,50.000000") "0, 0, 0" "1,1,1") true 0))
      (Variables|/Game/Mods/StructuresPlusMod/Items/PersonalTeleporter/TeleporterBeacon/BP_TeleporterBeacon.BP_TeleporterBeacon_C|SetOwningPC _returnvalue_5 _returnvalue_2)
      (Variables|/Script/Engine.Actor|SetTargetingTeam _returnvalue_5 (Variables|/Script/Engine.Actor|GetTargetingTeam _returnvalue) false)
      (Variables|/Script/ShooterGame.PrimalTargetableActor|SetDescriptiveName _returnvalue_5 _returnvalue_4)
      (Networking|ForceNetUpdate))))

(event Custom|SpawnTeleporterHelperEvent
  (bind _returnvalue (Game|SpawnActorfromClass "/Game/Mods/StructuresPlusMod/Items/PersonalTeleporter/TeleporterHelper/BP_TeleporterHelper.BP_TeleporterHelper_C" (Transformation|GetActorTransform (Components|GetOwner)) true 0))
  (bind _returnvalue_2 (Class|Actor|GetOwnerController))
  (Variables|/Script/Engine.Actor|SetTargetingTeam _returnvalue (Variables|/Script/Engine.Actor|GetTargetingTeam _returnvalue_2) false)
  (Default|TeleportRequestEvent _returnvalue _returnvalue_2))

(event EventBeginPlay
  (bind _returnvalue (Game|GetGameMode))
  (Utilities|FlowControl|Delay 0.2)
  (Utilities|FlowControl|Sequence
    (:then_0
      (bind _returnvalue_2 (Class|Actor|GetOwnerController))
      (if (Pawn|IsLocalController _returnvalue_2)
        (Input|EnableInput _returnvalue_2)))
    (:then_1
      (Networking|SwitchHasAuthority
        (:Authority
          (Utilities|FlowControl|Sequence
            (:then_0
              (bind _value (CallFunction|SPGetBoolOption _returnvalue "DisablePersonalTeleporterBeacon"))
              (Variables|Default|SetDisablePersonalBeacon _value))
            (:then_1
              (bind _value_2 (CallFunction|SPGetBoolOption _returnvalue "AllowPersonalTeleporterInBossArena"))
              (Variables|Default|SetAllowInBossArena _value_2))))))))

(event Input|ActionEvents|InputActionGamepadRightFire
  (:Pressed
    (bind _returnvalue (Class|Actor|GetOwnerController))
    (bind _asshooterplayercontroller (Utilities|Casting|CastToShooterPlayerController _returnvalue))
    (Utilities|IsValid (Class|ShooterCharacter|GetRidingDino (Class|ShooterPlayerController|GetPlayerCharacter _asshooterplayercontroller))
      (:Is%20Valid
        (CallFunction|SPMessageClient _returnvalue "Can't use while mounted." "NewEnumerator1"))
      (:Is%20Not%20Valid
        (CallFunction|SpawnTeleporterHelperEvent)))))

(event Input|ActionEvents|InputActionGamepadLeftFire
  (:Pressed
    (Class|ShooterWeapon|PlayWeaponAnimation (Variables|Default|GetSecondaryActionAnim) false false false false false false)
    (CallFunction|TryPlaceBeaconEvent)))

(event Input|ActionEvents|InputActionOpenMapMarkers
  (:Pressed
    (Utilities|FlowControl|Delay 0.2)))

(event Input|ActionEvents|InputActionFire
  (:Pressed
    (bind _returnvalue (Class|Actor|GetOwnerController))
    (bind _asshooterplayercontroller (Utilities|Casting|CastToShooterPlayerController _returnvalue))
    (Utilities|IsValid (Class|ShooterCharacter|GetRidingDino (Class|ShooterPlayerController|GetPlayerCharacter _asshooterplayercontroller))
      (:Is%20Valid
        (CallFunction|SPMessageClient _returnvalue "Can't use while mounted." "NewEnumerator1"))
      (:Is%20Not%20Valid
        (CallFunction|SpawnTeleporterHelperEvent)))))

(event Input|ActionEvents|InputActionTargeting
  (:Pressed
    (Class|ShooterWeapon|PlayWeaponAnimation (Variables|Default|GetSecondaryActionAnim) false false false false false false)
    (CallFunction|TryPlaceBeaconEvent)))

(fn ConstructionScript)

(fn DestroyExistingBeacon
  (bind _returnvalue (Class|Actor|GetOwnerController))
  (bind _outactors (Actor|GetAllActorsOfClass "/Game/Mods/StructuresPlusMod/Items/PersonalTeleporter/TeleporterBeacon/BP_TeleporterBeacon.BP_TeleporterBeacon_C"))
  (bind _array_element (Utilities|Array|ForEachLoopwithBreak _outactors :!label _label)
    (:LoopBody
      (bind _asbp_teleporterbeacon_c (Utilities|Casting|CastToBP_TeleporterBeacon _array_element))
      (if (== (Variables|/Game/Mods/StructuresPlusMod/Items/PersonalTeleporter/TeleporterBeacon/BP_TeleporterBeacon.BP_TeleporterBeacon_C|GetOwningPC _asbp_teleporterbeacon_c) _returnvalue)
        (Actor|DestroyActor _asbp_teleporterbeacon_c)
        (goto _label Break)))))

(fn IsAllowedtoPlaceBeacon
  (params (PC :type Player%20Controller%20Object%20Reference))
  (bind _returnvalue (Components|GetOwner))
  (bind _returnvalue_2 (Transformation|GetActorLocation _returnvalue))
  (Utilities|FlowControl|Sequence
    (:then_0
      (bind _returnvalue_3 (Class|PrimalItem|GetWeaponClipAmmo (Variables|Default|GetAssociatedPrimalItem)))
      (if (>= _returnvalue_3 10)
        (bind _foundnearbyenemy (CallFunction|SPServerCheckforNearbyEnemyStructure PC _returnvalue_2))
        (if (not _foundnearbyenemy)
          (if (or (Variables|Default|GetAllowInBossArena) (not (CallFunction|IsinBossArena _returnvalue_2)))
            (LocalVariables|SetCanPlaceBeacon true)
            (else
              (CallFunction|SPMessageClient PC "Disabled in Boss Arenas." "NewEnumerator1")))
          (else
            (CallFunction|SPMessageClient PC "Too Close to Enemy Structure." "NewEnumerator1")))
        (else
          (CallFunction|SPMessageClient PC "Creating a portal requires 10 element shards." "NewEnumerator1"))))
    (:then_1
      (return (LocalVariables|GetCanPlaceBeacon)))))

(fn IsinBossArena
  (params (PlayerLocation :type Vector))
  (bind _outactors (Actor|GetAllActorsOfClass "/Game/PrimalEarth/CoreBlueprints/BossTribute/BossArenaManager.BossArenaManager_C"))
  (bind _array_element (Utilities|Array|ForEachLoopwithBreak _outactors :!label _label)
    (:LoopBody
      (bind _asbossarenamanager_c (Utilities|Casting|CastToBossArenaManager _array_element))
      (Utilities|IsValid (Variables|/Game/PrimalEarth/CoreBlueprints/BossTribute/BossArenaManager.BossArenaManager_C|GetBossArenaCenterLoc _asbossarenamanager_c)
        (:Is%20Valid
          (if (< (Math|Vector|VectorLength (- (Transformation|GetActorLocation (Variables|/Game/PrimalEarth/CoreBlueprints/BossTribute/BossArenaManager.BossArenaManager_C|GetBossArenaCenterLoc _asbossarenamanager_c)) PlayerLocation)) (Variables|/Game/PrimalEarth/CoreBlueprints/BossTribute/BossArenaManager.BossArenaManager_C|GetTeleportActorsGatherRadius _asbossarenamanager_c))
            (LocalVariables|SetPlayerIsInArena true)
            (goto _label Break)))))
    (:Completed
      (return (LocalVariables|GetPlayerIsInArena)))))