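; Held Structures Plus transfer tool weapon that opens the item transfer UI and stores numbered transfer filter presets.
; Fire or targeting input applies Buff_StructuresPlus_Transfer, which initializes the UI, and EndPlay removes it on authority.
; SavePreset and LoadPreset persist request filters in the associated item's custom data under index-suffixed keys.
; Helpers split string/class struct arrays into parallel arrays for storage and rebuild them on load.
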(event Custom|ApplyBuffEvent
  (bind _buff (CallFunction|SPApplyBufffromWeapon self "/Game/Mods/StructuresPlusMod/_Buffs/Buff_StructuresPlus_Transfer.Buff_StructuresPlus_Transfer_C"))
  (Utilities|IsValid _buff
    (:Is%20Valid
      (bind _asbuff_structuresplus_transfer_c (Utilities|Casting|CastToBuff_StructuresPlus_Transfer _buff))
      (Variables|Default|SetBuffRef _asbuff_structuresplus_transfer_c))
    (:Is%20Not%20Valid
      _))
  (Default|InitializeTransferUI _asbuff_structuresplus_transfer_c self))

(event EventBeginPlay
  (Utilities|FlowControl|Delay 0.2)
  (bind _returnvalue (Class|Actor|GetOwnerController))
  (if (Pawn|IsLocalController _returnvalue)
    (Input|EnableInput _returnvalue)))

(event EventEndPlay
  (params (EndPlayReason :type EEndPlayReason%20Enum :default "ActorDestroyed"))
  (bind _buffref (Variables|Default|GetBuffRef))
  (Networking|SwitchHasAuthority
    (:Authority
      (Utilities|IsValid _buffref
        (:Is%20Valid
          (Default|RemoveBuffEvent _buffref))))))

(event Input|ActionEvents|InputActionGamepadRightFire
  (:Pressed
    (Utilities|IsValid (Variables|Default|GetBuffRef)
      (:Is%20Not%20Valid
        (Class|ShooterWeapon|PlayWeaponAnimation (Variables|Default|GetSecondaryActionAnim) false false false false false false)
        (CallFunction|ApplyBuffEvent)))))

(event Input|ActionEvents|InputActionGamepadLeftFire
  (:Pressed
    (Utilities|IsValid (Variables|Default|GetBuffRef)
      (:Is%20Not%20Valid
        (Class|ShooterWeapon|PlayWeaponAnimation (Variables|Default|GetSecondaryActionAnim) false false false false false false)
        (CallFunction|ApplyBuffEvent)))))

(event Input|ActionEvents|InputActionTargeting
  (:Pressed
    (Utilities|IsValid (Variables|Default|GetBuffRef)
      (:Is%20Not%20Valid
        (Class|ShooterWeapon|PlayWeaponAnimation (Variables|Default|GetSecondaryActionAnim) false false false false false false)
        (CallFunction|ApplyBuffEvent)))))

(event Input|ActionEvents|InputActionFire
  (:Pressed
    (Utilities|IsValid (Variables|Default|GetBuffRef)
      (:Is%20Not%20Valid
        (Class|ShooterWeapon|PlayWeaponAnimation (Variables|Default|GetSecondaryActionAnim) false false false false false false)
        (CallFunction|ApplyBuffEvent)))))

(fn ConstructionScript)

(fn SavePreset
  (params (Details :type SP%20Transfer%20Request%20Structure) (Index :type Integer))
  (bind (_sourceinclude _sourceexclude _targetinclude _targetexclude _items _sourcemax _targetmax _sourcecontains _sourcenotcontains _targetcontains _targetnotcontains _isblueprints) (Utilities|Struct|BreakSPTransferRequest Details))
  (Utilities|FlowControl|Sequence
    (:then_0
      (bind (_strings _classes) (CallFunction|SplitAlphaArray _sourceinclude))
      (CallFunction|WriteCustomData (Utilities|String|BuildString(Integer) "Splus_SourceInclude_" "" Index) _strings _classes))
    (:then_1
      (bind (_strings_2 _classes_2) (CallFunction|SplitAlphaArray _sourceexclude))
      (CallFunction|WriteCustomData (Utilities|String|BuildString(Integer) "Splus_SourceExclude_" "" Index) _strings_2 _classes_2))
    (:then_2
      (bind (_strings_3 _classes_3) (CallFunction|SplitAlphaArray _targetinclude))
      (CallFunction|WriteCustomData (Utilities|String|BuildString(Integer) "Splus_TargetInclude_" "" Index) _strings_3 _classes_3))
    (:then_3
      (bind (_strings_4 _classes_4) (CallFunction|SplitAlphaArray _targetexclude))
      (CallFunction|WriteCustomData (Utilities|String|BuildString(Integer) "Splus_TargetExclude_" "" Index) _strings_4 _classes_4))
    (:then_4
      (bind (_strings_5 _classes_5) (CallFunction|SplitAlphaArray _items))
      (CallFunction|WriteCustomData (Utilities|String|BuildString(Integer) "Splus_Items_" "" Index) _strings_5 _classes_5))
    (:then_5
      (Class|PrimalItem|SetCustomItemData (Variables|Default|GetAssociatedPrimalItem) (Utilities|Struct|MakeCustomItemData (Utilities|String|StringToName (Utilities|String|BuildString(Integer) "Splus_MiscTransfer_" "" Index)) (Utilities|Array|MakeArray _sourcecontains _sourcenotcontains _targetcontains _targetnotcontains (Utilities|String|SelectString "1" "0" _isblueprints)) (Utilities|Array|MakeArray (Math|Conversions|ToFloat(Integer) _sourcemax) (Math|Conversions|ToFloat(Integer) _targetmax)))))))

(fn LoadPreset
  (params (Index :type Integer))
  (bind _transferdetails_lp (LocalVariables|GetTransferDetails_LP))
  (Utilities|FlowControl|Sequence
    (:then_0
      (bind (_strings _classes) (CallFunction|ReadCustomData (Utilities|String|BuildString(Integer) "Splus_SourceInclude_" "" Index)))
      (bind _alphaarray (CallFunction|CreateAlphaArray _strings _classes))
      (Utilities|Struct|SetmembersinSPTransferRequest _transferdetails_lp _alphaarray))
    (:then_1
      (bind (_strings_2 _classes_2) (CallFunction|ReadCustomData (Utilities|String|BuildString(Integer) "Splus_SourceExclude_" "" Index)))
      (bind _alphaarray_2 (CallFunction|CreateAlphaArray _strings_2 _classes_2))
      (Utilities|Struct|SetmembersinSPTransferRequest _transferdetails_lp _alphaarray_2))
    (:then_2
      (bind (_strings_3 _classes_3) (CallFunction|ReadCustomData (Utilities|String|BuildString(Integer) "Splus_TargetInclude_" "" Index)))
      (bind _alphaarray_3 (CallFunction|CreateAlphaArray _strings_3 _classes_3))
      (Utilities|Struct|SetmembersinSPTransferRequest _transferdetails_lp _alphaarray_3))
    (:then_3
      (bind (_strings_4 _classes_4) (CallFunction|ReadCustomData (Utilities|String|BuildString(Integer) "Splus_TargetExclude_" "" Index)))
      (bind _alphaarray_4 (CallFunction|CreateAlphaArray _strings_4 _classes_4))
      (Utilities|Struct|SetmembersinSPTransferRequest _transferdetails_lp _alphaarray_4))
    (:then_4
      (bind (_strings_5 _classes_5) (CallFunction|ReadCustomData (Utilities|String|BuildString(Integer) "Splus_Items_" "" Index)))
      (bind _alphaarray_5 (CallFunction|CreateAlphaArray _strings_5 _classes_5))
      (Utilities|Struct|SetmembersinSPTransferRequest _transferdetails_lp _alphaarray_5))
    (:then_5
      (bind (_outdata _returnvalue) (Class|PrimalItem|GetCustomItemData (Variables|Default|GetAssociatedPrimalItem) (Utilities|String|StringToName (Utilities|String|BuildString(Integer) "Splus_MiscTransfer_" "" Index))))
      (if _returnvalue
        (if (and (== (Utilities|Array|Length (.CustomDataStrings (Utilities|Struct|BreakCustomItemData _outdata))) 5) (== (Utilities|Array|Length (.CustomDataFloats (Utilities|Struct|BreakCustomItemData _outdata))) 2))
          (Utilities|Struct|SetmembersinSPTransferRequest _transferdetails_lp (Math|Float|Floor (Utilities|Array|Get(acopy) (.CustomDataFloats (Utilities|Struct|BreakCustomItemData _outdata)))) (Math|Float|Floor (Utilities|Array|Get(acopy) (.CustomDataFloats (Utilities|Struct|BreakCustomItemData _outdata)) 1)) (Utilities|Array|Get(acopy) (.CustomDataStrings (Utilities|Struct|BreakCustomItemData _outdata))) (Utilities|Array|Get(acopy) (.CustomDataStrings (Utilities|Struct|BreakCustomItemData _outdata)) 1) (Utilities|Array|Get(acopy) (.CustomDataStrings (Utilities|Struct|BreakCustomItemData _outdata)) 2) (Utilities|Array|Get(acopy) (.CustomDataStrings (Utilities|Struct|BreakCustomItemData _outdata)) 3) (Utilities|Enum|Equal(Enum) (Utilities|Array|Get(acopy) (.CustomDataStrings (Utilities|Struct|BreakCustomItemData _outdata)) 4) "1")))))
    (:then_6
      (return _transferdetails_lp))))

(fn WriteCustomData
  (params (DataName :type String) (Strings :type Array%20of%20Strings) (Classes :type Array%20of%20Object%20Class%20References))
  (Class|PrimalItem|SetCustomItemData (Variables|Default|GetAssociatedPrimalItem) (Utilities|Struct|MakeCustomItemData (Utilities|String|StringToName DataName) Strings Classes)))

(fn ReadCustomData
  (params (DataName :type String))
  (Utilities|FlowControl|Sequence
    (:then_0
      (bind (_outdata _returnvalue) (Class|PrimalItem|GetCustomItemData (Variables|Default|GetAssociatedPrimalItem) (Utilities|String|StringToName DataName)))
      (if _returnvalue
        (for (_array_element _array_index) (.CustomDataStrings (Utilities|Struct|BreakCustomItemData _outdata))
          (if (<= _array_index (Utilities|Array|LastIndex (.CustomDataClasses (Utilities|Struct|BreakCustomItemData _outdata))))
            (Utilities|Array|Add (LocalVariables|GetStrings_RCD) _array_element)
            (Utilities|Array|Add (LocalVariables|GetClasses_RCD) (Utilities|Array|Get(acopy) (.CustomDataClasses (Utilities|Struct|BreakCustomItemData _outdata)) _array_index))))))
    (:then_1
      (return (LocalVariables|GetStrings_RCD) (LocalVariables|GetClasses_RCD)))))

(fn SplitAlphaArray
  (params (AlphaArray :type Array%20of%20SP%20Alphabetization%20Object%20Structures))
  (for _array_element AlphaArray
    (Utilities|Array|Add (LocalVariables|GetStrings_SAA) (.String (Utilities|Struct|BreakSP_AlphabetizationObject _array_element)))
    (Utilities|Array|Add (LocalVariables|GetObjects_SAA) (.Class (Utilities|Struct|BreakSP_AlphabetizationObject _array_element))))
  (return (LocalVariables|GetStrings_SAA) (LocalVariables|GetObjects_SAA)))

(fn CreateAlphaArray
  (params (Strings :type Array%20of%20Strings) (Classes :type Array%20of%20Object%20Class%20References))
  (for (_array_element _array_index) Strings
    (if (<= _array_index (Utilities|Array|LastIndex Classes))
      (Utilities|Array|Add (LocalVariables|GetAlphaArray_CAA) (Utilities|Struct|MakeSP_AlphabetizationObject _array_element (Utilities|Array|Get(acopy) Classes _array_index)))))
  (return (LocalVariables|GetAlphaArray_CAA)))