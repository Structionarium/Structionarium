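; ARK transfer gun weapon that moves items remotely between storage structures, creatures and the player.
; Line-trace aiming sets the source or target, with hotkeys for self and single-item transfers; the source persists on the associated item.
; Sources require tribe permission, removable contents and no "*" in the name.
; HandleTransfer checks game-mode pull range, then moves eligible items within the target's free slots and, for characters, weight capacity.
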(event Custom|GetSavedSourceEvent
  (bind _asprimalitem_transfergun_c (Utilities|Casting|CastToPrimalItem_TransferGun (Variables|Default|GetAssociatedPrimalItem)))
  (bind _asprimalinventorycomponent (Utilities|Casting|CastToPrimalInventoryComponent (Variables|/Game/Mods/StructuresPlusMod/Items/RemoteTransferGun/PrimalItem_TransferGun.PrimalItem_TransferGun_C|GetSourceInventory _asprimalitem_transfergun_c)))
  (Utilities|IsValid (Components|GetOwner _asprimalinventorycomponent)
    (:Is%20Valid
      (Variables|Default|SetSourceInventory _asprimalinventorycomponent)
      (bind _returnvalue (Class|Actor|GetOwnerController))
      (CallFunction|SPMessageClient _returnvalue (Utilities|String|Append "Source: " (Variables|/Game/Mods/StructuresPlusMod/Items/RemoteTransferGun/PrimalItem_TransferGun.PrimalItem_TransferGun_C|GetSourceInventoryName _asprimalitem_transfergun_c)) "NewEnumerator3"))))

(event Custom|SetSourceEvent
  (params (Source :type Actor%20Object%20Reference))
  (bind _isvalid (CallFunction|IsValidSource Source))
  (if _isvalid
    (CallFunction|SetSource Source)
    (else
      (bind _returnvalue (Class|Actor|GetOwnerController))
      (CallFunction|SPMessageClient _returnvalue "You can't transfer from this container." "NewEnumerator1"))))

(event Custom|TransferEvent
  (params (Target :type Actor%20Object%20Reference) (Single :type Boolean))
  (bind _asprimalstructureitemcontainer (Utilities|Casting|CastToPrimalStructureItemContainer Target)
    (:then
      (CallFunction|HandleTransfer (Variables|/Script/ShooterGame.PrimalStructureItemContainer|GetMyInventoryComponent _asprimalstructureitemcontainer) Single))
    (:CastFailed
      (bind _asprimaldinocharacter (Utilities|Casting|CastToPrimalDinoCharacter Target))
      (CallFunction|HandleTransfer (Variables|/Script/ShooterGame.PrimalCharacter|GetMyInventoryComponent _asprimaldinocharacter) Single))))

(event Custom|TransferToSelfEvent
  (params (TransferSingle :type Boolean))
  (bind _returnvalue (Class|Actor|GetOwnerController))
  (bind _asshooterplayercontroller (Utilities|Casting|CastToShooterPlayerController _returnvalue))
  (CallFunction|HandleTransfer (Variables|/Script/ShooterGame.PrimalCharacter|GetMyInventoryComponent (Class|ShooterPlayerController|GetPlayerCharacter _asshooterplayercontroller)) TransferSingle))

(event Custom|SetSelfAsSourceEvent
  (bind _returnvalue (Class|Actor|GetOwnerController))
  (CallFunction|SetSource _returnvalue))

(event EventBeginPlay
  (Utilities|FlowControl|Delay 0.2)
  (bind _returnvalue (Class|Actor|GetOwnerController))
  (if (Pawn|IsLocalController _returnvalue)
    (Input|EnableInput _returnvalue)
    (CallFunction|GetSavedSourceEvent)))

(event Input|ActionEvents|InputActionGamepadRightFire
  (:Pressed
    (bind _returnvalue (Class|Actor|GetOwnerController))
    (Utilities|SPIsRadialMenuOpen _returnvalue
      (:No
        (Utilities|SPIsPlacingStructure _returnvalue
          (:No
            (bind _result (CallFunction|SPDoItemLineTrace _returnvalue self (Utilities|Array|MakeArray "ObjectTypeQuery9" "ObjectTypeQuery7" "ObjectTypeQuery16") false))
            (Utilities|IsValid _result
              (:Is%20Valid
                (CallFunction|TransferEvent _result (Variables|Default|GetTransferSingle))))))))))

(event Input|ActionEvents|InputActionGamepadLeftFire
  (:Pressed
    (bind _returnvalue (Class|Actor|GetOwnerController))
    (Utilities|SPIsRadialMenuOpen _returnvalue
      (:No
        (Utilities|SPIsPlacingStructure _returnvalue
          (:No
            (bind _result (CallFunction|SPDoItemLineTrace _returnvalue self (Utilities|Array|MakeArray "ObjectTypeQuery9" "ObjectTypeQuery7" "ObjectTypeQuery16") false))
            (Utilities|IsValid _result
              (:Is%20Valid
                (CallFunction|SetSourceEvent _result)))))))))

(event Input|ActionEvents|InputActionTargeting
  (:Pressed
    (bind _returnvalue (Class|Actor|GetOwnerController))
    (Utilities|SPIsRadialMenuOpen _returnvalue
      (:No
        (Utilities|SPIsPlacingStructure _returnvalue
          (:No
            (bind _result (CallFunction|SPDoItemLineTrace _returnvalue self (Utilities|Array|MakeArray "ObjectTypeQuery9" "ObjectTypeQuery7" "ObjectTypeQuery16") false))
            (Utilities|IsValid _result
              (:Is%20Valid
                (CallFunction|SetSourceEvent _result)))))))))

(event Input|ActionEvents|InputActionFire
  (:Pressed
    (bind _returnvalue (Class|Actor|GetOwnerController))
    (Utilities|SPIsRadialMenuOpen _returnvalue
      (:No
        (Utilities|SPIsPlacingStructure _returnvalue
          (:No
            (bind _result (CallFunction|SPDoItemLineTrace _returnvalue self (Utilities|Array|MakeArray "ObjectTypeQuery9" "ObjectTypeQuery7" "ObjectTypeQuery16") false))
            (Utilities|IsValid _result
              (:Is%20Valid
                (CallFunction|TransferEvent _result (Variables|Default|GetTransferSingle))))))))))

(event Input|MouseEvents|RightMouseButton
  (:Pressed
    (bind _returnvalue (Class|Actor|GetOwnerController))
    (Utilities|SPIsRadialMenuOpen _returnvalue
      (:No
        (Utilities|SPIsPlacingStructure _returnvalue
          (:No
            (Class|ShooterWeapon|PlayWeaponAnimation (Variables|Default|GetFireAnim) false false false false false false)))))))

(event Input|MouseEvents|LeftMouseButton
  (:Pressed
    (bind _returnvalue (Class|Actor|GetOwnerController))
    (Utilities|SPIsRadialMenuOpen _returnvalue
      (:No
        (Utilities|SPIsPlacingStructure _returnvalue
          (:No
            (Class|ShooterWeapon|PlayWeaponAnimation (Variables|Default|GetFireAnim) false false false false false false)))))))

(event Input|GamepadEvents|GamepadRightTrigger
  (:Pressed
    (bind _returnvalue (Class|Actor|GetOwnerController))
    (Utilities|SPIsRadialMenuOpen _returnvalue
      (:No
        (Utilities|SPIsPlacingStructure _returnvalue
          (:No
            (Class|ShooterWeapon|PlayWeaponAnimation (Variables|Default|GetFireAnim) false false false false false false)))))))

(event Input|GamepadEvents|GamepadLeftTrigger
  (:Pressed
    (bind _returnvalue (Class|Actor|GetOwnerController))
    (Utilities|SPIsRadialMenuOpen _returnvalue
      (:No
        (Utilities|SPIsPlacingStructure _returnvalue
          (:No
            (Class|ShooterWeapon|PlayWeaponAnimation (Variables|Default|GetFireAnim) false false false false false false)))))))

(event Input|KeyboardEvents|LeftAlt
  (:Pressed
    (CallFunction|TransfertoSelfEvent (Variables|Default|GetTransferSingle))))

(event Input|KeyboardEvents|LeftShift
  (:Pressed
    (Variables|Default|SetTransferSingle true))
  (:Released
    (Variables|Default|SetTransferSingle false)))

(event Input|KeyboardEvents|G
  (:Pressed
    (CallFunction|SetSelfasSourceEvent)))

(fn ConstructionScript)

(fn HandleTransfer
  (params (TargetInventory :type Primal%20Inventory%20Component%20Object%20Reference) (Single :type Boolean))
  (bind _returnvalue (Class|Actor|GetOwnerController))
  (Utilities|IsValid (Variables|Default|GetSourceInventory)
    (:Is%20Valid
      (if (Variables|/Script/ShooterGame.PrimalInventoryComponent|GetbRemoteInventoryAllowAddItems TargetInventory)
        (if (!= TargetInventory (Variables|Default|GetSourceInventory))
          (bind _inrange (CallFunction|IsinRange TargetInventory))
          (if _inrange
            (LocalVariables|SetItems (Variables|/Script/ShooterGame.PrimalInventoryComponent|GetInventoryItems (Variables|Default|GetSourceInventory)))
            (bind _availableweight (CallFunction|GetAvailableWeightforCharacter TargetInventory))
            (LocalVariables|SetAvailableWeight_HT _availableweight)
            (bind _emptyslots (CallFunction|GetEmptySlotCount TargetInventory))
            (LocalVariables|SetEmptySlotCount_HT _emptyslots)
            (bind _array_element (Utilities|Array|ForEachLoopwithBreak (LocalVariables|GetItems) :!label _label)
              (:LoopBody
                (if (> (LocalVariables|GetEmptySlotCount_HT) 0)
                  (bind _isvalid (CallFunction|IsValidItemforTransfer _array_element))
                  (if _isvalid
                    (bind _isallowed (CallFunction|SPIsAllowedinInventory (Utilities|GetClass _array_element) TargetInventory))
                    (if _isallowed
                      (bind (_hasweight _itemweight) (CallFunction|GetItemWeight _array_element TargetInventory (LocalVariables|GetAvailableWeight_HT)))
                      (if _hasweight
                        (LocalVariables|SetAvailableWeight_HT (- (LocalVariables|GetAvailableWeight_HT) _itemweight))
                        (Class|PrimalInventoryComponent|AddItemObject TargetInventory _array_element)
                        (Class|PrimalInventoryComponent|RemoveItem (Variables|Default|GetSourceInventory) (Variables|/Script/ShooterGame.PrimalItem|GetItemID _array_element) false false true false)
                        (LocalVariables|SetEmptySlotCount_HT (- (LocalVariables|GetEmptySlotCount_HT) 1))
                        (if Single
                          (goto _label Break))
                        (else
                          (LocalVariables|SetDidntHaveRoom true)
                          (goto _label Break)))))
                  (else
                    (LocalVariables|SetDidntHaveRoom true))))
              (:Completed
                (Networking|ForceNetUpdate (Components|GetOwner TargetInventory))
                (if (LocalVariables|GetDidntHaveRoom)
                  (CallFunction|SPMessageClient _returnvalue "Target full." "NewEnumerator1")
                  (else
                    (CallFunction|SPMessageClient _returnvalue "Transfer Completed." "NewEnumerator3")))))
            (else
              (CallFunction|SPMessageClient _returnvalue "Target Is Too Far From Source" "NewEnumerator1")))
          (else
            (CallFunction|SPMessageClient _returnvalue "Source Can Not Be The Same As Target" "NewEnumerator1")))
        (else
          (CallFunction|SPMessageClient _returnvalue "Target Doesn't Accept Any Items." "NewEnumerator1"))))
    (:Is%20Not%20Valid
      (CallFunction|SPMessageClient _returnvalue "Source Not Set." "NewEnumerator1"))))

(fn IsinRange
  (params (TargetInventory :type Primal%20Inventory%20Component%20Object%20Reference))
  (bind _pullrange (CallFunction|SPGetPullSettings (Game|GetGameMode)))
  (bind _returnvalue (Transformation|GetDistanceTo (Components|GetOwner (Variables|Default|GetSourceInventory)) (Components|GetOwner TargetInventory)))
  (return (<= _returnvalue _pullrange)))

(fn SetSource
  (params (Source :type Actor%20Object%20Reference))
  (bind _asprimalstructureitemcontainer (Utilities|Casting|CastToPrimalStructureItemContainer Source)
    (:then
      (Variables|Default|SetSourceInventory (Variables|/Script/ShooterGame.PrimalStructureItemContainer|GetMyInventoryComponent _asprimalstructureitemcontainer))
      (bind _descriptivename (CallFunction|SPGetDescriptiveName 0 _asprimalstructureitemcontainer))
      (LocalVariables|SetInventoryName_SS _descriptivename))
    (:CastFailed
      (bind _asprimaldinocharacter (Utilities|Casting|CastToPrimalDinoCharacter Source)
        (:then
          (Variables|Default|SetSourceInventory (Variables|/Script/ShooterGame.PrimalCharacter|GetMyInventoryComponent _asprimaldinocharacter))
          (bind _descriptivename_2 (CallFunction|SPGetDescriptiveName 0 _asprimaldinocharacter))
          (LocalVariables|SetInventoryName_SS _descriptivename_2))
        (:CastFailed
          (bind _asshooterplayercontroller (Utilities|Casting|CastToShooterPlayerController Source))
          (Variables|Default|SetSourceInventory (Variables|/Script/ShooterGame.PrimalCharacter|GetMyInventoryComponent (Class|ShooterPlayerController|GetPlayerCharacter _asshooterplayercontroller)))
          (LocalVariables|SetInventoryName_SS "Self")))))
  (bind _returnvalue (Class|Actor|GetOwnerController))
  (CallFunction|SPMessageClient _returnvalue (Utilities|String|Append "Source Set: " (LocalVariables|GetInventoryName_SS)) "NewEnumerator3")
  (bind _asprimalitem_transfergun_c (Utilities|Casting|CastToPrimalItem_TransferGun (Variables|Default|GetAssociatedPrimalItem)))
  (Variables|/Game/Mods/StructuresPlusMod/Items/RemoteTransferGun/PrimalItem_TransferGun.PrimalItem_TransferGun_C|SetSourceInventory _asprimalitem_transfergun_c (Variables|Default|GetSourceInventory))
  (Variables|/Game/Mods/StructuresPlusMod/Items/RemoteTransferGun/PrimalItem_TransferGun.PrimalItem_TransferGun_C|SetSourceInventoryName _asprimalitem_transfergun_c (LocalVariables|GetInventoryName_SS)))

(fn IsValidSource
  (params (Source :type Actor%20Object%20Reference))
  (Utilities|FlowControl|Sequence
    (:then_0
      (bind _returnvalue (Class|Actor|GetOwnerController))
      (bind _asshooterplayercontroller (Utilities|Casting|CastToShooterPlayerController _returnvalue))
      (bind _asprimalstructureitemcontainer (Utilities|Casting|CastToPrimalStructureItemContainer Source)
        (:then
          (bind _returnvalue_2 (Class|ShooterPlayerController|AllowTribeGroupPermission _asshooterplayercontroller "STRUCTUREACTIVATE" _asprimalstructureitemcontainer))
          (LocalVariables|SetretVal_IVS (Math|Boolean|ANDBoolean _returnvalue_2 (== (Utilities|String|FindSubstring (Variables|/Script/ShooterGame.PrimalStructureItemContainer|GetBoxName _asprimalstructureitemcontainer) "*") -1) (not (Utilities|Array|ContainsItem (Variables|/Script/Engine.Actor|GetTags _asprimalstructureitemcontainer) (Utilities|Name|MakeLiteralName "PreventPulling"))) (Variables|/Script/ShooterGame.PrimalInventoryComponent|GetbRemoteInventoryAllowRemoveItems (Variables|/Script/ShooterGame.PrimalStructureItemContainer|GetMyInventoryComponent _asprimalstructureitemcontainer)))))
        (:CastFailed
          (bind _asprimaldinocharacter (Utilities|Casting|CastToPrimalDinoCharacter Source))
          (bind _returnvalue_3 (Class|ShooterPlayerController|AllowTribeGroupPermission _asshooterplayercontroller "INVENTORYACCESS" _asprimaldinocharacter))
          (LocalVariables|SetretVal_IVS (Math|Boolean|ANDBoolean _returnvalue_3 (== (Utilities|String|FindSubstring (Variables|/Script/ShooterGame.PrimalDinoCharacter|GetTamedName _asprimaldinocharacter) "*") -1) (Variables|/Script/ShooterGame.PrimalInventoryComponent|GetbRemoteInventoryAllowRemoveItems (Variables|/Script/ShooterGame.PrimalCharacter|GetMyInventoryComponent _asprimaldinocharacter)))))))
    (:then_1
      (return (LocalVariables|GetretVal_IVS)))))

(fn IsValidItemforTransfer
  (params (Item :type Primal%20Item%20Object%20Reference))
  (return (and (Variables|/Script/ShooterGame.PrimalItem|GetbAllowRemovalFromInventory Item) (== (Variables|/Script/ShooterGame.PrimalItem|GetSlotIndex Item) -1))))

(fn GetItemWeight
  (params (Item :type Primal%20Item%20Object%20Reference) (TargetInventory :type Primal%20Inventory%20Component%20Object%20Reference) (AvailableWeight :type Float%20%28single-precision%29))
  (bind _returnvalue (Components|GetOwner TargetInventory))
  (Utilities|FlowControl|Sequence
    (:then_0
      (Utilities|Casting|CastToPrimalStructureItemContainer _returnvalue
        (:then
          (LocalVariables|SetbHasWeight true)
          (LocalVariables|SetfItemWeight 0.0))
        (:CastFailed
          (Utilities|Casting|CastToPrimalCharacter _returnvalue)
          (bind _weightmultiplier (CallFunction|SPGetInventoryWeightMultiplier (Utilities|GetClass Item) TargetInventory))
          (bind _returnvalue_2 (Class|PrimalItem|GetItemWeight Item false false))
          (LocalVariables|SetfItemWeight (* _weightmultiplier _returnvalue_2))
          (LocalVariables|SetbHasWeight (<= (LocalVariables|GetfItemWeight) AvailableWeight)))))
    (:then_1
      (return (LocalVariables|GetbHasWeight) (LocalVariables|GetfItemWeight)))))

(fn GetAvailableWeightforCharacter
  (params (TargetInventory :type Primal%20Inventory%20Component%20Object%20Reference))
  (Utilities|FlowControl|Sequence
    (:then_0
      (bind _asprimalcharacter (Utilities|Casting|CastToPrimalCharacter (Components|GetOwner TargetInventory)))
      (bind _returnvalue (Class|PrimalCharacter|GetCharacterStatusComponent _asprimalcharacter))
      (Class|PrimalCharacterStatusComponent|UpdateWeightStat _returnvalue false)
      (bind (_maxweight _currentweight) (CallFunction|SPGetCharacterWeights _asprimalcharacter))
      (LocalVariables|SetWeight_GAW (- _maxweight _currentweight)))
    (:then_1
      (return (LocalVariables|GetWeight_GAW)))))

(fn GetEmptySlotCount
  (params (TargetInventory :type Primal%20Inventory%20Component%20Object%20Reference))
  (bind _returnvalue (Components|GetOwner TargetInventory))
  (Utilities|FlowControl|Sequence
    (:then_0
      (Utilities|Casting|CastToPrimalStructureItemContainer _returnvalue
        (:then
          (bind _emptyslots (CallFunction|SPGetEmptyInventorySlotCount TargetInventory))
          (LocalVariables|SetTargetEmptySlots _emptyslots))
        (:CastFailed
          (Utilities|Casting|CastToPrimalCharacter _returnvalue)
          (bind _availableslots (CallFunction|SPGetEmptyInventorySlotCount-Dino TargetInventory))
          (LocalVariables|SetTargetEmptySlots _availableslots))))
    (:then_1
      (return (LocalVariables|GetTargetEmptySlots)))))