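; Handheld command tool weapon that toggles wandering and following on the dino the player aims at.
; Targeting input cycles four modes (wandering on/off, follow on/off), messaging the player and tinting a dynamic gun material.
; Fire input line-traces and passes the hit through FiredEvent to HandleFiredEvent, which edits the PrimalDinoCharacter and forces a net update.
; Input is enabled only for the local owner; the radial menu blocks firing and mode cycling.
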(event Custom|FiredEvent
  (params (Target :type Actor%20Object%20Reference) (ModeIndex :type Integer))
  (CallFunction|HandleFiredEvent Target ModeIndex))

(event EventBeginPlay
  (Utilities|FlowControl|Delay 0.2)
  (bind _returnvalue (Class|Actor|GetOwnerController))
  (if (Pawn|IsLocalController _returnvalue)
    (Input|EnableInput _returnvalue)))

(event Input|ActionEvents|InputActionGamepadRightFire
  (:Pressed
    (bind _returnvalue (Class|Actor|GetOwnerController))
    (Utilities|SPIsRadialMenuOpen _returnvalue
      (:No
        (bind _result (CallFunction|SPDoItemLineTrace _returnvalue self (Utilities|Array|MakeArray "ObjectTypeQuery7" "ObjectTypeQuery16" "ObjectTypeQuery8") false))
        (Utilities|IsValid _result
          (:Is%20Valid
            (CallFunction|FiredEvent _result (Variables|Default|GetModeIndex))))))))

(event Input|ActionEvents|InputActionGamepadLeftFire
  (:Pressed
    (bind _returnvalue (Class|Actor|GetOwnerController))
    (Utilities|SPIsRadialMenuOpen _returnvalue
      (:No
        (CallFunction|CycleMode)))))

(event Input|ActionEvents|InputActionTargeting
  (:Pressed
    (bind _returnvalue (Class|Actor|GetOwnerController))
    (Utilities|SPIsRadialMenuOpen _returnvalue
      (:No
        (CallFunction|CycleMode)))))

(event Input|ActionEvents|InputActionFire
  (:Pressed
    (bind _returnvalue (Class|Actor|GetOwnerController))
    (Utilities|SPIsRadialMenuOpen _returnvalue
      (:No
        (bind _result (CallFunction|SPDoItemLineTrace _returnvalue self (Utilities|Array|MakeArray "ObjectTypeQuery7" "ObjectTypeQuery16" "ObjectTypeQuery8") false))
        (Utilities|IsValid _result
          (:Is%20Valid
            (CallFunction|FiredEvent _result (Variables|Default|GetModeIndex))))))))

(event Input|MouseEvents|RightMouseButton
  (:Pressed
    (Class|ShooterWeapon|PlayWeaponAnimation (Variables|Default|GetReloadAnim) false false false false false false)))

(event Input|MouseEvents|LeftMouseButton
  (:Pressed
    (bind _returnvalue (Class|Actor|GetOwnerController))
    (Utilities|SPIsRadialMenuOpen _returnvalue
      (:No
        (Class|ShooterWeapon|PlayWeaponAnimation (Variables|Default|GetFireAnim) false false false false false false)))))

(event Input|GamepadEvents|GamepadRightTrigger
  (:Pressed
    (bind _returnvalue (Class|Actor|GetOwnerController))
    (Utilities|SPIsRadialMenuOpen _returnvalue
      (:No
        (Class|ShooterWeapon|PlayWeaponAnimation (Variables|Default|GetFireAnim) false false false false false false)))))

(event Input|GamepadEvents|GamepadLeftTrigger
  (:Pressed
    (Class|ShooterWeapon|PlayWeaponAnimation (Variables|Default|GetReloadAnim) false false false false false false)))

(fn ConstructionScript
  (if (not (Networking|IsDedicatedServer))
    (bind _returnvalue (Rendering|Material|CreateDynamicMaterialInstance "/Game/PrimalEarth/WeaponPistolMachined/PistolMachined_Colorized_MIC.PistolMachined_Colorized_MIC" :!class /Script/Engine.KismetMaterialLibrary))
    (Variables|Default|SetGunMat _returnvalue)
    (Rendering|Material|SetMaterial (Variables|Default|GetMesh1P) 0 _returnvalue)))

(fn CycleMode
  (bind _gunmat (Variables|Default|GetGunMat))
  (Utilities|FlowControl|Sequence
    (:then_0
      (Variables|Default|SetModeIndex (Math|Integer|SelectInt 0 (+ (Variables|Default|GetModeIndex) 1) (> (+ (Variables|Default|GetModeIndex) 1) 3))))
    (:then_1
      (bind _returnvalue (Class|Actor|GetOwnerController))
      (CallFunction|SPMessageClient _returnvalue (Utilities|Select :Index (Variables|Default|GetModeIndex) :Option%200 "Mode: Enable Wandering" :Option%201 "Mode: Disable Wandering" :Option%202 "Mode: Enable Following" :Option%203 "Mode: Disable Following") "NewEnumerator3")
      (Rendering|Material|SetVectorParameterValue _gunmat "Color2" (Math|Conversions|ToLinearColor(Vector) (Utilities|Select :Index (Variables|Default|GetModeIndex) :Option%200 "0.100000,0.100000,0.100000" :Option%201 "0.350000,0.350000,0.350000" :Option%202 "0.600000,0.600000,0.600000" :Option%203 "0.900000,0.900000,0.900000")) :!class /Script/Engine.MaterialInstanceDynamic)
      (Rendering|Material|SetVectorParameterValue _gunmat "Color4" (Math|Conversions|ToLinearColor(Vector) (Utilities|Select :Index (Variables|Default|GetModeIndex) :Option%200 "0.100000,0.100000,0.100000" :Option%201 "0.350000,0.350000,0.350000" :Option%202 "0.600000,0.600000,0.600000" :Option%203 "0.900000,0.900000,0.900000")) :!class /Script/Engine.MaterialInstanceDynamic))))

(fn HandleFiredEvent
  (params (HitActor :type Actor%20Object%20Reference) (Mode :type Integer))
  (bind _asprimaldinocharacter (Utilities|Casting|CastToPrimalDinoCharacter HitActor))
  (Utilities|FlowControl|Sequence
    (:then_0
      (switch int Mode
        (:0
          (Variables|/Script/ShooterGame.PrimalDinoCharacter|SetbEnableTamedWandering _asprimaldinocharacter true false))
        (:1
          (Variables|/Script/ShooterGame.PrimalDinoCharacter|SetbEnableTamedWandering _asprimaldinocharacter false false))
        (:2
          (bind _returnvalue (Class|Actor|GetOwnerController))
          (bind _asshooterplayercontroller (Utilities|Casting|CastToShooterPlayerController _returnvalue))
          (Variables|/Script/ShooterGame.PrimalDinoCharacter|SetTamedFollowTarget _asprimaldinocharacter (Class|ShooterPlayerController|GetPlayerCharacter _asshooterplayercontroller) false))
        (:3
          (Variables|/Script/ShooterGame.PrimalDinoCharacter|SetTamedFollowTarget _asprimaldinocharacter 0 false))))
    (:then_1
      (Networking|ForceNetUpdate _asprimaldinocharacter))))