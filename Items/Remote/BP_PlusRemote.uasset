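; Handheld remote weapon that switches structures on or off and toggles doors at range in three modes.
; Targeting cycles the mode, saving it to the item's custom data for restore on BeginPlay and recoloring a dynamic material.
; Fire line-traces for a structure, unless placing or in a radial menu, and passes it to GunFiredEvent.
; Activation checks tribe permission, team and power or fuel; doors check CanOpen before TryMultiUse.
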(event Custom|GunFiredEvent
  (params (Structure :type Actor%20Object%20Reference) (GunMode :type Integer))
  (switch int GunMode
    (:0
      (CallFunction|ToggleActivation Structure true))
    (:1
      (CallFunction|ToggleActivation Structure false))
    (:2
      (CallFunction|ToggleDoor Structure))))

(event EventBeginPlay
  (Utilities|FlowControl|Delay 0.2)
  (bind _returnvalue (Class|Actor|GetOwnerController))
  (if (Pawn|IsLocalController _returnvalue)
    (Input|EnableInput _returnvalue)
    (bind (_outdata _returnvalue_2) (Class|PrimalItem|GetCustomItemData (Variables|Default|GetAssociatedPrimalItem) "GunMode"))
    (if _returnvalue_2
      (if (>= (Utilities|Array|LastIndex (Utilities|Struct|BreakCustomItemData _outdata)) 0)
        (Variables|Default|SetGunMode (Math|Float|Floor (Utilities|Array|Get(acopy) (Utilities|Struct|BreakCustomItemData _outdata))))
        (CallFunction|UpdateGunColor)))))

(event Input|ActionEvents|InputActionGamepadRightFire
  (:Pressed
    (bind _returnvalue (Class|Actor|GetOwnerController))
    (Utilities|SPIsPlacingStructure _returnvalue
      (:No
        (Utilities|SPIsRadialMenuOpen _returnvalue
          (:No
            (bind _result (CallFunction|SPDoItemLineTrace _returnvalue self (Utilities|Array|MakeArray "ObjectTypeQuery9") false))
            (Utilities|IsValid _result
              (:Is%20Valid
                (CallFunction|GunFiredEvent _result (Variables|Default|GetGunMode))))))))))

(event Input|ActionEvents|InputActionGamepadLeftFire
  (:Pressed
    (Variables|Default|SetGunMode (Math|Integer|SelectInt 0 (+ (Variables|Default|GetGunMode) 1) (> (+ (Variables|Default|GetGunMode) 1) 2)))
    (bind _returnvalue (Class|Actor|GetOwnerController))
    (bind _asshooterplayercontroller (Utilities|Casting|CastToShooterPlayerController _returnvalue))
    (Class|ShooterPlayerController|ClientServerNotification _asshooterplayercontroller (Utilities|Select :Index (Variables|Default|GetGunMode) :Option%200 "Activate Mode" :Option%201 "Deactivate Mode" :Option%202 "Door Mode") "(R=0.249093,G=0.164050,B=0.965000,A=1.000000)" 1.5 3.0)
    (CallFunction|UpdateGunColor)
    (Class|PrimalItem|SetCustomItemData (Variables|Default|GetAssociatedPrimalItem) (Utilities|Struct|MakeCustomItemData "GunMode" (Utilities|Array|MakeArray (Math|Conversions|ToFloat(Integer) (Variables|Default|GetGunMode)))))))

(event Input|ActionEvents|InputActionTargeting
  (:Pressed
    (Variables|Default|SetGunMode (Math|Integer|SelectInt 0 (+ (Variables|Default|GetGunMode) 1) (> (+ (Variables|Default|GetGunMode) 1) 2)))
    (bind _returnvalue (Class|Actor|GetOwnerController))
    (bind _asshooterplayercontroller (Utilities|Casting|CastToShooterPlayerController _returnvalue))
    (Class|ShooterPlayerController|ClientServerNotification _asshooterplayercontroller (Utilities|Select :Index (Variables|Default|GetGunMode) :Option%200 "Activate Mode" :Option%201 "Deactivate Mode" :Option%202 "Door Mode") "(R=0.249093,G=0.164050,B=0.965000,A=1.000000)" 1.5 3.0)
    (CallFunction|UpdateGunColor)
    (Class|PrimalItem|SetCustomItemData (Variables|Default|GetAssociatedPrimalItem) (Utilities|Struct|MakeCustomItemData "GunMode" (Utilities|Array|MakeArray (Math|Conversions|ToFloat(Integer) (Variables|Default|GetGunMode)))))))

(event Input|ActionEvents|InputActionFire
  (:Pressed
    (bind _returnvalue (Class|Actor|GetOwnerController))
    (Utilities|SPIsPlacingStructure _returnvalue
      (:No
        (Utilities|SPIsRadialMenuOpen _returnvalue
          (:No
            (bind _result (CallFunction|SPDoItemLineTrace _returnvalue self (Utilities|Array|MakeArray "ObjectTypeQuery9") false))
            (Utilities|IsValid _result
              (:Is%20Valid
                (CallFunction|GunFiredEvent _result (Variables|Default|GetGunMode))))))))))

(event Input|MouseEvents|RightMouseButton
  (:Pressed
    (Class|ShooterWeapon|PlayWeaponAnimation (Variables|Default|GetReloadAnim) false false false false false false)))

(event Input|MouseEvents|LeftMouseButton
  (:Pressed
    (bind _returnvalue (Class|Actor|GetOwnerController))
    (Utilities|SPIsRadialMenuOpen _returnvalue
      (:No
        (Utilities|SPIsPlacingStructure _returnvalue
          (:No
            (Class|ShooterWeapon|PlayWeaponAnimation (Variables|Default|GetFireAnim) false false false false false false)))))))

(event Input|GamepadEvents|GamepadRightTrigger
  (:Pressed
    (bind _returnvalue (Class|Actor|GetOwnerController))
    (Utilities|SPIsRadialMenuOpen _returnvalue
      (:No
        (Utilities|SPIsPlacingStructure _returnvalue
          (:No
            (Class|ShooterWeapon|PlayWeaponAnimation (Variables|Default|GetFireAnim) false false false false false false)))))))

(event Input|GamepadEvents|GamepadLeftTrigger
  (:Pressed
    (Class|ShooterWeapon|PlayWeaponAnimation (Variables|Default|GetReloadAnim) false false false false false false)))

(fn ConstructionScript
  (if (not (Networking|IsDedicatedServer))
    (bind _returnvalue (Rendering|Material|CreateDynamicMaterialInstance "/Game/PrimalEarth/WeaponPistolMachined/PistolMachined_Colorized_MIC.PistolMachined_Colorized_MIC" :!class /Script/Engine.KismetMaterialLibrary))
    (Variables|Default|SetGunMat _returnvalue)
    (Rendering|Material|SetMaterial (Variables|Default|GetMesh1P) 0 _returnvalue)
    (CallFunction|UpdateGunColor)))

(fn ToggleActivation
  (params (Structure :type Actor%20Object%20Reference) (DoActivate :type Boolean))
  (bind _asprimalstructureitemcontainer (Utilities|Casting|CastToPrimalStructureItemContainer Structure))
  (if (Variables|/Script/ShooterGame.PrimalStructureItemContainer|GetbCanToggleActivation _asprimalstructureitemcontainer)
    (bind _returnvalue (Class|Actor|GetOwnerController))
    (bind _asshooterplayercontroller (Utilities|Casting|CastToShooterPlayerController _returnvalue))
    (bind _returnvalue_2 (Class|ShooterPlayerController|AllowTribeGroupPermission _asshooterplayercontroller "STRUCTUREACTIVATE" Structure))
    (if (and _returnvalue_2 (== (Variables|/Script/Engine.Actor|GetTargetingTeam Structure) (Variables|Default|GetTargetingTeam)))
      (if DoActivate
        (if (and (not (Variables|/Script/ShooterGame.PrimalStructureItemContainer|GetbContainerActivated _asprimalstructureitemcontainer)) (or (and (Variables|/Script/ShooterGame.PrimalStructureItemContainer|GetbActiveRequiresPower _asprimalstructureitemcontainer) (Variables|/Script/ShooterGame.PrimalStructureItemContainer|GetbIsPowered _asprimalstructureitemcontainer)) (and (not (Variables|/Script/ShooterGame.PrimalStructureItemContainer|GetbActiveRequiresPower _asprimalstructureitemcontainer)) (Variables|/Script/ShooterGame.PrimalStructureItemContainer|GetbHasFuel _asprimalstructureitemcontainer))))
          (Class|PrimalStructure|SetContainerActive _asprimalstructureitemcontainer true)
          (Class|ShooterPlayerController|ClientServerNotification _asshooterplayercontroller (Utilities|String|Append (Variables|/Script/ShooterGame.PrimalTargetableActor|GetDescriptiveName _asprimalstructureitemcontainer) " turned on!") "(R=0.337667,G=0.535000,B=0.017403,A=1.000000)" 1.5 3.0))
        (elif (Variables|/Script/ShooterGame.PrimalStructureItemContainer|GetbContainerActivated _asprimalstructureitemcontainer)
          (Class|PrimalStructure|SetContainerActive _asprimalstructureitemcontainer false)
          (Class|ShooterPlayerController|ClientServerNotification _asshooterplayercontroller (Utilities|String|Append (Variables|/Script/ShooterGame.PrimalTargetableActor|GetDescriptiveName _asprimalstructureitemcontainer) " turned off!") "(R=0.910000,G=0.031850,B=0.079991,A=1.000000)" 1.5 3.0))))))

(fn UpdateGunColor
  (bind _gunmode (Variables|Default|GetGunMode))
  (bind _gunmat (Variables|Default|GetGunMat))
  (Rendering|Material|SetVectorParameterValue _gunmat "Color2" (Utilities|Select :Index _gunmode :Option%200 "(R=5.000000,G=10.000000,B=5.000000,A=1.000000)" :Option%201 "(R=1.000000,G=1.000000,B=1.000000,A=0.000000)" :Option%202 "(R=1.500000,G=1.500000,B=1.500000,A=1.000000)") :!class /Script/Engine.MaterialInstanceDynamic)
  (Rendering|Material|SetVectorParameterValue _gunmat "Color4" (Utilities|Select :Index _gunmode :Option%200 "(R=0.500000,G=1.000000,B=0.500000,A=1.000000)" :Option%201 "(R=0.250000,G=0.250000,B=0.250000,A=1.000000)" :Option%202 "(R=1.500000,G=1.500000,B=1.500000,A=1.000000)") :!class /Script/Engine.MaterialInstanceDynamic))

(fn ToggleDoor
  (params (Structure :type Actor%20Object%20Reference))
  (bind _returnvalue (Class|Actor|GetOwnerController))
  (bind _asprimalstructuredoor (Utilities|Casting|CastToPrimalStructureDoor Structure))
  (bind _returnvalue_2 (Class|PrimalStructureDoor|CanOpen _asprimalstructuredoor _returnvalue))
  (if _returnvalue_2
    (Class|Actor|TryMultiUse Structure _returnvalue 500)
    (else
      (CallFunction|SPMessageClient _returnvalue "You can't open this door." "NewEnumerator1"))))