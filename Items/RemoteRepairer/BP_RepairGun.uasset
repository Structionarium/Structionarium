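; Remote repair gun weapon that lets the local player repair a targeted structure by firing at it.
; Fire input line-traces for a target unless placing a structure or using the radial menu; separate mouse/trigger bindings play the fire animation.
; Damaged structures get a resource check against item repair or crafting costs scaled by missing health, then repair via TryMultiUse.
; Full-health targets or insufficient resources produce red notifications instead.
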(event Custom|ExecuteRepairEvent
  (params (Target :type Actor%20Object%20Reference))
  (bind _asprimalstructure (Utilities|Casting|CastToPrimalStructure Target))
  (bind _returnvalue (Class|Actor|GetOwnerController))
  (bind _asshooterplayercontroller (Utilities|Casting|CastToShooterPlayerController _returnvalue))
  (if (== (Variables|/Script/ShooterGame.PrimalTargetableActor|GetMaxHealth _asprimalstructure) (Variables|/Script/ShooterGame.PrimalTargetableActor|GetReplicatedHealth _asprimalstructure))
    (Class|ShooterPlayerController|ClientServerNotification _asshooterplayercontroller "Target doesn't need repairs." "(R=1.000000,G=0.000000,B=0.000000,A=1.000000)" 1.5 3.0)
    (else
      (bind _hasresources (CallFunction|HasRequiredResources _asprimalstructure))
      (if _hasresources
        (Class|Actor|TryMultiUse _asprimalstructure _returnvalue 202)
        (else
          (Class|ShooterPlayerController|ClientServerNotification _asshooterplayercontroller "Insufficient resources for this repair." "(R=1.000000,G=0.000000,B=0.000000,A=1.000000)" 1.5 3.0))))))

(event EventBeginPlay
  (Utilities|FlowControl|Delay 0.2)
  (bind _returnvalue (Class|Actor|GetOwnerController))
  (if (Pawn|IsLocalController _returnvalue)
    (Input|EnableInput _returnvalue)))

(event Input|ActionEvents|InputActionGamepadRightFire
  (:Pressed
    (bind _returnvalue (Class|Actor|GetOwnerController))
    (Utilities|SPIsPlacingStructure _returnvalue
      (:No
        (Utilities|SPIsRadialMenuOpen _returnvalue
          (:No
            (bind _result (CallFunction|SPDoItemLineTrace _returnvalue self (Utilities|Array|MakeArray "ObjectTypeQuery9") false))
            (Utilities|IsValid _result
              (:Is%20Valid
                (CallFunction|ExecuteRepairEvent _result)))))))))

(event Input|ActionEvents|InputActionFire
  (:Pressed
    (bind _returnvalue (Class|Actor|GetOwnerController))
    (Utilities|SPIsPlacingStructure _returnvalue
      (:No
        (Utilities|SPIsRadialMenuOpen _returnvalue
          (:No
            (bind _result (CallFunction|SPDoItemLineTrace _returnvalue self (Utilities|Array|MakeArray "ObjectTypeQuery9") false))
            (Utilities|IsValid _result
              (:Is%20Valid
                (CallFunction|ExecuteRepairEvent _result)))))))))

(event Input|MouseEvents|LeftMouseButton
  (:Pressed
    (bind _returnvalue (Class|Actor|GetOwnerController))
    (Utilities|SPIsRadialMenuOpen _returnvalue
      (:No
        (Utilities|SPIsPlacingStructure _returnvalue
          (:No
            (Class|ShooterWeapon|PlayWeaponAnimation (Variables|Default|GetFireAnim) false false false false false false)))))))

(event Input|GamepadEvents|GamepadRightTrigger
  (:Pressed
    (bind _returnvalue (Class|Actor|GetOwnerController))
    (Utilities|SPIsRadialMenuOpen _returnvalue
      (:No
        (Utilities|SPIsPlacingStructure _returnvalue
          (:No
            (Class|ShooterWeapon|PlayWeaponAnimation (Variables|Default|GetFireAnim) false false false false false false)))))))

(fn ConstructionScript)

(fn HasRequiredResources
  (params (Structure :type Primal%20Structure%20Object%20Reference))
  (LocalVariables|SetCanRepair true)
  (Utilities|FlowControl|Sequence
    (:then_0
      (bind _returnvalue (Class|VictoryCore|GetClassDefaultObject (Variables|/Script/ShooterGame.PrimalStructure|GetConsumesPrimalItem Structure)))
      (bind _asprimalitem (Utilities|Casting|CastToPrimalItem _returnvalue))
      (if (Variables|/Script/ShooterGame.PrimalItem|GetbOverrideRepairingRequirements _asprimalitem)
        (LocalVariables|SetRepairRequirements (Variables|/Script/ShooterGame.PrimalItem|GetOverrideRepairingRequirements _asprimalitem))
        (else
          (LocalVariables|SetRepairRequirements (Variables|/Script/ShooterGame.PrimalItem|GetBaseCraftingResourceRequirements _asprimalitem)))))
    (:then_1
      (bind _returnvalue_2 (Class|Actor|GetOwnerController))
      (bind _asshooterplayercontroller (Utilities|Casting|CastToShooterPlayerController _returnvalue_2))
      (bind _array_element (Utilities|Array|ForEachLoopwithBreak (LocalVariables|GetRepairRequirements) :!label _label)
        (:LoopBody
          (bind _returnvalue_3 (Class|PrimalInventoryComponent|GetItemTemplateQuantity (Variables|/Script/ShooterGame.PrimalCharacter|GetMyInventoryComponent (Class|ShooterPlayerController|GetPlayerCharacter _asshooterplayercontroller)) (.ResourceItemType (Utilities|Struct|BreakCraftingResourceRequirement _array_element)) 0 true false false))
          (if (< _returnvalue_3 (Math|Float|Ceil (* (.BaseResourceRequirement (Utilities|Struct|BreakCraftingResourceRequirement _array_element)) (Variables|/Script/ShooterGame.PrimalItem|GetRepairResourceRequirementMultiplier _asprimalitem) (Math|Float|Absolute(Float) (- (/ (Variables|/Script/ShooterGame.PrimalTargetableActor|GetReplicatedHealth Structure) (Variables|/Script/ShooterGame.PrimalTargetableActor|GetMaxHealth Structure)) 1.0)))))
            (LocalVariables|SetCanRepair false)
            (goto _label Break)))
        (:Completed
          (return (LocalVariables|GetCanRepair)))))))