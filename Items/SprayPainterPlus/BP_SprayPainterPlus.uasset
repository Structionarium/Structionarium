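; Spray painter weapon that applies its item's dye color to the selected color regions of a structure hit by a line trace.
; Alt+1 to 6 toggle the six regions, stored as "1"/"0" strings in item custom data.
; A server-added buff, removed on EndPlay, receives region data for UI.
; The owning client traces on fire; BroadcastChanges sets structure colors and multicasts the using-colors flag.
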(event Custom|HandleFired
  (params (Structure :type Primal%20Structure%20Object%20Reference) (ColorIndex :type Integer))
  (bind _regions (CallFunction|GetRegionArray))
  (CallFunction|BroadcastChanges Structure ColorIndex _regions))

(event Custom|HandleRegionToggle
  (params (RegionIndex :type Integer))
  (bind _buffref (Variables|Default|GetBuffRef))
  (CallFunction|ToggleRegion RegionIndex)
  (Utilities|IsValid _buffref
    (:Is%20Valid
      (bind _regions (CallFunction|GetRegionArray))
      (Default|SendNewDatatoClient _buffref _regions))))

(event Custom|BroadcastChanges
  (params (Structure :type Primal%20Structure%20Object%20Reference) (ColorIndex :type Integer) (Regions :type Array%20of%20Booleans))
  (Variables|/Script/ShooterGame.PrimalStructure|SetbUsingStructureColors Structure true false)
  (for (_array_element _array_index) Regions
    (if _array_element
      (Class|PrimalStructure|SetStructureColorValue Structure _array_index ColorIndex)))
  (Class|Actor|MulticastProperty Structure "bUsingStructureColors"))

(event EventEndPlay
  (params (EndPlayReason :type EEndPlayReason%20Enum :default "ActorDestroyed"))
  (bind _buffref (Variables|Default|GetBuffRef))
  (Networking|SwitchHasAuthority
    (:Authority
      (Utilities|IsValid _buffref
        (:Is%20Valid
          (Actor|DestroyActor _buffref))))))

(event EventBeginPlay
  (Utilities|FlowControl|Delay 0.2)
  (bind _returnvalue (Class|Actor|GetOwnerController))
  (Utilities|FlowControl|Sequence
    (:then_0
      (if (Pawn|IsLocalController _returnvalue)
        (Input|EnableInput _returnvalue)))
    (:then_1
      (Networking|SwitchHasAuthority
        (:Authority
          (bind _asshooterplayercontroller (Utilities|Casting|CastToShooterPlayerController _returnvalue))
          (bind _returnvalue_2 (Class|PrimalBuff|StaticAddBuff "/Game/Mods/StructuresPlusMod/_Buffs/Buff_StructuresPlus_SprayPainter.Buff_StructuresPlus_SprayPainter_C" (Class|ShooterPlayerController|GetPlayerCharacter _asshooterplayercontroller) 0 0 false))
          (bind _asbuff_structuresplus_spraypainter_c (Utilities|Casting|CastToBuff_StructuresPlus_SprayPainter _returnvalue_2))
          (Variables|Default|SetBuffRef _asbuff_structuresplus_spraypainter_c)
          (bind _regions (CallFunction|GetRegionArray))
          (Default|InitializeUI _asbuff_structuresplus_spraypainter_c _regions))))))

(event Input|KeyboardEvents|Alt1
  (:Pressed
    (CallFunction|HandleRegionToggle)))

(event Input|KeyboardEvents|Alt2
  (:Pressed
    (CallFunction|HandleRegionToggle 1)))

(event Input|KeyboardEvents|Alt3
  (:Pressed
    (CallFunction|HandleRegionToggle 2)))

(event Input|KeyboardEvents|Alt4
  (:Pressed
    (CallFunction|HandleRegionToggle 3)))

(event Input|KeyboardEvents|Alt5
  (:Pressed
    (CallFunction|HandleRegionToggle 4)))

(event Input|KeyboardEvents|Alt6
  (:Pressed
    (CallFunction|HandleRegionToggle 5)))

(fn ConstructionScript)

(fn BPFiredWeapon
  (bind _returnvalue (Class|Actor|GetOwnerController))
  (if (Pawn|IsLocalController _returnvalue)
    (bind _returnvalue_2 (Class|PrimalItem|GetItemColorID (Variables|Default|GetAssociatedPrimalItem)))
    (if (> _returnvalue_2 0)
      (bind _result (CallFunction|SPDoItemLineTrace _returnvalue self (Utilities|Array|MakeArray "ObjectTypeQuery9") false))
      (Utilities|IsValid _result
        (:Is%20Valid
          (bind _asprimalstructure (Utilities|Casting|CastToPrimalStructure _result))
          (CallFunction|HandleFired _asprimalstructure _returnvalue_2)))
      (else
        (CallFunction|SPMessageClient _returnvalue "No dye applied." "NewEnumerator1")))))

(fn GetRegionArray
  (Utilities|FlowControl|Sequence
    (:then_0
      (bind (_outdata _returnvalue) (Class|PrimalItem|GetCustomItemData (Variables|Default|GetAssociatedPrimalItem) "SplusColorRegions"))
      (if _returnvalue
        (for _array_element (.CustomDataStrings (Utilities|Struct|BreakCustomItemData _outdata))
          (Utilities|Array|Add (LocalVariables|GetRegions_GRA) (Utilities|Enum|Equal(Enum) _array_element "1")))
        (else
          (LocalVariables|SetRegions_GRA (Utilities|Array|MakeArray true false false false false false)))))
    (:then_1
      (return (LocalVariables|GetRegions_GRA)))))

(fn SetRegionArray
  (params (Regions :type Array%20of%20Booleans))
  (for _array_element Regions
    (Utilities|Array|Add (LocalVariables|GetRegions_SRA) (Utilities|String|SelectString "1" "0" _array_element)))
  (Class|PrimalItem|SetCustomItemData (Variables|Default|GetAssociatedPrimalItem) (Utilities|Struct|MakeCustomItemData "SplusColorRegions" (LocalVariables|GetRegions_SRA))))

(fn ToggleRegion
  (params (Index :type Integer))
  (bind _regions (CallFunction|GetRegionArray))
  (if (>= (Utilities|Array|LastIndex _regions) Index)
    (LocalVariables|SetTempRegions _regions)
    (Utilities|Array|SetArrayElem (LocalVariables|GetTempRegions) Index (not (Utilities|Array|Get(acopy) _regions Index)))
    (CallFunction|SetRegionArray (LocalVariables|GetTempRegions))))