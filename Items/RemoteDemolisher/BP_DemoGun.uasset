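; Remote demolition gun (Structures Plus) that demolishes structures or picks them up into the player's inventory.
; Targeting input toggles the mode on a cooldown, messaging the player and recoloring a dynamic gun material.
; Fire runs a delayed line trace, then filters targets by tribe permission, excluded classes, tags and server pickup settings.
; An INI option lets admins on dedicated servers bypass tribe checks for player-owned structures.
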(event Custom|PickupEvent
  (params (Target :type Actor%20Object%20Reference))
  (Utilities|Casting|CastToPrimalStructureTurretPlant Target
    (:CastFailed
      (bind _asprimalstructure (Utilities|Casting|CastToPrimalStructure Target))
      (bind _allowpickup (CallFunction|IsPickupAllowed _asprimalstructure (Variables|Default|GetAdminPickUpAll)))
      (if _allowpickup
        (CallFunction|HandlePickup _asprimalstructure)))))

(event Custom|DemolishEvent
  (params (Target :type Actor%20Object%20Reference))
  (Utilities|Casting|CastToPrimalStructureTurretPlant Target
    (:CastFailed
      (bind _asprimalstructure (Utilities|Casting|CastToPrimalStructure Target))
      (bind _allowdemolish (CallFunction|IsDemolishAllowed _asprimalstructure (Variables|Default|GetAdminPickUpAll)))
      (if _allowdemolish
        (bind _returnvalue (Class|Actor|GetOwnerController))
        (Class|PrimalStructure|Demolish _asprimalstructure _returnvalue)))))

(event EventBeginPlay
  (Utilities|FlowControl|Delay 0.2)
  (Utilities|FlowControl|Sequence
    (:then_0
      (bind _returnvalue (Class|Actor|GetOwnerController))
      (if (Pawn|IsLocalController _returnvalue)
        (Input|EnableInput _returnvalue)
        (Variables|Default|SetAllowModeSwitchTime (- (Utilities|Time|GetGameTimeinSeconds) (Math|Conversions|ToFloat(Integer) (* (Variables|Default|GetModeSwitchCooldown) -1.0))))))
    (:then_1
      (Networking|SwitchHasAuthority
        (:Authority
          (bind _asshootergamemode (Utilities|Casting|CastToShooterGameMode (Game|GetGameMode)))
          (Utilities|FlowControl|Sequence
            (:then_0
              (bind _returnvalue_2 (Class|ShooterGameMode|GetBoolOptionIni _asshootergamemode "StructuresPlus" "AllowAdminToDemoAnyTribeWithDemoGun"))
              (Variables|Default|SetAdminPickUpAll _returnvalue_2 true))
            (:then_1
              (bind _returnvalue_3 (Class|Actor|GetOwnerController))
              (bind _asshooterplayercontroller (Utilities|Casting|CastToShooterPlayerController _returnvalue_3))
              (bind _returnvalue_4 (Class|ShooterGameMode|IsPlayerAllowedtoCheat _asshootergamemode _asshooterplayercontroller))
              (Variables|Default|SetIsAdmin _returnvalue_4 true))))))))

(event Input|ActionEvents|InputActionGamepadRightFire
  (:Pressed
    (bind _returnvalue (Class|Actor|GetOwnerController))
    (Utilities|SPIsPlacingStructure _returnvalue
      (:No
        (Utilities|SPIsRadialMenuOpen _returnvalue
          (:No
            (Utilities|FlowControl|Delay 0.2)
            (bind _result (CallFunction|SPDoItemLineTrace _returnvalue self (Utilities|Array|MakeArray "ObjectTypeQuery9") (and (Variables|Default|GetIsAdmin) (Variables|Default|GetAdminPickUpAll))))
            (Utilities|IsValid _result
              (:Is%20Valid
                (if (Variables|Default|GetIsPickupMode)
                  (CallFunction|PickupEvent _result)
                  (else
                    (CallFunction|DemolishEvent _result)))))))))))

(event Input|ActionEvents|InputActionGamepadLeftFire
  (bind _gunmat (Variables|Default|GetGunMat))
  (:Pressed
    (bind _returnvalue (Class|Actor|GetOwnerController))
    (if (<= (Math|Conversions|ToFloat(Integer) (- (Variables|Default|GetAllowModeSwitchTime) (Utilities|Time|GetGameTimeinSeconds))) 0.0)
      (Variables|Default|SetIsPickupMode (not (Variables|Default|GetIsPickupMode)))
      (CallFunction|SPMessageClient _returnvalue (Utilities|String|SelectString "Pickup Mode Enabled" "Demolish Mode Enabled" (Variables|Default|GetIsPickupMode)) "NewEnumerator3")
      (Rendering|Material|SetVectorParameterValue _gunmat "Color2" (Math|Conversions|ToLinearColor(Vector) (Math|Vector|SelectVector "0.225000,0.225000,0.225000" "1.000000,0.000000, 0" (Variables|Default|GetIsPickupMode))) :!class /Script/Engine.MaterialInstanceDynamic)
      (Rendering|Material|SetVectorParameterValue _gunmat "Color4" (Math|Conversions|ToLinearColor(Vector) (Math|Vector|SelectVector "0.225000,0.225000,0.225000" "1.000000,0.000000, 0" (Variables|Default|GetIsPickupMode))) :!class /Script/Engine.MaterialInstanceDynamic)
      (Variables|Default|SetAllowModeSwitchTime (- (Utilities|Time|GetGameTimeinSeconds) (Math|Conversions|ToFloat(Integer) (* (Variables|Default|GetModeSwitchCooldown) -1.0))))
      (else
        (CallFunction|SPMessageClient _returnvalue "You must wait 1 second between mode changes." "NewEnumerator1")))))

(event Input|ActionEvents|InputActionTargeting
  (bind _gunmat (Variables|Default|GetGunMat))
  (:Pressed
    (bind _returnvalue (Class|Actor|GetOwnerController))
    (if (<= (Math|Conversions|ToFloat(Integer) (- (Variables|Default|GetAllowModeSwitchTime) (Utilities|Time|GetGameTimeinSeconds))) 0.0)
      (Variables|Default|SetIsPickupMode (not (Variables|Default|GetIsPickupMode)))
      (CallFunction|SPMessageClient _returnvalue (Utilities|String|SelectString "Pickup Mode Enabled" "Demolish Mode Enabled" (Variables|Default|GetIsPickupMode)) "NewEnumerator3")
      (Rendering|Material|SetVectorParameterValue _gunmat "Color2" (Math|Conversions|ToLinearColor(Vector) (Math|Vector|SelectVector "0.225000,0.225000,0.225000" "1.000000,0.000000, 0" (Variables|Default|GetIsPickupMode))) :!class /Script/Engine.MaterialInstanceDynamic)
      (Rendering|Material|SetVectorParameterValue _gunmat "Color4" (Math|Conversions|ToLinearColor(Vector) (Math|Vector|SelectVector "0.225000,0.225000,0.225000" "1.000000,0.000000, 0" (Variables|Default|GetIsPickupMode))) :!class /Script/Engine.MaterialInstanceDynamic)
      (Variables|Default|SetAllowModeSwitchTime (- (Utilities|Time|GetGameTimeinSeconds) (Math|Conversions|ToFloat(Integer) (* (Variables|Default|GetModeSwitchCooldown) -1.0))))
      (else
        (CallFunction|SPMessageClient _returnvalue "You must wait 1 second between mode changes." "NewEnumerator1")))))

(event Input|ActionEvents|InputActionFire
  (:Pressed
    (bind _returnvalue (Class|Actor|GetOwnerController))
    (Utilities|SPIsPlacingStructure _returnvalue
      (:No
        (Utilities|SPIsRadialMenuOpen _returnvalue
          (:No
            (Utilities|FlowControl|Delay 0.2)
            (bind _result (CallFunction|SPDoItemLineTrace _returnvalue self (Utilities|Array|MakeArray "ObjectTypeQuery9") (and (Variables|Default|GetIsAdmin) (Variables|Default|GetAdminPickUpAll))))
            (Utilities|IsValid _result
              (:Is%20Valid
                (if (Variables|Default|GetIsPickupMode)
                  (CallFunction|PickupEvent _result)
                  (else
                    (CallFunction|DemolishEvent _result)))))))))))

(event Input|MouseEvents|RightMouseButton
  (:Pressed
    (Class|ShooterWeapon|PlayWeaponAnimation (Variables|Default|GetReloadAnim) false false false false false false)))

(event Input|MouseEvents|LeftMouseButton
  (:Pressed
    (bind _returnvalue (Class|Actor|GetOwnerController))
    (Utilities|SPIsRadialMenuOpen _returnvalue
      (:No
        (Utilities|SPIsPlacingStructure _returnvalue
          (:No
            (Class|ShooterWeapon|PlayWeaponAnimation (Variables|Default|GetFireAnim) false false false false false false)))))))

(event Input|GamepadEvents|GamepadRightTrigger
  (:Pressed
    (bind _returnvalue (Class|Actor|GetOwnerController))
    (Utilities|SPIsRadialMenuOpen _returnvalue
      (:No
        (Utilities|SPIsPlacingStructure _returnvalue
          (:No
            (Class|ShooterWeapon|PlayWeaponAnimation (Variables|Default|GetFireAnim) false false false false false false)))))))

(event Input|GamepadEvents|GamepadLeftTrigger
  (:Pressed
    (Class|ShooterWeapon|PlayWeaponAnimation (Variables|Default|GetReloadAnim) false false false false false false)))

(fn ConstructionScript
  (if (not (Networking|IsDedicatedServer))
    (bind _returnvalue (Rendering|Material|CreateDynamicMaterialInstance "/Game/PrimalEarth/WeaponPistolMachined/PistolMachined_Colorized_MIC.PistolMachined_Colorized_MIC" :!class /Script/Engine.KismetMaterialLibrary))
    (Variables|Default|SetGunMat _returnvalue)
    (Rendering|Material|SetMaterial (Variables|Default|GetMesh1P) 0 _returnvalue)))

(fn IsDemolishAllowed
  (params (Structure :type Primal%20Structure%20Object%20Reference) (AllowAdminDemoAll :type Boolean))
  (bind _returnvalue (Utilities|GetClass Structure))
  (bind _targetingteam (Variables|/Script/Engine.Actor|GetTargetingTeam Structure))
  (bind _returnvalue_2 (Class|Actor|GetOwnerController))
  (bind _asshooterplayercontroller (Utilities|Casting|CastToShooterPlayerController _returnvalue_2))
  (bind _returnvalue_3 (Class|ShooterPlayerController|AllowTribeGroupPermission _asshooterplayercontroller "GENERAL_STRUCTUREDEMOLISH" Structure))
  (bind _asshootergamemode (Utilities|Casting|CastToShooterGameMode (Game|GetGameMode)))
  (bind _returnvalue_4 (Class|ShooterGameMode|IsPlayerAllowedtoCheat _asshootergamemode _asshooterplayercontroller))
  (bind _isplayerowned (CallFunction|SPIsPlayerOwnedStructure _targetingteam))
  (return (Math|Boolean|ANDBoolean (or (Math|Boolean|ANDBoolean _isplayerowned _returnvalue_4 (Networking|IsDedicatedServer) AllowAdminDemoAll) (and _returnvalue_3 (== (Variables|/Script/Engine.Actor|GetTargetingTeam _returnvalue_2) _targetingteam))) (not (Utilities|ClassIsChildOf _returnvalue "/Game/PrimalEarth/Structures/BuildingBases/TreePlatform_Base_SM.TreePlatform_Base_SM_C")) (== (Utilities|String|FindSubstring (Utilities|GetDisplayName (Variables|/Script/ShooterGame.PrimalStructure|GetMyStaticMesh Structure)) "SM_InteractionBox") -1) (not (== _returnvalue "/Game/PrimalEarth/Structures/DeathItemCache.DeathItemCache_C")) (not (Utilities|ClassIsChildOf _returnvalue "/Game/PrimalEarth/Structures/BeeHive/BeeHive.BeeHive_C")) (Variables|/Script/Engine.Actor|GetbCanBeDamaged Structure) (not (CallFunction|SPStructureHasTag Structure "PreventDemolish")))))

(fn IsPickupAllowed
  (params (Structure :type Primal%20Structure%20Object%20Reference) (AllowAdminDemoAll :type Boolean))
  (bind _returnvalue (Game|GetGameMode))
  (bind _allowdemolish (CallFunction|IsDemolishAllowed Structure AllowAdminDemoAll))
  (bind _asshootergamemode (Utilities|Casting|CastToShooterGameMode _returnvalue))
  (bind _returnvalue_2 (Class|ShooterGameMode|GetBoolOptionIni _asshootergamemode "StructuresPlus" "RestrictDemoGunPickup"))
  (bind (_dodisablepickup _dodisablepickupwhendamaged _pickuptime) (CallFunction|SPGetPickupSettings _returnvalue))
  (bind _assplus_ipickup_c (Utilities|Casting|CastToSPlus_IPickup (Class|TargetableInterface|ToUObject Structure))
    (:then
      (bind _timetodisablepickup (Default|IPickupGetTimetoDisablePickup _assplus_ipickup_c))
      (bind _asshootergamestate (Utilities|Casting|CastToShooterGameState (Game|GetGameState)))
      (bind _returnvalue_3 (Class|ShooterGameState|GetNetworkTimeDelta _asshootergamestate _timetodisablepickup true))
      (LocalVariables|SetDisablePickupTime _returnvalue_3))
    (:CastFailed
      _))
  (bind _returnvalue_4 (Class|Actor|GetOwnerController))
  (bind _asshooterplayercontroller (Utilities|Casting|CastToShooterPlayerController _returnvalue_4))
  (bind _returnvalue_5 (Class|ShooterGameMode|IsPlayerAllowedtoCheat _asshootergamemode _asshooterplayercontroller))
  (bind _isplayerowned (CallFunction|SPIsPlayerOwnedStructure (Variables|/Script/Engine.Actor|GetTargetingTeam Structure)))
  (return (Math|Boolean|ANDBoolean _allowdemolish (or (Math|Boolean|ANDBoolean _isplayerowned _returnvalue_5 (Networking|IsDedicatedServer) AllowAdminDemoAll) (Math|Boolean|ANDBoolean (not _dodisablepickup) (or (not _dodisablepickupwhendamaged) (and _dodisablepickupwhendamaged (== (Variables|/Script/ShooterGame.PrimalTargetableActor|GetMaxHealth Structure) (Variables|/Script/ShooterGame.PrimalTargetableActor|GetHealth Structure)))) (Math|Boolean|ORBoolean (== _pickuptime 0.0) (not (== (LocalVariables|GetDisablePickupTime) 0.0)) (not (Utilities|DoesObjectImplementInterface Structure "/Game/Mods/StructuresPlusMod/_Interfaces/SPlus_IPickup.SPlus_IPickup_C"))) (or (not _returnvalue_2) (!= (Variables|/Script/ShooterGame.PrimalStructure|GetPickupGivesItem Structure) 0)))) (not (CallFunction|SPStructureHasTag Structure "PreventPickup")))))

(fn HandlePickup
  (params (Structure :type Primal%20Structure%20Object%20Reference))
  (LocalVariables|SetStructureClass (Variables|/Script/ShooterGame.PrimalStructure|GetConsumesPrimalItem Structure))
  (Utilities|FlowControl|Sequence
    (:then_0
      (Variables|/Script/ShooterGame.PrimalTargetableActor|SetDestroyedMesh Structure 0)
      (Variables|/Script/ShooterGame.PrimalTargetableActor|SetDeathSound Structure 0)
      (Actor|DestroyActor Structure))
    (:then_1
      (bind _returnvalue (Class|Actor|GetOwnerController))
      (bind _asshooterplayercontroller (Utilities|Casting|CastToShooterPlayerController _returnvalue))
      (Class|PrimalInventoryComponent|BPIncrementItemTemplateQuantity (Variables|/Script/ShooterGame.PrimalCharacter|GetMyInventoryComponent (Class|ShooterPlayerController|GetPlayerCharacter _asshooterplayercontroller)) (LocalVariables|GetStructureClass) 1 true false true false false false 0 false))))