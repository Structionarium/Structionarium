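; S+ dynamic gate structure in six materials (wood to Tek), cycled with H/Shift+H during placement and gated by engrams.
; Replicated gateway data drives meshes and sizing; it spawns in a crafting state that self-destructs on a timer unless finished.
; Server-side overlap boxes auto-open and delay-close it, configurable through the radial menu alongside thickness, repair and demolish.
; Glass supports adjustable transparency; Tek swaps collision profiles and animates a forcefield material instead of swinging.
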(event OnComponentBeginOverlap(InsideBox)
  (params (OtherActor :type Actor%20Object%20Reference) (OtherComp :type Primitive%20Component%20Object%20Reference) (OtherBodyIndex :type Integer) (bFromSweep :type Boolean) (SweepResult :type Hit%20Result%20Structure%20%28by%20ref%29))
  (Networking|SwitchHasAuthority
    (:Authority
      (CallFunction|OpenDoor OtherActor false))))

(event OnComponentBeginOverlap(OutsideBox)
  (params (OtherActor :type Actor%20Object%20Reference) (OtherComp :type Primitive%20Component%20Object%20Reference) (OtherBodyIndex :type Integer) (bFromSweep :type Boolean) (SweepResult :type Hit%20Result%20Structure%20%28by%20ref%29))
  (Networking|SwitchHasAuthority
    (:Authority
      (CallFunction|OpenDoor OtherActor true))))

(event OnComponentEndOverlap(PlayerCheckBox)
  (params (OtherActor :type Actor%20Object%20Reference) (OtherComp :type Primitive%20Component%20Object%20Reference) (OtherBodyIndex :type Integer))
  (Networking|SwitchHasAuthority
    (:Authority
      (CallFunction|HandleCloseDelay OtherActor))))

(event Custom|SelfDestructEvent
  (if (Variables|Default|GetIsCrafting)
    (Actor|DestroyActor)))

(event Custom|StartDoorInterp
  (params (InterpDest :type Float%20%28single-precision%29))
  (Variables|Default|SetDoorInterpDestValue InterpDest)
  (if (> (Math|Float|Absolute(Float) (- (Variables|Default|GetDoorInterpDestValue) (Variables|Default|GetDoorInterpCurrentValue))) 0.001)
    (Class|KismetSystemLibrary|SetTimerforNextTick 0 "UpdateDoorInterp" false)))

(event Custom|UpdateDoorInterp
  (if (Class|VictoryCore|IsTimeSince (Class|Actor|GetWorld) (Variables|Default|GetCreationTime) 0.1 false)
    (Variables|Default|SetDoorInterpCurrentValue (Math|Interpolation|FInterptoConstant (Variables|Default|GetDoorInterpCurrentValue) (Variables|Default|GetDoorInterpDestValue) (Utilities|Time|GetWorldDeltaSeconds) (Variables|Default|GetDoorMatInterpSpeed)))
    (else
      (Variables|Default|SetDoorInterpCurrentValue (Variables|Default|GetDoorInterpDestValue))))
  (Rendering|Material|SetScalarParameterValue (Variables|Default|GetTekMIC) "CycleDoor" (Variables|Default|GetDoorInterpCurrentValue) :!class /Script/Engine.MaterialInstanceDynamic)
  (if (> (Math|Float|Absolute(Float) (- (Variables|Default|GetDoorInterpDestValue) (Variables|Default|GetDoorInterpCurrentValue))) 0.001)
    (Class|KismetSystemLibrary|SetTimerforNextTick 0 "UpdateDoorInterp" false)))

(event EventIGlassSetModel
  (params (ModelIndex :type Integer)))

(event EventIGlassSetTransparency
  (params (GlassSetting :type SP%20Glass%20Settings%20Structure))
  (Variables|Default|SetGlassSettings GlassSetting true))

(event Input|KeyboardEvents|ShiftH
  (bind _gatewaydata (Variables|Default|GetGatewayData))
  (bind _materialindex (Utilities|Struct|BreakSP_DynamicGatewayData _gatewaydata))
  (:Pressed
    (if (> _materialindex 0)
      (Utilities|Struct|SetmembersinSP_DynamicGatewayData _gatewaydata (- _materialindex 1))
      (CallFunction|OnRepGatewayData))))

(event Input|KeyboardEvents|H
  (bind _gatewaydata (Variables|Default|GetGatewayData))
  (bind _materialindex (Utilities|Struct|BreakSP_DynamicGatewayData _gatewaydata))
  (:Pressed
    (if (< _materialindex 5)
      (Utilities|Struct|SetmembersinSP_DynamicGatewayData _gatewaydata (+ _materialindex 1))
      (CallFunction|OnRepGatewayData))))

(fn ConstructionScript
  (|CallParentFunction))

(fn BPIsAllowedtoBuild
  (params (OutPlacementData :type Placement%20Data%20Structure%20%28by%20ref%29) (CurrentAllowedReason :type Integer))
  (bind _gatewaydata (Variables|Default|GetGatewayData))
  (bind _materialindex (Utilities|Struct|BreakSP_DynamicGatewayData _gatewaydata))
  (LocalVariables|SetBuildReason (Math|Integer|SelectInt 1 CurrentAllowedReason (== CurrentAllowedReason -9)))
  (Utilities|FlowControl|Sequence
    (:then_0
      (if (Variables|Default|GetbIsPreviewStructure)
        (bind _returnvalue (Class|Actor|GetOwnerController))
        (bind _asshooterplayercontroller (Utilities|Casting|CastToShooterPlayerController _returnvalue))
        (bind _asshooterplayerstate (Utilities|Casting|CastToShooterPlayerState (Variables|/Script/Engine.Controller|GetPlayerState _asshooterplayercontroller)))
        (if (not (Class|ShooterPlayerState|HasEngram _asshooterplayerstate (Utilities|Select :Index _materialindex :Option%200 "/Game/Mods/StructuresPlusMod/Doors/Gates/Small/Wood/PrimalItemStructure_Gate_Wood.PrimalItemStructure_Gate_Wood_C" :Option%201 "/Game/Mods/StructuresPlusMod/Doors/Gates/Small/Stone/PrimalItemStructure_Gate_Stone.PrimalItemStructure_Gate_Stone_C" :Option%202 "/Game/Mods/StructuresPlusMod/Doors/Gates/Small/Metal/PrimalItemStructure_Gate_Metal.PrimalItemStructure_Gate_Metal_C" :Option%203 "/Game/Mods/StructuresPlusMod/Doors/Gates/Small/Glass/PrimalItemStructure_Gate_Glass.PrimalItemStructure_Gate_Glass_C" :Option%204 "/Game/Mods/StructuresPlusMod/Doors/Gates/Small/Adobe/PrimalItemStructure_Gate_Adobe.PrimalItemStructure_Gate_Adobe_C" :Option%205 "/Game/Mods/StructuresPlusMod/Doors/Gates/Small/Tek/PrimalItemStructure_Gate_Tek.PrimalItemStructure_Gate_Tek_C")))
          (LocalVariables|SetBuildReason (Utilities|Select :Index _materialindex :Option%200 -111 :Option%201 -112 :Option%202 -113 :Option%203 -114 :Option%204 -115 :Option%205 -116)))))
    (:then_1
      (return (LocalVariables|GetBuildReason)))))

(fn BPGetMultiUseEntries
  (params (ForPC :type Player%20Controller%20Object%20Reference) (MultiUseEntries :type Array%20of%20Multi%20Use%20Entry%20Structures))
  (bind _color (CallFunction|SPGetSpecialMenuColor))
  (bind _repaircooldowntime (Variables|Default|GetRepairCooldownTime))
  (bind _gatethickness (Variables|Default|GetGateThickness))
  (bind (_canrepair _repairstring) (CallFunction|SPGetRepairMenuEntryData ForPC _repaircooldowntime))
  (bind _returnvalue (Math|Conversions|ToColor(LinearColor) _color))
  (bind _entriesout (CallFunction|CleanMultiUseEntries MultiUseEntries))
  (bind _entriesout_2 (CallFunction|SPAddMenuEntries _entriesout ForPC self false false (and (== (Utilities|Struct|BreakSP_DynamicGatewayData (Variables|Default|GetGatewayData)) 3) (not (Variables|Default|GetIsCrafting))) false 0.0 0.0))
  (Utilities|FlowControl|Sequence
    (:then_0
      (bind _returnvalue_2 (Class|PrimalStructureDoor|CanOpen ForPC))
      (bind _returnvalue_3 (Class|PrimalStructure|AllowStructureAccess ForPC))
      (if (and _returnvalue_3 _returnvalue_2)
        (Utilities|FlowControl|Sequence
          (:then_0
            (if (not (Variables|Default|GetIsCrafting))
              (Utilities|Array|Add _entriesout_2 (Utilities|Struct|MakeMultiUseEntry (Utilities|String|SelectString "Switch to Manual" "Switch to Automatic" (Variables|Default|GetIsAutomatic)) 9003 -1003))
              (if (Variables|Default|GetIsAutomatic)
                (Utilities|Array|Add _entriesout_2 (Utilities|Struct|MakeMultiUseEntry (Utilities|String|SelectString "Auto Open & Close" "Auto Close Only" (Variables|Default|GetAutoCloseOnly)) 9004 -1004))
                (Utilities|Array|Add _entriesout_2 (Utilities|Struct|MakeMultiUseEntry "Set Close Delay" 9005 -1010 true true (Math|Conversions|ToColor(LinearColor) (CallFunction|SPGetSpecialMenuColor))))
                (Utilities|Array|Add _entriesout_2 (Utilities|Struct|MakeMultiUseEntry "No Delay" 9006 -1000 1))
                (Utilities|Array|Add _entriesout_2 (Utilities|Struct|MakeMultiUseEntry "1 sec Delay" 9007 -1001 1))
                (Utilities|Array|Add _entriesout_2 (Utilities|Struct|MakeMultiUseEntry "5 sec Delay" 9008 -1002 1))
                (Utilities|Array|Add _entriesout_2 (Utilities|Struct|MakeMultiUseEntry "10 sec Delay" 9009 -1003 1))
                (Utilities|Array|Add _entriesout_2 (Utilities|Struct|MakeMultiUseEntry (Utilities|String|BuildString(Integer) "Current Delay: " "" (Math|Float|Floor (Variables|Default|GetCloseDelay)) " sec") 9999 -1004 true 1 (Math|Color|MakeColor 255 175 175 255))))))
          (:then_1
            (Utilities|Array|Add _entriesout_2 (Utilities|Struct|MakeMultiUseEntry "[Gate Thickness]" 9013 -1100 true true _returnvalue))
            (Utilities|Array|Add _entriesout_2 (Utilities|Struct|MakeMultiUseEntry (Utilities|String|BuildString(Integer) "Current Thickness: " "" (+ _gatethickness 1)) 9999 1000 true true 2 _returnvalue))
            (Utilities|Array|Add _entriesout_2 (Utilities|Struct|MakeMultiUseEntry "+1" 9014 0 (>= _gatethickness 4) true 2))
            (Utilities|Array|Add _entriesout_2 (Utilities|Struct|MakeMultiUseEntry "" 9999 -999 true 2))
            (Utilities|Array|Add _entriesout_2 (Utilities|Struct|MakeMultiUseEntry "-1" 9015 -1000 (<= _gatethickness 0) true 2)))
          (:then_2
            (Utilities|Array|Add _entriesout_2 (Utilities|Struct|MakeMultiUseEntry "Demolish" 9010 -2500 1.0 1.0))
            (if (Variables|Default|GetIsCrafting)
              (Utilities|Array|Add _entriesout_2 (Utilities|Struct|MakeMultiUseEntry "Finish Crafting" 9011 2500))
              (elif (!= (Math|Float|Floor (Variables|Default|GetHealth)) (Math|Float|Floor (Variables|Default|GetMaxHealth)))
                (Utilities|Array|Add _entriesout_2 (Utilities|Struct|MakeMultiUseEntry _repairstring 9012 -1000 (not _canrepair)))))))))
    (:then_1
      (return _entriesout_2))))

(fn BPTryMultiUse
  (params (ForPC :type Player%20Controller%20Object%20Reference) (UseIndex :type Integer))
  (bind _self self)
  (switch int UseIndex
    (:Default
      _)
    (:9002
      (CallFunction|SPApplyTransparencyBuff ForPC self))
    (:9003
      (Variables|Default|SetIsAutomatic (not (Variables|Default|GetIsAutomatic)) true))
    (:9004
      (Variables|Default|SetAutoCloseOnly (not (Variables|Default|GetAutoCloseOnly)) true))
    (:9005
      _)
    (:9006
      (Variables|Default|SetCloseDelay 0.0 true))
    (:9007
      (Variables|Default|SetCloseDelay 1.0 true))
    (:9008
      (Variables|Default|SetCloseDelay 5.0 true))
    (:9009
      (Variables|Default|SetCloseDelay 1e+01 true))
    (:9010
      (CallFunction|SPDemolishDynamicStructure ForPC (select (Variables|Default|GetIsCrafting) (Variables|Default|GetMaterialsStored) (Variables|Default|GetMaterialsRequired)) _self))
    (:9011
      (CallFunction|SPApplyDynamicCraftingBuff ForPC _self false))
    (:9012
      (CallFunction|SPApplyDynamicCraftingBuff ForPC _self true))
    (:9013
      _)
    (:9014
      (Variables|Default|SetDoorScale (+ (Variables|Default|GetDoorScale) "0,0.200000, 0") true)
      (Variables|Default|SetGateThickness (+ (Variables|Default|GetGateThickness) 1) true))
    (:9015
      (Variables|Default|SetDoorScale (- (Variables|Default|GetDoorScale) "0,0.200000, 0") true)
      (Variables|Default|SetGateThickness (- (Variables|Default|GetGateThickness) 1) true)))
  (return true))

(fn BPClientDoMultiUse
  (params (ForPC :type Player%20Controller%20Object%20Reference) (ClientUseIndex :type Integer))
  (bind _asshooterplayercontroller (Utilities|Casting|CastToShooterPlayerController ForPC))
  (if (== ClientUseIndex 9005)
    (Class|ShooterPlayerController|SetMultiUseWheelCategory _asshooterplayercontroller 1)
    (elif (== ClientUseIndex 9013)
      (Class|ShooterPlayerController|SetMultiUseWheelCategory _asshooterplayercontroller 2))))

(fn ReceiveBeginPlay
  (bind _returnvalue (Game|GetGameMode))
  (|CallParentFunction)
  (if (Variables|Default|GetbIsPreviewStructure)
    (bind _returnvalue_2 (Class|Actor|GetOwnerController))
    (Input|EnableInput _returnvalue_2)
    (bind _globalactor (CallFunction|SPGetGlobalActor self))
    (Utilities|IsValid _globalactor
      (:Is%20Valid
        (Class|PlayerController|ClientSendNetExecCommandtoServer _returnvalue_2 _globalactor "ApplyGateBuff" (Utilities|Struct|MakeBPNetExecParams) true))
      (:Is%20Not%20Valid
        (Development|PrintString "Global Actor Not Found")))
    (else
      (Utilities|FlowControl|Sequence
        (:then_0
          (Networking|SwitchHasAuthority
            (:Authority
              (Utilities|FlowControl|Sequence
                (:then_0
                  (if (not (Variables|Default|GetIsDefaultConfigSet))
                    (bind _value (CallFunction|SPGetIntIniOption _returnvalue "DefaultDoorConfig" 0 2))
                    (Variables|Default|SetIsDefaultConfigSet true)
                    (switch int _value
                      (:1
                        (Variables|Default|SetAutoCloseOnly true true))
                      (:2
                        (Variables|Default|SetIsAutomatic false true)))))
                (:then_1
                  (bind _value_2 (CallFunction|SPGetFloatIniOption _returnvalue "MinimumGlassTransparency" 0.0 1.0))
                  (Variables|Default|SetMinOpacity _value_2 true))
                (:then_3
                  (if (Variables|Default|GetIsCrafting)
                    (Utilities|Time|SetTimerbyFunctionName 0 "SelfDestructEvent" (Math|Conversions|ToFloat(Integer) (- (Variables|Default|GetDestructionTime) (Utilities|Time|GetGameTimeinSeconds))))))))))
        (:then_1
          (if (== (Utilities|Struct|BreakSP_DynamicGatewayData (Variables|Default|GetGatewayData)) 5)
            (Variables|Default|SetbPreventDoorInterpolation true)))
        (:then_2
          (if (and (not (Networking|IsDedicatedServer)) (Variables|Default|GetIsCrafting))
            (CallFunction|UpdateMaterials)))
        (:then_3
          (Utilities|SwitchNetAuthority
            (:PlayerServer
              (CallFunction|OnRepGlassSettings)
              (CallFunction|OnRepDoorScale)
              (CallFunction|OnRepGatewayData))))))))

(fn OnRepDoorScale
  (Transformation|SetActorRelativeScale3D (Variables|Default|GetDoorScale)))

(fn BPPreInitializeComponents
  (|CallParentFunction)
  (if (not (Variables|Default|GetbIsPreviewStructure))
    (Networking|SwitchHasAuthority
      (:Authority
        (bind _returnvalue (Class|VictoryCore|IsLoadingSaveGame))
        (if (not _returnvalue)
          (CallFunction|SPInitializeDynamicStructure self 1))))))

(fn OnRepIsCrafting
  (CallFunction|UpdateMaterials))

(fn OnRepGatewayData
  (bind _mystaticmesh (Variables|Default|GetMyStaticMesh))
  (bind _gatewaydata (Variables|Default|GetGatewayData))
  (bind _width (Utilities|Struct|BreakSP_DynamicGatewayData _gatewaydata))
  (bind _materialindex (Utilities|Struct|BreakSP_DynamicGatewayData _gatewaydata))
  (bind _returnvalue (== _materialindex 5))
  (Variables|Default|SetRotationSpeed (- 8e+01 (* (- _width 1) 5.0)))
  (Transformation|SetRelativeScale3D (Variables|Default|GetCheckBoxes) (Math|Vector|MakeVector 1.0 (+ (* (- _width 2) 0.25) 1.0) 1.0))
  (if (not (Networking|IsDedicatedServer))
    (Components|StaticMesh|SetStaticMesh _mystaticmesh (Utilities|Select :Index _materialindex :Option%200 "/Game/PrimalEarth/Test_Efecto/Wood_Structure/FrameGate/SM_DoorLeft.SM_DoorLeft" :Option%201 "/Game/PrimalEarth/Structures/Stone/Stone_GateDoor/SM_Stone_GateDoor.SM_Stone_GateDoor" :Option%202 "/Game/PrimalEarth/Test_Efecto/Metal_Structures/Gate/sm_gate_door.SM_Gate_Door" :Option%203 "/Game/Mods/StructuresPlusMod/Doors/Gates/Small/Glass/_Models/SM_Gate_Glass.SM_Gate_Glass" :Option%204 "/Game/ScorchedEarth/Structures/Adobe/Meshes/SM_AdobeGateDoor.SM_AdobeGateDoor" :Option%205 "/Game/PrimalEarth/Test_Efecto/Metal_Structures/Gate/sm_gate_door.SM_Gate_Door"))
    (Components|StaticMesh|SetStaticMesh (Variables|Default|GetSecondDoor) (Utilities|Select :Index _materialindex :Option%200 "/Game/PrimalEarth/Test_Efecto/Wood_Structure/FrameGate/SM_DoorRight.SM_DoorRight" :Option%201 "/Game/PrimalEarth/Structures/Stone/Stone_GateDoor/SM_Stone_GateDoor.SM_Stone_GateDoor" :Option%202 "/Game/PrimalEarth/Test_Efecto/Metal_Structures/Gate/sm_gate_door.SM_Gate_Door" :Option%203 "/Game/Mods/StructuresPlusMod/Doors/Gates/Small/Glass/_Models/SM_Gate_Glass.SM_Gate_Glass" :Option%204 "/Game/ScorchedEarth/Structures/Adobe/Meshes/SM_AdobeGateDoor.SM_AdobeGateDoor" :Option%205 "/Game/PrimalEarth/Test_Efecto/Metal_Structures/Gate/sm_gate_door.SM_Gate_Door"))
    (Rendering|SetVisibility _mystaticmesh (not _returnvalue) false)
    (Rendering|SetVisibility (Variables|Default|GetTekMesh) _returnvalue false)))

(fn UpdateMaterials
  (bind _mystaticmesh (Variables|Default|GetMyStaticMesh))
  (bind _gatewaydata (Variables|Default|GetGatewayData))
  (bind _materialindex (Utilities|Struct|BreakSP_DynamicGatewayData _gatewaydata))
  (if (not (or (Networking|IsDedicatedServer) (Variables|Default|GetbIsPreviewStructure)))
    (Variables|Default|SetTargetableDamageFXDefaultPhysMaterial (Utilities|Select :Index _materialindex :Option%200 "Wood" :Option%201 "Rock" :Option%202 "Metal" :Option%203 "Metal" :Option%204 "Rock" :Option%205 "Metal"))
    (if (Variables|Default|GetIsCrafting)
      (Rendering|Material|SetMaterial _mystaticmesh 0 "/Game/Mods/StructuresPlusMod/_Materials/PreviewMaterial.PreviewMaterial")
      (if (== _materialindex 3)
        (Rendering|Material|SetMaterial _mystaticmesh 1 "/Game/Mods/StructuresPlusMod/_Materials/PreviewMaterial.PreviewMaterial")
        (Rendering|Material|SetMaterial _mystaticmesh 2 "/Game/Mods/StructuresPlusMod/_Materials/PreviewMaterial.PreviewMaterial"))
      (else
        (switch int _materialindex
          (:Default
            (bind _returnvalue (Rendering|Material|CreateDynamicMaterialInstance (Utilities|Select :Index _materialindex :Option%200 "/Game/PrimalEarth/Test_Efecto/Wood_Structure/FrameGate/FrameGate_Colorize_MIC.FrameGate_Colorize_MIC" :Option%201 "/Game/PrimalEarth/Structures/Stone/Stone_GateDoor/StoneGate_Door_Colorize_MIC.StoneGate_Door_Colorize_MIC" :Option%202 "/Game/PrimalEarth/Test_Efecto/Metal_Structures/Materials/IndividualPieces/Metal_Gate_Colorize_MIC.Metal_Gate_Colorize_MIC" :Option%203 "/Game/PrimalEarth/Test_Efecto/Metal_Structures/Materials/IndividualPieces/Metal_Gate_Colorize_MIC.Metal_Gate_Colorize_MIC" :Option%204 "/Game/ScorchedEarth/Structures/Adobe/Material/MIC_AdobeGate_Plaster_Colorize.MIC_AdobeGate_Plaster_Colorize" :Option%205 "/Game/Mods/StructuresPlusMod/_Materials/ForceField_MIC.ForceField_MIC") :!class /Script/Engine.KismetMaterialLibrary))
            (Rendering|Material|SetMaterial _mystaticmesh 0 _returnvalue)
            (Variables|Default|SetTekMIC _returnvalue))
          (:3
            (CallFunction|ApplyGlassMaterial)))))))

(fn CleanMultiUseEntries
  (params (EntriesIn :type Array%20of%20Multi%20Use%20Entry%20Structures))
  (bind (_item _index) (Utilities|SPforEachReverse EntriesIn)
    (:Loop
      (LocalVariables|SetEntry _item)
      (if (== (Utilities|Struct|BreakMultiUseEntry _item) 201)
        (Utilities|Array|RemoveIndex EntriesIn _index :!label _label)
        (elif (Variables|Default|GetIsCrafting)
          (Utilities|FlowControl|Sequence
            (:then_0
              (if (or (== (Utilities|Struct|BreakMultiUseEntry _item) 501) (== (Utilities|Struct|BreakMultiUseEntry _item) 502))
                (goto _label)))
            (:then_1
              (if (== (Utilities|Struct|BreakMultiUseEntry _item) 500)
                (Utilities|Struct|SetmembersinMultiUseEntry (LocalVariables|GetEntry) -75)
                (Utilities|Array|SetArrayElem EntriesIn _index (LocalVariables|GetEntry))))))))
    (:Completed
      (return EntriesIn))))

(fn BPAllowPickupGiveItem
  (params (ForPC :type Player%20Controller%20Object%20Reference))
  (return (Variables|Default|GetIsCrafting)))

(fn BPOverrideCantBuildReasonString
  (params (CantBuildReason :type Integer))
  (return (Utilities|String|SelectString (Utilities|String|Append (Utilities|String|Append "You Require the S+ " (Utilities|Select :Index (Math|Integer|Clamp(Integer) (- 5 (+ CantBuildReason 116)) 0 5) :Option%200 "Wood" :Option%201 "Stone" :Option%202 "Metal" :Option%203 "Glass" :Option%204 "Adobe" :Option%205 "Tek")) " Gate Engram.") "" (and (<= CantBuildReason -111) (>= CantBuildReason -116)))))

(fn BlueprintDrawHUD
  (params (HUD :type Shooter%20HUD%20Object%20Reference) (CenterX :type Float%20%28single-precision%29) (CenterY :type Float%20%28single-precision%29))
  (if (Variables|Default|GetIsCrafting)
    (CallFunction|SPDrawDestructionTimer HUD CenterX CenterY (Variables|Default|GetDestructionTime))))

(fn BPUnstasis
  (Networking|SwitchHasAuthority
    (:Authority
      (CallFunction|OnRepDoorScale)
      (CallFunction|OnRepGatewayData)
      (if (Variables|Default|GetIsCrafting)
        (Utilities|Time|SetTimerbyFunctionName 0 "SelfDestructEvent" (Math|Conversions|ToFloat(Integer) (- (Variables|Default|GetDestructionTime) (Utilities|Time|GetGameTimeinSeconds))))))))

(fn OpenDoor
  (params (OtherActor :type Actor%20Object%20Reference) (OpenIn :type Boolean))
  (bind _nearbyplayers (Variables|Default|GetNearbyPlayers))
  (if (and (Variables|Default|GetIsAutomatic) (not (Variables|Default|GetIsCrafting)))
    (Utilities|Time|ClearTimerbyFunctionName 0 "CloseDoorEvent")
    (bind _asshootercharacter (Utilities|Casting|CastToShooterCharacter OtherActor))
    (bind _returnvalue (Class|Actor|GetOwnerController _asshootercharacter))
    (Utilities|IsValid _returnvalue
      (:Is%20Valid
        (bind _returnvalue_2 (Class|PrimalStructureDoor|CanOpen _returnvalue))
        (if _returnvalue_2
          (if (not (Utilities|Array|ContainsItem _nearbyplayers OtherActor))
            (Utilities|Array|Add _nearbyplayers OtherActor)
            (if (not (Math|Boolean|ORBoolean (> (Utilities|Array|Length _nearbyplayers) 1) (Variables|Default|GetAutoCloseOnly) (!= (Class|PrimalStructureDoor|GetDoorState) 0)))
              (Class|PrimalStructureDoor|BPSetDoorState (Math|Integer|SelectInt 1 2 OpenIn)))))))))

(fn CloseDoor
  (Utilities|FlowControl|Sequence
    (:then_0
      (if (Variables|Default|GetbStasised)
        (Class|Actor|Unstasis)))
    (:then_1
      (if (Variables|Default|GetIsAutomatic)
        (if (!= (Class|PrimalStructureDoor|GetDoorState) 0)
          (Class|PrimalStructureDoor|BPSetDoorState))))))

(fn HandleCloseDelay
  (params (OtherActor :type Actor%20Object%20Reference))
  (bind _nearbyplayers (Variables|Default|GetNearbyPlayers))
  (bind _closedelay (Variables|Default|GetCloseDelay))
  (Utilities|FlowControl|Sequence
    (:then_0
      (Utilities|Array|RemoveItem _nearbyplayers OtherActor))
    (:then_1
      (if (== (Utilities|Array|Length _nearbyplayers) 0)
        (if (== _closedelay 0.0)
          (CallFunction|CloseDoor)
          (else
            (Utilities|Time|SetTimerbyFunctionName 0 "CloseDoor" _closedelay)))))))

(fn OnRepGlassSettings
  (Utilities|SwitchNetAuthority
    (:PlayerServer
      _)
    (:Client
      _))
  (CallFunction|SPAlterGlassTransparency (Variables|Default|GetGlassSettings) (Variables|Default|GetInsideMIC) (Variables|Default|GetOutsideMIC)))

(fn OnRepMinOpacity
  (bind _minopacity (Variables|Default|GetMinOpacity))
  (Networking|SwitchHasAuthority
    (:Authority
      (if (< (.opacity (Variables|Default|GetGlassSettings)) _minopacity)
        (Variables|Default|SetGlassSettings (Utilities|Struct|MakeSPGlassSettings (.transparencytype (Variables|Default|GetGlassSettings)) _minopacity) true)))))

(fn ApplyGlassMaterial
  (bind _mystaticmesh (Variables|Default|GetMyStaticMesh))
  (Utilities|FlowControl|Sequence
    (:then_0
      (bind _returnvalue (Rendering|Material|CreateDynamicMaterialInstance "/Game/Mods/StructuresPlusMod/_Materials/GlassMIC.GlassMIC" :!class /Script/Engine.KismetMaterialLibrary))
      (Variables|Default|SetInsideMIC _returnvalue))
    (:then_1
      (bind _returnvalue_2 (Rendering|Material|CreateDynamicMaterialInstance "/Game/Mods/StructuresPlusMod/_Materials/GlassMIC.GlassMIC" :!class /Script/Engine.KismetMaterialLibrary))
      (Variables|Default|SetOutsideMIC _returnvalue_2))
    (:then_2
      (Rendering|Material|SetMaterial _mystaticmesh 0 (Variables|Default|GetInsideMIC))
      (Rendering|Material|SetMaterial _mystaticmesh 1 (Variables|Default|GetOutsideMIC))
      (bind _returnvalue_3 (Rendering|Material|CreateDynamicMaterialInstance "/Game/PrimalEarth/Test_Efecto/Metal_Structures/Materials/IndividualPieces/Metal_Gate_Colorize_MIC.Metal_Gate_Colorize_MIC" :!class /Script/Engine.KismetMaterialLibrary))
      (Rendering|Material|SetMaterial _mystaticmesh 2 _returnvalue_3))))

(fn BPPostSetStructureCollisionChannels
  (CallFunction|OnRepDoorScale))

(fn BPGotoDoorState
  (params (NewDoorState :type Integer))
  (bind _returnvalue (== NewDoorState 0))
  (if (== (Utilities|Struct|BreakSP_DynamicGatewayData (Variables|Default|GetGatewayData)) 5)
    (Collision|SetCollisionProfileName (Variables|Default|GetMyStaticMesh) (select _returnvalue "StructureWall" "UsableOnly") :!class /Script/Engine.PrimitiveComponent)
    (if (not (Networking|IsDedicatedServer))
      (CallFunction|StartDoorInterp (select _returnvalue 1.0 0.0)))))

(fn BPAdjustDamage
  (params (IncomingDamage :type Float%20%28single-precision%29) (TheDamageEvent :type Damage%20Event%20Structure) (EventInstigator :type Controller%20Object%20Reference) (DamageCauser :type Actor%20Object%20Reference) (bIsPointDamage :type Boolean) (PointHitInfo :type Hit%20Result%20Structure))
  (bind _outdamage (CallFunction|SPAdjustDamagetoDynamicStructure TheDamageEvent (Utilities|Struct|BreakSP_DynamicGatewayData (Variables|Default|GetGatewayData)) 1))
  (return _outdamage))

(fn IDynamicGetIsCrafting
  (return (Variables|Default|GetIsCrafting)))

(fn IDynamicGetMaterials
  (return (Variables|Default|GetMaterialsRequired) (Variables|Default|GetMaterialsStored)))

(fn IDynamicGetPerUnitCraftCostArray
  (return (Variables|Default|GetCraftingCosts)))

(fn IDynamicGetStructure
  (return self))

(fn IDynamicSetDestructionTime
  (params (DestructionTime :type Float%20%28double-precision%29))
  (Variables|Default|SetDestructionTime DestructionTime true)
  (return true))

(fn IDynamicSetGatewayData
  (params (GatewayData :type SP%20Dynamic%20Gateway%20Data%20Structure))
  (Variables|Default|SetGatewayData GatewayData true)
  (return true))

(fn IDynamicSetIsCrafting
  (params (IsCrafting :type Boolean))
  (Variables|Default|SetIsCrafting IsCrafting true)
  (return true))

(fn IDynamicSetMaterials
  (params (TotalResources :type Array%20of%20Crafting%20Resource%20Requirement%20Structures) (StoredResources :type Array%20of%20Crafting%20Resource%20Requirement%20Structures))
  (Variables|Default|SetMaterialsRequired TotalResources true)
  (Variables|Default|SetMaterialsStored StoredResources true)
  (return false))

(fn IDynamicSetRepairCooldown
  (params (RepairCooldownTime :type Float%20%28double-precision%29))
  (Variables|Default|SetRepairCooldownTime RepairCooldownTime true)
  (return true))

(fn IDynamicSetStructureSettings
  (params (StructureSettings :type Primal%20Structure%20Settings%20Class%20Reference))
  (Variables|Default|SetStructureSettingsClass StructureSettings)
  (return true))

(fn IGlassGetModel
  (return 0 false))

(fn IGlassGetTransparency
  (return (Variables|Default|GetGlassSettings) (Variables|Default|GetMinOpacity)))