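; Square internal pipe structure that adjusts where child structures land when snapped onto it.
; Its snapped-transform override calls AlterSnapPoint, which, for a middle range of snap indices, searches the pipe's linked structures for a Ceiling_Base.
; When one is found, it raises the snapped position slightly on Z and flags the override as used, returning zero rotation.
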(fn ConstructionScript
  (|CallParentFunction))

(fn BPOverrideSnappedtoTransform
  (params (childStructure :type Primal%20Structure%20Object%20Reference) (ChildSnapFromIndex :type Integer) (ChildSnapFromName :type Name :default "None") (UnsnappedPlacementPos :type Vector :default "0, 0, 0") (UnsnappedPlacementRot :type Rotator :default "0, 0, 0") (SnappedPlacementPos :type Vector :default "0, 0, 0") (SnappedPlacementRot :type Rotator :default "0, 0, 0") (SnapToIndex :type Integer) (SnapToName :type Name :default "None"))
  (bind (_useoverride _newlocaiton) (CallFunction|AlterSnapPoint SnapToIndex SnappedPlacementPos))
  (return _newlocaiton "0, 0, 0" 0 _useoverride))

(fn AlterSnapPoint
  (params (SnapToIndex :type Integer) (SnappedLocation :type Vector :default "0, 0, 0"))
  (Utilities|FlowControl|Sequence
    (:then_0
      (if (and (>= SnapToIndex 6) (<= SnapToIndex 10))
        (bind _array_element (Utilities|Array|ForEachLoopwithBreak (Variables|Default|GetLinkedStructures) :!label _label)
          (:LoopBody
            (Utilities|Casting|CastToCeiling_Base _array_element)
            (LocalVariables|SetIsPlacedOnCeiling true)
            (goto _label Break))
          (:Completed
            (if (LocalVariables|GetIsPlacedOnCeiling)
              (LocalVariables|SetOverrideLocation (+ SnappedLocation "0, 0,10.000000")))))))
    (:then_1
      (return (LocalVariables|GetIsPlacedOnCeiling) (LocalVariables|GetOverrideLocation)))))