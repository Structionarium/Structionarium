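; Flexible wire structure that joins two or more nearby wires through a central point, with placement blocked when fewer are in range.
; On the server it finds neighbours, links both ways and refreshes power status.
; It draws spline-mesh cables from the centre to each connection point, using a preview material during placement.
; When a linked wire is destroyed it recalculates, or drops its item and destroys itself if too few remain.
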(event Custom|ConnectionLostEvent
  (bind _returnvalue (Class|KismetMathLibrary|MakeRot 0.0 0.0 0.0))
  (bind _self self)
  (Utilities|FlowControl|Delay 0.5)
  (bind _nearbystructures (CallFunction|SPGetNearbyStructuresforFlexibleConnection _self "/Game/Mods/StructuresPlusMod/Wires/Base_Wire.Base_Wire_C"))
  (if (<= (Utilities|Array|Length _nearbystructures) 1)
    (bind _asprimalitem (Utilities|Casting|CastToPrimalItemClass (Variables|Default|GetConsumesPrimalItem)))
    (Class|PrimalInventoryComponent|StaticDropNewItem self _asprimalitem 0.0 true 1 false 0 _returnvalue true (Transformation|GetActorLocation) _returnvalue true false false true 0 "0, 0, 0" 0 0.0)
    (Actor|DestroyActor)
    (else
      (bind (_connectionpoints _centralpoint) (CallFunction|SPGetCentralPointforFlexibleConnection _nearbystructures _self))
      (Variables|Default|SetConnectionPoints _connectionpoints true)
      (Variables|Default|SetConnectionCenterPoint _centralpoint true)
      (CallFunction|UpdateSplineMeshesEvent)
      (CallFunction|SPHandlePowerStatus self))))

(event Custom|UpdateSplineMeshesEvent
  (Utilities|SwitchNetAuthority
    (:PlayerServer
      _)
    (:Client
      _))
  (CallFunction|AddSplineMeshComponents false))

(event EventBeginPlay
  (bind _self self)
  (Utilities|FlowControl|Delay 0.2)
  (if (not (Variables|Default|GetbIsPreviewStructure))
    (Networking|SwitchHasAuthority
      (:Authority
        (Utilities|FlowControl|Sequence
          (:then_0
            (if (== (Utilities|Array|Length (Variables|Default|GetConnectionPoints)) 0)
              (bind _nearbystructures (CallFunction|SPGetNearbyStructuresforFlexibleConnection _self "/Game/Mods/StructuresPlusMod/Wires/Base_Wire.Base_Wire_C"))
              (Utilities|FlowControl|Sequence
                (:then_0
                  (bind (_connectionpoints _centralpoint) (CallFunction|SPGetCentralPointforFlexibleConnection _nearbystructures _self))
                  (Variables|Default|SetConnectionPoints _connectionpoints true)
                  (Variables|Default|SetConnectionCenterPoint _centralpoint true))
                (:then_1
                  (CallFunction|LinkWires self _nearbystructures)
                  (CallFunction|SPHandlePowerStatus self)))))
          (:then_1
            (CallFunction|UpdateSplineMeshesEvent))
          (:then_2
            (for _array_element (Variables|Default|GetLinkedStructures)
              (bind _asbase_wire_c (Utilities|Casting|CastToBase_Wire _array_element))
              (Game|BindEventtoOnDestroyed _asbase_wire_c (delegate Custom|ConnectionLostEvent))))))
      (:Remote
        (CallFunction|AddSplineMeshComponents false)))))

(fn ConstructionScript)

(fn BPIsAllowedtoBuild
  (params (OutPlacementData :type Placement%20Data%20Structure%20%28by%20ref%29) (CurrentAllowedReason :type Integer))
  (bind _self self)
  (LocalVariables|SetBuildReason (Math|Integer|SelectInt 1 CurrentAllowedReason (== CurrentAllowedReason -9)))
  (if (Variables|Default|GetbIsPreviewStructure)
    (bind _nearbystructures (CallFunction|SPGetNearbyStructuresforFlexibleConnection _self "/Game/Mods/StructuresPlusMod/Wires/Base_Wire.Base_Wire_C"))
    (bind (_connectionpoints _centralpoint) (CallFunction|SPGetCentralPointforFlexibleConnection _nearbystructures _self))
    (Variables|Default|SetConnectionPoints _connectionpoints false)
    (Variables|Default|SetConnectionCenterPoint _centralpoint false)
    (if (< (Utilities|Array|Length _connectionpoints) 2)
      (LocalVariables|SetBuildReason -100)
      (else
        (CallFunction|AddSplineMeshComponents true))))
  (return (LocalVariables|GetBuildReason)))

(fn BPOverrideCantBuildReasonString
  (params (CantBuildReason :type Integer))
  (return (Utilities|String|SelectString "Requires 2 or more nearby wires." "" (== CantBuildReason -100))))

(fn AddSplineMeshComponents
  (params (UsePreviewMaterial :type Boolean))
  (for _array_element (Variables|Default|GetSplineMeshes)
    (Components|DestroyComponent _array_element))
  (for _array_element_2 (Variables|Default|GetConnectionPoints)
    (bind _returnvalue (AddComponent|AddSplineMeshComponent true))
    (Class|SceneComponent|Attachto _returnvalue (Variables|Default|GetMyRootTransform) "None" "KeepWorldPosition" true)
    (Components|StaticMesh|SetStaticMesh _returnvalue "/Game/PrimalEarth/Test_Efecto/PowerCablesStructures/SM_CablesStraight.SM_CablesStraight")
    (SplineMesh|SetStartandEnd _returnvalue (Variables|Default|GetConnectionCenterPoint) "0, 0, 0" _array_element_2 "0, 0, 0" :!class /Script/Engine.SplineMeshComponent)
    (Utilities|Array|Add (Variables|Default|GetSplineMeshes) _returnvalue)
    (if UsePreviewMaterial
      (Rendering|Material|SetMaterial _returnvalue 0 "/Game/Mods/StructuresPlusMod/_Materials/PreviewMaterial.PreviewMaterial")
      (else
        (Rendering|Material|SetMaterial _returnvalue 0 "/Game/Mods/StructuresPlusMod/_Materials/FlexWire_MIC.FlexWire_MIC")))))

(fn LinkWires
  (params (ThisWire :type Base%20Wire%20Object%20Reference) (Connections :type Array%20of%20Primal%20Structure%20Object%20References))
  (bind _linkedstructures (Variables|Default|GetLinkedStructures))
  (for _array_element Connections
    (Utilities|FlowControl|Sequence
      (:then_0
        (if (not (Utilities|Array|ContainsItem _linkedstructures _array_element))
          (Utilities|Array|Add _linkedstructures _array_element)))
      (:then_1
        (if (not (Utilities|Array|ContainsItem (Variables|/Script/ShooterGame.PrimalStructure|GetLinkedStructures _array_element) ThisWire))
          (Utilities|Array|Add (Variables|/Script/ShooterGame.PrimalStructure|GetLinkedStructures _array_element) ThisWire))))))