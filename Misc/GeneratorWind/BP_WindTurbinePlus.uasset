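; Structures Plus wind turbine that switches itself on and off by local wind, with no manual player activation.
; A randomized looping timer samples day-cycle wind, zeroed when an upward trace is blocked, and the server toggles activation against a minimum-wind threshold.
; INI options set that threshold, pickup rules and MaxPowerDistance, which gates the pipe-source check.
; Placement requires open sky, and the multi-use menu gains S+ entries.
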(event Custom|ForceUpdateWind
  (CallFunction|UpdateWind))

(event EventIPickupSetPickupSettings
  (params (DisablePickup :type Boolean) (DisablePickupWhenDamaged :type Boolean) (DisablePickupAfterTime :type Float%20%28single-precision%29) (TimeToDisablePickup :type Float%20%28double-precision%29))
  (Variables|Default|SetDisablePickup DisablePickup true)
  (Variables|Default|SetDisablePickupWhenDamaged DisablePickupWhenDamaged true)
  (Variables|Default|SetDisablePickupAfterTime DisablePickupAfterTime true)
  (Variables|Default|SetTimeToDisablePickup TimeToDisablePickup true))

(fn ConstructionScript
  (|CallParentFunction))

(fn BPContainerDeactivated)

(fn BPContainerActivated)

(fn BPCanbeActivated
  (return true))

(fn BPCanbeActivatedbyPlayer
  (params (PC :type Shooter%20Player%20Controller%20Object%20Reference))
  (return false))

(fn BPIsValidWaterSourceforPipe
  (params (ForWaterPipe :type Primal%20Structure%20Water%20Pipe%20Object%20Reference))
  (return (< (Math|Vector|VectorLength (- (Transformation|GetActorLocation ForWaterPipe) (Transformation|GetActorLocation))) (Variables|Default|GetMaxPowerDistance))))

(fn UpdateWind
  (bind _returnvalue (Transformation|GetActorLocation))
  (bind _returnvalue_2 (Class|Actor|GetWorld))
  (bind _returnvalue_3 (+ _returnvalue "0, 0,80.000000"))
  (if (not (Variables|Default|GetbIsPreviewStructure))
    (Utilities|FlowControl|Sequence
      (:then_0
        (bind _returnvalue_4 (Class|VictoryCore|BPFastTrace _returnvalue_2 (+ _returnvalue "0, 0,5000.000000") _returnvalue_3 self))
        (if _returnvalue_4
          (bind _returnvalue_5 (Class|PrimalGlobals|GetDayCycleManager _returnvalue_2))
          (Utilities|IsValid _returnvalue_5
            (:Is%20Valid
              (bind _returnvalue_6 (Class|DayCycleManager|GetWindatLocation _returnvalue_5 _returnvalue_3))
              (Variables|Default|SetCurrentWind _returnvalue_6)))
          (else
            (Variables|Default|SetCurrentWind 0.0))))
      (:then_1
        (if (Networking|IsServer)
          (bind _returnvalue_7 (Class|PrimalStructureItemContainer|CanbeActivated))
          (if (Math|Boolean|NotEqual(Boolean) (Variables|Default|GetbContainerActivated) (and _returnvalue_7 (>= (Variables|Default|GetCurrentWind) (Variables|Default|GetTurnOffForWindLessThan))))
            (Class|PrimalStructure|SetContainerActive (and _returnvalue_7 (>= (Variables|Default|GetCurrentWind) (Variables|Default|GetTurnOffForWindLessThan))))))))))

(fn BPUnstasis
  (CallFunction|UpdateWind))

(fn BPIsAllowedtoBuild
  (params (OutPlacementData :type Placement%20Data%20Structure%20%28by%20ref%29) (CurrentAllowedReason :type Integer))
  (bind _returnvalue (== CurrentAllowedReason -9))
  (bind _returnvalue_2 (Transformation|GetActorLocation))
  (bind _returnvalue_3 (Math|Integer|SelectInt 1 CurrentAllowedReason _returnvalue))
  (LocalVariables|SetretVal _returnvalue_3)
  (if (>= _returnvalue_3 1)
    (bind _returnvalue_4 (Class|VictoryCore|BPFastTrace (Class|Actor|GetWorld) (+ _returnvalue_2 "0, 0,4000.000000") (+ _returnvalue_2 "0, 0,50.000000") self))
    (if _returnvalue_4
      _
      (else
        (LocalVariables|SetretVal -100))))
  (return (LocalVariables|GetretVal)))

(fn BPOverrideCantBuildReasonString
  (params (CantBuildReason :type Integer))
  (if (== CantBuildReason -100)
    (LocalVariables|SetretVal "Needs open access to the sky!"))
  (return (LocalVariables|GetretVal)))

(fn BPGetMultiUseEntries
  (params (ForPC :type Player%20Controller%20Object%20Reference) (MultiUseEntries :type Array%20of%20Multi%20Use%20Entry%20Structures))
  (bind _entriesout (CallFunction|SPAddMenuEntries MultiUseEntries ForPC self (Variables|Default|GetDisablePickup) (Variables|Default|GetDisablePickupWhenDamaged) false false (Variables|Default|GetDisablePickupAfterTime) (Variables|Default|GetTimeToDisablePickup)))
  (return _entriesout))

(fn SetTurbineSettings
  (bind _returnvalue (Game|GetGameMode))
  (bind _asshootergamemode (Utilities|Casting|CastToShooterGameMode _returnvalue))
  (Utilities|FlowControl|Sequence
    (:then_0
      (bind _returnvalue_2 (Class|ShooterGameMode|GetFloatOptionIni _asshootergamemode "StructuresPlus" "MinWindForTurbine"))
      (Variables|Default|SetTurnOffForWindLessThan (Math|Float|SelectFloat 1e+02 (Math|Float|SelectFloat 2e+01 (Math|Float|SelectFloat 0.0 _returnvalue_2 (== _returnvalue_2 -1.0)) (== _returnvalue_2 0.0)) (> (Math|Float|SelectFloat 2e+01 (Math|Float|SelectFloat 0.0 _returnvalue_2 (== _returnvalue_2 -1.0)) (== _returnvalue_2 0.0)) 1e+02)) true))
    (:then_1
      (bind _value (CallFunction|SPGetIntIniOption _returnvalue "TurbineMaxPowerDistanceInFoundations" 30 1000))
      (Variables|Default|SetMaxPowerDistance (* _value 3e+02) true))))

(fn ReceiveBeginPlay
  (|CallParentFunction)
  (if (not (Variables|Default|GetbIsPreviewStructure))
    (Utilities|Time|SetTimerbyFunctionName 0 "ForceUpdateWind" (Math|Random|RandomFloatinRange 16.0 34.0) true)
    (Networking|SwitchHasAuthority
      (:Authority
        (CallFunction|SPSetPickUpSettings (Game|GetGameMode) self)
        (CallFunction|SetTurbineSettings)
        (CallFunction|UpdateWind)))))

(fn IPickupGetDisablePickupAfterTime
  (return (Variables|Default|GetDisablePickupAfterTime)))

(fn IPickupGetTimetoDisablePickup
  (return (Variables|Default|GetTimeToDisablePickup)))