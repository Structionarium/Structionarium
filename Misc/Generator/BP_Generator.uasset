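; Generator structure with configurable pickup, inventory slots, electric-storm shutdown and wire-hiding availability.
; On authority BeginPlay it reads game-mode settings through SP helpers, then triggers a delayed multicast that unlinks snapped non-pipe structures.
; Multi-use entries add pickup options and team-only Hide/Show Wires, which update every connected Base_Wire found through a water-pipe search.
; It also overrides one placement failure code and notifies the day-cycle manager when active health decreases.
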(event Custom|ClearSnappedStructureEvent
  (Utilities|FlowControl|Delay 1.0)
  (CallFunction|MulticastClearSnappedStructuresEvent))

(event Custom|MulticastClearSnappedStructuresEvent
  (bind _linkedstructures (Variables|Default|GetLinkedStructures))
  (for (_array_element _array_index) _linkedstructures
    (Utilities|Casting|CastToPrimalStructureWaterPipe _array_element
      (:CastFailed
        (bind (_item _index) (Utilities|SPforEachReverse (Variables|/Script/ShooterGame.PrimalStructure|GetLinkedStructures _array_element))
          (:Loop
            (Utilities|Casting|CastToBP_GeneratorClass (Utilities|GetClass _item))
            (Utilities|Array|RemoveIndex (Variables|/Script/ShooterGame.PrimalStructure|GetLinkedStructures _array_element) _index))
          (:Completed
            (Utilities|Array|RemoveIndex _linkedstructures _array_index)))))))

(event Custom|UpdateWiresEvent
  (params (DoHide :type Boolean) (Wires :type Array%20of%20Primal%20Structure%20Object%20References))
  (for _array_element Wires
    (bind _asbase_wire_c (Utilities|Casting|CastToBase_Wire _array_element))
    (Default|UpdateSelf _asbase_wire_c DoHide)))

(event EventIPickupSetPickupSettings
  (params (DisablePickup :type Boolean) (DisablePickupWhenDamaged :type Boolean) (DisablePickupAfterTime :type Float%20%28single-precision%29) (TimeToDisablePickup :type Float%20%28double-precision%29))
  (Variables|Default|SetDisablePickup DisablePickup true)
  (Variables|Default|SetDisablePickupWhenDamaged DisablePickupWhenDamaged true)
  (Variables|Default|SetDisablePickupAfterTime DisablePickupAfterTime true)
  (Variables|Default|SetTimeToDisablePickup TimeToDisablePickup true))

(fn ConstructionScript)

(fn BPGetMultiUseEntries
  (params (ForPC :type Player%20Controller%20Object%20Reference) (MultiUseEntries :type Array%20of%20Multi%20Use%20Entry%20Structures))
  (bind _entriesout (CallFunction|SPAddMenuEntries MultiUseEntries ForPC self (Variables|Default|GetDisablePickup) (Variables|Default|GetDisablePickupWhenDamaged) false false (Variables|Default|GetDisablePickupAfterTime) (Variables|Default|GetTimeToDisablePickup)))
  (if (and (== (Variables|/Script/Engine.Actor|GetTargetingTeam ForPC) (Variables|Default|GetTargetingTeam)) (not (Variables|Default|GetDisableHide)))
    (Utilities|Array|Add _entriesout (Utilities|Struct|MakeMultiUseEntry "Hide Wires" 9001 -1005))
    (Utilities|Array|Add _entriesout (Utilities|Struct|MakeMultiUseEntry "Show Wires" 9002 -1004)))
  (return _entriesout))

(fn BPTryMultiUse
  (params (ForPC :type Player%20Controller%20Object%20Reference) (UseIndex :type Integer))
  (bind _array (Utilities|Array|MakeArray "/Script/ShooterGame.PrimalStructureWaterPipe"))
  (bind _self self)
  (Utilities|FlowControl|Sequence
    (:then_0
      (if (== UseIndex 601)
        (Variables|Default|SetIsUnlocked (not (Variables|Default|GetbIsLocked)))))
    (:then_1
      (switch int UseIndex
        (:Default
          _)
        (:9001
          (bind _connectedstructures (CallFunction|SPGetAllConnectedStructureOfTypes _self _array))
          (CallFunction|UpdateWiresEvent true _connectedstructures))
        (:9002
          (bind _connectedstructures_2 (CallFunction|SPGetAllConnectedStructureOfTypes _self _array))
          (CallFunction|UpdateWiresEvent false _connectedstructures_2)))
      (return true))))

(fn BPIsAllowedtoBuild
  (params (OutPlacementData :type Placement%20Data%20Structure%20%28by%20ref%29) (CurrentAllowedReason :type Integer))
  (return (Math|Integer|SelectInt 1 CurrentAllowedReason (== CurrentAllowedReason -9))))

(fn BPonContainerActiveHealthDecrease
  (bind _returnvalue (Class|PrimalGlobals|GetDayCycleManager (Class|Actor|GetWorld)))
  (bind _asdaycyclemanagerbase_c (Utilities|Casting|CastToDayCycleManagerBase _returnvalue))
  (Default|ActivatedStructureUpdated _asdaycyclemanagerbase_c self))

(fn OnRepInventorySlots
  (Variables|/Script/ShooterGame.PrimalInventoryComponent|SetMaxInventoryItems (Variables|Default|GetMyInventoryComponent) (Variables|Default|GetInventorySlots)))

(fn ReceiveBeginPlay
  (bind _returnvalue (Game|GetGameMode))
  (|CallParentFunction)
  (if (not (Variables|Default|GetbIsPreviewStructure))
    (Networking|SwitchHasAuthority
      (:Authority
        (Utilities|FlowControl|Sequence
          (:then_0
            (CallFunction|SPSetPickUpSettings _returnvalue self))
          (:then_1
            (bind _disablehide (CallFunction|SPGetHideSettings _returnvalue))
            (Variables|Default|SetDisableHide _disablehide true))
          (:then_2
            (bind _value (CallFunction|SPGetBoolOption _returnvalue "DisableGeneratorDuringStorm"))
            (Variables|Default|SetbDisableStructureOnElectricStorm _value))
          (:then_3
            (bind _slotcount (CallFunction|SPGetInventorySlotSetting _returnvalue "GeneratorSlotCount" 8))
            (Variables|Default|SetInventorySlots _slotcount true))
          (:then_4
            (Variables|Default|SetbIsLocked (not (Variables|Default|GetIsUnlocked)) true))
          (:then_5
            (CallFunction|ClearSnappedStructureEvent)))))))

(fn IPickupGetDisablePickupAfterTime
  (return (Variables|Default|GetDisablePickupAfterTime)))

(fn IPickupGetTimetoDisablePickup
  (return (Variables|Default|GetTimeToDisablePickup)))