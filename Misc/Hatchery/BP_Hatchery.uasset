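; Structures Plus hatchery container that gathers same-team fertilized eggs dropped within range and incubates them in its inventory.
; While active, server timers collect non-blacklisted eggs, stamp egg-boost time on nearby team dinos, and drain egg durability down to a floor of 1.
; Game-mode settings supply slots, range, incubation speed and pickup rules.
; Multi-use entries toggle collection and range display or edit the blacklist, while RepNotifies and Dodo animation handle visuals.
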(event EventIPickupSetPickupSettings
  (params (DisablePickup :type Boolean) (DisablePickupWhenDamaged :type Boolean) (DisablePickupAfterTime :type Float%20%28single-precision%29) (TimeToDisablePickup :type Float%20%28double-precision%29))
  (Variables|Default|SetDisablePickup DisablePickup true)
  (Variables|Default|SetDisablePickupWhenDamaged DisablePickupWhenDamaged true)
  (Variables|Default|SetDisablePickupAfterTime DisablePickupAfterTime true)
  (Variables|Default|SetTimeToDisablePickup TimeToDisablePickup true))

(event EventBPContainerActivated
  (CallFunction|HandleAnimation true)
  (Networking|SwitchHasAuthority
    (:Authority
      (CallFunction|HandleCollectItems)
      (Utilities|Time|SetTimerbyFunctionName 0 "HandleCollectItems" 45.0 true)
      (Utilities|Time|SetTimerbyFunctionName 0 "HandleEggs" (Variables|Default|GetIncubationInterval) true))))

(event EventBPContainerDeactivated
  (CallFunction|HandleAnimation false)
  (Networking|SwitchHasAuthority
    (:Authority
      (Utilities|Time|ClearTimerbyFunctionName 0 "HandleCollectItems")
      (Utilities|Time|ClearTimerbyFunctionName 0 "HandleEggs"))))

(event EventBPPostLoadedfromSaveGame
  (Networking|SwitchHasAuthority
    (:Authority
      (Utilities|FlowControl|Delay 0.2)
      (Utilities|Time|SetTimerbyFunctionName 0 "HandleCollectItems" (Math|Random|RandomFloatinRange 4e+01 5e+01) true)
      (Utilities|Time|SetTimerbyFunctionName 0 "HandleEggs" (Variables|Default|GetIncubationInterval) true))))

(fn ConstructionScript
  (|CallParentFunction)
  (Utilities|SwitchNetAuthority
    (:PlayerServer
      _)
    (:Client
      _))
  (bind _returnvalue (Class|PrimalInventoryComponent|GetItemTemplateQuantity (Variables|Default|GetMyInventoryComponent) "/Game/PrimalEarth/CoreBlueprints/Items/Consumables/PrimalItemConsumable_Egg.PrimalItemConsumable_Egg_C" 0 true false false))
  (Rendering|SetVisibility (Variables|Default|GetEggs) (> _returnvalue 0) true)
  (Components|Animation|PlayAnimation (Variables|Default|GetDodo) (select (> _returnvalue 0) (Variables|Default|GetIncubatingAnimation) (Variables|Default|GetIdleAnimation)) true))

(fn BPIsAllowedtoBuild
  (params (OutPlacementData :type Placement%20Data%20Structure%20%28by%20ref%29) (CurrentAllowedReason :type Integer))
  (return (Math|Integer|SelectInt 1 CurrentAllowedReason (== CurrentAllowedReason -9))))

(fn BPGetMultiUseEntries
  (params (ForPC :type Player%20Controller%20Object%20Reference) (MultiUseEntries :type Array%20of%20Multi%20Use%20Entry%20Structures))
  (bind _entriesout (CallFunction|SPAddMenuEntries MultiUseEntries ForPC self (Variables|Default|GetDisablePickup) (Variables|Default|GetDisablePickupWhenDamaged) false false (Variables|Default|GetDisablePickupAfterTime) (Variables|Default|GetTimeToDisablePickup)))
  (Utilities|FlowControl|Sequence
    (:then_0
      (if (== (Variables|/Script/Engine.Actor|GetTargetingTeam ForPC) (Variables|Default|GetTargetingTeam))
        (Utilities|Array|Add _entriesout (Utilities|Struct|MakeMultiUseEntry (Utilities|String|SelectString "Show Range" "Hide Range" (Variables|Default|GetIsRangeHidden)) 9001 -1009))
        (Utilities|Array|Add _entriesout (Utilities|Struct|MakeMultiUseEntry (Utilities|String|SelectString "Start Collecting Eggs" "Stop Collecting Eggs" (Variables|Default|GetDisableEggCollection)) 9003 -1006))
        (Utilities|Array|Add _entriesout (Utilities|Struct|MakeMultiUseEntry "Add to Blacklist" 9004 -1006 true true))
        (Utilities|Array|Add _entriesout (Utilities|Struct|MakeMultiUseEntry "Remove from Blacklist" 9005 -1010 true true))))
    (:then_1
      (return _entriesout))))

(fn BPTryMultiUse
  (params (ForPC :type Player%20Controller%20Object%20Reference) (UseIndex :type Integer))
  (Utilities|FlowControl|Sequence
    (:then_0
      (if (== UseIndex 601)
        (Variables|Default|SetIsUnlocked (not (Variables|Default|GetbIsLocked)))))
    (:then_1
      (switch int UseIndex
        (:9001
          (Variables|Default|SetIsRangeHidden (not (Variables|Default|GetIsRangeHidden)) true))
        (:9003
          (Variables|Default|SetDisableEggCollection (not (Variables|Default|GetDisableEggCollection)) true))
        (:9004
          (CallFunction|HandleAddBlacklist ForPC))
        (:9005
          (CallFunction|HandleRemoveBlacklist ForPC))))
    (:then_2
      (return true))))

(fn OnRepCollectionRange
  (bind _collectionrange (Variables|Default|GetCollectionRange))
  (Transformation|SetWorldScale3D (Variables|Default|GetRangeMesh) (Math|Vector|MakeVector _collectionrange _collectionrange _collectionrange)))

(fn OnRepInventorySlots
  (Variables|/Script/ShooterGame.PrimalInventoryComponent|SetMaxInventoryItems (Variables|Default|GetMyInventoryComponent) (Variables|Default|GetInventorySlots)))

(fn HandleCollectItems
  (if (Variables|Default|GetbContainerActivated)
    (if (not (Variables|Default|GetDisableEggCollection))
      (bind (_outactors _returnvalue) (Class|KismetSystemLibrary|SphereOverlapActorsSimple (Transformation|GetActorLocation) (Variables|Default|GetCollectionRange) "ObjectTypeQuery11" "/Script/ShooterGame.DroppedItem" (Utilities|Array|MakeArray)))
      (if _returnvalue
        (bind _array_element (Utilities|Array|ForEachLoopwithBreak _outactors :!label _label)
          (:LoopBody
            (bind _isnotfull (CallFunction|SPDoesInventoryHaveEmptySlots (Variables|Default|GetMyInventoryComponent)))
            (if _isnotfull
              (if (== (Variables|Default|GetTargetingTeam) (Variables|/Script/Engine.Actor|GetTargetingTeam _array_element))
                (bind _asdroppeditem (Utilities|Casting|CastToDroppedItem _array_element))
                (if (Math|Boolean|ANDBoolean (Variables|/Script/ShooterGame.PrimalItem|GetbIsEgg (Variables|/Script/ShooterGame.DroppedItem|GetMyItem _asdroppeditem)) (!= (Variables|/Script/ShooterGame.PrimalItem|GetEggDinoClassToSpawn (Variables|/Script/ShooterGame.DroppedItem|GetMyItem _asdroppeditem)) 0) (> (Variables|/Script/ShooterGame.PrimalItem|GetItemDurability (Variables|/Script/ShooterGame.DroppedItem|GetMyItem _asdroppeditem)) 1.0) (not (Utilities|Array|ContainsItem (Variables|Default|GetBlacklist) (Utilities|GetClass (Variables|/Script/ShooterGame.DroppedItem|GetMyItem _asdroppeditem)))))
                  (Class|PrimalInventoryComponent|AddItemObject (Variables|Default|GetMyInventoryComponent) (Variables|/Script/ShooterGame.DroppedItem|GetMyItem _asdroppeditem))
                  (Actor|DestroyActor _asdroppeditem)))
              (else
                (goto _label Break)))))))
    (else
      (Utilities|Time|ClearTimerbyFunctionName 0 "HandleCollectItems"))))

(fn HandleAnimation
  (params (IsActive :type Boolean))
  (bind _dodo (Variables|Default|GetDodo))
  (if (not (Networking|IsDedicatedServer))
    (Components|Animation|PlayAnimation _dodo (select IsActive (Variables|Default|GetIncubatingAnimation) (Variables|Default|GetIdleAnimation)) true)
    (Variables|/Script/Engine.SkeletalMeshComponent|SetGlobalAnimRateScale _dodo (Math|Float|SelectFloat 0.25 1.0 IsActive))))

(fn BPNotifyInventoryItemChange
  (params (bIsItemAdd :type Boolean) (theItem :type Primal%20Item%20Object%20Reference) (bEquipItem :type Boolean))
  (bind _returnvalue (Class|PrimalInventoryComponent|GetItemTemplateQuantity (Variables|Default|GetMyInventoryComponent) "/Game/PrimalEarth/CoreBlueprints/Items/Consumables/PrimalItemConsumable_Egg.PrimalItemConsumable_Egg_C" 0 true false false))
  (Variables|Default|SetAreEggsVisible (> _returnvalue 0) true))

(fn OnRepAreEggsVisible
  (Rendering|SetVisibility (Variables|Default|GetEggs) (Variables|Default|GetAreEggsVisible) true))

(fn HandleEggs
  (if (Variables|Default|GetbContainerActivated)
    (CallFunction|GiveEggBoost)
    (CallFunction|IncubateEggs)
    (else
      (Utilities|Time|ClearTimerbyFunctionName 0 "HandleEggs"))))

(fn GiveEggBoost
  (LocalVariables|SetCurrentTime (Utilities|Time|GetGameTimeinSeconds))
  (bind _asshootergamemode (Utilities|Casting|CastToShooterGameMode (Game|GetGameMode)))
  (bind _returnvalue (Class|ShooterGameMode|GetOverlappingDinoCharactersOfTeamandClass _asshootergamemode (Transformation|GetActorLocation) (Variables|Default|GetCollectionRange) 0 (Variables|Default|GetTargetingTeam) false true))
  (for _array_element _returnvalue
    (Variables|/Script/ShooterGame.PrimalDinoCharacter|SetLastEggBoostedTime _array_element (LocalVariables|GetCurrentTime))))

(fn IncubateEggs
  (bind _asshootergamestate (Utilities|Casting|CastToShooterGameState (Game|GetGameState)))
  (for _array_element (Variables|/Script/ShooterGame.PrimalInventoryComponent|GetInventoryItems (Variables|Default|GetMyInventoryComponent))
    (if (and (Variables|/Script/ShooterGame.PrimalItem|GetbIsEgg _array_element) (> (Variables|/Script/ShooterGame.PrimalItem|GetItemDurability _array_element) 1.0))
      (Variables|/Script/ShooterGame.PrimalItem|SetItemDurability _array_element (Math|Float|Clamp(Float) (- (Variables|/Script/ShooterGame.PrimalItem|GetItemDurability _array_element) (* (Variables|/Script/ShooterGame.PrimalItem|GetEggLoseDurabilityPerSecond _array_element) (Variables|/Script/ShooterGame.PrimalItem|GetExtraEggLoseDurabilityPerSecondMultiplier _array_element) (Variables|/Script/ShooterGame.ShooterGameState|GetEggHatchSpeedMultiplier _asshootergamestate) (Variables|Default|GetIncubationMultiplier) (Variables|Default|GetIncubationInterval))) 1.0 1e+02)))))

(fn ReceiveBeginPlay
  (bind _returnvalue (Game|GetGameMode))
  (|CallParentFunction)
  (if (not (Variables|Default|GetbIsPreviewStructure))
    (Networking|SwitchHasAuthority
      (:Authority
        (Utilities|FlowControl|Sequence
          (:then_0
            (CallFunction|SPSetPickUpSettings _returnvalue self))
          (:then_1
            (bind _slotcount (CallFunction|SPGetInventorySlotSetting _returnvalue "HatcherySlotCount" 50))
            (Variables|Default|SetInventorySlots _slotcount true))
          (:then_2
            (bind _value (CallFunction|SPGetIntIniOption _returnvalue "HatcheryRangeInFoundations" 25 100))
            (Variables|Default|SetCollectionRange (* _value 3e+02) true))
          (:then_3
            (Variables|Default|SetbIsLocked (not (Variables|Default|GetIsUnlocked)) true))
          (:then_4
            (bind _value_2 (CallFunction|SPGetFloatIniOption _returnvalue "HatcheryIncubationMultiplier" 2.0 999999.0))
            (Variables|Default|SetIncubationMultiplier _value_2 false))
          (:then_5
            (Utilities|SwitchNetAuthority
              (:PlayerServer
                (CallFunction|HandleAnimation (Variables|Default|GetbContainerActivated))
                (CallFunction|OnRepAreEggsVisible))))))
      (:Remote
        (CallFunction|HandleAnimation (Variables|Default|GetbContainerActivated))))))

(fn OnRepIsRangeHidden
  (bind _rangemesh (Variables|Default|GetRangeMesh))
  (bind _israngehidden (Variables|Default|GetIsRangeHidden))
  (Development|SetHiddeninGame _rangemesh _israngehidden false)
  (Rendering|SetVisibility _rangemesh (not _israngehidden) false))

(fn HandleAddBlacklist
  (params (PC :type Player%20Controller%20Object%20Reference))
  (for _array_element (Variables|/Script/ShooterGame.PrimalInventoryComponent|GetInventoryItems (Variables|Default|GetMyInventoryComponent))
    (if (Utilities|ClassIsChildOf (Utilities|GetClass _array_element) "/Game/PrimalEarth/CoreBlueprints/Items/Consumables/PrimalItemConsumable_Egg.PrimalItemConsumable_Egg_C")
      (if (not (Utilities|Array|ContainsItem (Variables|Default|GetBlacklist) (Utilities|GetClass _array_element)))
        (Utilities|SPAddifUnique (LocalVariables|GetClassesToBlacklist) (Utilities|GetClass _array_element)))))
  (if (> (Utilities|Array|Length (LocalVariables|GetClassesToBlacklist)) 0)
    (bind _asshooterplayercontroller (Utilities|Casting|CastToShooterPlayerController PC))
    (bind _returnvalue (Class|PrimalBuff|StaticAddBuff "/Game/Mods/StructuresPlusMod/_Buffs/Buff_StructuresPlus_SelectBox_Hatchery.Buff_StructuresPlus_SelectBox_Hatchery_C" (Class|ShooterPlayerController|GetPlayerCharacter _asshooterplayercontroller) 0 0 false))
    (bind _asbuff_structuresplus_selectbox_hatchery_c (Utilities|Casting|CastToBuff_StructuresPlus_SelectBox_Hatchery _returnvalue))
    (Default|InitializeHatcherySelectUI _asbuff_structuresplus_selectbox_hatchery_c self (LocalVariables|GetClassesToBlacklist) true)
    (else
      (CallFunction|SPMessageClient PC "No items in hatchery inventory." "NewEnumerator1"))))

(fn HandleRemoveBlacklist
  (params (PC :type Player%20Controller%20Object%20Reference))
  (if (> (Utilities|Array|Length (Variables|Default|GetBlacklist)) 0)
    (bind _asshooterplayercontroller (Utilities|Casting|CastToShooterPlayerController PC))
    (bind _returnvalue (Class|PrimalBuff|StaticAddBuff "/Game/Mods/StructuresPlusMod/_Buffs/Buff_StructuresPlus_SelectBox_Hatchery.Buff_StructuresPlus_SelectBox_Hatchery_C" (Class|ShooterPlayerController|GetPlayerCharacter _asshooterplayercontroller) 0 0 false))
    (bind _asbuff_structuresplus_selectbox_hatchery_c (Utilities|Casting|CastToBuff_StructuresPlus_SelectBox_Hatchery _returnvalue))
    (Default|InitializeHatcherySelectUI _asbuff_structuresplus_selectbox_hatchery_c self (Variables|Default|GetBlacklist) false)
    (else
      (CallFunction|SPMessageClient PC "Blacklist is empty." "NewEnumerator1"))))

(fn IPickupGetDisablePickupAfterTime
  (return (Variables|Default|GetDisablePickupAfterTime)))

(fn IPickupGetTimetoDisablePickup
  (return (Variables|Default|GetTimeToDisablePickup)))