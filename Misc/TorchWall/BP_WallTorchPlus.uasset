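; Structures Plus wall torch with configurable pickup rules, recolorable flame and optional automatic day/night lighting.
; Same-team players get a multi-use entry that opens the light settings UI through a buff.
; Adding dye sets the replicated TorchColor and consumes one; the color drives the child emitter's flame and light parameters.
; In auto mode, a server-side looping timer switches the torch on at night and off by day, using dawn/dusk offsets.
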(event Custom|HandleBeginPlayEvent
  (Utilities|FlowControl|Delay 2.0)
  (if (.isauto (Variables|Default|GetTorchSettings))
    (Utilities|Time|SetTimerbyFunctionName 0 "CheckTime" 1e+01 true)))

(event Custom|ChangeFlameColorEvent
  (params (FlameColor :type Vector))
  (CallFunction|UpdateTorchColor FlameColor))

(event Custom|RemoveDyeEvent
  (params (DyeClass :type Primal%20Item%20Dye%20Class%20Reference))
  (Utilities|FlowControl|Delay 0.1)
  (Class|PrimalInventoryComponent|BPIncrementItemTemplateQuantity (Variables|Default|GetMyInventoryComponent) DyeClass -1 true false false false false false 0 false))

(event Custom|SetLightSettingsEvent
  (params (Settings :type SP%20Light%20Settings%20Structure))
  (Variables|Default|SetTorchSettings Settings false)
  (Networking|SwitchHasAuthority
    (:Authority
      (Utilities|Time|ClearTimerbyFunctionName 0 "CheckTime")
      (CallFunction|ChangeFlameColorEvent (Variables|Default|GetTorchColor))
      (if (.isauto (Variables|Default|GetTorchSettings))
        (Utilities|Time|SetTimerbyFunctionName 0 "CheckTime" 1e+01 true)))))

(event EventIPickupSetPickupSettings
  (params (DisablePickup :type Boolean) (DisablePickupWhenDamaged :type Boolean) (DisablePickupAfterTime :type Float%20%28single-precision%29) (TimeToDisablePickup :type Float%20%28double-precision%29))
  (Variables|Default|SetDisablePickup DisablePickup true)
  (Variables|Default|SetDisablePickupWhenDamaged DisablePickupWhenDamaged true)
  (Variables|Default|SetDisablePickupAfterTime DisablePickupAfterTime true)
  (Variables|Default|SetTimeToDisablePickup TimeToDisablePickup true))

(fn ConstructionScript)

(fn BPIsAllowedtoBuild
  (params (OutPlacementData :type Placement%20Data%20Structure%20%28by%20ref%29) (CurrentAllowedReason :type Integer))
  (return (Math|Integer|SelectInt 1 CurrentAllowedReason (== CurrentAllowedReason -9))))

(fn BPGetMultiUseEntries
  (params (ForPC :type Player%20Controller%20Object%20Reference) (MultiUseEntries :type Array%20of%20Multi%20Use%20Entry%20Structures))
  (bind _entriesout (CallFunction|SPAddMenuEntries MultiUseEntries ForPC self (Variables|Default|GetDisablePickup) (Variables|Default|GetDisablePickupWhenDamaged) false false (Variables|Default|GetDisablePickupAfterTime) (Variables|Default|GetTimeToDisablePickup)))
  (if (== (Variables|/Script/Engine.Actor|GetTargetingTeam ForPC) (Variables|Default|GetTargetingTeam))
    (Utilities|Array|Add _entriesout (Utilities|Struct|MakeMultiUseEntry "[Change Settings]" 9001 -10 true (Math|Conversions|ToColor(LinearColor) (CallFunction|SPGetSpecialMenuColor)))))
  (return _entriesout))

(fn BPTryMultiUse
  (params (ForPC :type Player%20Controller%20Object%20Reference) (UseIndex :type Integer))
  (switch int UseIndex
    (:Default
      _)
    (:9001
      (Networking|SwitchHasAuthority
        (:Authority
          (bind _asshooterplayercontroller (Utilities|Casting|CastToShooterPlayerController ForPC))
          (bind _returnvalue (Class|PrimalBuff|StaticAddBuff "/Game/Mods/StructuresPlusMod/_Buffs/Buff_StructuresPlus_Lights.Buff_StructuresPlus_Lights_C" (Class|ShooterPlayerController|GetPlayerCharacter _asshooterplayercontroller) 0 0 false))
          (bind _asbuff_structuresplus_lights_c (Utilities|Casting|CastToBuff_StructuresPlus_Lights _returnvalue))
          (Default|InitializeLightUI _asbuff_structuresplus_lights_c self (Variables|Default|GetTorchSettings))))))
  (return true))

(fn BPNotifyInventoryItemChange
  (params (bIsItemAdd :type Boolean) (theItem :type Primal%20Item%20Object%20Reference) (bEquipItem :type Boolean))
  (if bIsItemAdd
    (Utilities|FlowControl|Sequence
      (:then_0
        (bind _asprimalitem_dye (Utilities|Casting|CastToPrimalItem_Dye theItem))
        (Variables|Default|SetTorchColor (Math|Vector|MakeVector (.r (Variables|/Script/ShooterGame.PrimalItem_Dye|GetDyeColor _asprimalitem_dye)) (.g (Variables|/Script/ShooterGame.PrimalItem_Dye|GetDyeColor _asprimalitem_dye)) (.b (Variables|/Script/ShooterGame.PrimalItem_Dye|GetDyeColor _asprimalitem_dye))) false))
      (:then_1
        (bind _asprimalitem_dye_2 (Utilities|Casting|CastToPrimalItem_DyeClass (Utilities|GetClass theItem)))
        (CallFunction|RemoveDyeEvent _asprimalitem_dye_2)))))

(fn OnRepTorchColor
  (bind _torchcolor (Variables|Default|GetTorchColor))
  (Networking|SwitchHasAuthority
    (:Authority
      (CallFunction|ChangeFlameColorEvent _torchcolor))
    (:Remote
      (CallFunction|UpdateTorchColor _torchcolor))))

(fn UpdateTorchColor
  (params (FlameColor :type Vector))
  (bind _returnvalue (* FlameColor 25.0))
  (bind _asemitter_standingtorchplus_c (Utilities|Casting|CastToEmitter_StandingTorchPlus (Variables|/Script/Engine.ChildActorComponent|GetChildActor (Variables|Default|GetActivatedEmitter))))
  (Effects|Components|ParticleSystem|SetVectorParameter (Variables|/Script/Engine.Emitter|GetParticleSystemComponent _asemitter_standingtorchplus_c) "FlameColorA" _returnvalue)
  (Effects|Components|ParticleSystem|SetVectorParameter (Variables|/Script/Engine.Emitter|GetParticleSystemComponent _asemitter_standingtorchplus_c) "FlameColorB" _returnvalue)
  (Effects|Components|ParticleSystem|SetVectorParameter (Variables|/Script/Engine.Emitter|GetParticleSystemComponent _asemitter_standingtorchplus_c) "FlameLightColor" (* FlameColor (* (/ (.a (.primarycolor (Variables|Default|GetTorchSettings))) 3.0) 1.3))))

(fn CheckTime
  (bind _torchsettings (Variables|Default|GetTorchSettings))
  (bind _bcontaineractivated (Variables|Default|GetbContainerActivated))
  (bind (_postdawnoffset _preduskoffset) (Utilities|Struct|BreakSPLightSettings _torchsettings))
  (bind _isday (CallFunction|SPIsDayTime self _postdawnoffset _preduskoffset))
  (if (or (Math|Boolean|NotEqual(Boolean) _isday (Variables|Default|GetIsDaytime)) (Math|Boolean|Equal(Boolean) _isday (Variables|Default|GetbContainerActivated)))
    (Variables|Default|SetIsDaytime _isday)
    (if (Variables|Default|GetIsDayTime)
      (if _bcontaineractivated
        (Class|PrimalStructure|SetContainerActive false))
      (elif (not _bcontaineractivated)
        (Class|PrimalStructure|SetContainerActive true)))))

(fn ReceiveBeginPlay
  (|CallParentFunction)
  (if (not (Variables|Default|GetbIsPreviewStructure))
    (Networking|SwitchHasAuthority
      (:Authority
        (CallFunction|SPSetPickUpSettings (Game|GetGameMode) self)
        (Utilities|FlowControl|Sequence
          (:then_0
            (Utilities|SwitchNetAuthority
              (:PlayerServer
                (CallFunction|UpdateTorchColor (Variables|Default|GetTorchColor)))))
          (:then_1
            (CallFunction|HandleBeginPlayEvent)))))))

(fn IPickupGetDisablePickupAfterTime
  (return (Variables|Default|GetDisablePickupAfterTime)))

(fn IPickupGetTimetoDisablePickup
  (return (Variables|Default|GetTimeToDisablePickup)))