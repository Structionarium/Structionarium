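; S+ flamethrower auto turret that burns characters along its line of fire, with configurable targeting options.
; Any inventory change counts as ammo use, extending a flame window that a looping timer services and a replicated flag mirrors on the emitter.
; Each tick line-traces toward the target, box-traces that path and applies a flame buff to living characters hit.
; Shared SP helpers handle placement, targeting filters, menu, HUD and slot settings.
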(event EventITurretSetOptions
  (params (TurretOptions :type SP%20Turret%20Options%20Structure))
  (Variables|Default|SetTurretOptions TurretOptions false))

(event EventBPContainerActivated
  (CallFunction|UpdateFlameEmitter))

(event EventBPContainerDeactivated
  (CallFunction|UpdateFlameEmitter))

(fn ConstructionScript
  (|CallParentFunction)
  (CallFunction|UpdateFlameEmitter))

(fn BPIsAllowedtoBuild
  (params (OutPlacementData :type Placement%20Data%20Structure%20%28by%20ref%29) (CurrentAllowedReason :type Integer))
  (return (CallFunction|SPIsTurretAllowedtoBuild OutPlacementData CurrentAllowedReason)))

(fn BPGetMultiUseEntries
  (params (ForPC :type Player%20Controller%20Object%20Reference) (MultiUseEntries :type Array%20of%20Multi%20Use%20Entry%20Structures))
  (bind _asshooterplayercontroller (Utilities|Casting|CastToShooterPlayerController ForPC))
  (bind _returnvalue (Class|PrimalStructure|AllowStructureAccess _asshooterplayercontroller))
  (if (and _returnvalue (== (Variables|/Script/Engine.Actor|GetTargetingTeam _asshooterplayercontroller) (Variables|Default|GetTargetingTeam)))
    (Utilities|FlowControl|Sequence
      (:then_0
        (bind _entriesout (CallFunction|SPCleanUpTurretMenuEntries MultiUseEntries))
        (bind _entriesout_2 (CallFunction|SPAddMenuEntries _entriesout ForPC self false false false false 0.0 0.0))
        (LocalVariables|SetEntries _entriesout_2)
        (Utilities|Array|Add (LocalVariables|GetEntries) (Utilities|Struct|MakeMultiUseEntry "[Turret Options]" 9002 -1000 true (Math|Conversions|ToColor(LinearColor) (CallFunction|SPGetSpecialMenuColor)))))
      (:then_1
        (return (LocalVariables|GetEntries))))
    (else
      (return (LocalVariables|GetEntries)))))

(fn BPTryMultiUse
  (params (ForPC :type Player%20Controller%20Object%20Reference) (UseIndex :type Integer))
  (Utilities|FlowControl|Sequence
    (:then_0
      (if (== UseIndex 601)
        (Variables|Default|SetIsUnlocked (not (Variables|Default|GetbIsLocked)))
        (elif (== UseIndex 9002)
          (CallFunction|SPApplyTurretSettingsBuff ForPC self))))
    (:then_1
      (return true))))

(fn OnRepInventorySlots
  (Variables|/Script/ShooterGame.PrimalInventoryComponent|SetMaxInventoryItems (Variables|Default|GetMyInventoryComponent) (Variables|Default|GetInventorySlots)))

(fn BPTurretPreventsTargeting
  (params (PotentialTarget :type Primal%20Character%20Object%20Reference))
  (bind _preventtargeting (CallFunction|SPHandleTurretTargeting PotentialTarget (Variables|Default|GetTurretOptions)))
  (return _preventtargeting))

(fn ReceiveBeginPlay
  (|CallParentFunction)
  (if (not (Variables|Default|GetbIsPreviewStructure))
    (Networking|SwitchHasAuthority
      (:Authority
        (bind _slotcount (CallFunction|SPGetInventorySlotSetting (Game|GetGameMode) "SPlusAutoTurretSlotCount" 75))
        (Variables|Default|SetInventorySlots _slotcount true)
        (Variables|Default|SetbIsLocked (not (Variables|Default|GetIsUnlocked)) true)))))

(fn UpdateFlameEmitter
  (if (and (not (Variables|Default|GetbIsPreviewStructure)) (not (Networking|IsDedicatedServer)))
    (Components|Activation|SetActive (Variables|Default|GetActivatedEmitter) (Variables|Default|GetbContainerActivated) false)))

(fn AmmoConsumed
  (bind _returnvalue (Utilities|Time|GetGameTimeinSeconds))
  (Variables|Default|SetFlameOffTime (- (select (< (Math|Conversions|ToFloat(Integer) (- (Variables|Default|GetFlameOffTime) _returnvalue)) 0.0) _returnvalue (Variables|Default|GetFlameOffTime)) (Math|Conversions|ToFloat(Integer) (* (+ (Variables|Default|GetFireInterval) 0.25) -1.0))))
  (Utilities|FlowControl|Sequence
    (:then_0
      (if (not (Variables|Default|GetIsTimerStarted))
        (Utilities|Time|ClearTimerbyFunctionName 0 "FireFlame")
        (Utilities|Time|SetTimerbyFunctionName 0 "FireFlame" 0.5 true)
        (Variables|Default|SetIsTimerStarted true)
        (CallFunction|FireFlame)
        (Variables|Default|SetFlameVisibility true true)))))

(fn FireFlame
  (if (> (Math|Conversions|ToFloat(Integer) (- (Variables|Default|GetFlameOffTime) (Utilities|Time|GetGameTimeinSeconds))) 0.0)
    (bind _victims (CallFunction|GetVictims))
    (for _array_element _victims
      (Class|PrimalBuff|StaticAddBuff "/Game/Mods/StructuresPlusMod/Misc/AutoTurretFlame/Buff_AutoTurret_Flame.Buff_AutoTurret_Flame_C" _array_element 0 self false))
    (else
      (Utilities|Time|ClearTimerbyFunctionName 0 "FireFlame")
      (Variables|Default|SetIsTimerStarted false)
      (Variables|Default|SetFlameVisibility false true))))

(fn GetVictims
  (bind _target (Variables|Default|GetTarget))
  (bind _inlineofsight (LocalVariables|GetInLineOfSight))
  (bind _skeletalmesh1 (Variables|Default|GetSkeletalMesh1))
  (bind _returnvalue (Transformation|GetSocketLocation _skeletalmesh1 "MuzzleFlashSocket"))
  (Utilities|IsValid _target
    (:Is%20Valid
      (LocalVariables|SetEndVector (+ _returnvalue (* (Math|Vector|GetForwardVector (Math|Rotator|FindLookatRotation _returnvalue (Transformation|GetActorLocation _target))) (Variables|Default|GetTargetingRange))))
      (bind (_outhit _returnvalue_2) (Collision|LineTraceByChannel _returnvalue (LocalVariables|GetEndVector) "ECC_WorldDynamic" false (Utilities|Array|MakeArray) "None"))
      (if _returnvalue_2
        (LocalVariables|SetEndVector (.Location (Collision|BreakHitResult _outhit))))
      (bind (_outhits _returnvalue_3) (Class|KismetSystemLibrary|BoxTraceMultiforObjects _returnvalue (LocalVariables|GetEndVector) "75.000000,75.000000,75.000000" (Transformation|GetSocketRotation _skeletalmesh1 "AimPivotSocket") (Utilities|Array|MakeArray "ObjectTypeQuery6" "ObjectTypeQuery7" "ObjectTypeQuery16") false (Utilities|Array|MakeArray) "None" true))
      (if _returnvalue_3
        (for _array_element _outhits
          (bind _asprimalcharacter (Utilities|Casting|CastToPrimalCharacter (.HitActor (Collision|BreakHitResult _array_element))))
          (if (and (not (Variables|/Script/ShooterGame.PrimalCharacter|GetbIsDead _asprimalcharacter)) (not (Utilities|Array|ContainsItem _inlineofsight _asprimalcharacter)))
            (Utilities|Array|Add _inlineofsight _asprimalcharacter)))))
    (:Is%20Not%20Valid
      _))
  (return (LocalVariables|GetInLineOfSight)))

(fn OnRepFlameVisibility
  (Utilities|SwitchNetAuthority
    (:PlayerServer
      _)
    (:Client
      _))
  (Components|Activation|SetActive (Variables|Default|GetFlameEmitter) (Variables|Default|GetFlameVisibility) false))

(fn BPNotifyInventoryItemChange
  (params (bIsItemAdd :type Boolean) (theItem :type Primal%20Item%20Object%20Reference) (bEquipItem :type Boolean))
  (CallFunction|AmmoConsumed))

(fn BPIsAllowedtoBuildEx
  (params (OutPlacementData :type Placement%20Data%20Structure%20%28by%20ref%29) (CurrentAllowedReason :type Integer) (PC :type Player%20Controller%20Object%20Reference) (bFinalPlacement :type Boolean) (bChoosingRotation :type Boolean))
  (return (CallFunction|SPIsTurretAllowedtoBuildEx OutPlacementData CurrentAllowedReason PC self)))

(fn BlueprintDrawHUD
  (params (HUD :type Shooter%20HUD%20Object%20Reference) (CenterX :type Float%20%28single-precision%29) (CenterY :type Float%20%28single-precision%29))
  (CallFunction|SPDrawTurretHUD HUD CenterX CenterY self))

(fn ITurretGetOptions
  (bind _turretoptions (Variables|Default|GetTurretOptions))
  (bind (_mindinolevel _maxdinolevel _dinolist _isinclusionlist) (Utilities|Struct|BreakSPTurretOptions _turretoptions))
  (return (Utilities|Struct|MakeSPTurretOptions (Variables|Default|GetRangeSetting) (Variables|Default|GetAISetting) (Variables|Default|GetWarningSetting) _mindinolevel _maxdinolevel _dinolist _isinclusionlist)))