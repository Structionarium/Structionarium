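; Sheep Herder structure for ARK: while activated, it shears fully woolled same-team sheep in range and stores the wool in its inventory.
; A looping server timer runs Harvest, which octree-searches sheep within a configurable range.
; Slot count, range and pickup rules come from game-mode settings.
; Armour added to its inventory dresses the female mannequin through replicated mesh paths loaded on clients, with menu entries to reset it or toggle the range display.
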(event EventIPickupSetPickupSettings
  (params (DisablePickup :type Boolean) (DisablePickupWhenDamaged :type Boolean) (DisablePickupAfterTime :type Float%20%28single-precision%29) (TimeToDisablePickup :type Float%20%28double-precision%29))
  (Variables|Default|SetDisablePickup DisablePickup true)
  (Variables|Default|SetDisablePickupWhenDamaged DisablePickupWhenDamaged true)
  (Variables|Default|SetDisablePickupAfterTime DisablePickupAfterTime true)
  (Variables|Default|SetTimeToDisablePickup TimeToDisablePickup true))

(event EventBPContainerActivated
  (CallFunction|HandleAnimation)
  (Networking|SwitchHasAuthority
    (:Authority
      (CallFunction|Harvest)
      (Utilities|Time|SetTimerbyFunctionName 0 "Harvest" 6e+02 true))))

(event EventBPContainerDeactivated
  (CallFunction|HandleAnimation)
  (Networking|SwitchHasAuthority
    (:Authority
      (Utilities|Time|ClearTimerbyFunctionName 0 "Harvest"))))

(event EventBPPostLoadedfromSaveGame
  (Networking|SwitchHasAuthority
    (:Authority
      (Utilities|FlowControl|Delay 0.2)
      (Utilities|Time|SetTimerbyFunctionName 0 "Harvest" (Math|Random|RandomFloatinRange 5.5e+02 6e+02) true))))

(fn ConstructionScript
  (|CallParentFunction))

(fn BPIsAllowedtoBuild
  (params (OutPlacementData :type Placement%20Data%20Structure%20%28by%20ref%29) (CurrentAllowedReason :type Integer))
  (return (Math|Integer|SelectInt 1 CurrentAllowedReason (== CurrentAllowedReason -9))))

(fn BPGetMultiUseEntries
  (params (ForPC :type Player%20Controller%20Object%20Reference) (MultiUseEntries :type Array%20of%20Multi%20Use%20Entry%20Structures))
  (bind _entriesout (CallFunction|SPAddMenuEntries MultiUseEntries ForPC self (Variables|Default|GetDisablePickup) (Variables|Default|GetDisablePickupWhenDamaged) false false (Variables|Default|GetDisablePickupAfterTime) (Variables|Default|GetTimeToDisablePickup)))
  (if (== (Variables|/Script/Engine.Actor|GetTargetingTeam ForPC) (Variables|Default|GetTargetingTeam))
    (Utilities|Array|Add _entriesout (Utilities|Struct|MakeMultiUseEntry (Utilities|String|SelectString "Show Range" "Hide Range" (Variables|Default|GetIsRangeHidden)) 9001 -1009))
    (Utilities|Array|Add _entriesout (Utilities|Struct|MakeMultiUseEntry "Reset Armor" 9002 -1006 true true)))
  (return _entriesout))

(fn BPTryMultiUse
  (params (ForPC :type Player%20Controller%20Object%20Reference) (UseIndex :type Integer))
  (Utilities|FlowControl|Sequence
    (:then_0
      (if (== UseIndex 601)
        (Variables|Default|SetIsUnlocked (not (Variables|Default|GetbIsLocked)))))
    (:then_1
      (switch int UseIndex
        (:Default
          _)
        (:9001
          (Variables|Default|SetIsRangeHidden (not (Variables|Default|GetIsRangeHidden)) true))
        (:9002
          (Variables|Default|SetShirtMeshPath "" true)
          (Variables|Default|SetPantsMeshPath "" true)
          (Variables|Default|SetGlovesMeshPath "" true)
          (Variables|Default|SetBootsMeshPath "" true)))
      (return true))))

(fn OnRepHarvestRange
  (bind _harvestrange (Variables|Default|GetHarvestRange))
  (Transformation|SetWorldScale3D (Variables|Default|GetRangeMesh) (Math|Vector|MakeVector _harvestrange _harvestrange _harvestrange)))

(fn Harvest
  (if (Variables|Default|GetbContainerActivated)
    (Class|PrimalInventoryComponent|InventoryRefresh (Variables|Default|GetMyInventoryComponent))
    (bind _sheep (CallFunction|GetSheep))
    (bind _array_element (Utilities|Array|ForEachLoopwithBreak _sheep :!label _label)
      (:LoopBody
        (bind _emptyslots (CallFunction|SPGetEmptyInventorySlotCount (Variables|Default|GetMyInventoryComponent)))
        (if (== _emptyslots 0)
          (goto _label Break)
          (else
            (Default|BPDinoPrepareforARKUploading _array_element)
            (if (== (Variables|/Game/PrimalEarth/Dinos/Sheep/Sheep_Character_BP.Sheep_Character_BP_C|GetARKTransferWoolPercentage _array_element) 1.0)
              (Default|SetWoolPercentage _array_element 0.0)
              (Default|UpdateWoolMaterial _array_element)
              (Class|PrimalInventoryComponent|BPIncrementItemTemplateQuantity (Variables|Default|GetMyInventoryComponent) "/Game/PrimalEarth/CoreBlueprints/Resources/PrimalItemResource_Wool.PrimalItemResource_Wool_C" (Math|Float|Floor (Variables|/Game/PrimalEarth/Dinos/Sheep/Sheep_Character_BP.Sheep_Character_BP_C|GetGiveWoolItemsForFullPercent _array_element)) true false true false false false 0 false))))))
    (else
      (Utilities|Time|ClearTimerbyFunctionName 0 "Harvest"))))

(fn GetSheep
  (bind _returnvalue (Class|VictoryCore|ServerOctreeOverlapActorsClass (Class|Actor|GetWorld) (Transformation|GetActorLocation) (Variables|Default|GetHarvestRange) "DINOPAWNS" "/Game/PrimalEarth/Dinos/Sheep/Sheep_Character_BP.Sheep_Character_BP_C" false))
  (for _array_element _returnvalue
    (bind _returnvalue_2 (Transformation|GetDistanceTo _array_element self))
    (if (and (<= _returnvalue_2 (Variables|Default|GetHarvestRange)) (== (Variables|/Script/Engine.Actor|GetTargetingTeam _array_element) (Variables|Default|GetTargetingTeam)))
      (bind _assheep_character_bp_c (Utilities|Casting|CastToSheep_Character_BP _array_element))
      (Utilities|Array|Add (LocalVariables|GetSheepInRange) _assheep_character_bp_c)))
  (return (LocalVariables|GetSheepInRange)))

(fn OnRepInventorySlots
  (Variables|/Script/ShooterGame.PrimalInventoryComponent|SetMaxInventoryItems (Variables|Default|GetMyInventoryComponent) (Variables|Default|GetInventorySlots)))

(fn HandleAnimation
  (bind _pawnmesh (Variables|Default|GetPawnMesh))
  (Variables|/Script/Engine.SkeletalMeshComponent|SetbPauseAnims _pawnmesh (not (Variables|Default|GetbContainerActivated)))
  (bind _asanimbp_female_c (Utilities|Casting|CastToAnimBP_Female (Components|SkeletalMesh|GetAnimInstance _pawnmesh)))
  (Variables|/Game/Mods/StructuresPlusMod/Misc/Nanny/AnimBP_Female.AnimBP_Female_C|SetJustIdle _asanimbp_female_c true))

(fn ReceiveBeginPlay
  (bind _returnvalue (Game|GetGameMode))
  (|CallParentFunction)
  (if (not (Variables|Default|GetbIsPreviewStructure))
    (bind _returnvalue_2 (Class|VictoryCore|ConstructObjectAutoNameBP "/Script/ShooterGame.VictoryCore" self))
    (Variables|Default|SetVictoryCore _returnvalue_2)
    (Networking|SwitchHasAuthority
      (:Authority
        (Utilities|FlowControl|Sequence
          (:then_0
            (CallFunction|SPSetPickUpSettings _returnvalue self))
          (:then_1
            (bind _slotcount (CallFunction|SPGetInventorySlotSetting _returnvalue "SheepHerderSlotCount" 300))
            (Variables|Default|SetInventorySlots _slotcount true))
          (:then_2
            (bind _value (CallFunction|SPGetIntIniOption _returnvalue "SheepHerderRangeInFoundations" 10 50))
            (Variables|Default|SetHarvestRange (* _value 3e+02) true))
          (:then_3
            (Variables|Default|SetbIsLocked (not (Variables|Default|GetIsUnlocked)) true))
          (:then_4
            (Utilities|SwitchNetAuthority
              (:PlayerServer
                (CallFunction|HandleonReps))))))
      (:Remote
        (CallFunction|HandleonReps)))))

(fn BPNotifyInventoryItemChange
  (params (bIsItemAdd :type Boolean) (theItem :type Primal%20Item%20Object%20Reference) (bEquipItem :type Boolean))
  (bind _myequipmenttype (Variables|/Script/ShooterGame.PrimalItem|GetMyEquipmentType theItem))
  (bind _myitemskin (Variables|/Script/ShooterGame.PrimalItem|GetMyItemSkin theItem))
  (if bIsItemAdd
    (bind _asvictorycore (Utilities|Casting|CastToVictoryCore (Variables|Default|GetVictoryCore)))
    (bind _femalesk (CallFunction|SPGetSkeletalMeshesfromItem (select (Utilities|IsValid _myitemskin) _myitemskin theItem)))
    (if (Utilities|Enum|Equal(Enum) _myequipmenttype "Shirt")
      (Variables|Default|SetShirtMeshPath (Class|VictoryCore|GetClassPathName _asvictorycore _femalesk) true)
      (elif (Utilities|Enum|Equal(Enum) _myequipmenttype "Pants")
        (Variables|Default|SetPantsMeshPath (Class|VictoryCore|GetClassPathName _asvictorycore _femalesk) true)
        (elif (Utilities|Enum|Equal(Enum) _myequipmenttype "Boots")
          (Variables|Default|SetBootsMeshPath (Class|VictoryCore|GetClassPathName _asvictorycore _femalesk) true)
          (elif (Utilities|Enum|Equal(Enum) _myequipmenttype "Gloves")
            (Variables|Default|SetGlovesMeshPath (Class|VictoryCore|GetClassPathName _asvictorycore _femalesk) true)))))))

(fn OnRepShirtMeshPath
  (bind _shirtmeshpath (Variables|Default|GetShirtMeshPath))
  (bind _shirt (Variables|Default|GetShirt))
  (if (not (Networking|IsDedicatedServer))
    (if (Utilities|Enum|NotEqual(Enum) _shirtmeshpath "")
      (bind _asvictorycore (Utilities|Casting|CastToVictoryCore (Variables|Default|GetVictoryCore)))
      (bind _returnvalue (Class|VictoryCore|BPLoadObject _asvictorycore _shirtmeshpath))
      (Utilities|IsValid _returnvalue
        (:Is%20Valid
          (bind _asskeletalmesh (Utilities|Casting|CastToSkeletalMesh _returnvalue))
          (CallFunction|SPSetEquippedMesh _shirt _asskeletalmesh)))
      (else
        (CallFunction|SPSetEquippedMesh _shirt "/Game/PrimalEarth/Human/Female/Outfits/Ghillie/ghilie_suit_female_shirt.ghilie_suit_female_shirt")))))

(fn OnRepPantsMeshPath
  (bind _pantsmeshpath (Variables|Default|GetPantsMeshPath))
  (bind _pants (Variables|Default|GetPants))
  (if (not (Networking|IsDedicatedServer))
    (if (Utilities|Enum|NotEqual(Enum) _pantsmeshpath "")
      (bind _asvictorycore (Utilities|Casting|CastToVictoryCore (Variables|Default|GetVictoryCore)))
      (bind _returnvalue (Class|VictoryCore|BPLoadObject _asvictorycore _pantsmeshpath))
      (Utilities|IsValid _returnvalue
        (:Is%20Valid
          (bind _asskeletalmesh (Utilities|Casting|CastToSkeletalMesh _returnvalue))
          (CallFunction|SPSetEquippedMesh _pants _asskeletalmesh)))
      (else
        (CallFunction|SPSetEquippedMesh _pants "/Game/PrimalEarth/Human/Female/Outfits/Ghillie/ghilie_suit_female_pants.ghilie_suit_female_pants")))))

(fn OnRepGlovesMeshPath
  (bind _glovesmeshpath (Variables|Default|GetGlovesMeshPath))
  (bind _gloves (Variables|Default|GetGloves))
  (if (not (Networking|IsDedicatedServer))
    (if (Utilities|Enum|NotEqual(Enum) _glovesmeshpath "")
      (bind _asvictorycore (Utilities|Casting|CastToVictoryCore (Variables|Default|GetVictoryCore)))
      (bind _returnvalue (Class|VictoryCore|BPLoadObject _asvictorycore _glovesmeshpath))
      (Utilities|IsValid _returnvalue
        (:Is%20Valid
          (bind _asskeletalmesh (Utilities|Casting|CastToSkeletalMesh _returnvalue))
          (CallFunction|SPSetEquippedMesh _gloves _asskeletalmesh)))
      (else
        (CallFunction|SPSetEquippedMesh _gloves "/Game/PrimalEarth/Human/Female/Outfits/Ghillie/ghilie_suit_female_gloves.ghilie_suit_female_gloves")))))

(fn OnRepBootsMeshPath
  (bind _bootsmeshpath (Variables|Default|GetBootsMeshPath))
  (bind _boots (Variables|Default|GetBoots))
  (if (not (Networking|IsDedicatedServer))
    (if (Utilities|Enum|NotEqual(Enum) _bootsmeshpath "")
      (bind _asvictorycore (Utilities|Casting|CastToVictoryCore (Variables|Default|GetVictoryCore)))
      (bind _returnvalue (Class|VictoryCore|BPLoadObject _asvictorycore _bootsmeshpath))
      (Utilities|IsValid _returnvalue
        (:Is%20Valid
          (bind _asskeletalmesh (Utilities|Casting|CastToSkeletalMesh _returnvalue))
          (CallFunction|SPSetEquippedMesh _boots _asskeletalmesh)))
      (else
        (CallFunction|SPSetEquippedMesh _boots "/Game/PrimalEarth/Human/Female/Outfits/Ghillie/ghilie_suit_female_boots.ghilie_suit_female_boots")))))

(fn HandleonReps
  (CallFunction|HandleAnimation)
  (CallFunction|OnRepShirtMeshPath)
  (CallFunction|OnRepPantsMeshPath)
  (CallFunction|OnRepGlovesMeshPath)
  (CallFunction|OnRepBootsMeshPath))

(fn OnRepIsRangeHidden
  (bind _rangemesh (Variables|Default|GetRangeMesh))
  (bind _israngehidden (Variables|Default|GetIsRangeHidden))
  (Development|SetHiddeninGame _rangemesh _israngehidden false)
  (Rendering|SetVisibility _rangemesh (not _israngehidden) false))

(fn IPickupGetDisablePickupAfterTime
  (return (Variables|Default|GetDisablePickupAfterTime)))

(fn IPickupGetTimetoDisablePickup
  (return (Variables|Default|GetTimeToDisablePickup)))