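; Minigun auto turret structure that delegates placement checks, target filtering, HUD and menu entries to shared SP (S+) helper functions.
; Same-team players with access get a Turret Options entry that applies a settings buff; options are exchanged through turret interface functions.
; The authority reads inventory slot count from game-mode settings, with OnRep updating the inventory limit.
; Any inventory item change triggers the shot animation and muzzle flash on player servers and clients.
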(event Custom|UpdateTurretAnimationEvent
  (bind _skeletalmesh1 (Variables|Default|GetSkeletalMesh1))
  (bind _returnvalue (Transformation|GetSocketRotation _skeletalmesh1 "MuzzleFlashSocket"))
  (Utilities|SwitchNetAuthority
    (:PlayerServer
      _)
    (:Client
      _))
  (bind _asanimbp_autoturret_minigun_c (Utilities|Casting|CastToAnimBP_AutoTurret_Minigun (Components|SkeletalMesh|GetAnimInstance (Variables|Default|GetSkeletalMesh1))))
  (Default|ShotFiredEvent _asanimbp_autoturret_minigun_c)
  (Game|SpawnActorfromClass "/Game/PrimalEarth/General/BigTurretMuzzleFlashEmitter.BigTurretMuzzleFlashEmitter_C" (Math|Transform|MakeTransform (+ (* (Math|Vector|GetForwardVector _returnvalue) (.x (Variables|Default|GetMuzzleLocOffset))) (Transformation|GetSocketLocation _skeletalmesh1 "MuzzleFlashSocket")) _returnvalue "1,1,1") true 0))

(event EventITurretSetOptions
  (params (TurretOptions :type SP%20Turret%20Options%20Structure))
  (Variables|Default|SetTurretOptions TurretOptions false))

(fn ConstructionScript
  (|CallParentFunction))

(fn BPIsAllowedtoBuild
  (params (OutPlacementData :type Placement%20Data%20Structure%20%28by%20ref%29) (CurrentAllowedReason :type Integer))
  (return (CallFunction|SPIsTurretAllowedtoBuild OutPlacementData CurrentAllowedReason)))

(fn BPGetMultiUseEntries
  (params (ForPC :type Player%20Controller%20Object%20Reference) (MultiUseEntries :type Array%20of%20Multi%20Use%20Entry%20Structures))
  (bind _asshooterplayercontroller (Utilities|Casting|CastToShooterPlayerController ForPC))
  (bind _returnvalue (Class|PrimalStructure|AllowStructureAccess _asshooterplayercontroller))
  (if (and _returnvalue (== (Variables|/Script/Engine.Actor|GetTargetingTeam _asshooterplayercontroller) (Variables|Default|GetTargetingTeam)))
    (Utilities|FlowControl|Sequence
      (:then_0
        (bind _entriesout (CallFunction|SPCleanUpTurretMenuEntries MultiUseEntries))
        (bind _entriesout_2 (CallFunction|SPAddMenuEntries _entriesout ForPC self false false false false 0.0 0.0))
        (LocalVariables|SetEntries _entriesout_2)
        (Utilities|Array|Add (LocalVariables|GetEntries) (Utilities|Struct|MakeMultiUseEntry "[Turret Options]" 9002 -1000 true (Math|Conversions|ToColor(LinearColor) (CallFunction|SPGetSpecialMenuColor)))))
      (:then_1
        (return (LocalVariables|GetEntries))))
    (else
      (return (LocalVariables|GetEntries)))))

(fn BPTryMultiUse
  (params (ForPC :type Player%20Controller%20Object%20Reference) (UseIndex :type Integer))
  (Utilities|FlowControl|Sequence
    (:then_0
      (if (== UseIndex 601)
        (Variables|Default|SetIsUnlocked (not (Variables|Default|GetbIsLocked)))
        (elif (== UseIndex 9002)
          (CallFunction|SPApplyTurretSettingsBuff ForPC self))))
    (:then_1
      (return true))))

(fn OnRepInventorySlots
  (Variables|/Script/ShooterGame.PrimalInventoryComponent|SetMaxInventoryItems (Variables|Default|GetMyInventoryComponent) (Variables|Default|GetInventorySlots)))

(fn BPTurretPreventsTargeting
  (params (PotentialTarget :type Primal%20Character%20Object%20Reference))
  (bind _preventtargeting (CallFunction|SPHandleTurretTargeting PotentialTarget (Variables|Default|GetTurretOptions)))
  (return _preventtargeting))

(fn ReceiveBeginPlay
  (|CallParentFunction)
  (if (not (Variables|Default|GetbIsPreviewStructure))
    (Networking|SwitchHasAuthority
      (:Authority
        (bind _slotcount (CallFunction|SPGetInventorySlotSetting (Game|GetGameMode) "SPlusAutoTurretSlotCount" 75))
        (Variables|Default|SetInventorySlots _slotcount true)
        (Variables|Default|SetbIsLocked (not (Variables|Default|GetIsUnlocked)) true)))))

(fn BPNotifyInventoryItemChange
  (params (bIsItemAdd :type Boolean) (theItem :type Primal%20Item%20Object%20Reference) (bEquipItem :type Boolean))
  (CallFunction|UpdateTurretAnimationEvent))

(fn BPIsAllowedtoBuildEx
  (params (OutPlacementData :type Placement%20Data%20Structure%20%28by%20ref%29) (CurrentAllowedReason :type Integer) (PC :type Player%20Controller%20Object%20Reference) (bFinalPlacement :type Boolean) (bChoosingRotation :type Boolean))
  (return (CallFunction|SPIsTurretAllowedtoBuildEx OutPlacementData CurrentAllowedReason PC self)))

(fn BlueprintDrawHUD
  (params (HUD :type Shooter%20HUD%20Object%20Reference) (CenterX :type Float%20%28single-precision%29) (CenterY :type Float%20%28single-precision%29))
  (CallFunction|SPDrawTurretHUD HUD CenterX CenterY self))

(fn ITurretGetOptions
  (bind _turretoptions (Variables|Default|GetTurretOptions))
  (bind (_mindinolevel _maxdinolevel _dinolist _isinclusionlist) (Utilities|Struct|BreakSPTurretOptions _turretoptions))
  (return (Utilities|Struct|MakeSPTurretOptions (Variables|Default|GetRangeSetting) (Variables|Default|GetAISetting) (Variables|Default|GetWarningSetting) _mindinolevel _maxdinolevel _dinolist _isinclusionlist)))