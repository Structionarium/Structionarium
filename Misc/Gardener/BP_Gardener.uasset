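; Gardener container structure for ARK Structures Plus that automatically harvests nearby same-team crop plots while activated.
; A looping server timer gathers planted plots by octree overlap and moves their items in, capacity permitting, skipping fertilizer, water, blueprints and blacklisted classes.
; Menu entries toggle range display and seed collection or destruction, and edit the blacklist via a selection buff.
; Equipped armor dresses the gardener mesh through replicated mesh paths loaded on clients.
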(event EventIPickupSetPickupSettings
  (params (DisablePickup :type Boolean) (DisablePickupWhenDamaged :type Boolean) (DisablePickupAfterTime :type Float%20%28single-precision%29) (TimeToDisablePickup :type Float%20%28double-precision%29))
  (Variables|Default|SetDisablePickup DisablePickup true)
  (Variables|Default|SetDisablePickupWhenDamaged DisablePickupWhenDamaged true)
  (Variables|Default|SetDisablePickupAfterTime DisablePickupAfterTime true)
  (Variables|Default|SetTimeToDisablePickup TimeToDisablePickup true))

(event EventBPContainerActivated
  (CallFunction|HandleAnimation)
  (Networking|SwitchHasAuthority
    (:Authority
      (CallFunction|Harvest)
      (Utilities|Time|SetTimerbyFunctionName 0 "Harvest" 1.5e+02 true))))

(event EventBPContainerDeactivated
  (CallFunction|HandleAnimation)
  (Networking|SwitchHasAuthority
    (:Authority
      (Utilities|Time|ClearTimerbyFunctionName 0 "Harvest"))))

(event EventBPPostLoadedfromSaveGame
  (Networking|SwitchHasAuthority
    (:Authority
      (Utilities|FlowControl|Delay 0.2)
      (Utilities|Time|SetTimerbyFunctionName 0 "Harvest" (Math|Random|RandomFloatinRange 1.4e+02 2e+02) true))))

(fn ConstructionScript
  (|CallParentFunction))

(fn BPIsAllowedtoBuild
  (params (OutPlacementData :type Placement%20Data%20Structure%20%28by%20ref%29) (CurrentAllowedReason :type Integer))
  (return (Math|Integer|SelectInt 1 CurrentAllowedReason (== CurrentAllowedReason -9))))

(fn BPGetMultiUseEntries
  (params (ForPC :type Player%20Controller%20Object%20Reference) (MultiUseEntries :type Array%20of%20Multi%20Use%20Entry%20Structures))
  (bind _entriesout (CallFunction|SPAddMenuEntries MultiUseEntries ForPC self (Variables|Default|GetDisablePickup) (Variables|Default|GetDisablePickupWhenDamaged) false false (Variables|Default|GetDisablePickupAfterTime) (Variables|Default|GetTimeToDisablePickup)))
  (Utilities|FlowControl|Sequence
    (:then_0
      (if (== (Variables|/Script/Engine.Actor|GetTargetingTeam ForPC) (Variables|Default|GetTargetingTeam))
        (Utilities|Array|Add _entriesout (Utilities|Struct|MakeMultiUseEntry (Utilities|String|SelectString "Show Range" "Hide Range" (Variables|Default|GetIsRangeHidden)) 9001 -1009))
        (Utilities|Array|Add _entriesout (Utilities|Struct|MakeMultiUseEntry (Utilities|String|SelectString "Destroy Seeds" "Collect Seeds" (Variables|Default|GetCollectSeeds)) 9003 -1005))
        (Utilities|Array|Add _entriesout (Utilities|Struct|MakeMultiUseEntry "Reset Armor" 9004 -1006))
        (Utilities|Array|Add _entriesout (Utilities|Struct|MakeMultiUseEntry "Add to Blacklist" 9005 -1006 true true))
        (Utilities|Array|Add _entriesout (Utilities|Struct|MakeMultiUseEntry "Remove from Blacklist" 9006 -1010 true true))))
    (:then_1
      (return _entriesout))))

(fn BPTryMultiUse
  (params (ForPC :type Player%20Controller%20Object%20Reference) (UseIndex :type Integer))
  (Utilities|FlowControl|Sequence
    (:then_0
      (if (== UseIndex 601)
        (Variables|Default|SetIsUnlocked (not (Variables|Default|GetbIsLocked)))))
    (:then_1
      (switch int UseIndex
        (:9001
          (Variables|Default|SetIsRangeHidden (not (Variables|Default|GetIsRangeHidden)) true))
        (:9003
          (Variables|Default|SetCollectSeeds (not (Variables|Default|GetCollectSeeds)) true))
        (:9004
          (Variables|Default|SetShirtMeshPath "" true)
          (Variables|Default|SetPantsMeshPath "" true)
          (Variables|Default|SetGlovesMeshPath "" true)
          (Variables|Default|SetBootsMeshPath "" true))
        (:9005
          (CallFunction|HandleAddBlacklist ForPC))
        (:9006
          (CallFunction|HandleRemoveBlacklist ForPC))))
    (:then_2
      (return true))))

(fn OnRepHarvestRange
  (bind _harvestrange (Variables|Default|GetHarvestRange))
  (Transformation|SetWorldScale3D (Variables|Default|GetRangeMesh) (Math|Vector|MakeVector _harvestrange _harvestrange _harvestrange)))

(fn Harvest
  (bind _itemclassestotake (LocalVariables|GetItemClassesToTake))
  (bind _transferqtyitemclasses (LocalVariables|GetTransferQtyItemClasses))
  (bind _capacityforitemclasses (LocalVariables|GetCapacityForItemClasses))
  (if (Variables|Default|GetbContainerActivated)
    (Class|PrimalInventoryComponent|InventoryRefresh (Variables|Default|GetMyInventoryComponent))
    (bind _cropplots (CallFunction|GetCropPlots))
    (for _array_element _cropplots
      (Utilities|FlowControl|Sequence
        (:then_0
          (if (Variables|/Script/Engine.Actor|GetbStasised _array_element)
            (Class|Actor|Unstasis _array_element)))
        (:then_1
          (Class|PrimalInventoryComponent|InventoryRefresh (Variables|/Script/ShooterGame.PrimalStructureItemContainer|GetMyInventoryComponent _array_element))
          (for _array_element_2 (Variables|/Script/ShooterGame.PrimalInventoryComponent|GetInventoryItems (Variables|/Script/ShooterGame.PrimalStructureItemContainer|GetMyInventoryComponent _array_element))
            (if (not (Math|Boolean|ORBoolean (Utilities|ClassIsChildOf (Utilities|GetClass _array_element_2) "/Game/PrimalEarth/CoreBlueprints/Items/Consumables/BaseBPs/PrimalItemConsumable_Fertilizer_Base.PrimalItemConsumable_Fertilizer_Base_C") (Utilities|ClassIsChildOf (Utilities|GetClass _array_element_2) "/Game/PrimalEarth/Test/PrimalItemConsumableEatable_WaterContainer.PrimalItemConsumableEatable_WaterContainer_C") (Variables|/Script/ShooterGame.PrimalItem|GetbIsBlueprint _array_element_2) (Utilities|Array|ContainsItem (Variables|Default|GetBlacklist) (Utilities|GetClass _array_element_2))))
              (Utilities|Array|Add (LocalVariables|GetItemsToTake) _array_element_2)
              (if (not (Utilities|Array|ContainsItem _itemclassestotake (Utilities|GetClass _array_element_2)))
                (Utilities|Array|Add _itemclassestotake (Utilities|GetClass _array_element_2))
                (bind _asprimalitem (Utilities|Casting|CastToPrimalItemClass (Utilities|GetClass _array_element_2)))
                (bind _capacity (CallFunction|SPGetStructureInventoryCapacityforItem _asprimalitem self))
                (Utilities|Array|Add (LocalVariables|GetCapacityForItemClasses) _capacity)
                (Utilities|Array|Add (LocalVariables|GetTransferQtyItemClasses) (Class|KismetSystemLibrary|MakeLiteralInteger))))))))
    (for _array_element_3 (LocalVariables|GetItemsToTake)
      (LocalVariables|SetItemClassIndex (Utilities|Array|FindItem (LocalVariables|GetItemClassesToTake) (Utilities|GetClass _array_element_3)))
      (if (>= (LocalVariables|GetItemClassIndex) 0)
        (if (> (Utilities|Array|Get(acopy) (LocalVariables|GetCapacityForItemClasses) (LocalVariables|GetItemClassIndex)) 0)
          (bind _returnvalue (Class|PrimalItem|IncrementItemQuantity _array_element_3 (* (Math|Integer|Min(Integer) (Utilities|Array|Get(acopy) (LocalVariables|GetCapacityForItemClasses) (LocalVariables|GetItemClassIndex)) (Variables|/Script/ShooterGame.PrimalItem|GetItemQuantity _array_element_3)) -1) true false false false false))
          (Utilities|Array|SetArrayElem _transferqtyitemclasses (LocalVariables|GetItemClassIndex) (+ (Utilities|Array|Get(acopy) _transferqtyitemclasses (LocalVariables|GetItemClassIndex)) (* _returnvalue -1)))
          (Utilities|Array|SetArrayElem _capacityforitemclasses (LocalVariables|GetItemClassIndex) (- (Utilities|Array|Get(acopy) _capacityforitemclasses (LocalVariables|GetItemClassIndex)) (* _returnvalue -1))))))
    (for (_array_element_4 _array_index) (LocalVariables|GetItemClassesToTake)
      (if (or (not (Utilities|ClassIsChildOf _array_element_4 "/Game/PrimalEarth/CoreBlueprints/Items/Consumables/Seeds/PrimalItemConsumableSeed.PrimalItemConsumableSeed_C")) (and (Utilities|ClassIsChildOf _array_element_4 "/Game/PrimalEarth/CoreBlueprints/Items/Consumables/Seeds/PrimalItemConsumableSeed.PrimalItemConsumableSeed_C") (Variables|Default|GetCollectSeeds)))
        (if (> (Utilities|Array|Get(acopy) (LocalVariables|GetTransferQtyItemClasses) _array_index) 0)
          (bind _asprimalitem_2 (Utilities|Casting|CastToPrimalItemClass _array_element_4))
          (Class|PrimalInventoryComponent|BPIncrementItemTemplateQuantity (Variables|Default|GetMyInventoryComponent) _asprimalitem_2 (Utilities|Array|Get(acopy) (LocalVariables|GetTransferQtyItemClasses) _array_index) true false true false false false 0 false))))
    (else
      (Utilities|Time|ClearTimerbyFunctionName 0 "Harvest"))))

(fn GetCropPlots
  (bind _returnvalue (Class|VictoryCore|ServerOctreeOverlapActorsClass (Class|Actor|GetWorld) (Transformation|GetActorLocation) (Variables|Default|GetHarvestRange) "STRUCTURES" "/Script/ShooterGame.PrimalStructureItemContainer_CropPlot" false))
  (for _array_element _returnvalue
    (bind _asprimalstructureitemcontainer_cropplot (Utilities|Casting|CastToPrimalStructureItemContainer_CropPlot _array_element))
    (bind _returnvalue_2 (Transformation|GetDistanceTo _array_element self))
    (if (Math|Boolean|ANDBoolean (<= _returnvalue_2 (Variables|Default|GetHarvestRange)) (!= (Variables|/Script/ShooterGame.PrimalStructureItemContainer_CropPlot|GetPlantedCrop _asprimalstructureitemcontainer_cropplot) 0) (== (Variables|/Script/Engine.Actor|GetTargetingTeam _array_element) (Variables|Default|GetTargetingTeam)))
      (Utilities|Array|Add (LocalVariables|GetPlotsInRange) _asprimalstructureitemcontainer_cropplot)))
  (return (LocalVariables|GetPlotsInRange)))

(fn OnRepInventorySlots
  (Variables|/Script/ShooterGame.PrimalInventoryComponent|SetMaxInventoryItems (Variables|Default|GetMyInventoryComponent) (Variables|Default|GetInventorySlots)))

(fn HandleAnimation
  (Variables|/Script/Engine.SkeletalMeshComponent|SetbPauseAnims (Variables|Default|GetPawnMesh) (not (Variables|Default|GetbContainerActivated))))

(fn ReceiveBeginPlay
  (bind _returnvalue (Game|GetGameMode))
  (|CallParentFunction)
  (if (not (Variables|Default|GetbIsPreviewStructure))
    (bind _returnvalue_2 (Class|VictoryCore|ConstructObjectAutoNameBP "/Script/ShooterGame.VictoryCore" self))
    (Variables|Default|SetVictoryCore _returnvalue_2)
    (Networking|SwitchHasAuthority
      (:Authority
        (Utilities|FlowControl|Sequence
          (:then_0
            (CallFunction|SPSetPickUpSettings _returnvalue self))
          (:then_1
            (bind _slotcount (CallFunction|SPGetInventorySlotSetting _returnvalue "GardenerSlotCount" 300))
            (Variables|Default|SetInventorySlots _slotcount true))
          (:then_2
            (bind _value (CallFunction|SPGetIntIniOption _returnvalue "GardenerRangeInFoundations" 10 50))
            (Variables|Default|SetHarvestRange (* _value 3e+02) true))
          (:then_3
            (Variables|Default|SetbIsLocked (not (Variables|Default|GetIsUnlocked)) true))
          (:then_4
            (Utilities|SwitchNetAuthority
              (:PlayerServer
                (CallFunction|HandleonReps))))))
      (:Remote
        (CallFunction|HandleonReps)))))

(fn BPNotifyInventoryItemChange
  (params (bIsItemAdd :type Boolean) (theItem :type Primal%20Item%20Object%20Reference) (bEquipItem :type Boolean))
  (bind _myequipmenttype (Variables|/Script/ShooterGame.PrimalItem|GetMyEquipmentType theItem))
  (bind _myitemskin (Variables|/Script/ShooterGame.PrimalItem|GetMyItemSkin theItem))
  (if bIsItemAdd
    (bind _asvictorycore (Utilities|Casting|CastToVictoryCore (Variables|Default|GetVictoryCore)))
    (bind _femalesk (CallFunction|SPGetSkeletalMeshesfromItem (select (Utilities|IsValid _myitemskin) _myitemskin theItem)))
    (if (Utilities|Enum|Equal(Enum) _myequipmenttype "Shirt")
      (Variables|Default|SetShirtMeshPath (Class|VictoryCore|GetClassPathName _asvictorycore _femalesk) true)
      (elif (Utilities|Enum|Equal(Enum) _myequipmenttype "Pants")
        (Variables|Default|SetPantsMeshPath (Class|VictoryCore|GetClassPathName _asvictorycore _femalesk) true)
        (elif (Utilities|Enum|Equal(Enum) _myequipmenttype "Boots")
          (Variables|Default|SetBootsMeshPath (Class|VictoryCore|GetClassPathName _asvictorycore _femalesk) true)
          (elif (Utilities|Enum|Equal(Enum) _myequipmenttype "Gloves")
            (Variables|Default|SetGlovesMeshPath (Class|VictoryCore|GetClassPathName _asvictorycore _femalesk) true)))))))

(fn OnRepShirtMeshPath
  (bind _shirtmeshpath (Variables|Default|GetShirtMeshPath))
  (bind _shirt (Variables|Default|GetShirt))
  (if (not (Networking|IsDedicatedServer))
    (if (Utilities|Enum|NotEqual(Enum) _shirtmeshpath "")
      (bind _asvictorycore (Utilities|Casting|CastToVictoryCore (Variables|Default|GetVictoryCore)))
      (bind _returnvalue (Class|VictoryCore|BPLoadObject _asvictorycore _shirtmeshpath))
      (Utilities|IsValid _returnvalue
        (:Is%20Valid
          (bind _asskeletalmesh (Utilities|Casting|CastToSkeletalMesh _returnvalue))
          (CallFunction|SPSetEquippedMesh _shirt _asskeletalmesh)))
      (else
        (CallFunction|SPSetEquippedMesh _shirt "/Game/PrimalEarth/Human/Female/Outfits/Burlap/femaleBurlap_Shirt.femaleBurlap_Shirt")))))

(fn OnRepPantsMeshPath
  (bind _pantsmeshpath (Variables|Default|GetPantsMeshPath))
  (bind _pants (Variables|Default|GetPants))
  (if (not (Networking|IsDedicatedServer))
    (if (Utilities|Enum|NotEqual(Enum) _pantsmeshpath "")
      (bind _asvictorycore (Utilities|Casting|CastToVictoryCore (Variables|Default|GetVictoryCore)))
      (bind _returnvalue (Class|VictoryCore|BPLoadObject _asvictorycore _pantsmeshpath))
      (Utilities|IsValid _returnvalue
        (:Is%20Valid
          (bind _asskeletalmesh (Utilities|Casting|CastToSkeletalMesh _returnvalue))
          (CallFunction|SPSetEquippedMesh _pants _asskeletalmesh)))
      (else
        (CallFunction|SPSetEquippedMesh _pants "/Game/PrimalEarth/Human/Female/Outfits/Burlap/femaleBurlap_Pants.femaleBurlap_Pants")))))

(fn OnRepGlovesMeshPath
  (bind _glovesmeshpath (Variables|Default|GetGlovesMeshPath))
  (bind _gloves (Variables|Default|GetGloves))
  (if (not (Networking|IsDedicatedServer))
    (if (Utilities|Enum|NotEqual(Enum) _glovesmeshpath "")
      (bind _asvictorycore (Utilities|Casting|CastToVictoryCore (Variables|Default|GetVictoryCore)))
      (bind _returnvalue (Class|VictoryCore|BPLoadObject _asvictorycore _glovesmeshpath))
      (Utilities|IsValid _returnvalue
        (:Is%20Valid
          (bind _asskeletalmesh (Utilities|Casting|CastToSkeletalMesh _returnvalue))
          (CallFunction|SPSetEquippedMesh _gloves _asskeletalmesh)))
      (else
        (CallFunction|SPSetEquippedMesh _gloves "/Game/PrimalEarth/Human/Female/Outfits/Burlap/femaleBurlap_Gloves.femaleBurlap_Gloves")))))

(fn OnRepBootsMeshPath
  (bind _bootsmeshpath (Variables|Default|GetBootsMeshPath))
  (bind _boots (Variables|Default|GetBoots))
  (if (not (Networking|IsDedicatedServer))
    (if (Utilities|Enum|NotEqual(Enum) _bootsmeshpath "")
      (bind _asvictorycore (Utilities|Casting|CastToVictoryCore (Variables|Default|GetVictoryCore)))
      (bind _returnvalue (Class|VictoryCore|BPLoadObject _asvictorycore _bootsmeshpath))
      (Utilities|IsValid _returnvalue
        (:Is%20Valid
          (bind _asskeletalmesh (Utilities|Casting|CastToSkeletalMesh _returnvalue))
          (CallFunction|SPSetEquippedMesh _boots _asskeletalmesh)))
      (else
        (CallFunction|SPSetEquippedMesh _boots "/Game/PrimalEarth/Human/Female/Outfits/Burlap/femaleBurlap_Boots.femaleBurlap_Boots")))))

(fn HandleonReps
  (CallFunction|HandleAnimation)
  (CallFunction|OnRepShirtMeshPath)
  (CallFunction|OnRepPantsMeshPath)
  (CallFunction|OnRepGlovesMeshPath)
  (CallFunction|OnRepBootsMeshPath))

(fn OnRepIsRangeHidden
  (bind _rangemesh (Variables|Default|GetRangeMesh))
  (bind _israngehidden (Variables|Default|GetIsRangeHidden))
  (Development|SetHiddeninGame _rangemesh _israngehidden false)
  (Rendering|SetVisibility _rangemesh (not _israngehidden) false))

(fn HandleAddBlacklist
  (params (PC :type Player%20Controller%20Object%20Reference))
  (for _array_element (Variables|/Script/ShooterGame.PrimalInventoryComponent|GetInventoryItems (Variables|Default|GetMyInventoryComponent))
    (if (not (Utilities|ClassIsChildOf (Utilities|GetClass _array_element) "/Game/PrimalEarth/CoreBlueprints/Items/Consumables/BaseBPs/PrimalItemConsumable_Fertilizer_Base.PrimalItemConsumable_Fertilizer_Base_C"))
      (if (not (Utilities|Array|ContainsItem (Variables|Default|GetBlacklist) (Utilities|GetClass _array_element)))
        (Utilities|SPAddifUnique (LocalVariables|GetClassesInInventory) (Utilities|GetClass _array_element)))))
  (if (> (Utilities|Array|Length (LocalVariables|GetClassesInInventory)) 0)
    (bind _asshooterplayercontroller (Utilities|Casting|CastToShooterPlayerController PC))
    (bind _returnvalue (Class|PrimalBuff|StaticAddBuff "/Game/Mods/StructuresPlusMod/_Buffs/Buff_StructuresPlus_SelectBox_Gardener.Buff_StructuresPlus_SelectBox_Gardener_C" (Class|ShooterPlayerController|GetPlayerCharacter _asshooterplayercontroller) 0 0 false))
    (bind _asbuff_structuresplus_selectbox_gardener_c (Utilities|Casting|CastToBuff_StructuresPlus_SelectBox_Gardener _returnvalue))
    (Default|InitializeGardenerSelectUI _asbuff_structuresplus_selectbox_gardener_c self (LocalVariables|GetClassesInInventory) true)
    (else
      (CallFunction|SPMessageClient PC "No items in gardener inventory." "NewEnumerator1"))))

(fn HandleRemoveBlacklist
  (params (PC :type Player%20Controller%20Object%20Reference))
  (if (> (Utilities|Array|Length (Variables|Default|GetBlacklist)) 0)
    (bind _asshooterplayercontroller (Utilities|Casting|CastToShooterPlayerController PC))
    (bind _returnvalue (Class|PrimalBuff|StaticAddBuff "/Game/Mods/StructuresPlusMod/_Buffs/Buff_StructuresPlus_SelectBox_Gardener.Buff_StructuresPlus_SelectBox_Gardener_C" (Class|ShooterPlayerController|GetPlayerCharacter _asshooterplayercontroller) 0 0 false))
    (bind _asbuff_structuresplus_selectbox_gardener_c (Utilities|Casting|CastToBuff_StructuresPlus_SelectBox_Gardener _returnvalue))
    (Default|InitializeGardenerSelectUI _asbuff_structuresplus_selectbox_gardener_c self (Variables|Default|GetBlacklist) false)
    (else
      (CallFunction|SPMessageClient PC "Blacklist is empty." "NewEnumerator1"))))

(fn IPickupGetDisablePickupAfterTime
  (return (Variables|Default|GetDisablePickupAfterTime)))

(fn IPickupGetTimetoDisablePickup
  (return (Variables|Default|GetTimeToDisablePickup)))