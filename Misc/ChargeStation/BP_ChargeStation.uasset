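; Charge station structure that drains charge from nearby lantern pets into its own store and uses it to recharge battery items in its inventory.
; While active, a randomized server timer alternates recharging and leeching, unstasising pets as needed, and switches the station off when its store fills.
; It avoids stasis while active and not full.
; It also draws stored charge on the HUD, offers a range-mesh toggle and supports configurable pickup.
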(event EventIPickupSetPickupSettings
  (params (DisablePickup :type Boolean) (DisablePickupWhenDamaged :type Boolean) (DisablePickupAfterTime :type Float%20%28single-precision%29) (TimeToDisablePickup :type Float%20%28double-precision%29))
  (Variables|Default|SetDisablePickup DisablePickup true)
  (Variables|Default|SetDisablePickupWhenDamaged DisablePickupWhenDamaged true)
  (Variables|Default|SetDisablePickupAfterTime DisablePickupAfterTime true)
  (Variables|Default|SetTimeToDisablePickup TimeToDisablePickup true))

(fn ConstructionScript)

(fn BlueprintDrawHUD
  (params (HUD :type Shooter%20HUD%20Object%20Reference) (CenterX :type Float%20%28single-precision%29) (CenterY :type Float%20%28single-precision%29))
  (bind _canvas (Variables|/Script/Engine.HUD|GetCanvas HUD))
  (Class|Canvas|SetDrawColor _canvas (Math|Conversions|ToColor(LinearColor) "(R=0.000000,G=0.825000,B=0.031290,A=1.000000)"))
  (Class|Canvas|BPDrawTextCentered _canvas (Variables|/Script/ShooterGame.ShooterHUD|GetNormalFont HUD) (Utilities|String|Append (Utilities|String|Append (Utilities|String|Append "Current Charge: " (Utilities|String|ToString(Integer) (Variables|Default|GetStoredCharge_Current))) " / ") (Utilities|String|ToString(Integer) (Variables|Default|GetStoredCharge_Max))) CenterX (+ CenterY -7e+01) 1.0 1.0 true true))

(fn BPNotifyInventoryItemChange
  (params (bIsItemAdd :type Boolean) (theItem :type Primal%20Item%20Object%20Reference) (bEquipItem :type Boolean))
  (if bIsItemAdd
    (CallFunction|ChargeBatteries)))

(fn BPGetMultiUseEntries
  (params (ForPC :type Player%20Controller%20Object%20Reference) (MultiUseEntries :type Array%20of%20Multi%20Use%20Entry%20Structures))
  (bind _entriesout (CallFunction|SPAddMenuEntries MultiUseEntries ForPC self (Variables|Default|GetDisablePickup) (Variables|Default|GetDisablePickupWhenDamaged) false false (Variables|Default|GetDisablePickupAfterTime) (Variables|Default|GetTimeToDisablePickup)))
  (Utilities|FlowControl|Sequence
    (:then_0
      (bind _returnvalue (Class|PrimalStructure|AllowStructureAccess ForPC))
      (if _returnvalue
        (Utilities|Array|Add _entriesout (Utilities|Struct|MakeMultiUseEntry (Utilities|String|SelectString "Show Range" "Hide Range" (Variables|Default|GetIsRangeMeshHidden)) 9000 -1000))))
    (:then_1
      (return _entriesout))))

(fn BPContainerActivated
  (Networking|SwitchHasAuthority
    (:Authority
      (Utilities|Time|SetTimerbyFunctionName 0 "HandleChargeStation" (Math|Random|RandomFloatinRange 45.0 6e+01) true))))

(fn BPContainerDeactivated
  (Networking|SwitchHasAuthority
    (:Authority
      (Utilities|Time|ClearTimerbyFunctionName 0 "HandleChargeStation"))))

(fn OnRepIsRangeMeshHidden
  (Rendering|SetVisibility (Variables|Default|GetRangeMesh) (not (Variables|Default|GetIsRangeMeshHidden)) false))

(fn BPTryMultiUse
  (params (ForPC :type Player%20Controller%20Object%20Reference) (UseIndex :type Integer))
  (switch int UseIndex
    (:Default
      _)
    (:9000
      (Variables|Default|SetIsRangeMeshHidden (not (Variables|Default|GetIsRangeMeshHidden)) true)))
  (return true))

(fn ReceiveBeginPlay
  (|CallParentFunction)
  (if (not (Variables|Default|GetbIsPreviewStructure))
    (Networking|SwitchHasAuthority
      (:Authority
        (CallFunction|SPSetPickUpSettings (Game|GetGameMode) self)
        (if (Variables|Default|GetbContainerActivated)
          (Utilities|Time|SetTimerbyFunctionName 0 "HandleChargeStation" (Math|Random|RandomFloatinRange 45.0 6e+01) true))))))

(fn HandleChargeStation
  (CallFunction|ChargeBatteries)
  (CallFunction|LeechChargefromPets)
  (CallFunction|ChargeBatteries)
  (if (== (Variables|Default|GetStoredCharge_Current) (Variables|Default|GetStoredCharge_Max))
    (Class|PrimalStructure|SetContainerActive false)))

(fn LeechChargefromPets
  (if (> (- (Variables|Default|GetStoredCharge_Max) (Variables|Default|GetStoredCharge_Current)) 0)
    (bind _returnvalue (Class|VictoryCore|ServerOctreeOverlapActorsClass (Class|Actor|GetWorld) (Transformation|GetActorLocation) 1.5e+03 "DINOPAWNS" "/Game/Aberration/CoreBlueprints/LanternPet_Character_BP.LanternPet_Character_BP_C" true))
    (bind _array_element (Utilities|Array|ForEachLoopwithBreak _returnvalue :!label _label)
      (:LoopBody
        (bind _aslanternpet_character_bp_c (Utilities|Casting|CastToLanternPet_Character_BP _array_element))
        (if (Variables|/Script/Engine.Actor|GetbStasised _aslanternpet_character_bp_c)
          (Class|Actor|Unstasis _aslanternpet_character_bp_c))
        (if (> (Math|Float|Floor (/ (Variables|/Game/Aberration/CoreBlueprints/LanternPet_Character_BP.LanternPet_Character_BP_C|GetcurrentChargeAmount _aslanternpet_character_bp_c) 5.0)) 0)
          (LocalVariables|SetChargeLeechAmt (Math|Conversions|ToFloat(Integer) (Math|Integer|Min(Integer) (Math|Float|Floor (/ (Variables|/Game/Aberration/CoreBlueprints/LanternPet_Character_BP.LanternPet_Character_BP_C|GetcurrentChargeAmount _aslanternpet_character_bp_c) 5.0)) (- (Variables|Default|GetStoredCharge_Max) (Variables|Default|GetStoredCharge_Current)))))
          (Variables|/Game/Aberration/CoreBlueprints/LanternPet_Character_BP.LanternPet_Character_BP_C|SetcurrentChargeAmount _aslanternpet_character_bp_c (- (Variables|/Game/Aberration/CoreBlueprints/LanternPet_Character_BP.LanternPet_Character_BP_C|GetcurrentChargeAmount _aslanternpet_character_bp_c) (* (LocalVariables|GetChargeLeechAmt) 5.0)) false)
          (Variables|Default|SetStoredCharge_Current (+ (Math|Float|Floor (LocalVariables|GetChargeLeechAmt)) (Variables|Default|GetStoredCharge_Current)) false)
          (Class|Actor|MulticastProperty _aslanternpet_character_bp_c "currentChargeAmount")
          (Variables|/Game/Aberration/CoreBlueprints/LanternPet_Character_BP.LanternPet_Character_BP_C|SetbAutoChargeActive _aslanternpet_character_bp_c false false)
          (Class|Actor|MulticastProperty "bAutoChargeActive")
          (if (<= (Variables|Default|GetStoredCharge_Current) 0)
            (goto _label Break))))
      (:Completed
        (Class|Actor|MulticastProperty "StoredCharge_Current")))))

(fn ChargeBatteries
  (if (> (Variables|Default|GetStoredCharge_Current) 0)
    (bind _array_element (Utilities|Array|ForEachLoopwithBreak (Variables|/Script/ShooterGame.PrimalInventoryComponent|GetInventoryItems (Variables|Default|GetMyInventoryComponent)) :!label _label)
      (:LoopBody
        (bind _asprimalitem_chargebattery_c (Utilities|Casting|CastToPrimalItem_ChargeBattery _array_element))
        (if (> (- (Variables|/Script/ShooterGame.PrimalItem|GetMaxDurabiltiyOverride _asprimalitem_chargebattery_c) (Variables|/Script/ShooterGame.PrimalItem|GetItemDurability _asprimalitem_chargebattery_c)) 0.0)
          (LocalVariables|SetChargeTransferAmt (Math|Float|Min(Float) (- (Variables|/Script/ShooterGame.PrimalItem|GetMaxDurabiltiyOverride _asprimalitem_chargebattery_c) (Variables|/Script/ShooterGame.PrimalItem|GetItemDurability _asprimalitem_chargebattery_c)) (Math|Conversions|ToFloat(Integer) (Variables|Default|GetStoredCharge_Current))))
          (Default|AddDurabilitySafe _asprimalitem_chargebattery_c (LocalVariables|GetChargeTransferAmt))
          (Variables|Default|SetStoredCharge_Current (- (Variables|Default|GetStoredCharge_Current) (Math|Float|Floor (LocalVariables|GetChargeTransferAmt))) false)
          (if (<= (Variables|Default|GetStoredCharge_Current) 0)
            (goto _label Break))))
      (:Completed
        (Class|Actor|MulticastProperty "StoredCharge_Current")))))

(fn BPUnstasis
  (bind _returnvalue (Class|VictoryCore|IsLoadingSaveGame))
  (if (not _returnvalue)
    (Networking|SwitchHasAuthority
      (:Authority
        (if (Variables|Default|GetbContainerActivated)
          (Utilities|Time|SetTimerbyFunctionName 0 "HandleChargeStation" (Math|Random|RandomFloatinRange 45.0 6e+01) true))))))

(fn BPPreventStasis
  (bind _returnvalue (Class|VictoryCore|IsLoadingSaveGame))
  (return (Math|Boolean|ANDBoolean (not _returnvalue) (< (Variables|Default|GetStoredCharge_Current) (Variables|Default|GetStoredCharge_Max)) (Variables|Default|GetbContainerActivated))))

(fn IPickupGetDisablePickupAfterTime
  (return (Variables|Default|GetDisablePickupAfterTime)))

(fn IPickupGetTimetoDisablePickup
  (return (Variables|Default|GetTimeToDisablePickup)))