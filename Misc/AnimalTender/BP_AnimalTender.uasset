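; Animal Tender structure that automatically gathers creature produce and feeds owl pellets to Gachas.
; While activated, a looping server timer scans same-team dinos in range, classified by name-tag substrings, pulling selected paste, polymer and oil from Achatinas and oil producers, then distributing pellets up to a chosen per-Gacha limit.
; Multi-use wheels set those choices and range display.
; Game-mode settings supply range, slot count and pickup rules.
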(event EventIPickupSetPickupSettings
  (params (DisablePickup :type Boolean) (DisablePickupWhenDamaged :type Boolean) (DisablePickupAfterTime :type Float%20%28single-precision%29) (TimeToDisablePickup :type Float%20%28double-precision%29))
  (Variables|Default|SetDisablePickup DisablePickup true)
  (Variables|Default|SetDisablePickupWhenDamaged DisablePickupWhenDamaged true)
  (Variables|Default|SetDisablePickupAfterTime DisablePickupAfterTime true)
  (Variables|Default|SetTimeToDisablePickup TimeToDisablePickup true))

(event EventBPContainerActivated
  (Networking|SwitchHasAuthority
    (:Authority
      (CallFunction|HandleCollectItems)
      (Utilities|Time|SetTimerbyFunctionName 0 "HandleCollectItems" 1.8e+02 true)
      (Variables|Default|SetDoAnimation true true))))

(event EventBPContainerDeactivated
  (Networking|SwitchHasAuthority
    (:Authority
      (Utilities|Time|ClearTimerbyFunctionName 0 "HandleCollectItems")
      (Variables|Default|SetDoAnimation false true))))

(event EventBPPostLoadedfromSaveGame
  (Networking|SwitchHasAuthority
    (:Authority
      (Utilities|FlowControl|Delay 0.2)
      (Utilities|Time|SetTimerbyFunctionName 0 "HandleCollectItems" (Math|Random|RandomFloatinRange 1.8e+02 225.0) true))))

(fn ConstructionScript
  (|CallParentFunction))

(fn BPIsAllowedtoBuild
  (params (OutPlacementData :type Placement%20Data%20Structure%20%28by%20ref%29) (CurrentAllowedReason :type Integer))
  (return (Math|Integer|SelectInt 1 CurrentAllowedReason (== CurrentAllowedReason -9))))

(fn BPGetMultiUseEntries
  (params (ForPC :type Player%20Controller%20Object%20Reference) (MultiUseEntries :type Array%20of%20Multi%20Use%20Entry%20Structures))
  (bind _color (CallFunction|SPGetSpecialMenuColor))
  (bind _returnvalue (Math|Conversions|ToColor(LinearColor) _color))
  (bind _entriesout (CallFunction|SPAddMenuEntries MultiUseEntries ForPC self (Variables|Default|GetDisablePickup) (Variables|Default|GetDisablePickupWhenDamaged) false false (Variables|Default|GetDisablePickupAfterTime) (Variables|Default|GetTimeToDisablePickup)))
  (Utilities|FlowControl|Sequence
    (:then_0
      (if (== (Variables|/Script/Engine.Actor|GetTargetingTeam ForPC) (Variables|Default|GetTargetingTeam))
        (Utilities|Array|Add _entriesout (Utilities|Struct|MakeMultiUseEntry (Utilities|String|SelectString "Show Range" "Hide Range" (Variables|Default|GetIsRangeHidden)) 9002 -1009))
        (Utilities|FlowControl|Sequence
          (:then_0
            (Utilities|Array|Add _entriesout (Utilities|Struct|MakeMultiUseEntry "[Tender Options]" 9000 -1005 true true _returnvalue))
            (CallFunction|AddWheelCategoryMultiUse _entriesout (Variables|Default|GetItemsData) (Variables|Default|GetItemsToCollect) 9900 1 "Collecting:"))
          (:then_1
            (Utilities|Array|Add _entriesout (Utilities|Struct|MakeMultiUseEntry "[Pellet Distribution]" 9001 -1005 true true _returnvalue))
            (Utilities|Array|Add _entriesout (Utilities|Struct|MakeMultiUseEntry "# to Keep on Gachas" -1 5000 true 2))
            (for (_array_element _array_index) (Variables|Default|GetPelletQtyOptions)
              (Utilities|Array|Add _entriesout (Utilities|Struct|MakeMultiUseEntry (Utilities|String|ToString(Integer) _array_element) (+ _array_index 9950) (* _array_index -1) true (== _array_index (Variables|Default|GetSelectedPelletQtyIndex)) 2 _returnvalue)))))))
    (:then_1
      (return _entriesout))))

(fn BPTryMultiUse
  (params (ForPC :type Player%20Controller%20Object%20Reference) (UseIndex :type Integer))
  (bind _returnvalue (- UseIndex 9900))
  (bind _itemstocollect (Variables|Default|GetItemsToCollect))
  (Utilities|FlowControl|Sequence
    (:then_0
      (if (== UseIndex 601)
        (Variables|Default|SetIsUnlocked (not (Variables|Default|GetbIsLocked)))
        (elif (== UseIndex 9002)
          (Variables|Default|SetIsRangeHidden (not (Variables|Default|GetIsRangeHidden)) true)
          (elif (and (>= UseIndex 9900) (< UseIndex 9910))
            (Utilities|Array|SetArrayElem _itemstocollect _returnvalue (not (Utilities|Array|Get(acopy) _itemstocollect _returnvalue)))
            (Class|Actor|MulticastProperty "ItemsToCollect")
            (elif (and (>= UseIndex 9950) (< UseIndex 9960))
              (Variables|Default|SetSelectedPelletQtyIndex (- UseIndex 9950) true))))))
    (:then_1
      (return true))))

(fn OnRepCollectionRange
  (bind _collectionrange (Variables|Default|GetCollectionRange))
  (Transformation|SetWorldScale3D (Variables|Default|GetRangeMesh) (Math|Vector|MakeVector _collectionrange _collectionrange _collectionrange)))

(fn OnRepInventorySlots
  (Variables|/Script/ShooterGame.PrimalInventoryComponent|SetMaxInventoryItems (Variables|Default|GetMyInventoryComponent) (Variables|Default|GetInventorySlots)))

(fn BPClientDoMultiUse
  (params (ForPC :type Player%20Controller%20Object%20Reference) (ClientUseIndex :type Integer))
  (switch int ClientUseIndex
    (:9000
      (bind _asshooterplayercontroller (Utilities|Casting|CastToShooterPlayerController ForPC))
      (Class|ShooterPlayerController|SetMultiUseWheelCategory _asshooterplayercontroller 1))
    (:9001
      (bind _asshooterplayercontroller_2 (Utilities|Casting|CastToShooterPlayerController ForPC))
      (Class|ShooterPlayerController|SetMultiUseWheelCategory _asshooterplayercontroller_2 2))))

(fn HandleCollectItems
  (bind _itemstocollect (Variables|Default|GetItemsToCollect))
  (if (Variables|Default|GetbContainerActivated)
    (Class|PrimalInventoryComponent|InventoryRefresh (Variables|Default|GetMyInventoryComponent))
    (bind (_snails _oildinos _gachas) (CallFunction|GetNearbyDinos))
    (for _array_element _snails
      (Class|PrimalInventoryComponent|InventoryRefresh (Variables|/Script/ShooterGame.PrimalCharacter|GetMyInventoryComponent _array_element))
      (Class|PrimalInventoryComponent|BPInventoryRefresh (Variables|/Script/ShooterGame.PrimalCharacter|GetMyInventoryComponent _array_element))
      (Utilities|FlowControl|Sequence
        (:then_0
          (if (Utilities|Array|Get(acopy) _itemstocollect)
            (CallFunction|CollectItem (Variables|/Script/ShooterGame.PrimalCharacter|GetMyInventoryComponent _array_element) "/Game/PrimalEarth/CoreBlueprints/Resources/PrimalItemResource_Polymer_Organic.PrimalItemResource_Polymer_Organic_C")))
        (:then_1
          (if (Utilities|Array|Get(acopy) _itemstocollect 1)
            (CallFunction|CollectItem (Variables|/Script/ShooterGame.PrimalCharacter|GetMyInventoryComponent _array_element) "/Game/PrimalEarth/Dinos/Achatina/PrimalItemResource_SnailPaste.PrimalItemResource_SnailPaste_C")))))
    (for _array_element_2 _oildinos
      (Class|PrimalInventoryComponent|InventoryRefresh (Variables|/Script/ShooterGame.PrimalCharacter|GetMyInventoryComponent _array_element_2))
      (Class|PrimalInventoryComponent|BPInventoryRefresh (Variables|/Script/ShooterGame.PrimalCharacter|GetMyInventoryComponent _array_element_2))
      (if (Utilities|Array|Get(acopy) _itemstocollect 2)
        (CallFunction|CollectItem (Variables|/Script/ShooterGame.PrimalCharacter|GetMyInventoryComponent _array_element_2) "/Game/PrimalEarth/CoreBlueprints/Resources/PrimalItemResource_Oil.PrimalItemResource_Oil_C")))
    (if (> (Variables|Default|GetSelectedPelletQtyIndex) 0)
      (CallFunction|DistributePellets _gachas))
    (else
      (Utilities|Time|ClearTimerbyFunctionName 0 "HandleCollectItems"))))

(fn GetNearbyDinos
  (bind _returnvalue (Class|VictoryCore|ServerOctreeOverlapActorsClass (Class|Actor|GetWorld) (Transformation|GetActorLocation) (Variables|Default|GetCollectionRange) "DINOPAWNS" "/Script/ShooterGame.PrimalDinoCharacter" true))
  (for _array_element _returnvalue
    (if (== (Variables|/Script/Engine.Actor|GetTargetingTeam _array_element) (Variables|Default|GetTargetingTeam))
      (bind _asprimaldinocharacter (Utilities|Casting|CastToPrimalDinoCharacter _array_element))
      (switch int (CallFunction|GetDinoType _asprimaldinocharacter)
        (:1
          (Utilities|Array|Add (LocalVariables|GetSnalList) _asprimaldinocharacter))
        (:2
          (Utilities|Array|Add (LocalVariables|GetOilDinoList) _asprimaldinocharacter))
        (:3
          (Utilities|Array|Add (LocalVariables|GetGachaList) _asprimaldinocharacter)))))
  (return (LocalVariables|GetSnalList) (LocalVariables|GetOilDinoList) (LocalVariables|GetGachaList)))

(fn ReceiveBeginPlay
  (bind _returnvalue (Game|GetGameMode))
  (|CallParentFunction)
  (if (not (Variables|Default|GetbIsPreviewStructure))
    (Networking|SwitchHasAuthority
      (:Authority
        (Utilities|FlowControl|Sequence
          (:then_0
            (CallFunction|SPSetPickUpSettings _returnvalue self))
          (:then_1
            (bind _slotcount (CallFunction|SPGetInventorySlotSetting _returnvalue "AnimalTenderSlotCount" 300))
            (Variables|Default|SetInventorySlots _slotcount true))
          (:then_2
            (bind _value (CallFunction|SPGetIntIniOption _returnvalue "AnimalTenderRangeInFoundations" 50 100))
            (Variables|Default|SetCollectionRange (* _value 3e+02) true))
          (:then_3
            (Variables|Default|SetbIsLocked (not (Variables|Default|GetIsUnlocked)) true))
          (:then_4
            (Utilities|SwitchNetAuthority
              (:PlayerServer
                (CallFunction|OnRepDoAnimation)))))))))

(fn GetDinoType
  (params (Dino :type Primal%20Dino%20Character%20Object%20Reference))
  (bind _dinonametag (Variables|/Script/ShooterGame.PrimalDinoCharacter|GetDinoNameTag Dino))
  (bind _customtag (Variables|/Script/Engine.Actor|GetCustomTag Dino))
  (bind _returnvalue (Utilities|String|ToString(Name) _dinonametag))
  (bind _returnvalue_2 (Utilities|String|ToString(Name) _customtag))
  (return (Math|Integer|SelectInt 3 (Math|Integer|SelectInt 2 (Math|Integer|SelectInt 1 0 (or (>= (Utilities|String|FindSubstring _returnvalue "Achatina") 0) (>= (Utilities|String|FindSubstring _returnvalue_2 "Achatina") 0))) (Math|Boolean|ORBoolean (>= (Utilities|String|FindSubstring _returnvalue "Beetle") 0) (>= (Utilities|String|FindSubstring _returnvalue_2 "Beetle") 0) (>= (Utilities|String|FindSubstring _returnvalue "Tusoteuthis") 0) (>= (Utilities|String|FindSubstring _returnvalue_2 "Tusoteuthis") 0) (>= (Utilities|String|FindSubstring _returnvalue "Basilosaurus") 0) (>= (Utilities|String|FindSubstring _returnvalue_2 "Basilosaurus") 0))) (or (>= (Utilities|String|FindSubstring _returnvalue "Gacha") 0) (>= (Utilities|String|FindSubstring _returnvalue_2 "Gacha") 0)))))

(fn CollectItem
  (params (SourceInventory :type Primal%20Inventory%20Component%20Object%20Reference) (TargetItemClass :type Primal%20Item%20Class%20Reference))
  (bind _capacity (CallFunction|SPGetStructureInventoryCapacityforItem TargetItemClass self))
  (if (> _capacity 0)
    (bind _returnvalue (Class|PrimalInventoryComponent|GetItemTemplateQuantity SourceInventory TargetItemClass 0 true false false))
    (if (> _returnvalue 0)
      (bind _returnvalue_2 (Class|PrimalInventoryComponent|BPGetItemOfTemplate SourceInventory TargetItemClass true false false false false false false false false false))
      (bind _asprimalitem (Utilities|Casting|CastToPrimalItemClass (Utilities|GetClass _returnvalue_2)))
      (bind _actuallyremoved (CallFunction|SPSafeRemovefromInventory _asprimalitem SourceInventory (Math|Integer|Min(Integer) _returnvalue _capacity) true true))
      (Class|PrimalInventoryComponent|BPIncrementItemTemplateQuantity (Variables|Default|GetMyInventoryComponent) _asprimalitem _actuallyremoved true false true false false false 0 false))))

(fn OnRepDoAnimation
  (Variables|/Script/Engine.SkeletalMeshComponent|SetGlobalAnimRateScale (Variables|Default|GetSkeletalMesh1) (Math|Float|SelectFloat 1.0 0.0 (Variables|Default|GetDoAnimation))))

(fn OnRepIsRangeHidden
  (bind _rangemesh (Variables|Default|GetRangeMesh))
  (bind _israngehidden (Variables|Default|GetIsRangeHidden))
  (Development|SetHiddeninGame _rangemesh _israngehidden false)
  (Rendering|SetVisibility _rangemesh (not _israngehidden) false))

(fn BPOverrideAllowStructureAccess
  (params (ForPC :type Shooter%20Player%20Controller%20Object%20Reference) (bIsAccessAllowed :type Boolean))
  (return (> (Variables|Default|GetSelectedPelletQtyIndex) 0)))

(fn AddWheelCategoryMultiUse
  (params (Entries :type Array%20of%20Multi%20Use%20Entry%20Structures) (OptionsData :type Array%20of%20SP%20Alphabetization%20Object%20Structures) (OptionsUsed :type Array%20of%20Booleans) (UseIndexStart :type Integer) (WheelCategory :type Integer) (Header :type String))
  (for (_array_element _array_index) OptionsData
    (Utilities|Array|Add Entries (Utilities|Struct|MakeMultiUseEntry (Utilities|String|Append (Utilities|String|SelectString "Stop " "Start " (Utilities|Array|Get(acopy) OptionsUsed _array_index)) (Utilities|Struct|BreakSP_AlphabetizationObject _array_element)) (+ _array_index UseIndexStart) (* _array_index -1) true true WheelCategory (select (Utilities|Array|Get(acopy) OptionsUsed _array_index) (Math|Color|MakeColor 200 200 255 255) (Math|Color|MakeColor 200 255 200 255)))))
  (for (_array_element_2 _array_index_2) OptionsUsed
    (if _array_element_2
      (LocalVariables|SetCollectionString (Utilities|String|Append (Utilities|String|Append (LocalVariables|GetCollectionString) (Utilities|Struct|BreakSP_AlphabetizationObject (Utilities|Array|Get(acopy) OptionsData _array_index_2))) ", "))))
  (Utilities|Array|Add Entries (Utilities|Struct|MakeMultiUseEntry (Utilities|String|Append (Utilities|String|Append Header "           ") (Utilities|String|SelectString "Nothing" (Utilities|String|GetSubstring (LocalVariables|GetCollectionString) 0 (- (Utilities|String|Len (LocalVariables|GetCollectionString)) 2)) (== (Utilities|String|Len (LocalVariables|GetCollectionString)) 0))) -1 500 true true WheelCategory (Math|Color|MakeColor 255 255 255 255))))

(fn DistributePellets
  (params (Gachas :type Array%20of%20Primal%20Dino%20Character%20Object%20References))
  (for _array_element (Variables|/Script/ShooterGame.PrimalInventoryComponent|GetInventoryItems (Variables|Default|GetMyInventoryComponent))
    (if (Utilities|ClassIsChildOf (Utilities|GetClass _array_element) "/Game/Extinction/Dinos/Owl/Pellet/PrimalItemConsumable_OwlPellet.PrimalItemConsumable_OwlPellet_C")
      (Utilities|Array|Add (LocalVariables|GetItemsToDistribute_DP) _array_element)))
  (if (> (Utilities|Array|Length (LocalVariables|GetItemsToDistribute_DP)) 0)
    (for _array_element_2 Gachas
      (Utilities|Array|Add (LocalVariables|GetInventoriesToDeposit_DP) (Variables|/Script/ShooterGame.PrimalCharacter|GetMyInventoryComponent _array_element_2)))
    (CallFunction|SPDistributeSingleItemClass (Variables|Default|GetMyInventoryComponent) (LocalVariables|GetItemsToDistribute_DP) (LocalVariables|GetInventoriesToDeposit_DP) (Utilities|Array|Get(acopy) (Variables|Default|GetPelletQtyOptions) (Variables|Default|GetSelectedPelletQtyIndex)) true)))

(fn IPickupGetDisablePickupAfterTime
  (return (Variables|Default|GetDisablePickupAfterTime)))

(fn IPickupGetTimetoDisablePickup
  (return (Variables|Default|GetTimeToDisablePickup)))