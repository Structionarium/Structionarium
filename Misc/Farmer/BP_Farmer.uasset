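; Farmer structure that, while activated, moves fertilizer from nearby same-team compost bins, tagged containers and dung beetles to crop plots in range.
; The server runs Farm on a looping timer, collecting into its own inventory and then topping up the least-fertilized plots first.
; Menu entries toggle range display, collection and distribution.
; Added armor items set replicated mesh path strings that clients load to dress the farmer, with burlap and leather defaults.
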(event EventIPickupSetPickupSettings
  (params (DisablePickup :type Boolean) (DisablePickupWhenDamaged :type Boolean) (DisablePickupAfterTime :type Float%20%28single-precision%29) (TimeToDisablePickup :type Float%20%28double-precision%29))
  (Variables|Default|SetDisablePickup DisablePickup true)
  (Variables|Default|SetDisablePickupWhenDamaged DisablePickupWhenDamaged true)
  (Variables|Default|SetDisablePickupAfterTime DisablePickupAfterTime true)
  (Variables|Default|SetTimeToDisablePickup TimeToDisablePickup true))

(event EventBPContainerActivated
  (CallFunction|HandleAnimation)
  (Networking|SwitchHasAuthority
    (:Authority
      (CallFunction|Farm)
      (Utilities|Time|SetTimerbyFunctionName 0 "Farm" 3e+02 true))))

(event EventBPContainerDeactivated
  (CallFunction|HandleAnimation)
  (Networking|SwitchHasAuthority
    (:Authority
      (Utilities|Time|ClearTimerbyFunctionName 0 "Farm"))))

(event EventBPPostLoadedfromSaveGame
  (Networking|SwitchHasAuthority
    (:Authority
      (Utilities|FlowControl|Delay 0.2)
      (Utilities|Time|SetTimerbyFunctionName 0 "Farm" (Math|Random|RandomFloatinRange 2.8e+02 3e+02) true))))

(fn ConstructionScript
  (|CallParentFunction))

(fn BPIsAllowedtoBuild
  (params (OutPlacementData :type Placement%20Data%20Structure%20%28by%20ref%29) (CurrentAllowedReason :type Integer))
  (return (Math|Integer|SelectInt 1 CurrentAllowedReason (== CurrentAllowedReason -9))))

(fn BPGetMultiUseEntries
  (params (ForPC :type Player%20Controller%20Object%20Reference) (MultiUseEntries :type Array%20of%20Multi%20Use%20Entry%20Structures))
  (bind _entriesout (CallFunction|SPAddMenuEntries MultiUseEntries ForPC self (Variables|Default|GetDisablePickup) (Variables|Default|GetDisablePickupWhenDamaged) false false (Variables|Default|GetDisablePickupAfterTime) (Variables|Default|GetTimeToDisablePickup)))
  (if (== (Variables|/Script/Engine.Actor|GetTargetingTeam ForPC) (Variables|Default|GetTargetingTeam))
    (Utilities|Array|Add _entriesout (Utilities|Struct|MakeMultiUseEntry (Utilities|String|SelectString "Show Range" "Hide Range" (Variables|Default|GetIsRangeHidden)) 9001 -1009))
    (Utilities|Array|Add _entriesout (Utilities|Struct|MakeMultiUseEntry (Utilities|String|SelectString "Enable Fertilizer Collection" "Disable Fertilizer Collection" (Variables|Default|GetDisableCollection)) 9003 -1005))
    (Utilities|Array|Add _entriesout (Utilities|Struct|MakeMultiUseEntry (Utilities|String|SelectString "Enable Fertilizer Distribution" "Disable Fertilizer Distribution" (Variables|Default|GetDisableDistribution)) 9004 -1006))
    (Utilities|Array|Add _entriesout (Utilities|Struct|MakeMultiUseEntry "Reset Armor" 9005 -1006 true true)))
  (return _entriesout))

(fn BPTryMultiUse
  (params (ForPC :type Player%20Controller%20Object%20Reference) (UseIndex :type Integer))
  (Utilities|FlowControl|Sequence
    (:then_0
      (if (== UseIndex 601)
        (Variables|Default|SetIsUnlocked (not (Variables|Default|GetbIsLocked)))))
    (:then_1
      (switch int UseIndex
        (:Default
          _)
        (:9001
          (Variables|Default|SetIsRangeHidden (not (Variables|Default|GetIsRangeHidden)) true))
        (:9002
          _)
        (:9003
          (Variables|Default|SetDisableCollection (not (Variables|Default|GetDisableCollection)) true))
        (:9004
          (Variables|Default|SetDisableDistribution (not (Variables|Default|GetDisableDistribution)) true))
        (:9005
          (Variables|Default|SetShirtMeshPath "" true)
          (Variables|Default|SetPantsMeshPath "" true)
          (Variables|Default|SetGlovesMeshPath "" true)
          (Variables|Default|SetBootsMeshPath "" true)))
      (return true))))

(fn OnRepHarvestRange
  (bind _harvestrange (Variables|Default|GetHarvestRange))
  (Transformation|SetWorldScale3D (Variables|Default|GetRangeMesh) (Math|Vector|MakeVector _harvestrange _harvestrange _harvestrange)))

(fn GetCropPlots
  (LocalVariables|SetLowestFertQty 99999)
  (bind _returnvalue (Class|VictoryCore|ServerOctreeOverlapActorsClass (Class|Actor|GetWorld) (Transformation|GetActorLocation) (Variables|Default|GetHarvestRange) "STRUCTURES" "/Script/ShooterGame.PrimalStructureItemContainer_CropPlot" false))
  (for _array_element _returnvalue
    (bind _asprimalstructureitemcontainer_cropplot (Utilities|Casting|CastToPrimalStructureItemContainer_CropPlot _array_element))
    (bind _returnvalue_2 (Transformation|GetDistanceTo _array_element self))
    (if (Math|Boolean|ANDBoolean (<= _returnvalue_2 (Variables|Default|GetHarvestRange)) (Variables|/Script/ShooterGame.PrimalStructureItemContainer_CropPlot|GetbUsesCrop _asprimalstructureitemcontainer_cropplot) (== (Variables|/Script/Engine.Actor|GetTargetingTeam _array_element) (Variables|Default|GetTargetingTeam)) (!= (Variables|/Script/ShooterGame.PrimalStructureItemContainer_CropPlot|GetSeedBaseItemTemplate _asprimalstructureitemcontainer_cropplot) 0))
      (Class|Actor|Unstasis _asprimalstructureitemcontainer_cropplot)
      (bind _isnotfull (CallFunction|SPDoesInventoryHaveEmptySlots (Variables|/Script/ShooterGame.PrimalStructureItemContainer|GetMyInventoryComponent _asprimalstructureitemcontainer_cropplot)))
      (if _isnotfull
        (bind _returnvalue_3 (Class|PrimalInventoryComponent|GetItemTemplateQuantity (Variables|/Script/ShooterGame.PrimalStructureItemContainer|GetMyInventoryComponent _asprimalstructureitemcontainer_cropplot) "/Game/PrimalEarth/CoreBlueprints/Items/Consumables/BaseBPs/PrimalItemConsumable_Fertilizer_Base.PrimalItemConsumable_Fertilizer_Base_C" 0 true false false))
        (LocalVariables|SetFertQty _returnvalue_3)
        (Utilities|Array|Add (LocalVariables|GetCrops) (Utilities|Struct|MakeSPCropPlotFertilizer _asprimalstructureitemcontainer_cropplot (LocalVariables|GetFertQty)))
        (if (< (LocalVariables|GetFertQty) (LocalVariables|GetLowestFertQty))
          (LocalVariables|SetLowestFertQty (LocalVariables|GetFertQty))))))
  (return (LocalVariables|GetCrops) (LocalVariables|GetLowestFertQty)))

(fn OnRepInventorySlots
  (Variables|/Script/ShooterGame.PrimalInventoryComponent|SetMaxInventoryItems (Variables|Default|GetMyInventoryComponent) (Variables|Default|GetInventorySlots)))

(fn CollectFertilizer
  (bind _itemstoremove (LocalVariables|GetItemsToRemove))
  (Utilities|FlowControl|Sequence
    (:then_0
      (bind _inventories (CallFunction|GetCompostBins))
      (LocalVariables|SetCollectInventories _inventories))
    (:then_1
      (bind _inventories_2 (CallFunction|GetDungBeetles))
      (Utilities|Array|AppendArray (LocalVariables|GetCollectInventories) _inventories_2))
    (:then_2
      (bind _array_element (Utilities|Array|ForEachLoopwithBreak (LocalVariables|GetCollectInventories) :!label _label)
        (:LoopBody
          (if (LocalVariables|GetIsFull)
            (goto _label Break)
            (else
              (Class|Actor|Unstasis (Components|GetOwner _array_element))
              (bind _array_element_2 (Utilities|Array|ForEachLoopwithBreak (Variables|/Script/ShooterGame.PrimalInventoryComponent|GetInventoryItems _array_element) :!label _label_2)
                (:LoopBody
                  (if (Math|Boolean|ANDBoolean (not (Variables|/Script/ShooterGame.PrimalItem|GetbIsBlueprint _array_element_2)) (Utilities|ClassIsChildOf (Utilities|GetClass _array_element_2) "/Game/PrimalEarth/CoreBlueprints/Items/Consumables/BaseBPs/PrimalItemConsumable_Fertilizer_Base.PrimalItemConsumable_Fertilizer_Base_C") (not (Utilities|ClassIsChildOf (Utilities|GetClass _array_element_2) "/Game/PrimalEarth/CoreBlueprints/Items/Consumables/BaseBPs/PrimalItemConsumablePoop.PrimalItemConsumablePoop_C")))
                    (bind _isnotfull (CallFunction|SPDoesInventoryHaveEmptySlots (Variables|Default|GetMyInventoryComponent)))
                    (if (not _isnotfull)
                      (LocalVariables|SetIsFull false)
                      (goto _label_2 Break)
                      (else
                        (Class|PrimalInventoryComponent|AddItemObject (Variables|Default|GetMyInventoryComponent) _array_element_2)
                        (Utilities|Array|Add (LocalVariables|GetItemsToRemove) _array_element_2)))))
                (:Completed
                  (for _array_element_3 _itemstoremove
                    (Class|PrimalInventoryComponent|RemoveItem _array_element (Variables|/Script/ShooterGame.PrimalItem|GetItemID _array_element_3) false false true false))
                  (Utilities|Array|Clear _itemstoremove))))))))))

(fn DistributeFertilizer
  (bind _fertilizers (LocalVariables|GetFertilizers))
  (bind _item (Utilities|Array|Get(acopy) _fertilizers))
  (for _array_element (Variables|/Script/ShooterGame.PrimalInventoryComponent|GetInventoryItems (Variables|Default|GetMyInventoryComponent))
    (if (Math|Boolean|ANDBoolean (not (Variables|/Script/ShooterGame.PrimalItem|GetbIsBlueprint _array_element)) (Utilities|ClassIsChildOf (Utilities|GetClass _array_element) "/Game/PrimalEarth/CoreBlueprints/Items/Consumables/BaseBPs/PrimalItemConsumable_Fertilizer_Base.PrimalItemConsumable_Fertilizer_Base_C") (not (Utilities|ClassIsChildOf (Utilities|GetClass _array_element) "/Game/PrimalEarth/CoreBlueprints/Items/Consumables/BaseBPs/PrimalItemConsumablePoop.PrimalItemConsumablePoop_C")))
      (Utilities|Array|Add (LocalVariables|GetFertilizers) _array_element)))
  (bind (_cropplots _lowestqty) (CallFunction|GetCropPlots))
  (LocalVariables|SetCropsInRange _cropplots)
  (LocalVariables|SetLowFertQty _lowestqty)
  (while (Math|Boolean|ANDBoolean (> (Utilities|Array|Length (LocalVariables|GetFertilizers)) 0) (not (LocalVariables|GetStopLoop)) (< (LocalVariables|GetIteration) 1000))
    (LocalVariables|SetIteration (+ (LocalVariables|GetIteration) 1))
    (bind (_array_element_2 _array_index) (Utilities|Array|ForEachLoopwithBreak (LocalVariables|GetCropsInRange) :!label _label)
      (:LoopBody
        (bind _isnotfull (CallFunction|SPDoesInventoryHaveEmptySlots (Variables|/Script/ShooterGame.PrimalStructureItemContainer|GetMyInventoryComponent (.CropPlot (Utilities|Struct|BreakSPCropPlotFertilizer _array_element_2)))))
        (if _isnotfull
          (LocalVariables|SetFoundNotFullCropPlot true)
          (if (== (.FertilizerQty (Utilities|Struct|BreakSPCropPlotFertilizer _array_element_2)) (LocalVariables|GetLowFertQty))
            (if (== (Utilities|Array|Length (LocalVariables|GetFertilizers)) 0)
              (goto _label Break)
              (else
                (bind _returnvalue (Class|PrimalInventoryComponent|AddItemObject (Variables|/Script/ShooterGame.PrimalStructureItemContainer|GetMyInventoryComponent (.CropPlot (Utilities|Struct|BreakSPCropPlotFertilizer _array_element_2))) _item))
                (Class|PrimalInventoryComponent|RemoveItem (Variables|Default|GetMyInventoryComponent) (Variables|/Script/ShooterGame.PrimalItem|GetItemID _item) false false true false)
                (Utilities|Array|RemoveIndex _fertilizers)
                (Utilities|Array|SetArrayElem (LocalVariables|GetCropsInRange) _array_index (Utilities|Struct|MakeSPCropPlotFertilizer (.CropPlot (Utilities|Struct|BreakSPCropPlotFertilizer _array_element_2)) (+ (.FertilizerQty (Utilities|Struct|BreakSPCropPlotFertilizer _array_element_2)) (Variables|/Script/ShooterGame.PrimalItem|GetItemQuantity _returnvalue)))))))))
      (:Completed
        (LocalVariables|SetLowFertQty (+ (LocalVariables|GetLowFertQty) 1))
        (if (LocalVariables|GetFoundNotFullCropPlot)
          (LocalVariables|SetFoundNotFullCropPlot false)
          (else
            (LocalVariables|SetStopLoop true)))))))

(fn Farm
  (if (Variables|Default|GetbContainerActivated)
    (Class|PrimalInventoryComponent|InventoryRefresh (Variables|Default|GetMyInventoryComponent))
    (Utilities|FlowControl|Sequence
      (:then_0
        (if (not (Variables|Default|GetDisableCollection))
          (CallFunction|CollectFertilizer)))
      (:then_1
        (if (not (Variables|Default|GetDisableDistribution))
          (CallFunction|DistributeFertilizer))))
    (else
      (Utilities|Time|ClearTimerbyFunctionName 0 "Farm"))))

(fn GetCompostBins
  (bind _returnvalue (Class|VictoryCore|ServerOctreeOverlapActorsClass (Class|Actor|GetWorld) (Transformation|GetActorLocation) (Variables|Default|GetHarvestRange) "STRUCTURES" "/Script/ShooterGame.PrimalStructureItemContainer" false))
  (for _array_element _returnvalue
    (bind _returnvalue_2 (Transformation|GetDistanceTo _array_element self))
    (if (and (<= _returnvalue_2 (Variables|Default|GetHarvestRange)) (== (Variables|/Script/Engine.Actor|GetTargetingTeam _array_element) (Variables|Default|GetTargetingTeam)))
      (bind _asprimalstructureitemcontainer (Utilities|Casting|CastToPrimalStructureItemContainer _array_element))
      (if (or (CallFunction|SPStructureHasTag _asprimalstructureitemcontainer "SPlusCollect") (Utilities|ClassIsChildOf (Utilities|GetClass _array_element) "/Game/PrimalEarth/Structures/CompostBin.CompostBin_C"))
        (Utilities|Array|Add (LocalVariables|GetCompostInventories) (Variables|/Script/ShooterGame.PrimalStructureItemContainer|GetMyInventoryComponent _asprimalstructureitemcontainer)))))
  (return (LocalVariables|GetCompostInventories)))

(fn GetDungBeetles
  (bind _returnvalue (Class|VictoryCore|ServerOctreeOverlapActorsClass (Class|Actor|GetWorld) (Transformation|GetActorLocation) (Variables|Default|GetHarvestRange) "DINOPAWNS" "/Script/ShooterGame.PrimalDinoCharacter" false))
  (for _array_element _returnvalue
    (bind _returnvalue_2 (Transformation|GetDistanceTo _array_element self))
    (if (and (<= _returnvalue_2 (Variables|Default|GetHarvestRange)) (== (Variables|/Script/Engine.Actor|GetTargetingTeam _array_element) (Variables|Default|GetTargetingTeam)))
      (bind _asprimaldinocharacter (Utilities|Casting|CastToPrimalDinoCharacter _array_element))
      (if (Math|Boolean|ORBoolean (Utilities|ClassIsChildOf (Utilities|GetClass _array_element) "/Game/PrimalEarth/Dinos/DungBeetle/DungBeetle_Character_BP.DungBeetle_Character_BP_C") (>= (Utilities|String|FindSubstring (Utilities|String|ToString(Name) (Variables|/Script/ShooterGame.PrimalDinoCharacter|GetDinoNameTag _asprimaldinocharacter)) "Beetle") 0) (>= (Utilities|String|FindSubstring (Utilities|String|ToString(Name) (Variables|/Script/Engine.Actor|GetCustomTag _asprimaldinocharacter)) "Beetle") 0))
        (Utilities|Array|Add (LocalVariables|GetBeetleInventories) (Variables|/Script/ShooterGame.PrimalCharacter|GetMyInventoryComponent _asprimaldinocharacter)))))
  (return (LocalVariables|GetBeetleInventories)))

(fn HandleAnimation
  (Variables|/Script/Engine.SkeletalMeshComponent|SetbPauseAnims (Variables|Default|GetPawnMesh) (not (Variables|Default|GetbContainerActivated))))

(fn ReceiveBeginPlay
  (bind _returnvalue (Game|GetGameMode))
  (|CallParentFunction)
  (if (not (Variables|Default|GetbIsPreviewStructure))
    (bind _returnvalue_2 (Class|VictoryCore|ConstructObjectAutoNameBP "/Script/ShooterGame.VictoryCore" self))
    (Variables|Default|SetVictoryCore _returnvalue_2)
    (Networking|SwitchHasAuthority
      (:Authority
        (Utilities|FlowControl|Sequence
          (:then_0
            (CallFunction|SPSetPickUpSettings _returnvalue self))
          (:then_1
            (bind _slotcount (CallFunction|SPGetInventorySlotSetting _returnvalue "FarmerSlotCount" 300))
            (Variables|Default|SetInventorySlots _slotcount true))
          (:then_2
            (bind _value (CallFunction|SPGetIntIniOption _returnvalue "FarmerRangeInFoundations" 30 100))
            (Variables|Default|SetHarvestRange (* _value 3e+02) true))
          (:then_3
            (Variables|Default|SetbIsLocked (not (Variables|Default|GetIsUnlocked)) true))
          (:then_4
            (Utilities|SwitchNetAuthority
              (:PlayerServer
                (CallFunction|HandleonReps))))))
      (:Remote
        (CallFunction|HandleonReps)))))

(fn BPNotifyInventoryItemChange
  (params (bIsItemAdd :type Boolean) (theItem :type Primal%20Item%20Object%20Reference) (bEquipItem :type Boolean))
  (bind _myequipmenttype (Variables|/Script/ShooterGame.PrimalItem|GetMyEquipmentType theItem))
  (bind _myitemskin (Variables|/Script/ShooterGame.PrimalItem|GetMyItemSkin theItem))
  (if bIsItemAdd
    (bind _asvictorycore (Utilities|Casting|CastToVictoryCore (Variables|Default|GetVictoryCore)))
    (bind _malesk (CallFunction|SPGetSkeletalMeshesfromItem (select (Utilities|IsValid _myitemskin) _myitemskin theItem)))
    (if (Utilities|Enum|Equal(Enum) _myequipmenttype "Shirt")
      (Variables|Default|SetShirtMeshPath (Class|VictoryCore|GetClassPathName _asvictorycore _malesk) true)
      (elif (Utilities|Enum|Equal(Enum) _myequipmenttype "Pants")
        (Variables|Default|SetPantsMeshPath (Class|VictoryCore|GetClassPathName _asvictorycore _malesk) true)
        (elif (Utilities|Enum|Equal(Enum) _myequipmenttype "Boots")
          (Variables|Default|SetBootsMeshPath (Class|VictoryCore|GetClassPathName _asvictorycore _malesk) true)
          (elif (Utilities|Enum|Equal(Enum) _myequipmenttype "Gloves")
            (Variables|Default|SetGlovesMeshPath (Class|VictoryCore|GetClassPathName _asvictorycore _malesk) true)))))))

(fn OnRepShirtMeshPath
  (bind _shirtmeshpath (Variables|Default|GetShirtMeshPath))
  (bind _shirt (Variables|Default|GetShirt))
  (if (not (Networking|IsDedicatedServer))
    (if (Utilities|Enum|NotEqual(Enum) _shirtmeshpath "")
      (bind _asvictorycore (Utilities|Casting|CastToVictoryCore (Variables|Default|GetVictoryCore)))
      (bind _returnvalue (Class|VictoryCore|BPLoadObject _asvictorycore _shirtmeshpath))
      (Utilities|IsValid _returnvalue
        (:Is%20Valid
          (bind _asskeletalmesh (Utilities|Casting|CastToSkeletalMesh _returnvalue))
          (CallFunction|SPSetEquippedMesh _shirt _asskeletalmesh)))
      (else
        (CallFunction|SPSetEquippedMesh _shirt "/Game/PrimalEarth/Human/Male/Outfits/Burlap/male_Burlap_Shirt.male_Burlap_Shirt")))))

(fn OnRepPantsMeshPath
  (bind _pantsmeshpath (Variables|Default|GetPantsMeshPath))
  (bind _pants (Variables|Default|GetPants))
  (if (not (Networking|IsDedicatedServer))
    (if (Utilities|Enum|NotEqual(Enum) _pantsmeshpath "")
      (bind _asvictorycore (Utilities|Casting|CastToVictoryCore (Variables|Default|GetVictoryCore)))
      (bind _returnvalue (Class|VictoryCore|BPLoadObject _asvictorycore _pantsmeshpath))
      (Utilities|IsValid _returnvalue
        (:Is%20Valid
          (bind _asskeletalmesh (Utilities|Casting|CastToSkeletalMesh _returnvalue))
          (CallFunction|SPSetEquippedMesh _pants _asskeletalmesh)))
      (else
        (CallFunction|SPSetEquippedMesh _pants "/Game/PrimalEarth/Human/Male/Outfits/Burlap/male_Burlap_Pants.male_Burlap_Pants")))))

(fn OnRepGlovesMeshPath
  (bind _glovesmeshpath (Variables|Default|GetGlovesMeshPath))
  (bind _gloves (Variables|Default|GetGloves))
  (if (not (Networking|IsDedicatedServer))
    (if (Utilities|Enum|NotEqual(Enum) _glovesmeshpath "")
      (bind _asvictorycore (Utilities|Casting|CastToVictoryCore (Variables|Default|GetVictoryCore)))
      (bind _returnvalue (Class|VictoryCore|BPLoadObject _asvictorycore _glovesmeshpath))
      (Utilities|IsValid _returnvalue
        (:Is%20Valid
          (bind _asskeletalmesh (Utilities|Casting|CastToSkeletalMesh _returnvalue))
          (CallFunction|SPSetEquippedMesh _gloves _asskeletalmesh)))
      (else
        (CallFunction|SPSetEquippedMesh _gloves "/Game/PrimalEarth/Human/Male/Outfits/Leather/maleLeather_gloves.maleLeather_gloves")))))

(fn OnRepBootsMeshPath
  (bind _bootsmeshpath (Variables|Default|GetBootsMeshPath))
  (bind _boots (Variables|Default|GetBoots))
  (if (not (Networking|IsDedicatedServer))
    (if (Utilities|Enum|NotEqual(Enum) _bootsmeshpath "")
      (bind _asvictorycore (Utilities|Casting|CastToVictoryCore (Variables|Default|GetVictoryCore)))
      (bind _returnvalue (Class|VictoryCore|BPLoadObject _asvictorycore _bootsmeshpath))
      (Utilities|IsValid _returnvalue
        (:Is%20Valid
          (bind _asskeletalmesh (Utilities|Casting|CastToSkeletalMesh _returnvalue))
          (CallFunction|SPSetEquippedMesh _boots _asskeletalmesh)))
      (else
        (CallFunction|SPSetEquippedMesh _boots "/Game/PrimalEarth/Human/Male/Outfits/Burlap/male_Burlap_Boots.male_Burlap_Boots")))))

(fn HandleonReps
  (CallFunction|HandleAnimation)
  (CallFunction|OnRepShirtMeshPath)
  (CallFunction|OnRepPantsMeshPath)
  (CallFunction|OnRepGlovesMeshPath)
  (CallFunction|OnRepBootsMeshPath))

(fn OnRepIsRangeHidden
  (bind _rangemesh (Variables|Default|GetRangeMesh))
  (bind _israngehidden (Variables|Default|GetIsRangeHidden))
  (Development|SetHiddeninGame _rangemesh _israngehidden false)
  (Rendering|SetVisibility _rangemesh (not _israngehidden) false))

(fn IPickupGetDisablePickupAfterTime
  (return (Variables|Default|GetDisablePickupAfterTime)))

(fn IPickupGetTimetoDisablePickup
  (return (Variables|Default|GetTimeToDisablePickup)))