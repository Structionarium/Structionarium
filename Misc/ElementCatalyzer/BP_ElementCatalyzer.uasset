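; BP_ElementCatalyzer is a placeable crafting structure that can only be built in liquid Element.
; Placement checks overlap nearby pain-causing volumes and require one with Element pool damage to encompass the location, otherwise returning a custom can't-build reason.
; On authority BeginPlay, non-preview instances load pickup settings and set inventory crafting speed from a game-mode option.
; It implements a pickup interface whose settings feed its multi-use menu entries through shared SP helpers.
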(event EventIPickupSetPickupSettings
  (params (DisablePickup :type Boolean) (DisablePickupWhenDamaged :type Boolean) (DisablePickupAfterTime :type Float%20%28single-precision%29) (TimeToDisablePickup :type Float%20%28double-precision%29))
  (Variables|Default|SetDisablePickup DisablePickup true)
  (Variables|Default|SetDisablePickupWhenDamaged DisablePickupWhenDamaged true)
  (Variables|Default|SetDisablePickupAfterTime DisablePickupAfterTime true)
  (Variables|Default|SetTimeToDisablePickup TimeToDisablePickup true))

(fn ConstructionScript
  (|CallParentFunction))

(fn BPGetMultiUseEntries
  (params (ForPC :type Player%20Controller%20Object%20Reference) (MultiUseEntries :type Array%20of%20Multi%20Use%20Entry%20Structures))
  (bind _entriesout (CallFunction|SPAddMenuEntries MultiUseEntries ForPC self (Variables|Default|GetDisablePickup) (Variables|Default|GetDisablePickupWhenDamaged) false false (Variables|Default|GetDisablePickupAfterTime) (Variables|Default|GetTimeToDisablePickup)))
  (return _entriesout))

(fn ReceiveBeginPlay
  (|CallParentFunction)
  (if (not (Variables|Default|GetbIsPreviewStructure))
    (Networking|SwitchHasAuthority
      (:Authority
        (CallFunction|SPSetPickUpSettings (Game|GetGameMode) self)
        (bind _value (CallFunction|SPGetFloatIniOption (Game|GetGameMode) "ElementCatalyzerCraftingSpeed" 1.0 1e+02))
        (Variables|/Script/ShooterGame.PrimalInventoryComponent|SetCraftingItemSpeed (Variables|Default|GetMyInventoryComponent) _value)))))

(fn BPIsAllowedtoBuildEx
  (params (OutPlacementData :type Placement%20Data%20Structure%20%28by%20ref%29) (CurrentAllowedReason :type Integer) (PC :type Player%20Controller%20Object%20Reference) (bFinalPlacement :type Boolean))
  (LocalVariables|SetBuildReason CurrentAllowedReason)
  (Utilities|FlowControl|Sequence
    (:then_0
      (if (== (LocalVariables|GetBuildReason) 1)
        (LocalVariables|SetBuildReason (Math|Integer|SelectInt 1 -100 (CallFunction|IsinElement (.AdjustedLocation (Utilities|Struct|BreakPlacementData OutPlacementData)))))))
    (:then_1
      (return (LocalVariables|GetBuildReason)))))

(fn BPOverrideCantBuildReasonString
  (params (CantBuildReason :type Integer))
  (return (Utilities|String|SelectString "Must be placed in liquid Element" "" (== CantBuildReason -100))))

(fn IsinElement
  (params (Location :type Vector))
  (Utilities|FlowControl|Sequence
    (:then_0
      (bind (_outactors _returnvalue) (Class|KismetSystemLibrary|SphereOverlapActorsSimple Location 115.0 "ObjectTypeQuery14" "/Script/Engine.PainCausingVolume" (Utilities|Array|MakeArray)))
      (if _returnvalue
        (bind _array_element (Utilities|Array|ForEachLoopwithBreak _outactors :!label _label)
          (:LoopBody
            (bind _aspaincausingvolume (Utilities|Casting|CastToPainCausingVolume _array_element))
            (bind _returnvalue_2 (Class|Volume|BPEncompassesPoint _aspaincausingvolume Location 1.0))
            (if (and _returnvalue_2 (== (Variables|/Script/Engine.PainCausingVolume|GetDamageType _aspaincausingvolume) "/Game/PrimalEarth/CoreBlueprints/DamageTypes/DmgType_ElementPool.DmgType_ElementPool_C"))
              (LocalVariables|SetretVal true)
              (goto _label Break))))))
    (:then_1
      (return (LocalVariables|GetretVal)))))

(fn IPickupGetDisablePickupAfterTime
  (return (Variables|Default|GetDisablePickupAfterTime)))

(fn IPickupGetTimetoDisablePickup
  (return (Variables|Default|GetTimeToDisablePickup)))