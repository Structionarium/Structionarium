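; Gas Collector Tek structure: collects gas in its inventory, disables its linked gas vein and takes slot count and pickup rules from SP game-mode settings.
; An inventory-UI toggle (PhoneHome) lets a randomized-interval server timer move gas to a random same-team gas Dedicated Storage with space.
; PhoneHome also prevents stasis, except while loading saves.
; Inventory fill ratio drives the liquid, meter and running effects through an OnRep.
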(event Custom|DisableVentEvent
  (Utilities|FlowControl|Delay 0.5)
  (CallFunction|MulticastDisableVent))

(event Custom|MulticastDisableVent
  (CallFunction|DisableGasVent))

(event EventIPickupSetPickupSettings
  (params (DisablePickup :type Boolean) (DisablePickupWhenDamaged :type Boolean) (DisablePickupAfterTime :type Float%20%28single-precision%29) (TimeToDisablePickup :type Float%20%28double-precision%29))
  (Variables|Default|SetDisablePickup DisablePickup true)
  (Variables|Default|SetDisablePickupWhenDamaged DisablePickupWhenDamaged true)
  (Variables|Default|SetDisablePickupAfterTime DisablePickupAfterTime true)
  (Variables|Default|SetTimeToDisablePickup TimeToDisablePickup true))

(event EventBeginPlay
  (bind _returnvalue (Game|GetGameMode))
  (Utilities|FlowControl|Delay 0.2)
  (if (not (Variables|Default|GetbIsPreviewStructure))
    (Utilities|FlowControl|Sequence
      (:then_0
        (Networking|SwitchHasAuthority
          (:Authority
            (CallFunction|SPSetPickUpSettings _returnvalue self)
            (bind _slotcount (CallFunction|SPGetInventorySlotSetting _returnvalue "GasCollectorSlotCount" 24))
            (Variables|Default|SetInventorySlots _slotcount true)
            (Utilities|Time|SetTimerbyFunctionName 0 "HandleGasTransfer" (Math|Random|RandomFloatinRange 275.0 3e+02) true)
            (CallFunction|MulticastDisableVent))))
      (:then_1
        (Networking|CanExecuteCosmeticEvents
          (:True
            (Components|Activation|Activate (Variables|Default|GetPump%20SFX) false)
            (Components|Activation|Activate (Variables|Default|GetCollectorRunningFX) false)
            (Rendering|SetVisibility (Variables|Default|GetPointLight1) true false)
            (Rendering|SetVisibility (Variables|Default|GetGasVolume) true false)
            (CallFunction|UpdateGasFX (Variables|Default|GetCurrentGasFXHeight))))))))

(event EventBPNotifyInventoryItemChange
  (params (bIsItemAdd :type Boolean) (theItem :type Primal%20Item%20Object%20Reference) (bEquipItem :type Boolean))
  (CallFunction|RecalculateGasFXHeight))

(fn ConstructionScript
  (bind _returnvalue (Rendering|Material|CreateDynamicMaterialInstance "/Game/Aberration/Structures/GasCollector/MIC_SimpleGasLiquid.MIC_SimpleGasLiquid" :!class /Script/Engine.KismetMaterialLibrary))
  (Variables|Default|SetGasMIC _returnvalue)
  (Rendering|Material|SetMaterial (Variables|Default|GetGasVolume) 0 (Variables|Default|GetGasMIC))
  (bind _returnvalue_2 (Rendering|Material|CreateDynamicMaterialInstance "/Game/Aberration/Structures/GasCollector/GasCollector_MIC.GasCollector_MIC" :!class /Script/Engine.KismetMaterialLibrary))
  (Variables|Default|SetCollectorMIC _returnvalue_2)
  (Rendering|Material|SetMaterial (Variables|Default|GetStaticMeshGasCollector) 0 (Variables|Default|GetCollectorMIC)))

(fn RecalculateGasFXHeight
  (bind _returnvalue (Class|PrimalInventoryComponent|GetMaxInventoryItems (Variables|Default|GetMyInventoryComponent) true))
  (Variables|Default|SetCurrentGasFXHeight (Math|Float|Min(Float) (/ (Math|Conversions|ToFloat(Integer) (Utilities|Array|Length (Variables|/Script/ShooterGame.PrimalInventoryComponent|GetInventoryItems (Variables|Default|GetMyInventoryComponent)))) (Math|Conversions|ToFloat(Integer) _returnvalue)) 1.0) true)
  (return))

(fn OnRepCurrentGasFXHeight
  (CallFunction|UpdateGasFX (Variables|Default|GetCurrentGasFXHeight)))

(fn UpdateGasFX
  (params (InputPin :type Float%20%28single-precision%29))
  (bind _returnvalue (== InputPin 1.0))
  (bind _collectorrunningfx (Variables|Default|GetCollectorRunningFX))
  (bind _liquidgas (Variables|Default|GetLiquidGas))
  (bind _relativescale3d (Variables|/Script/Engine.SceneComponent|GetRelativeScale3D _liquidgas))
  (bind (_x _y) (Math|Vector|BreakVector _relativescale3d))
  (Networking|CanExecuteCosmeticEvents
    (:True
      (Transformation|SetRelativeScale3D _liquidgas (Math|Vector|MakeVector _x _y (* InputPin (Variables|Default|GetMaxGasFXHeight))))
      (Rendering|Material|SetScalarParameterValue (Variables|Default|GetGasMIC) "Amount" InputPin :!class /Script/Engine.MaterialInstanceDynamic)
      (Rendering|Material|SetScalarParameterValue (Variables|Default|GetCollectorMIC) "Meter Rotation" InputPin :!class /Script/Engine.MaterialInstanceDynamic)
      (if (not (Math|Boolean|Equal(Boolean) _returnvalue (not (Components|Activation|IsActive _collectorrunningfx))))
        (if _returnvalue
          (Components|Activation|Deactivate _collectorrunningfx)
          (else
            (Components|Activation|Activate _collectorrunningfx false)))))))

(fn BPGetMultiUseEntries
  (params (ForPC :type Player%20Controller%20Object%20Reference) (MultiUseEntries :type Array%20of%20Multi%20Use%20Entry%20Structures))
  (bind _entriesout (CallFunction|SPAddMenuEntries MultiUseEntries ForPC self (Variables|Default|GetDisablePickup) (Variables|Default|GetDisablePickupWhenDamaged) false false (Variables|Default|GetDisablePickupAfterTime) (Variables|Default|GetTimeToDisablePickup)))
  (Utilities|FlowControl|Sequence
    (:then_0
      (bind _returnvalue (Class|PrimalStructure|AllowStructureAccess ForPC))
      (if _returnvalue
        (Utilities|Array|Add _entriesout (Utilities|Struct|MakeMultiUseEntry (Utilities|String|SelectString "Transferring to Dedicated Storage" "Holding Inventory" (Variables|Default|GetPhoneHome)) 9000 -1000 true true))))
    (:then_1
      (return _entriesout))))

(fn OnRepInventorySlots
  (Variables|/Script/ShooterGame.PrimalInventoryComponent|SetMaxInventoryItems (Variables|Default|GetMyInventoryComponent) (Variables|Default|GetInventorySlots)))

(fn HandleGasTransfer
  (bind _myinventorycomponent (Variables|Default|GetMyInventoryComponent))
  (if (Variables|Default|GetPhoneHome)
    (Class|PrimalInventoryComponent|BPInventoryRefresh _myinventorycomponent)
    (bind _storage (CallFunction|GetGasDedicatedStorageUnit))
    (Utilities|IsValid _storage
      (:Is%20Valid
        (bind _outitem (CallFunction|SPGetRemappedItem "/Game/Aberration/CoreBlueprints/Resources/PrimalItemResource_Gas.PrimalItemResource_Gas_C"))
        (bind _capacity (CallFunction|SPGetStructureInventoryCapacityforItem _outitem _storage))
        (if (> _capacity 0)
          (bind _returnvalue (Class|PrimalInventoryComponent|GetItemTemplateQuantity _myinventorycomponent _outitem 0 true false false))
          (if (> _returnvalue 0)
            (LocalVariables|SetTransferQty (Math|Integer|Min(Integer) _returnvalue _capacity))
            (Class|PrimalInventoryComponent|BPIncrementItemTemplateQuantity _myinventorycomponent _outitem (* (LocalVariables|GetTransferQty) -1) true false true false false false 0 false)
            (Class|PrimalInventoryComponent|BPIncrementItemTemplateQuantity (Variables|/Script/ShooterGame.PrimalStructureItemContainer|GetMyInventoryComponent _storage) _outitem (LocalVariables|GetTransferQty) true false true false false false 0 false)))))))

(fn GetGasDedicatedStorageUnit
  (bind _gasstoragelist (LocalVariables|GetGasStorageList))
  (bind _returnvalue (Utilities|Array|Length _gasstoragelist))
  (bind _outactors (Actor|GetAllActorsOfClass "/Game/Mods/StructuresPlusMod/Misc/DedicatedStorage/BP_DedicatedStorage.BP_DedicatedStorage_C"))
  (for _array_element _outactors
    (bind _asbp_dedicatedstorage_c (Utilities|Casting|CastToBP_DedicatedStorage _array_element))
    (bind _isnotfull (CallFunction|SPDoesInventoryHaveEmptySlots (Variables|/Script/ShooterGame.PrimalStructureItemContainer|GetMyInventoryComponent _asbp_dedicatedstorage_c)))
    (if (Math|Boolean|ANDBoolean _isnotfull (Utilities|ClassIsChildOf (Variables|/Game/Mods/StructuresPlusMod/Misc/DedicatedStorage/BP_DedicatedStorage.BP_DedicatedStorage_C|GetSelectedResourceClass _asbp_dedicatedstorage_c) "/Game/Aberration/CoreBlueprints/Resources/PrimalItemResource_Gas.PrimalItemResource_Gas_C") (== (Variables|/Script/Engine.Actor|GetTargetingTeam _array_element) (Variables|Default|GetTargetingTeam)))
      (Utilities|Array|Add (LocalVariables|GetGasStorageList) _asbp_dedicatedstorage_c)))
  (return (select (> _returnvalue 0) (Utilities|Array|Get(acopy) _gasstoragelist (Math|Random|RandomIntegerinRange 0 (- _returnvalue 1))) 0)))

(fn BPTryMultiUse
  (params (ForPC :type Player%20Controller%20Object%20Reference) (UseIndex :type Integer))
  (Utilities|FlowControl|Sequence
    (:then_0
      (switch int UseIndex
        (:9000
          (Variables|Default|SetPhoneHome (not (Variables|Default|GetPhoneHome)) true))))
    (:then_1
      (return true))))

(fn BPPreventStasis
  (bind _returnvalue (Class|VictoryCore|IsLoadingSaveGame))
  (return (and (not _returnvalue) (Variables|Default|GetPhoneHome))))

(fn BPUnstasis
  (bind _returnvalue (Class|VictoryCore|IsLoadingSaveGame))
  (if (not _returnvalue)
    (Class|PrimalInventoryComponent|BPInventoryRefresh (Variables|Default|GetMyInventoryComponent))
    (CallFunction|DisableVentEvent)))

(fn DisableGasVent
  (bind _array_element (Utilities|Array|ForEachLoopwithBreak (Variables|Default|GetLinkedStructures) :!label _label)
    (:LoopBody
      (if (== (Utilities|GetClass _array_element) "/Game/Aberration/Structures/GasCollector/GasVein_Base_BP.GasVein_Base_BP_C")
        (Class|PrimalStructure|BPHandleStructureEnabled _array_element false)
        (goto _label Break)))))

(fn IPickupGetDisablePickupAfterTime
  (return (Variables|Default|GetDisablePickupAfterTime)))

(fn IPickupGetTimetoDisablePickup
  (return (Variables|Default|GetTimeToDisablePickup)))