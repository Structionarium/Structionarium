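; BP_AutoTurretPlant is a plant auto turret that adds configurable targeting options through shared SP turret helpers.
; A multi-use entry for same-team players applies a settings buff, and the turret options interface stores the resulting options.
; Targeting and HUD drawing delegate to SP functions.
; The options getter merges the turret's own range, AI and warning settings with stored dino level and list filters.
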(event EventITurretSetOptions
  (params (TurretOptions :type SP%20Turret%20Options%20Structure))
  (Variables|Default|SetTurretOptions TurretOptions false))

(fn ConstructionScript
  (|CallParentFunction))

(fn BPGetMultiUseEntries
  (params (ForPC :type Player%20Controller%20Object%20Reference) (MultiUseEntries :type Array%20of%20Multi%20Use%20Entry%20Structures))
  (bind _entriesout (CallFunction|SPCleanUpTurretMenuEntries MultiUseEntries))
  (if (== (Variables|/Script/Engine.Actor|GetTargetingTeam ForPC) (Variables|Default|GetTargetingTeam))
    (Utilities|Array|Add _entriesout (Utilities|Struct|MakeMultiUseEntry "[Turret Options]" 9001 -1000 true (Math|Conversions|ToColor(LinearColor) (CallFunction|SPGetSpecialMenuColor)))))
  (return _entriesout))

(fn BPTryMultiUse
  (params (ForPC :type Player%20Controller%20Object%20Reference) (UseIndex :type Integer))
  (Utilities|FlowControl|Sequence
    (:then_0
      (if (== UseIndex 9001)
        (CallFunction|SPApplyTurretSettingsBuff ForPC self)))
    (:then_1
      (return true))))

(fn BPTurretPreventsTargeting
  (params (PotentialTarget :type Primal%20Character%20Object%20Reference))
  (bind _preventtargeting (CallFunction|SPHandleTurretTargeting PotentialTarget (Variables|Default|GetTurretOptions)))
  (return _preventtargeting))

(fn BlueprintDrawHUD
  (params (HUD :type Shooter%20HUD%20Object%20Reference) (CenterX :type Float%20%28single-precision%29) (CenterY :type Float%20%28single-precision%29))
  (CallFunction|SPDrawTurretHUD HUD CenterX CenterY self))

(fn ITurretGetOptions
  (bind _turretoptions (Variables|Default|GetTurretOptions))
  (bind (_mindinolevel _maxdinolevel _dinolist _isinclusionlist) (Utilities|Struct|BreakSPTurretOptions _turretoptions))
  (return (Utilities|Struct|MakeSPTurretOptions (Variables|Default|GetRangeSetting) (Variables|Default|GetAISetting) (Variables|Default|GetWarningSetting) _mindinolevel _maxdinolevel _dinolist _isinclusionlist)))