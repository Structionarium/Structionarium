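; S+ Transmitter structure with configurable pickup, a multi-use dino scan and boss tribute crafting.
; Server BeginPlay reads game-mode options for pickup, storm shutdown and scanning, then adds missing tribute blueprints for arena managers found in the level.
; The scan entry applies a scanner buff to the player and opens its UI, warning about hibernation in singleplayer.
; It also mutes the emitter sound and overrides placement failure -9.
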(event EventIPickupSetPickupSettings
  (params (DisablePickup :type Boolean) (DisablePickupWhenDamaged :type Boolean) (DisablePickupAfterTime :type Float%20%28single-precision%29) (TimeToDisablePickup :type Float%20%28double-precision%29))
  (Variables|Default|SetDisablePickup DisablePickup true)
  (Variables|Default|SetDisablePickupWhenDamaged DisablePickupWhenDamaged true)
  (Variables|Default|SetDisablePickupAfterTime DisablePickupAfterTime true)
  (Variables|Default|SetTimeToDisablePickup TimeToDisablePickup true))

(fn ConstructionScript
  (|CallParentFunction))

(fn BPGetMultiUseEntries
  (params (ForPC :type Player%20Controller%20Object%20Reference) (MultiUseEntries :type Array%20of%20Multi%20Use%20Entry%20Structures))
  (bind _entriesout (CallFunction|SPAddMenuEntries MultiUseEntries ForPC self (Variables|Default|GetDisablePickup) (Variables|Default|GetDisablePickupWhenDamaged) false false (Variables|Default|GetDisablePickupAfterTime) (Variables|Default|GetTimeToDisablePickup)))
  (bind _returnvalue (Class|PrimalStructure|AllowStructureAccess ForPC))
  (if (and _returnvalue (not (Variables|Default|GetDisableDinoScan)))
    (Utilities|Array|Add _entriesout (Utilities|Struct|MakeMultiUseEntry "[Dino Scan]" 9001 -1000 true (Math|Conversions|ToColor(LinearColor) (CallFunction|SPGetSpecialMenuColor)))))
  (return _entriesout))

(fn BPTryMultiUse
  (params (ForPC :type Player%20Controller%20Object%20Reference) (UseIndex :type Integer))
  (Utilities|FlowControl|Sequence
    (:then_0
      (if (== UseIndex 601)
        (Variables|Default|SetIsUnlocked (not (Variables|Default|GetbIsLocked)))))
    (:then_1
      (if (and (== UseIndex 9001) (not (Variables|Default|GetDisableDinoScan)))
        (Utilities|FlowControl|Sequence
          (:then_0
            (Utilities|SwitchNetAuthority
              (:PlayerServer
                (bind _asshooterplayercontroller (Utilities|Casting|CastToShooterPlayerController ForPC))
                (Class|ShooterPlayerController|ClientServerNotification _asshooterplayercontroller "Dino scan will not work correctly on singleplayer unless you prevent hibernation." "(R=1.000000,G=0.000000,B=0.000000,A=1.000000)" 1.5 5.0))))
          (:then_1
            (CallFunction|PerformDinoScan ForPC)))))
    (:then_2
      (return true))))

(fn ForceTributeCrafting
  (bind _myinventorycomponent (Variables|Default|GetMyInventoryComponent))
  (bind _outactors (Actor|GetAllActorsOfClass "/Game/PrimalEarth/CoreBlueprints/BossTribute/BossArenaManager.BossArenaManager_C"))
  (for _array_element _outactors
    (bind _asbossarenamanager_c (Utilities|Casting|CastToBossArenaManager _array_element))
    (bind _asbossarenamanager_c_2 (Utilities|Casting|CastToBossArenaManagerClass (Utilities|GetClass _asbossarenamanager_c)))
    (Utilities|Array|Add (LocalVariables|GetArenaManagers) _asbossarenamanager_c_2))
  (for _array_element_2 (Variables|Default|GetTributes)
    (bind _returnvalue (Class|VictoryCore|GetClassDefaultObject _array_element_2))
    (bind _asprimalitem_bosstributegeneric_c (Utilities|Casting|CastToPrimalItem_BossTributeGeneric _returnvalue))
    (if (Utilities|Array|ContainsItem (LocalVariables|GetArenaManagers) (Variables|/Game/PrimalEarth/CoreBlueprints/Items/Armor/Cloth/PrimalItem_BossTributeGeneric.PrimalItem_BossTributeGeneric_C|GetBossArenaManagerClass _asprimalitem_bosstributegeneric_c))
      (bind _returnvalue_2 (Class|PrimalInventoryComponent|GetItemTemplateQuantity _myinventorycomponent _array_element_2 0 false false false))
      (if (== _returnvalue_2 0)
        (Class|PrimalItem|AddNewItem _array_element_2 _myinventorycomponent false false 0.0 false 1 true 0.0 false 0 0.0)))))

(fn PerformDinoScan
  (params (PC :type Player%20Controller%20Object%20Reference))
  (bind _asshooterplayercontroller (Utilities|Casting|CastToShooterPlayerController PC))
  (bind _returnvalue (Class|PrimalBuff|StaticAddBuff "/Game/Mods/StructuresPlusMod/_Buffs/Buff_StructuresPlus_DinoScanner.Buff_StructuresPlus_DinoScanner_C" (Class|ShooterPlayerController|GetPlayerCharacter _asshooterplayercontroller) 0 0 false))
  (bind _asbuff_structuresplus_dinoscanner_c (Utilities|Casting|CastToBuff_StructuresPlus_DinoScanner _returnvalue))
  (Default|InitializeScannerUI _asbuff_structuresplus_dinoscanner_c))

(fn BPIsAllowedtoBuild
  (params (OutPlacementData :type Placement%20Data%20Structure%20%28by%20ref%29) (CurrentAllowedReason :type Integer))
  (return (Math|Integer|SelectInt 1 CurrentAllowedReason (== CurrentAllowedReason -9))))

(fn ReceiveBeginPlay
  (bind _returnvalue (Game|GetGameMode))
  (|CallParentFunction)
  (if (not (Variables|Default|GetbIsPreviewStructure))
    (Utilities|FlowControl|Sequence
      (:then_0
        (bind _astransmitteremitter_c (Utilities|Casting|CastToTransmitterEmitter (Variables|/Script/Engine.ChildActorComponent|GetChildActor (Variables|Default|GetActivatedEmitter))))
        (Audio|Components|Audio|SetVolumeMultiplier (Variables|/Script/ShooterGame.PrimalEmitterSpawnable|GetSoundToPlay _astransmitteremitter_c) 0.0 :!class /Script/Engine.AudioComponent))
      (:then_1
        (Networking|SwitchHasAuthority
          (:Authority
            (Utilities|FlowControl|Sequence
              (:then_0
                (CallFunction|SPSetPickUpSettings _returnvalue self))
              (:then_1
                (bind _dodisable (CallFunction|SPGetDisableElectronicsDuringStormSetting _returnvalue))
                (Variables|Default|SetbDisableStructureOnElectricStorm _dodisable))
              (:then_2
                (Variables|Default|SetbIsLocked (not (Variables|Default|GetIsUnlocked)) true))
              (:then_3
                (bind _value (CallFunction|SPGetBoolOption _returnvalue "DisableDinoScan"))
                (Variables|Default|SetDisableDinoScan _value true))
              (:then_4
                (bind _value_2 (CallFunction|SPGetBoolOption _returnvalue "PreventTransmitterPickup"))
                (if _value_2
                  (Variables|Default|SetDisablePickup true true)
                  (Utilities|SPAddifUnique (Variables|Default|GetTags) "PreventPickup")))
              (:then_5
                (CallFunction|ForceTributeCrafting)))))))))

(fn IPickupGetDisablePickupAfterTime
  (return (Variables|Default|GetDisablePickupAfterTime)))

(fn IPickupGetTimetoDisablePickup
  (return (Variables|Default|GetTimeToDisablePickup)))