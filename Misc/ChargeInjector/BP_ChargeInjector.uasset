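; Charge Injector: a placeable, activatable structure that acts as a charge emitter with player-adjustable range.
; A Buff_ChargeManager, destroyed on stasis and recreated on unstasis, receives charge variables forwarded through interface events and ChargeFunctions_FakeLibrary.
; Multi-use wheel entries adjust or show the range; its RepNotify rescales the range mesh and sets battery drain by range squared.
; Activation raises the animated drone; a game option can block Tek Generator power.
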(event Custom|CancelTekGen
  (Utilities|FlowControl|Delay 5.0)
  (if (and (> (Variables|Default|GetPoweredOverrideCounter) 0) (not (Variables|Default|GetAllowTekGen)))
    (Class|PrimalStructureItemContainer|SetPoweredOverrideCounter)))

(event Custom|HandleActivationAnimation
  (bind _progress (Timeline|ActivateTimeline Play)
    (:Update
      (if (not (Networking|IsDedicatedServer))
        (Transformation|SetRelativeLocation (Variables|Default|GetMeshScene) (Math|Vector|MakeVector 0.0 0.0 (* _progress 2e+02)) false)))
    (:Finished
      (Networking|SwitchHasAuthority
        (:Authority
          (Variables|Default|SetIsElevated (== _progress 1.0) false))))))

(event Custom|HandleDeactivationAnimation
  (bind _progress (Timeline|ActivateTimeline Reverse)
    (:Update
      (if (not (Networking|IsDedicatedServer))
        (Transformation|SetRelativeLocation (Variables|Default|GetMeshScene) (Math|Vector|MakeVector 0.0 0.0 (* _progress 2e+02)) false)))
    (:Finished
      (Networking|SwitchHasAuthority
        (:Authority
          (Variables|Default|SetIsElevated (== _progress 1.0) false))))))

(event Custom|SetDefaultsEvent
  (Utilities|FlowControl|Delay 0.5)
  (Variables|Default|SetRangeSetting 15 true))

(event Custom|CheckForBatteriesAndUpdate_Multicast
  ;[0.335 1 0.7682] Charge Buff logic
  (bind _asbuff_chargemanager_c (Utilities|Casting|CastToBuff_ChargeManager (Variables|ChargeBuff|GetchargeManagerBuff)))
  (Default|CheckBatteriesandUpdate _asbuff_chargemanager_c))

(event Custom|ChargeVariableEvent_Float_Multicast
  (params (variableType :type E_ChargeVariableNames%20Enum :default "NewEnumerator0") (fValue :type Float%20%28single-precision%29))
  ;[0.335 1 0.7682] Charge Buff logic
  (CallFunction|ChargeVariableEventFloat variableType fValue))

(event Custom|CreateChargeBuff
  ;[1 1 1] Charge buff
  (if (Utilities|IsValid (Variables|ChargeBuff|GetchargeManagerBuff))
    (CallFunction|DestroyChargeBuff))
  (ChargeBuff|CreateChargeManager))

(event Custom|ChargeVariableEvent_Int_Multicast
  (params (variableType :type E_ChargeVariableNames%20Enum :default "NewEnumerator0") (iValue :type Integer))
  ;[0.335 1 0.7682] Charge Buff logic
  (CallFunction|ChargeVariableEventInt variableType iValue))

(event Custom|ChargeVariableEvent_Int
  (params (variableType :type E_ChargeVariableNames%20Enum :default "NewEnumerator0") (ivalue :type Integer))
  ;[0.335 1 0.7682] Charge Buff logic
  (bind _asbuff_chargemanager_c (Utilities|Casting|CastToBuff_ChargeManager (Variables|ChargeBuff|GetchargeManagerBuff)))
  (CallFunction|SetChargeVariableInterface variableType false 0.0 0.0 false false false ivalue)
  (Default|ChargeVariableEvent _asbuff_chargemanager_c variableType false 0.0 0.0 ivalue))

(event Custom|ChargeVariableEvent_Float
  (params (variableType :type E_ChargeVariableNames%20Enum :default "NewEnumerator0") (fValue :type Float%20%28single-precision%29))
  ;[0.335 1 0.7682] Charge Buff logic
  (bind _asbuff_chargemanager_c (Utilities|Casting|CastToBuff_ChargeManager (Variables|ChargeBuff|GetchargeManagerBuff)))
  (CallFunction|SetChargeVariableInterface variableType false fValue 0.0 false false false)
  (Default|ChargeVariableEvent _asbuff_chargemanager_c variableType false fValue 0.0))

(event Custom|ChargeVariableEvent_Double
  (params (variableType :type E_ChargeVariableNames%20Enum :default "NewEnumerator0") (dValue :type Float%20%28double-precision%29))
  ;[0.335 1 0.7682] Charge Buff logic
  (bind _asbuff_chargemanager_c (Utilities|Casting|CastToBuff_ChargeManager (Variables|ChargeBuff|GetchargeManagerBuff)))
  (CallFunction|SetChargeVariableInterface variableType false 0.0 dValue false false false)
  (Default|ChargeVariableEvent _asbuff_chargemanager_c variableType false 0.0 dValue))

(event Custom|ChargeVariableEvent_Double_Multicast
  (params (variableType :type E_ChargeVariableNames%20Enum :default "NewEnumerator0") (dValue :type Float%20%28double-precision%29))
  ;[0.335 1 0.7682] Charge Buff logic
  (CallFunction|ChargeVariableEventDouble variableType dValue))

(event Custom|DestroyChargeBuff_Multicast
  ;[1 1 1] Charge buff
  (CallFunction|DestroyChargeBuff))

(event Custom|ChargeVariableEvent_Boolean
  (params (variableType :type E_ChargeVariableNames%20Enum :default "NewEnumerator0") (bBValue :type Boolean))
  ;[0.335 1 0.7682] Charge Buff logic
  (bind _asbuff_chargemanager_c (Utilities|Casting|CastToBuff_ChargeManager (Variables|ChargeBuff|GetchargeManagerBuff)))
  (CallFunction|SetChargeVariableInterface variableType false 0.0 0.0 bBValue false false)
  (Default|ChargeVariableEvent _asbuff_chargemanager_c variableType bBValue 0.0 0.0))

(event Custom|ChargeVariableEvent_Boolean_Multicast
  (params (variableType :type E_ChargeVariableNames%20Enum :default "NewEnumerator0") (bBValue :type Boolean))
  ;[0.335 1 0.7682] Charge Buff logic
  (CallFunction|ChargeVariableEventBoolean variableType bBValue))

(event Custom|CreateChargeBuff_Multicast
  ;[1 1 1] Charge buff
  (CallFunction|CreateChargeBuff))

(event EventIPickupSetPickupSettings
  (params (DisablePickup :type Boolean) (DisablePickupWhenDamaged :type Boolean) (DisablePickupAfterTime :type Float%20%28single-precision%29) (TimeToDisablePickup :type Float%20%28double-precision%29))
  (Variables|Default|SetDisablePickup DisablePickup false)
  (Variables|Default|SetDisablePickupWhenDamaged DisablePickupWhenDamaged false)
  (Variables|Default|SetDisablePickupAfterTime DisablePickupAfterTime false)
  (Variables|Default|SetTimeToDisablePickup TimeToDisablePickup false))

(event EventInterfaceCheckforBatteriesandUpdateMulticast
  ;[0.335 1 0.7682] Charge Buff logic
  (CallFunction|CheckforBatteriesandUpdateMulticast))

(event EventChargeVariableEventIntInterface
  (params (variableType :type E_ChargeVariableNames%20Enum :default "NewEnumerator0") (iValue :type Integer))
  ;[0.335 1 0.7682] Charge Buff logic
  (CallFunction|ChargeVariableEventInt variableType iValue))

(event EventChargeVariableEventIntMulticastInterface
  (params (variableType :type E_ChargeVariableNames%20Enum :default "NewEnumerator0") (iValue :type Integer))
  ;[0.335 1 0.7682] Charge Buff logic
  (CallFunction|ChargeVariableEventIntMulticast variableType iValue))

(event EventSetChargeVariableInterface
  (params (variableType :type E_ChargeVariableNames%20Enum :default "NewEnumerator0") (multicast :type Boolean) (fValue :type Float%20%28single-precision%29) (dValue :type Float%20%28double-precision%29) (bBValue :type Boolean) (triggerEvent :type Boolean) (multicastEvent :type Boolean) (iValue :type Integer))
  ;[0.335 1 0.7682] Charge Buff logic
  (switch Utilities|FlowControl|Switch|SwitchonE_ChargeVariableNames variableType
    (:NewEnumerator0
      (if (and multicast (Networking|IsServer))
        (Variables|ChargeBuff|SetcurrentChargeAmountStruct fValue true)
        (else
          (Variables|ChargeBuff|SetcurrentChargeAmountStruct fValue false)))
      (if triggerEvent :!label _label
        (bind _returnvalue (Class|VictoryCore|GetClassDefaultObject "/Game/Aberration/CoreBlueprints/ChargeFunctions_FakeLibrary.ChargeFunctions_FakeLibrary_C"))
        (bind _aschargefunctions_fakelibrary_c (Utilities|Casting|CastToChargeFunctions_FakeLibrary _returnvalue))
        (Default|ChargeVariableEventFloatLibrary _aschargefunctions_fakelibrary_c variableType fValue self (Variables|ChargeBuff|GetchargeManagerBuff) multicast)))
    (:NewEnumerator3
      (if multicast
        (Variables|ChargeBuff|SetemitterIsActive bBValue true)
        (else
          (Variables|ChargeBuff|SetemitterIsActive bBValue false)))
      (if triggerEvent
        (bind _returnvalue_2 (Class|VictoryCore|GetClassDefaultObject "/Game/Aberration/CoreBlueprints/ChargeFunctions_FakeLibrary.ChargeFunctions_FakeLibrary_C"))
        (bind _aschargefunctions_fakelibrary_c_2 (Utilities|Casting|CastToChargeFunctions_FakeLibrary _returnvalue_2))
        (Default|ChargeVariableEventBooleanLibrary _aschargefunctions_fakelibrary_c_2 variableType bBValue self (Variables|ChargeBuff|GetchargeManagerBuff) multicast)))
    (:NewEnumerator4
      (Variables|ChargeBuff|SetemitterRange fValue)
      (goto _label))
    (:NewEnumerator5
      (Variables|ChargeBuff|SetemitterChargeConsumedPerSecond fValue)
      (goto _label))
    (:NewEnumerator6
      (Variables|ChargeBuff|SetchargeEmittedPerSecond fValue)
      (goto _label))
    (:NewEnumerator10
      (Variables|ChargeBuff|SetlastTimeChargeUpdatedOnTimer dValue)
      (if triggerEvent
        (bind _returnvalue_3 (Class|VictoryCore|GetClassDefaultObject "/Game/Aberration/CoreBlueprints/ChargeFunctions_FakeLibrary.ChargeFunctions_FakeLibrary_C"))
        (bind _aschargefunctions_fakelibrary_c_3 (Utilities|Casting|CastToChargeFunctions_FakeLibrary _returnvalue_3))
        (Default|ChargeVariableEventDoubleLibrary _aschargefunctions_fakelibrary_c_3 variableType dValue self (Variables|ChargeBuff|GetchargeManagerBuff) multicastEvent)))
    (:NewEnumerator13
      (Variables|Default|SetchargeConsumedByReceivers fValue)
      (goto _label))))

(event EventChargeVariableEventBooleanInterface
  (params (variableType :type E_ChargeVariableNames%20Enum :default "NewEnumerator0") (bBValue :type Boolean))
  ;[0.335 1 0.7682] Charge Buff logic
  (CallFunction|ChargeVariableEventBoolean variableType bBValue))

(event EventChargeVariableEventFloatInterface
  (params (variableType :type E_ChargeVariableNames%20Enum :default "NewEnumerator0") (fValue :type Float%20%28single-precision%29))
  ;[0.335 1 0.7682] Charge Buff logic
  (CallFunction|ChargeVariableEventFloat variableType fValue))

(event EventChargeVariableEventBooleanMulticastInterface
  (params (variableType :type E_ChargeVariableNames%20Enum :default "NewEnumerator0") (bBValue :type Boolean))
  ;[0.335 1 0.7682] Charge Buff logic
  (CallFunction|ChargeVariableEventBooleanMulticast variableType bBValue))

(event EventChargeVariableEventFloatMulticastInterface
  (params (variableType :type E_ChargeVariableNames%20Enum :default "NewEnumerator0") (fValue :type Float%20%28single-precision%29))
  ;[0.335 1 0.7682] Charge Buff logic
  (CallFunction|ChargeVariableEventFloatMulticast variableType fValue))

(event EventChargeVariableEventDoubleInterface
  (params (variableType :type E_ChargeVariableNames%20Enum :default "NewEnumerator0") (dValue :type Float%20%28double-precision%29))
  ;[0.335 1 0.7682] Charge Buff logic
  (CallFunction|ChargeVariableEventDouble variableType dValue))

(event EventChargeVariableEventDoubleMulticastInterface
  (params (variableType :type E_ChargeVariableNames%20Enum :default "NewEnumerator0") (dValue :type Float%20%28double-precision%29))
  ;[0.335 1 0.7682] Charge Buff logic
  (CallFunction|ChargeVariableEventDoubleMulticast variableType dValue))

(fn ConstructionScript
  (|CallParentFunction)
  (if (not (or (Variables|Default|GetbIsPreviewStructure) (Networking|IsDedicatedServer)))
    (bind _returnvalue (Rendering|Material|CreateDynamicMaterialInstance "/Game/EndGame/Dinos/Drone/Drone_MIC.Drone_MIC" :!class /Script/Engine.KismetMaterialLibrary))
    (Rendering|Material|SetMaterial (Variables|Default|GetDroneMesh) 0 _returnvalue)
    (Rendering|Material|SetVectorParameterValue _returnvalue "Color5" "(R=0.000000,G=0.760000,B=0.000000,A=1.000000)" :!class /Script/Engine.MaterialInstanceDynamic)
    (Rendering|Material|SetScalarParameterValue _returnvalue "TheSSAOIntensity" 0.5 :!class /Script/Engine.MaterialInstanceDynamic)))

(fn BPGetMultiUseEntries
  (params (ForPC :type Player%20Controller%20Object%20Reference) (MultiUseEntries :type Array%20of%20Multi%20Use%20Entry%20Structures))
  (bind _color (CallFunction|SPGetSpecialMenuColor))
  (bind _rangesetting (Variables|Default|GetRangeSetting))
  (bind _returnvalue (Math|Conversions|ToColor(LinearColor) _color))
  (bind _entriesout (CallFunction|SPAddMenuEntries MultiUseEntries ForPC self (Variables|Default|GetDisablePickup) (Variables|Default|GetDisablePickupWhenDamaged) false false (Variables|Default|GetDisablePickupAfterTime) (Variables|Default|GetTimeToDisablePickup)))
  (Utilities|FlowControl|Sequence
    (:then_0
      (bind _returnvalue_2 (Class|PrimalStructure|AllowStructureAccess ForPC))
      (if _returnvalue_2
        (Utilities|Array|Add _entriesout (Utilities|Struct|MakeMultiUseEntry (Utilities|String|SelectString "Show Range" "Hide Range" (Variables|Default|GetIsRangeHidden)) 9000 -1000))
        (Utilities|Array|Add _entriesout (Utilities|Struct|MakeMultiUseEntry "[Adjust Range]" 8999 -500 true true _returnvalue))
        (Utilities|Array|Add _entriesout (Utilities|Struct|MakeMultiUseEntry (Utilities|String|BuildString(Integer) "Current Range: " "" _rangesetting) 9999 3000 true true 1 _returnvalue))
        (Utilities|Array|Add _entriesout (Utilities|Struct|MakeMultiUseEntry "+1" 9001 2000 (>= _rangesetting 50) true 1))
        (Utilities|Array|Add _entriesout (Utilities|Struct|MakeMultiUseEntry "+10" 9002 1000 (>= _rangesetting 41) true 1))
        (Utilities|Array|Add _entriesout (Utilities|Struct|MakeMultiUseEntry "" 9999 0 true true 1))
        (Utilities|Array|Add _entriesout (Utilities|Struct|MakeMultiUseEntry "-10" 9003 -1000 (<= _rangesetting 10) true 1))
        (Utilities|Array|Add _entriesout (Utilities|Struct|MakeMultiUseEntry "-1" 9004 -2000 (<= _rangesetting 1) true 1))))
    (:then_1
      (return _entriesout))))

(fn BPTryMultiUse
  (params (ForPC :type Player%20Controller%20Object%20Reference) (UseIndex :type Integer))
  (Utilities|FlowControl|Sequence
    (:then_0
      (switch int UseIndex
        (:9000
          (Variables|Default|SetIsRangeHidden (not (Variables|Default|GetIsRangeHidden)) true))
        (:9001
          (Variables|Default|SetRangeSetting (+ (Variables|Default|GetRangeSetting) 1) true))
        (:9002
          (Variables|Default|SetRangeSetting (+ (Variables|Default|GetRangeSetting) 10) true))
        (:9003
          (Variables|Default|SetRangeSetting (+ (Variables|Default|GetRangeSetting) -10) true))
        (:9004
          (Variables|Default|SetRangeSetting (+ (Variables|Default|GetRangeSetting) -1) true))))
    (:then_1
      (return true))))

(fn ReceiveDestroyed
  (|CallParentFunction)
  (CallFunction|DestroyChargeBuff))

(fn CreateChargeManager
  (bind _returnvalue (Class|VictoryCore|GetClassDefaultObject "/Game/Aberration/CoreBlueprints/ChargeFunctions_FakeLibrary.ChargeFunctions_FakeLibrary_C"))
  (bind _aschargefunctions_fakelibrary_c (Utilities|Casting|CastToChargeFunctions_FakeLibrary _returnvalue))
  (bind _chargemanager (Default|StructureCreateChargeManagerLibrary _aschargefunctions_fakelibrary_c self (Variables|ChargeBuff|GetchargeManagerBuffClass)))
  (Variables|ChargeBuff|SetchargeManagerBuff _chargemanager))

(fn BPTriggerStasisEvent
  (CallFunction|DestroyChargeBuffMulticast))

(fn DestroyChargeBuff
  (bind _chargemanagerbuff (Variables|ChargeBuff|GetchargeManagerBuff))
  (bind _asbuff_chargemanager_c (Utilities|Casting|CastToBuff_ChargeManager _chargemanagerbuff))
  (Variables|/Game/Aberration/CoreBlueprints/Buffs/Buff_ChargeManager.Buff_ChargeManager_C|SetchargeActor _asbuff_chargemanager_c 0)
  (Class|PrimalBuff|BPDeactivate _chargemanagerbuff))

(fn BPContainerActivated
  (Utilities|FlowControl|Sequence
    (:then_0
      (Networking|SwitchHasAuthority
        (:Authority
          (CallFunction|SetChargeVariableInterface "NewEnumerator3" true 0.0 0.0 true true true)
          (CallFunction|HandleActivationAnimation)
          (CallFunction|CancelTekGen))))
    (:then_1
      (if (not (Networking|IsDedicatedServer))
        (Variables|/Script/Engine.SkeletalMeshComponent|SetbPauseAnims (Variables|Default|GetDroneMesh) false)))))

(fn BPContainerDeactivated
  (Utilities|FlowControl|Sequence
    (:then_0
      (Networking|SwitchHasAuthority
        (:Authority
          (CallFunction|SetChargeVariableInterface "NewEnumerator3" true 0.0 0.0 false true true)
          (CallFunction|HandleDeactivationAnimation))))
    (:then_1
      (if (not (Networking|IsDedicatedServer))
        (Variables|/Script/Engine.SkeletalMeshComponent|SetbPauseAnims (Variables|Default|GetDroneMesh) true)))))

(fn ReceiveBeginPlay
  (bind _returnvalue (Game|GetGameMode))
  (|CallParentFunction)
  (if (not (Variables|Default|GetbIsPreviewStructure))
    (CallFunction|CreateChargeBuff)
    (Utilities|FlowControl|Sequence
      (:then_0
        (Networking|SwitchHasAuthority
          (:Authority
            (CallFunction|SPSetPickUpSettings _returnvalue self)
            (bind _value (CallFunction|SPGetBoolOption _returnvalue "ChargeInjectorAllowTekGen"))
            (Variables|Default|SetAllowTekGen _value)
            (Utilities|FlowControl|Sequence
              (:then_0
                (if (== (Variables|Default|GetRangeSetting) 0)
                  (CallFunction|SetDefaultsEvent)))
              (:then_1
                (if (not _value)
                  (CallFunction|CancelTekGen)))))))
      (:then_1
        (if (not (Networking|IsDedicatedServer))
          (bind _asemitter_chargeinjector_c (Utilities|Casting|CastToEmitter_ChargeInjector (Variables|/Script/Engine.ChildActorComponent|GetChildActor (Variables|Default|GetActivatedEmitter))))
          (Effects|Components|ParticleSystem|SetVectorParameter (Variables|/Script/Engine.Emitter|GetParticleSystemComponent _asemitter_chargeinjector_c) "EndPoint01" (Transformation|GetActorLocation))
          (Variables|/Script/Engine.SkeletalMeshComponent|SetbPauseAnims (Variables|Default|GetDroneMesh) (not (Variables|Default|GetbContainerActivated)))))
      (:then_2
        (Utilities|SwitchNetAuthority
          (:PlayerServer
            (CallFunction|OnRepIsElevated)))))))

(fn BPUnstasis
  (|CallParentFunction)
  (if (not (Variables|Default|GetbNoCollision))
    (bind _returnvalue (Class|VictoryCore|IsLoadingSaveGame))
    (if (not _returnvalue)
      (Networking|SwitchHasAuthority
        (:Authority
          (CallFunction|CreateChargeBuffMulticast))))))

(fn BPClientDoMultiUse
  (params (ForPC :type Player%20Controller%20Object%20Reference) (ClientUseIndex :type Integer))
  (switch int ClientUseIndex
    (:8999
      (bind _asshooterplayercontroller (Utilities|Casting|CastToShooterPlayerController ForPC))
      (Class|ShooterPlayerController|SetMultiUseWheelCategory _asshooterplayercontroller 1))))

(fn OnRepIsRangeHidden
  (bind _israngehidden (Variables|Default|GetIsRangeHidden))
  (bind _rangesetting (Variables|Default|GetRangeSetting))
  (bind _returnvalue (not _israngehidden))
  (bind _returnvalue_2 (* _rangesetting 3e+02))
  (Rendering|SetVisibility (Variables|Default|GetRangeMesh) _returnvalue false)
  (if _returnvalue
    (Transformation|SetWorldScale3D (Variables|Default|GetRangeMesh) (Math|Vector|MakeVector _returnvalue_2 _returnvalue_2 _returnvalue_2))))

(fn OnRepRangeSetting
  (bind _rangesetting (Variables|Default|GetRangeSetting))
  (bind _returnvalue (Math|Conversions|ToFloat(Integer) _rangesetting))
  (bind _returnvalue_2 (* _rangesetting 3e+02))
  (bind _returnvalue_3 (Math|Float|Power _returnvalue 2.0))
  (bind _returnvalue_4 (- 2.5e+03 _returnvalue_3))
  (bind _returnvalue_5 (/ _returnvalue_4 2.5e+03))
  (bind _returnvalue_6 (/ _returnvalue_5 1e+01))
  (bind _returnvalue_7 (- 0.1 _returnvalue_6))
  (Transformation|SetWorldScale3D (Variables|Default|GetRangeMesh) (Math|Vector|MakeVector _returnvalue_2 _returnvalue_2 _returnvalue_2))
  (Networking|SwitchHasAuthority
    (:Authority
      (CallFunction|SetChargeVariableInterface "NewEnumerator4" true _returnvalue_2 0.0 false true false)
      (Variables|Default|SetPoweredBatteryDurabilityToDecreasePerSecond _returnvalue_7)
      (Development|PrintString (Utilities|String|ToString(Float) _returnvalue_7)))))

(fn OnRepIsElevated
  (if (not (Networking|IsDedicatedServer))
    (Transformation|SetRelativeLocation (Variables|Default|GetMeshScene) (Math|Vector|MakeVector 0.0 0.0 (Math|Float|SelectFloat 2e+02 0.0 (Variables|Default|GetIsElevated))) false)))

(fn GetChargeVariableInterface
  (params (variableType :type E_ChargeVariableNames%20Enum :default "NewEnumerator0"))
  (Utilities|FlowControl|Sequence
    (:then_0
      (switch Utilities|FlowControl|Switch|SwitchonE_ChargeVariableNames variableType
        (:NewEnumerator0
          (LocalVariables|SetfinalFValue (Variables|ChargeBuff|GetcurrentChargeAmountStruct)))
        (:NewEnumerator1
          (LocalVariables|SetfinalFValue (Variables|ChargeBuff|GetcurrentChargeReceivedPerSecond)))
        (:NewEnumerator2
          (LocalVariables|SetfinalBValue (Variables|ChargeBuff|GetisReceiver)))
        (:NewEnumerator3
          (LocalVariables|SetfinalBValue (Variables|ChargeBuff|GetemitterIsActive)))
        (:NewEnumerator4
          (LocalVariables|SetfinalFValue (Variables|ChargeBuff|GetemitterRange)))
        (:NewEnumerator5
          (LocalVariables|SetfinalFValue (Variables|ChargeBuff|GetemitterChargeConsumedPerSecond)))
        (:NewEnumerator6
          (LocalVariables|SetfinalFValue (Variables|ChargeBuff|GetchargeEmittedPerSecond)))
        (:NewEnumerator7
          (LocalVariables|SetfinalFValue (Variables|ChargeBuff|GetchargeAddedToBatteryPerSecond)))
        (:NewEnumerator10
          (LocalVariables|SetfinalDValue (Variables|ChargeBuff|GetlastTimeChargeUpdatedOnTimer)))
        (:NewEnumerator13
          (LocalVariables|SetfinalFValue (Variables|Default|GetchargeConsumedByReceivers)))))
    (:then_1
      (return (LocalVariables|GetfinalFValue) (LocalVariables|GetfinalDValue) (LocalVariables|GetfinalBValue) 0))))

(fn GetNumBatteries
  (return 0))

(fn IPickupGetDisablePickupAfterTime
  (return (Variables|Default|GetDisablePickupAfterTime)))

(fn IPickupGetTimetoDisablePickup
  (return (Variables|Default|GetTimeToDisablePickup)))