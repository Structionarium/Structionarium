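; S+ Tek Light structure with configurable color, intensity, blink or fade, and automatic night-time switching.
; A team-only multi-use entry adds a buff that opens the settings UI, while pickup options come from S+ game settings.
; Authority-side timers check day/night and power or fuel, and step a lerp between primary and secondary colors.
; Visual updates skip dedicated servers, tinting the child emitter's lights and particles plus a dynamic emissive material.
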(event Custom|SetLightingEvent
  (params (Settings :type SP%20Light%20Settings%20Structure))
  (Variables|Default|SetLightSettings Settings false)
  (CallFunction|HandlePrimaryColor)
  (Networking|SwitchHasAuthority
    (:Authority
      (CallFunction|HandleIntervalStart)
      (if (Utilities|Struct|BreakSPLightSettings Settings)
        (Utilities|Time|SetTimerbyFunctionName 0 "CheckTime" 1e+01 true)
        (else
          (Utilities|Time|ClearTimerbyFunctionName 0 "CheckTime"))))))

(event Custom|HandleBeginPlayEvent
  (Utilities|FlowControl|Delay 2.0)
  (Utilities|FlowControl|Sequence
    (:then_0
      (if (Utilities|Struct|BreakSPLightSettings (Variables|Default|GetLightSettings))
        (Utilities|Time|SetTimerbyFunctionName 0 "CheckTime" 1e+01 true)))
    (:then_1
      (CallFunction|HandleIntervalStart))))

(event Custom|HandleIntervalLightEvent
  (Utilities|FlowControl|Sequence
    (:then_0
      (if (.doblink (Variables|Default|GetLightSettings))
        (Variables|Default|SetLerpValue (Math|Float|SelectFloat 1.0 0.0 (== (Variables|Default|GetLerpValue) 0.0)))
        (else
          (Variables|Default|SetLerpValue (+ (Variables|Default|GetLerpValue) (* (Variables|Default|GetLerpIncrement) (Variables|Default|GetLerpMultiplier))))
          (if (<= (Variables|Default|GetLerpValue) 0.0)
            (Variables|Default|SetLerpMultiplier 1.0)
            (elif (>= (Variables|Default|GetLerpValue) 1.0)
              (Variables|Default|SetLerpMultiplier -1.0))))))
    (:then_1
      (CallFunction|IntervalLightEvent (Variables|Default|GetLerpValue)))))

(event Custom|IntervalLightEvent
  (params (CurrentLerp :type Float%20%28single-precision%29))
  (bind _lightsettings (Variables|Default|GetLightSettings))
  (bind _returnvalue (Math|Float|Lerp (.a (.primarycolor _lightsettings)) (.a (.secondarycolor _lightsettings)) CurrentLerp))
  (bind _returnvalue_2 (Math|Color|Lerp(LinearColor) (Utilities|Struct|MakeLinearColor (.r (.primarycolor _lightsettings)) (.g (.primarycolor _lightsettings)) (.b (.primarycolor _lightsettings)) 1.0) (Utilities|Struct|MakeLinearColor (.r (.secondarycolor _lightsettings)) (.g (.secondarycolor _lightsettings)) (.b (.secondarycolor _lightsettings)) 1.0) CurrentLerp))
  (bind (_r _g _b) (Utilities|Struct|BreakLinearColor _returnvalue_2))
  (Utilities|SwitchNetAuthority
    (:PlayerServer
      _)
    (:Client
      _))
  (bind _asteklightemitter_c (Utilities|Casting|CastToTekLightEmitter (Variables|/Script/Engine.ChildActorComponent|GetChildActor (Variables|Default|GetActivatedEmitter))))
  (Rendering|Components|Light|SetLightColor (Variables|/Game/PrimalEarth/Test/TekLightEmitter.TekLightEmitter_C|GetSpotLight1 _asteklightemitter_c) (Utilities|Struct|MakeLinearColor _r _g _b 1.0))
  (Rendering|Components|Light|SetIntensity (Variables|/Game/PrimalEarth/Test/TekLightEmitter.TekLightEmitter_C|GetSpotLight1 _asteklightemitter_c) _returnvalue)
  (Effects|Components|ParticleSystem|SetVectorParameter (Variables|/Script/Engine.Emitter|GetParticleSystemComponent _asteklightemitter_c) "LightColor" (Math|Vector|MakeVector _r _g _b))
  (CallFunction|SetActiveMaterialProperties _r _g _b _returnvalue))

(event EventIPickupSetPickupSettings
  (params (DisablePickup :type Boolean) (DisablePickupWhenDamaged :type Boolean) (DisablePickupAfterTime :type Float%20%28single-precision%29) (TimeToDisablePickup :type Float%20%28double-precision%29))
  (Variables|Default|SetDisablePickup DisablePickup true)
  (Variables|Default|SetDisablePickupWhenDamaged DisablePickupWhenDamaged true)
  (Variables|Default|SetDisablePickupAfterTime DisablePickupAfterTime true)
  (Variables|Default|SetTimeToDisablePickup TimeToDisablePickup true))

(event EventBPContainerActivated
  (CallFunction|HandlePrimaryColor)
  (Networking|SwitchHasAuthority
    (:Authority
      (CallFunction|HandleIntervalStart))))

(event EventBPContainerDeactivated
  (Utilities|Time|ClearTimerbyFunctionName 0 "HandleIntervalLightEvent"))

(fn ConstructionScript
  (|CallParentFunction)
  (if (not (Variables|Default|GetbIsPreviewStructure))
    (bind _returnvalue (Rendering|Material|CreateDynamicMaterialInstance "/Game/PrimalEarth/TekTier/tek_light/Tek_Light_Colorize_MIC.Tek_Light_Colorize_MIC" :!class /Script/Engine.KismetMaterialLibrary))
    (Variables|Default|SetActiveMat _returnvalue)))

(fn BPGetMultiUseEntries
  (params (ForPC :type Player%20Controller%20Object%20Reference) (MultiUseEntries :type Array%20of%20Multi%20Use%20Entry%20Structures))
  (bind _entriesout (CallFunction|SPAddMenuEntries MultiUseEntries ForPC self (Variables|Default|GetDisablePickup) (Variables|Default|GetDisablePickupWhenDamaged) false false (Variables|Default|GetDisablePickupAfterTime) (Variables|Default|GetTimeToDisablePickup)))
  (if (== (Variables|/Script/Engine.Actor|GetTargetingTeam ForPC) (Variables|Default|GetTargetingTeam))
    (Utilities|Array|Add _entriesout (Utilities|Struct|MakeMultiUseEntry "[Change Settings]" 9001 -10 true (Math|Conversions|ToColor(LinearColor) (CallFunction|SPGetSpecialMenuColor)))))
  (return _entriesout))

(fn ReceiveBeginPlay
  (|CallParentFunction)
  (if (not (Variables|Default|GetbIsPreviewStructure))
    (CallFunction|HandlePrimaryColor)
    (Networking|SwitchHasAuthority
      (:Authority
        (CallFunction|SPSetPickUpSettings (Game|GetGameMode) self)
        (CallFunction|HandleBeginPlayEvent)))))

(fn BPTryMultiUse
  (params (ForPC :type Player%20Controller%20Object%20Reference) (UseIndex :type Integer))
  (switch int UseIndex
    (:Default
      _)
    (:9001
      (bind _asshooterplayercontroller (Utilities|Casting|CastToShooterPlayerController ForPC))
      (bind _returnvalue (Class|PrimalBuff|StaticAddBuff "/Game/Mods/StructuresPlusMod/_Buffs/Buff_StructuresPlus_Lights.Buff_StructuresPlus_Lights_C" (Class|ShooterPlayerController|GetPlayerCharacter _asshooterplayercontroller) 0 0 false))
      (bind _asbuff_structuresplus_lights_c (Utilities|Casting|CastToBuff_StructuresPlus_Lights _returnvalue))
      (Default|InitializeLightUI _asbuff_structuresplus_lights_c self (Variables|Default|GetLightSettings))))
  (return true))

(fn BPIsAllowedtoBuild
  (params (OutPlacementData :type Placement%20Data%20Structure%20%28by%20ref%29) (CurrentAllowedReason :type Integer))
  (return (Math|Integer|SelectInt 1 CurrentAllowedReason (== CurrentAllowedReason -9))))

(fn CheckTime
  (bind _lightsettings (Variables|Default|GetLightSettings))
  (bind (_postdawnoffset _preduskoffset) (Utilities|Struct|BreakSPLightSettings _lightsettings))
  (bind _isday (CallFunction|SPIsDayTime self _postdawnoffset _preduskoffset))
  (if (or (Math|Boolean|NotEqual(Boolean) _isday (Variables|Default|GetIsDaytime)) (Math|Boolean|Equal(Boolean) _isday (Variables|Default|GetbContainerActivated)))
    (Variables|Default|SetIsDaytime _isday)
    (if (Variables|Default|GetIsDaytime)
      (if (Variables|Default|GetbContainerActivated)
        (Class|PrimalStructure|SetContainerActive false))
      (elif (and (not (Variables|Default|GetbContainerActivated)) (or (Variables|Default|GetbIsPowered) (Variables|Default|GetbHasFuel)))
        (Class|PrimalStructure|SetContainerActive true)))))

(fn HandlePrimaryColor
  (bind _lightsettings (Variables|Default|GetLightSettings))
  (if (Variables|Default|GetbContainerActivated)
    (Utilities|SwitchNetAuthority
      (:PlayerServer
        _)
      (:Client
        _))
    (Rendering|Material|SetMaterial (Variables|Default|GetMyStaticMesh) 0 (Variables|Default|GetActiveMat))
    (bind _asteklightemitter_c (Utilities|Casting|CastToTekLightEmitter (Variables|/Script/Engine.ChildActorComponent|GetChildActor (Variables|Default|GetActivatedEmitter))))
    (Rendering|Components|Light|SetLightColor (Variables|/Game/PrimalEarth/Test/TekLightEmitter.TekLightEmitter_C|GetSpotLight1 _asteklightemitter_c) (Utilities|Struct|MakeLinearColor (.r (.primarycolor _lightsettings)) (.g (.primarycolor _lightsettings)) (.b (.primarycolor _lightsettings)) 1.0))
    (Rendering|Components|Light|SetIntensity (Variables|/Game/PrimalEarth/Test/TekLightEmitter.TekLightEmitter_C|GetSpotLight1 _asteklightemitter_c) (.a (.primarycolor _lightsettings)))
    (Effects|Components|ParticleSystem|SetVectorParameter (Variables|/Script/Engine.Emitter|GetParticleSystemComponent _asteklightemitter_c) "LightColor" (Math|Vector|MakeVector (.r (.primarycolor _lightsettings)) (.g (.primarycolor _lightsettings)) (.b (.primarycolor _lightsettings))))
    (CallFunction|SetActiveMaterialProperties (.r (.primarycolor _lightsettings)) (.g (.primarycolor _lightsettings)) (.b (.primarycolor _lightsettings)) (.a (.primarycolor _lightsettings)))))

(fn SetActiveMaterialProperties
  (params (R :type Float%20%28single-precision%29) (G :type Float%20%28single-precision%29) (B :type Float%20%28single-precision%29) (A :type Float%20%28single-precision%29))
  (bind _returnvalue (Math|Float|MakeLiteralFloat 5.0))
  (Rendering|Material|SetVectorParameterValue (Variables|Default|GetActiveMat) "Emissive - Color and Intensity" (Utilities|Struct|MakeLinearColor (+ (* R A) (* R _returnvalue)) (+ (* G A) (* G _returnvalue)) (+ (* B A) (* B _returnvalue)) 1.0) :!class /Script/Engine.MaterialInstanceDynamic))

(fn HandleIntervalStart
  (bind _lightsettings (Variables|Default|GetLightSettings))
  (if (and (Variables|Default|GetbContainerActivated) (.usesecondarycolor _lightsettings))
    (Variables|Default|SetLerpIncrement (/ 0.03333 (.secondaryinterval _lightsettings)))
    (Utilities|Time|SetTimerbyFunctionName 0 "HandleIntervalLightEvent" (Math|Float|SelectFloat (.secondaryinterval _lightsettings) 0.03333 (.doblink _lightsettings)) true)
    (else
      (Utilities|Time|ClearTimerbyFunctionName 0 "HandleIntervalLightEvent"))))

(fn IPickupGetDisablePickupAfterTime
  (return (Variables|Default|GetDisablePickupAfterTime)))

(fn IPickupGetTimetoDisablePickup
  (return (Variables|Default|GetTimeToDisablePickup)))