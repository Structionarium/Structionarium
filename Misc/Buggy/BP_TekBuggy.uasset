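; BP_TekBuggy is a Tek Buggy that same-team players can pick up as an inventory item.
; It adds a timed "Pick Up" multi-use entry, disabled and labeled as damaged when health is below maximum.
; On use, it gives the player a PrimalItem_TekBuggy, drops the buggy's inventory contents, clears death sound and FX, then destroys itself.
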(fn ConstructionScript
  (|CallParentFunction))

(fn BPGetMultiUseEntries
  (params (ForPC :type Player%20Controller%20Object%20Reference) (MultiUseEntries :type Array%20of%20Multi%20Use%20Entry%20Structures))
  (bind _mycharacterstatuscomponent (Variables|Default|GetMyCharacterStatusComponent))
  (bind _returnvalue (Class|PrimalCharacterStatusComponent|BPGetCurrentStatusValue _mycharacterstatuscomponent "Health"))
  (bind _returnvalue_2 (Class|PrimalCharacterStatusComponent|BPGetMaxStatusValue _mycharacterstatuscomponent "Health"))
  (bind _returnvalue_3 (Math|Float|Floor _returnvalue))
  (bind _returnvalue_4 (Math|Float|Floor _returnvalue_2))
  (bind _returnvalue_5 (< _returnvalue_3 _returnvalue_4))
  (if (== (Variables|/Script/Engine.Actor|GetTargetingTeam ForPC) (Variables|Default|GetTargetingTeam))
    (Utilities|Array|Add MultiUseEntries (Utilities|Struct|MakeMultiUseEntry (Utilities|String|SelectString "Pick Up (Damaged)" "Pick Up" _returnvalue_5) 9001 -1000 _returnvalue_5 1e+01 1e+01)))
  (return MultiUseEntries))

(fn BPTryMultiUse
  (params (ForPC :type Player%20Controller%20Object%20Reference) (UseIndex :type Integer))
  (bind _myinventorycomponent (Variables|Default|GetMyInventoryComponent))
  (switch int UseIndex
    (:Default
      _)
    (:9001
      (bind _asshooterplayercontroller (Utilities|Casting|CastToShooterPlayerController ForPC))
      (Class|PrimalItem|AddNewItem "/Game/Mods/StructuresPlusMod/Misc/Buggy/PrimalItem_TekBuggy.PrimalItem_TekBuggy_C" (Variables|/Script/ShooterGame.PrimalCharacter|GetMyInventoryComponent (Class|ShooterPlayerController|GetPlayerCharacter _asshooterplayercontroller)) false false 0.0 true 1 false 0.0 false)
      (for _array_element (Variables|/Script/ShooterGame.PrimalInventoryComponent|GetInventoryItems _myinventorycomponent)
        (Class|PrimalInventoryComponent|RemoveItem _myinventorycomponent (Variables|/Script/ShooterGame.PrimalItem|GetItemID _array_element) true false true false))
      (Variables|Default|SetDeathSound 0)
      (Variables|Default|SetDeathFX 0)
      (Actor|DestroyActor)))
  (return true))