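; Tek dino leash structure that, while active, movement-tethers team and baby dinos within a selectable radius.
; Activation or radius changes run an octree scan, and a detection sphere tethers dinos ridden by entering teammates.
; Nearby active leashes cap the allowed range or block activation, shown in the placement HUD and multi-use wheel.
; The server drives state; OnRep handlers update the radius visual, and team dino damage is nullified.
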(event OnComponentBeginOverlap(PlayerDetectSphere)
  (params (OtherActor :type Actor%20Object%20Reference) (OtherComp :type Primitive%20Component%20Object%20Reference) (OtherBodyIndex :type Integer) (bFromSweep :type Boolean) (SweepResult :type Hit%20Result%20Structure%20%28by%20ref%29))
  (if (CallFunction|GetIsActive)
    (bind _asshootercharacter (Utilities|Casting|CastToShooterCharacter OtherActor))
    (if (== (Variables|/Script/Engine.Actor|GetTargetingTeam _asshootercharacter) (Variables|Default|GetTargetingTeam))
      (Utilities|FlowControl|Sequence
        (:then_0
          (Utilities|IsValid (Variables|/Script/ShooterGame.ShooterCharacter|GetRidingDino _asshootercharacter)
            (:Is%20Valid
              (Class|Pawn|SetMovementTether (Variables|/Script/ShooterGame.ShooterCharacter|GetRidingDino _asshootercharacter) self (Variables|Default|GetEffectRadius) 0.0))))
        (:then_1
          (Utilities|IsValid (Variables|/Script/ShooterGame.PrimalCharacter|GetMountedDino _asshootercharacter)
            (:Is%20Valid
              (Class|Pawn|SetMovementTether (Variables|/Script/ShooterGame.PrimalCharacter|GetMountedDino _asshootercharacter) self (Variables|Default|GetEffectRadius) 0.0))))))))

(event Custom|HandleBeginPlayEvent
  (if (Variables|Default|GetActivated)
    (Utilities|FlowControl|Delay 1.0)
    (CallFunction|SetEffectRadius (Variables|Default|GetEffectRadius) true)))

(event Custom|AddTetherToDino
  (params (Dino :type Primal%20Dino%20Character%20Object%20Reference))
  (EventDispatchers|BindEventtoOnMovementTetherSet Dino (delegate Custom|MovementTetherEvent__DelegateSignature_Event))
  (Class|PrimalDinoCharacter|SetMovementTether Dino self (Variables|Default|GetEffectRadius) 0.0))

(event Custom|MovementTetherEvent__DelegateSignature_Event
  (params (Pawn :type Pawn%20Object%20Reference) (TetherObject :type Actor%20Object%20Reference))
  (bind _asprimaldinocharacter (Utilities|Casting|CastToPrimalDinoCharacter Pawn))
  (if (!= TetherObject self)
    (CallFunction|RemoveTetherfromDino _asprimaldinocharacter)))

(event Custom|RemoveTetherFromDino
  (params (Dino :type Primal%20Dino%20Character%20Object%20Reference))
  (EventDispatchers|UnbindEventfromOnMovementTetherSet Dino (delegate Custom|MovementTetherEvent__DelegateSignature_Event))
  (Utilities|Array|RemoveItem (Variables|Default|GetTetheredDinos) Dino))

(event EventIPickupSetPickupSettings
  (params (DisablePickup :type Boolean) (DisablePickupWhenDamaged :type Boolean) (DisablePickupAfterTime :type Float%20%28single-precision%29) (TimeToDisablePickup :type Float%20%28double-precision%29))
  (Variables|Default|SetDisablePickup DisablePickup true)
  (Variables|Default|SetDisablePickupWhenDamaged DisablePickupWhenDamaged true)
  (Variables|Default|SetDisablePickupAfterTime DisablePickupAfterTime true)
  (Variables|Default|SetTimeToDisablePickup TimeToDisablePickup true))

(fn ConstructionScript
  (|CallParentFunction)
  (if (not (Variables|Default|GetbIsPreviewStructure))
    (Collision|SetCollisionEnabled (Variables|Default|GetPlayerDetectSphere) "NoCollision")
    (if (not (Networking|IsDedicatedServer))
      (bind _returnvalue (Rendering|Material|CreateDynamicMaterialInstance "/Game/Extinction/Effects/Gameplay/DinoLeash/MIC_DinoLeash_Area.MIC_DinoLeash_Area" :!class /Script/Engine.KismetMaterialLibrary))
      (Variables|Default|SetRadialMaterialInstance _returnvalue)
      (Rendering|Material|SetMaterial (Variables|Default|GetEffectField) 0 _returnvalue))))

(fn BPGetMultiUseEntries
  (params (ForPC :type Player%20Controller%20Object%20Reference) (MultiUseEntries :type Array%20of%20Multi%20Use%20Entry%20Structures))
  (bind _returnvalue (Class|KismetSystemLibrary|MakeLiteralInteger 67101))
  (bind _activated (Variables|Default|GetActivated))
  (bind _returnvalue_2 (not _activated))
  (bind _entriesout (CallFunction|SPAddMenuEntries MultiUseEntries ForPC self (Variables|Default|GetDisablePickup) (Variables|Default|GetDisablePickupWhenDamaged) false false (Variables|Default|GetDisablePickupAfterTime) (Variables|Default|GetTimeToDisablePickup)))
  (Utilities|FlowControl|Sequence
    (:then_0
      (if (== (Variables|/Script/Engine.Actor|GetTargetingTeam ForPC) (Variables|Default|GetTargetingTeam))
        (bind _maxsetting (CallFunction|GetMaximumAllowedRadius))
        (LocalVariables|SetMaxSetting _maxsetting)
        (Utilities|Array|Add _entriesout (Utilities|Struct|MakeMultiUseEntry (Utilities|String|SelectString "Deactivate" (Utilities|String|SelectString "Can't Activate (Interference)" "Activate" (< (LocalVariables|GetMaxSetting) 0)) _activated) 67100 (Math|Integer|SelectInt 1000 -1 _returnvalue_2) (and _returnvalue_2 (< (LocalVariables|GetMaxSetting) 0)) (Math|Conversions|ToColor(LinearColor) (Variables|Default|GetDisabledWheelColor)) 1.0 1.0))
        (bind _returnvalue_3 (Class|PrimalGameData|BPGetGameData))
        (Utilities|Array|Add _entriesout (Utilities|Struct|MakeMultiUseEntry "[Change Range]" _returnvalue -2 true true true (Variables|/Script/ShooterGame.PrimalGameData|GetWheelFolderColor _returnvalue_3)))
        (for (_array_element _array_index) (Variables|Default|GetSettingNames)
          (Utilities|Array|Add _entriesout (Utilities|Struct|MakeMultiUseEntry _array_element (+ _array_index 67110) (+ _array_index 1) (and (< (LocalVariables|GetMaxSetting) _array_index) (Variables|Default|GetActivated)) (== _array_index (Variables|Default|GetRadiusSetting)) _returnvalue (Math|Conversions|ToColor(LinearColor) (Variables|Default|GetDisabledWheelColor)) (Variables|/Script/ShooterGame.PrimalGameData|GetWheelFolderColor _returnvalue_3))))
        (Utilities|Array|Add _entriesout (Utilities|Struct|MakeMultiUseEntry "[Back]" 88810 999 true true true _returnvalue (Variables|/Script/ShooterGame.PrimalGameData|GetWheelBackColor _returnvalue_3)))
        (if (Variables|Default|GetActivated)
          (Utilities|Array|Add _entriesout (Utilities|Struct|MakeMultiUseEntry (Utilities|String|SelectString "Show Radius" "Hide Radius" (Variables|Default|GetHideRadiusEffect)) 67099 5000)))))
    (:then_1
      (return _entriesout))))

(fn BPTryMultiUse
  (params (ForPC :type Player%20Controller%20Object%20Reference) (UseIndex :type Integer))
  (Utilities|FlowControl|Sequence
    (:then_0
      (if (== (Variables|/Script/Engine.Actor|GetTargetingTeam ForPC) (Variables|Default|GetTargetingTeam))
        (switch int UseIndex
          (:Default
            (switch int UseIndex
              (:67110
                (Variables|Default|SetRadiusSetting 0 true))
              (:67111
                (Variables|Default|SetRadiusSetting 1 true))
              (:67112
                (Variables|Default|SetRadiusSetting 2 true))
              (:67113
                (Variables|Default|SetRadiusSetting 3 true)))
            (CallFunction|SetEffectRadius (Utilities|Array|Get(acopy) (Variables|Default|GetRadiusOptions) (Variables|Default|GetRadiusSetting)) false))
          (:67099
            (Variables|Default|SetHideRadiusEffect (not (Variables|Default|GetHideRadiusEffect)) true))
          (:67100
            (CallFunction|Activate (not (Variables|Default|GetActivated)))))))
    (:then_1
      (return false))))

(fn OnRepActivated
  (if (not (Networking|IsDedicatedServer))
    (Class|KismetSystemLibrary|CanRunCosmeticEvents
      (:Yes
        (CallFunction|UpdateVisibility)))))

(fn Activate
  (params (Activated :type Boolean))
  (bind _tethereddinos (Variables|Default|GetTetheredDinos))
  (bind _playerdetectsphere (Variables|Default|GetPlayerDetectSphere))
  (bind _item (Utilities|Array|Get(acopy) _tethereddinos))
  (Class|KismetSystemLibrary|IsRunningonServer
    (:Yes
      (Variables|Default|SetActivated Activated true)
      (if (CallFunction|GetIsActive)
        (Collision|SetCollisionEnabled (Variables|Default|GetPlayerDetectSphere) "QueryAndPhysics")
        (bind _maxsetting (CallFunction|GetMaximumAllowedRadius))
        (Variables|Default|SetRadiusSetting (Math|Integer|Min(Integer) _maxsetting (Variables|Default|GetRadiusSetting)) true)
        (CallFunction|SetEffectRadius (Utilities|Array|Get(acopy) (Variables|Default|GetRadiusOptions) (Variables|Default|GetRadiusSetting)) true)
        (else
          (while (> (Utilities|Array|Length (Variables|Default|GetTetheredDinos)) 0)
            (if (and (Utilities|IsValid (Variables|/Script/Engine.Pawn|GetTetherActor _item)) (Utilities|IsValid _item))
              (Class|PrimalDinoCharacter|ClearMovementTether _item)
              (else
                (Utilities|Array|RemoveIndex _tethereddinos))))
          (Collision|SetCollisionEnabled _playerdetectsphere "NoCollision")
          (Components|Sphere|SetSphereRadius _playerdetectsphere 1.0 false)))
      (return))))

(fn BPPlacedStructure
  (params (ForPC :type Player%20Controller%20Object%20Reference))
  (bind _maxsetting (CallFunction|GetMaximumAllowedRadius))
  (CallFunction|Activate (>= _maxsetting 0)))

(fn BPIsAllowedtoBuild
  (params (OutPlacementData :type Placement%20Data%20Structure%20%28by%20ref%29) (CurrentAllowedReason :type Integer))
  (return (Math|Integer|SelectInt 1 CurrentAllowedReason (== CurrentAllowedReason -9))))

(fn BPClientDoMultiUse
  (params (ForPC :type Player%20Controller%20Object%20Reference) (ClientUseIndex :type Integer))
  (bind _returnvalue (Class|KismetSystemLibrary|MakeLiteralInteger 67101))
  (Utilities|FlowControl|Sequence
    (:then_0
      (bind _asshooterplayercontroller (Utilities|Casting|CastToShooterPlayerController ForPC))
      (if (== ClientUseIndex _returnvalue)
        (Class|ShooterPlayerController|SetMultiUseWheelCategory _asshooterplayercontroller _returnvalue)))
    (:then_1
      (|CallParentFunction ForPC ClientUseIndex))))

(fn OnRepEffectRadius
  (if (Variables|Default|GetActivated)
    (Transformation|SetWorldScale3D (Variables|Default|GetEffectField) (Math|Conversions|ToVector(Float) (/ (Variables|Default|GetEffectRadius) (Variables|Default|GetEffectScalar))))
    (if (not (Networking|IsDedicatedServer))
      (Rendering|Material|SetScalarParameterValue (Variables|Default|GetRadialMaterialInstance) "NearDistanceFade" (+ (Variables|Default|GetEffectRadius) 3e+03) :!class /Script/Engine.MaterialInstanceDynamic))))

(fn SetEffectRadius
  (params (EffectRadius :type Float%20%28single-precision%29) (ForceSet :type Boolean))
  (Class|KismetSystemLibrary|IsRunningonServer
    (:Yes
      (if (or ForceSet (!= (Variables|Default|GetEffectRadius) EffectRadius))
        (Variables|Default|SetEffectRadius EffectRadius true)
        (if (CallFunction|GetIsActive)
          (for _array_element (Variables|Default|GetTetheredDinos)
            (Class|Pawn|SetMovementTether _array_element self (Variables|Default|GetEffectRadius) 0.0))
          (CallFunction|TetherDinosinRadius)
          (Transformation|SetWorldScale3D (Variables|Default|GetEffectField) (Math|Conversions|ToVector(Float) (/ (Variables|Default|GetEffectRadius) (Variables|Default|GetEffectScalar))))
          (return))))))

(fn TetherDinosinRadius
  (Utilities|FlowControl|Sequence
    (:then_0
      (bind _returnvalue (Class|VictoryCore|ServerOctreeOverlapActorsClass (Class|Actor|GetWorld) (Transformation|GetActorLocation) (Variables|Default|GetEffectRadius) "SPATIALNETWORKEDACTORS" "/Script/ShooterGame.PrimalDinoCharacter" false))
      (for _array_element _returnvalue
        (bind _asprimaldinocharacter (Utilities|Casting|CastToPrimalDinoCharacter _array_element))
        (if (and (or (== (Variables|/Script/Engine.Actor|GetTargetingTeam _asprimaldinocharacter) (Variables|Default|GetTargetingTeam)) (< (Variables|/Script/ShooterGame.PrimalDinoCharacter|GetBabyAge _asprimaldinocharacter) 1.0)) (< (Utilities|Array|FindItem (Variables|Default|GetTetheredDinos) _asprimaldinocharacter) 0))
          (CallFunction|AddTethertoDino _asprimaldinocharacter)
          (Utilities|Array|Insert (Variables|Default|GetTetheredDinos) _asprimaldinocharacter))))
    (:then_1
      (Components|Sphere|SetSphereRadius (Variables|Default|GetPlayerDetectSphere) (/ (Variables|Default|GetEffectRadius) (Variables|Default|GetScaleFactor)) true)
      (return))))

(fn GetMaximumAllowedRadius
  (bind _returnvalue (Transformation|GetActorLocation))
  (LocalVariables|SetIndex (- (Utilities|Array|Length (Variables|Default|GetRadiusOptions)) 1))
  (LocalVariables|SetMax (Utilities|Array|Get(acopy) (Variables|Default|GetRadiusOptions) (LocalVariables|GetIndex)))
  (Utilities|FlowControl|Sequence
    (:then_0
      (Class|KismetSystemLibrary|IsRunningonServer
        (:Yes
          ;[1 1 1] Check Server
          (bind _returnvalue_2 (Class|VictoryCore|ServerOctreeOverlapActorsClass (Class|Actor|GetWorld) _returnvalue (+ (LocalVariables|GetMax) (Utilities|Array|Get(acopy) (Variables|Default|GetRadiusOptions))) "STRUCTURES" "/Game/Extinction/Structures/DinoLeash/Structure_DinoLeash.Structure_DinoLeash_C" true))
          (for _array_element _returnvalue_2
            (if (!= _array_element self)
              (bind (_isactive _effectradius) (CallFunction|GetNearbyLeashDetails _array_element))
              (if _isactive
                (LocalVariables|SetMax (Math|Float|Min(Float) (- (Utilities|Distance2D (Transformation|GetActorLocation) (Transformation|GetActorLocation _array_element)) _effectradius) (LocalVariables|GetMax)))))))
        (:No
          ;[1 1 1] Check Client
          (Utilities|Array|Add (LocalVariables|GetIgnore) self)
          (bind _outactors (Class|KismetSystemLibrary|SphereOverlapActorsSimple _returnvalue (+ (LocalVariables|GetMax) (Utilities|Array|Get(acopy) (Variables|Default|GetRadiusOptions))) "ObjectTypeQuery9" (Utilities|GetClass self) (LocalVariables|GetIgnore)))
          (for _array_element_2 _outactors
            (if (!= _array_element_2 self)
              (bind (_isactive_2 _effectradius_2) (CallFunction|GetNearbyLeashDetails _array_element_2))
              (if _isactive_2
                (LocalVariables|SetMax (Math|Float|Min(Float) (- (Utilities|Distance2D (Transformation|GetActorLocation) (Transformation|GetActorLocation _array_element_2)) _effectradius_2) (LocalVariables|GetMax)))))))))
    (:then_1
      (while (and (>= (LocalVariables|GetIndex) 0) (> (Utilities|Array|Get(acopy) (Variables|Default|GetRadiusOptions) (LocalVariables|GetIndex)) (LocalVariables|GetMax)))
        (LocalVariables|SetIndex (- (LocalVariables|GetIndex) 1)))
      (return (LocalVariables|GetMax) (LocalVariables|GetIndex)))))

(fn BlueprintDrawPreviewHUD
  (params (HUD :type Shooter%20HUD%20Object%20Reference) (CenterX :type Float%20%28single-precision%29) (CenterY :type Float%20%28single-precision%29))
  (bind _canvas (Variables|/Script/Engine.HUD|GetCanvas HUD))
  (bind _maxsetting (CallFunction|GetMaximumAllowedRadius))
  (Class|Canvas|SetDrawColor _canvas (Math|Conversions|ToColor(LinearColor) (Math|Color|SelectColor "(R=0.000000,G=1.000000,B=0.000000,A=0.750000)" "(R=1.000000,G=0.000000,B=0.000000,A=0.750000)" (>= _maxsetting 0))))
  (Class|Canvas|BPDrawTextCentered _canvas (Variables|/Script/ShooterGame.ShooterHUD|GetNormalFont HUD) (Utilities|String|SelectString (Utilities|String|ToString(Text) (Utilities|Text|FormatText "Max Range: {0}" (Utilities|Text|ToText(String) (Utilities|Array|Get(acopy) (Variables|Default|GetSettingNames) _maxsetting)))) "Interference" (>= _maxsetting 0)) CenterX (+ CenterY 25.0) 1.0 1.0 true true))

(fn BPContainerActivated
  (bind _maxsetting (CallFunction|GetMaximumAllowedRadius))
  (CallFunction|Activate (and (Variables|Default|GetActivated) (>= _maxsetting 0))))

(fn BPContainerDeactivated
  (CallFunction|Activate (Variables|Default|GetActivated)))

(fn GetIsActive
  (return (Variables|Default|GetActivated)))

(fn ReceiveBeginPlay
  (|CallParentFunction)
  (if (not (Variables|Default|GetbIsPreviewStructure))
    (Networking|SwitchHasAuthority
      (:Authority
        (Utilities|FlowControl|Sequence
          (:then_0
            (CallFunction|SPSetPickUpSettings (Game|GetGameMode) self)
            (Utilities|SwitchNetAuthority
              (:PlayerServer
                (CallFunction|OnRepActivated)
                (CallFunction|OnRepEffectRadius)
                (CallFunction|OnRepHideRadiusEffect))))
          (:then_1
            (CallFunction|HandleBeginPlayEvent)))))))

(fn UpdateVisibility
  (bind _effectfield (Variables|Default|GetEffectField))
  (Utilities|FlowControl|Sequence
    (:then_0
      (Transformation|SetWorldScale3D _effectfield (Math|Conversions|ToVector(Float) (/ (Variables|Default|GetEffectRadius) (Variables|Default|GetEffectScalar))))
      (if (Variables|Default|GetHideRadiusEffect)
        (Rendering|SetVisibility _effectfield false true)
        (else
          (Rendering|SetVisibility _effectfield (CallFunction|GetIsActive) true))))
    (:then_1
      (return))))

(fn BPAdjustDamage
  (params (IncomingDamage :type Float%20%28single-precision%29) (TheDamageEvent :type Damage%20Event%20Structure) (EventInstigator :type Controller%20Object%20Reference) (DamageCauser :type Actor%20Object%20Reference) (bIsPointDamage :type Boolean) (PointHitInfo :type Hit%20Result%20Structure))
  (LocalVariables|SetDamage IncomingDamage)
  (Utilities|FlowControl|Sequence
    (:then_0
      (bind _asprimaldinocharacter (Utilities|Casting|CastToPrimalDinoCharacter DamageCauser))
      (if (== (Variables|/Script/Engine.Actor|GetTargetingTeam _asprimaldinocharacter) (Variables|Default|GetTargetingTeam))
        (LocalVariables|SetDamage 0.0)))
    (:then_1
      (if (== (.HitComponent (Collision|BreakHitResult PointHitInfo)) (Variables|Default|GetPlayerDetectSphere))
        (LocalVariables|SetDamage 0.0)))
    (:then_2
      (return (LocalVariables|GetDamage)))))

(fn OnRepHideRadiusEffect
  (if (not (Networking|IsDedicatedServer))
    (Rendering|SetVisibility (Variables|Default|GetEffectField) (not (Variables|Default|GetHideRadiusEffect)) false)))

(fn GetNearbyLeashDetails
  (params (LeashRef :type Actor%20Object%20Reference))
  (Utilities|FlowControl|Sequence
    (:then_0
      (bind _asstructure_dinoleash_c (Utilities|Casting|CastToStructure_DinoLeash LeashRef)
        (:then
          (if (and (Variables|/Game/Extinction/Structures/DinoLeash/Structure_DinoLeash.Structure_DinoLeash_C|GetActivated _asstructure_dinoleash_c) (Variables|/Script/ShooterGame.PrimalStructureItemContainer|GetbIsPowered _asstructure_dinoleash_c))
            (LocalVariables|SetbIsOtherLeashActive true)
            (LocalVariables|SetOtherLeashRadius (Variables|/Game/Extinction/Structures/DinoLeash/Structure_DinoLeash.Structure_DinoLeash_C|GetEffectRadius _asstructure_dinoleash_c))))
        (:CastFailed
          (bind _asbp_leashtek_c (Utilities|Casting|CastToBP_LeashTek LeashRef))
          (if (Variables|BP_LeashTek_C|GetActivated _asbp_leashtek_c)
            (LocalVariables|SetbIsOtherLeashActive true)
            (LocalVariables|SetOtherLeashRadius (Variables|BP_LeashTek_C|GetEffectRadius _asbp_leashtek_c))))))
    (:then_1
      (return (LocalVariables|GetbIsOtherLeashActive) (LocalVariables|GetOtherLeashRadius)))))

(fn IPickupGetDisablePickupAfterTime
  (return (Variables|Default|GetDisablePickupAfterTime)))

(fn IPickupGetTimetoDisablePickup
  (return (Variables|Default|GetTimeToDisablePickup)))