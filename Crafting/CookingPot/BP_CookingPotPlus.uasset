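; BP_CookingPotPlus is an enhanced cooking pot structure with configurable pickup, team locking and an auto-crafting toggle.
; On BeginPlay the authority reads game-mode settings for pickup, slot count and crafting speed, with rep notifies updating the inventory component.
; Multi-use entries combine shared SP pickup options with the auto-craft toggle, while activation is limited to the owning team when locked.
; The build check overrides one specific placement failure code.
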(event EventIPickupSetPickupSettings
  (params (DisablePickup :type Boolean) (DisablePickupWhenDamaged :type Boolean) (DisablePickupAfterTime :type Float%20%28single-precision%29) (TimeToDisablePickup :type Float%20%28double-precision%29))
  (Variables|Default|SetDisablePickup DisablePickup true)
  (Variables|Default|SetDisablePickupWhenDamaged DisablePickupWhenDamaged true)
  (Variables|Default|SetDisablePickupAfterTime DisablePickupAfterTime true)
  (Variables|Default|SetTimeToDisablePickup TimeToDisablePickup true))

(fn ConstructionScript
  (|CallParentFunction))

(fn BPIsAllowedtoBuild
  (params (OutPlacementData :type Placement%20Data%20Structure%20%28by%20ref%29) (CurrentAllowedReason :type Integer))
  (return (Math|Integer|SelectInt 1 CurrentAllowedReason (== CurrentAllowedReason -9))))

(fn BPGetMultiUseEntries
  (params (ForPC :type Player%20Controller%20Object%20Reference) (MultiUseEntries :type Array%20of%20Multi%20Use%20Entry%20Structures))
  (bind _entriesout (CallFunction|SPAddMenuEntries MultiUseEntries ForPC self (Variables|Default|GetDisablePickup) (Variables|Default|GetDisablePickupWhenDamaged) false false (Variables|Default|GetDisablePickupAfterTime) (Variables|Default|GetTimeToDisablePickup)))
  (Utilities|FlowControl|Sequence
    (:then_0
      (bind _returnvalue (Class|PrimalStructure|AllowStructureAccess ForPC))
      (if _returnvalue
        (Utilities|Array|Add _entriesout (Utilities|Struct|MakeMultiUseEntry (Utilities|String|SelectString "Enable Auto Crafting" "Disable Auto Crafting" (Variables|Default|GetDisableAutoCrafting)) 9001 -1020 true true))))
    (:then_1
      (return _entriesout))))

(fn OnRepInventorySlots
  (Variables|/Script/ShooterGame.PrimalInventoryComponent|SetMaxInventoryItems (Variables|Default|GetMyInventoryComponent) (Variables|Default|GetInventorySlots)))

(fn BPTryMultiUse
  (params (ForPC :type Player%20Controller%20Object%20Reference) (UseIndex :type Integer))
  (Utilities|FlowControl|Sequence
    (:then_0
      (switch int UseIndex
        (:Default
          (switch int UseIndex
            (:9001
              (Variables|Default|SetDisableAutoCrafting (not (Variables|Default|GetDisableAutoCrafting)) true))))
        (:601
          (Variables|Default|SetIsUnlocked (not (Variables|Default|GetbIsLocked))))))
    (:then_1
      (return true))))

(fn BPCanbeActivatedbyPlayer
  (params (PC :type Shooter%20Player%20Controller%20Object%20Reference))
  (return (or (== (Variables|/Script/Engine.Actor|GetTargetingTeam PC) (Variables|Default|GetTargetingTeam)) (not (Variables|Default|GetbIsLocked)))))

(fn ReceiveBeginPlay
  (bind _returnvalue (Game|GetGameMode))
  (|CallParentFunction)
  (if (not (Variables|Default|GetbIsPreviewStructure))
    (Networking|SwitchHasAuthority
      (:Authority
        (Utilities|FlowControl|Sequence
          (:then_0
            (CallFunction|SPSetPickUpSettings _returnvalue self))
          (:then_1
            (bind _slotcount (CallFunction|SPGetInventorySlotSetting _returnvalue "CookingPotSlotCount" 25))
            (Variables|Default|SetInventorySlots _slotcount true))
          (:then_2
            (Variables|Default|SetbIsLocked (not (Variables|Default|GetIsUnlocked)) true))
          (:then_3
            (bind _value (CallFunction|SPGetFloatIniOption _returnvalue "CookingPotCraftingSpeed" 1.0 1e+02))
            (Variables|/Script/ShooterGame.PrimalInventoryComponent|SetCraftingItemSpeed (Variables|Default|GetMyInventoryComponent) _value))
          (:then_4
            (Utilities|SwitchNetAuthority
              (:PlayerServer
                (CallFunction|OnRepDisableAutoCrafting)))))))))

(fn OnRepDisableAutoCrafting
  (Variables|/Script/ShooterGame.PrimalInventoryComponent|SetbCheckForAutoCraftBlueprints (Variables|Default|GetMyInventoryComponent) (not (Variables|Default|GetDisableAutoCrafting))))

(fn IPickupGetDisablePickupAfterTime
  (return (Variables|Default|GetDisablePickupAfterTime)))

(fn IPickupGetTimetoDisablePickup
  (return (Variables|Default|GetTimeToDisablePickup)))