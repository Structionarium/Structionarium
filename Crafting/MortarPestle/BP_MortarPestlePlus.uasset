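; S+ Mortar and Pestle crafting structure with configurable pickup, slot count and crafting speed.
; On begin play the authority loads those settings through SP helpers using the game mode; an InventorySlots RepNotify sets the inventory's item limit.
; SP menu entries receive the pickup state exposed via IPickup.
; Placement turns rejection reason -9 into 1 and drops the floor requirement when the S+ global actor says so.
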(event EventIPickupSetPickupSettings
  (params (DisablePickup :type Boolean) (DisablePickupWhenDamaged :type Boolean) (DisablePickupAfterTime :type Float%20%28single-precision%29) (TimeToDisablePickup :type Float%20%28double-precision%29))
  (Variables|Default|SetDisablePickup DisablePickup true)
  (Variables|Default|SetDisablePickupWhenDamaged DisablePickupWhenDamaged true)
  (Variables|Default|SetDisablePickupAfterTime DisablePickupAfterTime true)
  (Variables|Default|SetTimeToDisablePickup TimeToDisablePickup true))

(fn ConstructionScript
  (|CallParentFunction)
  (if (Variables|Default|GetbIsPreviewStructure)
    _
    (else
      (Networking|SwitchHasAuthority
        (:Authority
          _))))
  (bind _globalactor (CallFunction|SPGetGlobalActor self))
  (Utilities|IsValid _globalactor
    (:Is%20Valid
      (if (Variables|/Game/Mods/StructuresPlusMod/SPlusGlobalActor.SPlusGlobalActor_C|GetRemoveFloorRequirement _globalactor)
        (Variables|Default|SetbRequiresPlacementOnStructureFloors false)))))

(fn BPIsAllowedtoBuild
  (params (OutPlacementData :type Placement%20Data%20Structure%20%28by%20ref%29) (CurrentAllowedReason :type Integer))
  (return (Math|Integer|SelectInt 1 CurrentAllowedReason (== CurrentAllowedReason -9))))

(fn BPGetMultiUseEntries
  (params (ForPC :type Player%20Controller%20Object%20Reference) (MultiUseEntries :type Array%20of%20Multi%20Use%20Entry%20Structures))
  (bind _entriesout (CallFunction|SPAddMenuEntries MultiUseEntries ForPC self (Variables|Default|GetDisablePickup) (Variables|Default|GetDisablePickupWhenDamaged) false false (Variables|Default|GetDisablePickupAfterTime) (Variables|Default|GetTimeToDisablePickup)))
  (return _entriesout))

(fn BPTryMultiUse
  (params (ForPC :type Player%20Controller%20Object%20Reference) (UseIndex :type Integer))
  (switch int UseIndex
    (:Default
      _)
    (:601
      (Variables|Default|SetIsUnlocked (not (Variables|Default|GetbIsLocked)))))
  (return (Math|Boolean|ORBoolean (== UseIndex 602) (== UseIndex 604) (== UseIndex 699))))

(fn OnRepInventorySlots
  (Variables|/Script/ShooterGame.PrimalInventoryComponent|SetMaxInventoryItems (Variables|Default|GetMyInventoryComponent) (Variables|Default|GetInventorySlots)))

(fn ReceiveBeginPlay
  (bind _returnvalue (Game|GetGameMode))
  (bind _myinventorycomponent (Variables|Default|GetMyInventoryComponent))
  (|CallParentFunction)
  (if (not (Variables|Default|GetbIsPreviewStructure))
    (Variables|/Script/ShooterGame.PrimalInventoryComponent|SetInventoryNameOverride _myinventorycomponent "S+ Mortar and Pestle")
    (Variables|/Script/ShooterGame.PrimalInventoryComponent|SetAbsoluteMaxInventoryItems _myinventorycomponent 10000)
    (Networking|SwitchHasAuthority
      (:Authority
        (Utilities|FlowControl|Sequence
          (:then_0
            (CallFunction|SPSetPickUpSettings _returnvalue self))
          (:then_1
            (bind _slotcount (CallFunction|SPGetInventorySlotSetting _returnvalue "MortarAndPestleSlotCount" 50))
            (Variables|Default|SetInventorySlots _slotcount true))
          (:then_2
            (Variables|Default|SetbIsLocked (not (Variables|Default|GetIsUnlocked)) true))
          (:then_3
            (bind _value (CallFunction|SPGetFloatIniOption _returnvalue "MortarAndPestleCraftingSpeed" 1.0 1e+02))
            (Variables|/Script/ShooterGame.PrimalInventoryComponent|SetCraftingItemSpeed (Variables|Default|GetMyInventoryComponent) _value)))))))

(fn IPickupGetDisablePickupAfterTime
  (return (Variables|Default|GetDisablePickupAfterTime)))

(fn IPickupGetTimetoDisablePickup
  (return (Variables|Default|GetTimeToDisablePickup)))