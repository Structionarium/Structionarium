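; Triangular Tek elevator ceiling structure that teleports a player standing on it to the nearest matching elevator above or below.
; A trigger box enables client input, so jump, crouch or thumbstick presses send Up/Down commands to the server, where shared SP helper functions check access, find the destination and teleport.
; Team members can toggle a lock and an opacity setting that shows or hides the bottom mesh.
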(event OnComponentBeginOverlap(CheckBox)
  (params (OtherActor :type Actor%20Object%20Reference) (OtherComp :type Primitive%20Component%20Object%20Reference) (OtherBodyIndex :type Integer) (bFromSweep :type Boolean) (SweepResult :type Hit%20Result%20Structure%20%28by%20ref%29))
  (bind _islocked (Variables|Default|GetIsLocked))
  (if (not (Networking|IsDedicatedServer))
    (bind _asprimalcharacter (Utilities|Casting|CastToPrimalCharacter OtherActor))
    (bind _returnvalue (Class|PrimalCharacter|IsAlliedwithOtherTeam _asprimalcharacter (Variables|Default|GetTargetingTeam)))
    (if (or (and _returnvalue _islocked) (not _islocked))
      (bind _returnvalue_2 (Class|Actor|GetOwnerController _asprimalcharacter))
      (Input|EnableInput _returnvalue_2))))

(event OnComponentEndOverlap(CheckBox)
  (params (OtherActor :type Actor%20Object%20Reference) (OtherComp :type Primitive%20Component%20Object%20Reference) (OtherBodyIndex :type Integer))
  (if (not (Networking|IsDedicatedServer))
    (bind _asprimalcharacter (Utilities|Casting|CastToPrimalCharacter OtherActor))
    (bind _returnvalue (Class|Actor|GetOwnerController _asprimalcharacter))
    (Input|DisableInput _returnvalue)))

(event Custom|HandleTeleport
  (params (Actor :type Actor%20Object%20Reference) (Location :type Vector))
  (Transformation|SetActorLocation Actor Location false))

(event Input|ActionEvents|InputActionJump
  (bind _returnvalue (Game|GetPlayerController 0))
  (:Pressed
    (if (== (Components|GetOwner (Class|CharacterMovementComponent|GetMovementBase (Variables|/Script/Engine.Character|GetCharacterMovement (Game|GetPlayerCharacter 0)))) self)
      (Class|PlayerController|ClientSendNetExecCommandtoServer _returnvalue self "Up" (Utilities|Struct|MakeBPNetExecParams) true)
      (else
        (Input|DisableInput _returnvalue)))))

(event Input|ActionEvents|InputActionCrouch
  (bind _returnvalue (Game|GetPlayerController 0))
  (:Pressed
    (if (== (Components|GetOwner (Class|CharacterMovementComponent|GetMovementBase (Variables|/Script/Engine.Character|GetCharacterMovement (Game|GetPlayerCharacter 0)))) self)
      (Class|PlayerController|ClientSendNetExecCommandtoServer _returnvalue self "Down" (Utilities|Struct|MakeBPNetExecParams) true)
      (else
        (Input|DisableInput _returnvalue)))))

(event Input|GamepadEvents|GamepadRightThumbstick
  (bind _returnvalue (Game|GetPlayerController 0))
  (:Pressed
    (if (== (Components|GetOwner (Class|CharacterMovementComponent|GetMovementBase (Variables|/Script/Engine.Character|GetCharacterMovement (Game|GetPlayerCharacter 0)))) self)
      (Class|PlayerController|ClientSendNetExecCommandtoServer _returnvalue self "Down" (Utilities|Struct|MakeBPNetExecParams) true)
      (else
        (Input|DisableInput _returnvalue)))))

(event Input|GamepadEvents|GamepadLeftThumbstick
  (bind _returnvalue (Game|GetPlayerController 0))
  (:Pressed
    (if (== (Components|GetOwner (Class|CharacterMovementComponent|GetMovementBase (Variables|/Script/Engine.Character|GetCharacterMovement (Game|GetPlayerCharacter 0)))) self)
      (Class|PlayerController|ClientSendNetExecCommandtoServer _returnvalue self "Up" (Utilities|Struct|MakeBPNetExecParams) true)
      (else
        (Input|DisableInput _returnvalue)))))

(fn ConstructionScript
  (|CallParentFunction))

(fn BPGetMultiUseEntries
  (params (ForPC :type Player%20Controller%20Object%20Reference) (MultiUseEntries :type Array%20of%20Multi%20Use%20Entry%20Structures))
  (bind _returnvalue (|CallParentFunction ForPC MultiUseEntries))
  (Utilities|FlowControl|Sequence
    (:then_0
      (if (== (Variables|/Script/Engine.Actor|GetTargetingTeam ForPC) (Variables|Default|GetTargetingTeam))
        (Utilities|Array|Add _returnvalue (Utilities|Struct|MakeMultiUseEntry (Utilities|String|SelectString "Unlock" "Lock" (Variables|Default|GetIsLocked)) 9100 -1500))
        (Utilities|Array|Add _returnvalue (Utilities|Struct|MakeMultiUseEntry (Utilities|String|SelectString "Make Transparent" "Make Opaque" (Variables|Default|GetIsOpaque)) 9101 -1250))))
    (:then_1
      (return _returnvalue))))

(fn BPTryMultiUse
  (params (ForPC :type Player%20Controller%20Object%20Reference) (UseIndex :type Integer))
  (bind _returnvalue (|CallParentFunction ForPC UseIndex))
  (Utilities|FlowControl|Sequence
    (:then_0
      (switch int UseIndex
        (:9100
          (Variables|Default|SetIsLocked (not (Variables|Default|GetIsLocked)) true))
        (:9101
          (Variables|Default|SetIsOpaque (not (Variables|Default|GetIsOpaque)) true))))
    (:then_1
      (return _returnvalue))))

(fn BPServerHandleNetExecCommand
  (params (FromPC :type Player%20Controller%20Object%20Reference) (CommandName :type Name :default "None") (ExecParams :type BP%20Net%20Exec%20Params%20Structure%20%28by%20ref%29))
  (Utilities|FlowControl|Sequence
    (:then_0
      (switch name CommandName
        (:Default
          (|CallParentFunction FromPC CommandName ExecParams))
        (:Up
          (LocalVariables|SetUp true)
          (if (CallFunction|SPAllowElevatorUse FromPC (Variables|Default|GetTargetingTeam) (Variables|Default|GetIsLocked)) :!label _label
            (bind _nextelevator (CallFunction|SPGetNearestElevator self (LocalVariables|GetUp)))
            (Utilities|IsValid _nextelevator
              (:Is%20Valid
                (bind (_domulticast _actortoteleport _teleportlocation) (CallFunction|SPDoElevatorTeleport FromPC _nextelevator))
                (if _domulticast
                  (CallFunction|HandleTeleport _actortoteleport _teleportlocation)))
              (:Is%20Not%20Valid
                (CallFunction|SPMessageClient FromPC "No matching elevator found." "NewEnumerator1")))))
        (:Down
          (LocalVariables|SetUp false)
          (goto _label))))
    (:then_1
      (return true))))

(fn OnRepIsOpaque
  (if (not (Networking|IsDedicatedServer))
    (Rendering|SetVisibility (Variables|Default|GetBottomMesh) (Variables|Default|GetIsOpaque) false)))

(fn ReceiveBeginPlay
  (|CallParentFunction)
  (if (not (Variables|Default|GetbIsPreviewStructure))
    (Utilities|SwitchNetAuthority
      (:PlayerServer
        (CallFunction|OnRepIsOpaque)))))