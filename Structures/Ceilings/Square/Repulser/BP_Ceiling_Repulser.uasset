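; Ceiling repulser structure that launches a player, or their ridden dino, standing on it when they press jump.
; A client overlap box enables input, which sends a Launch command to the server, limited to allies when locked.
; Radial-menu entries adjust pitch, roll and strength, stored in one replicated vector that aims a preview arrow.
; Strength is capped by a server INI option, with the top level doubling the multiplier.
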(event OnComponentBeginOverlap(CheckBox)
  (params (OtherActor :type Actor%20Object%20Reference) (OtherComp :type Primitive%20Component%20Object%20Reference) (OtherBodyIndex :type Integer) (bFromSweep :type Boolean) (SweepResult :type Hit%20Result%20Structure%20%28by%20ref%29))
  (bind _islocked (Variables|Default|GetIsLocked))
  (if (not (Networking|IsDedicatedServer))
    (bind _asprimalcharacter (Utilities|Casting|CastToPrimalCharacter OtherActor))
    (bind _returnvalue (Class|PrimalCharacter|IsAlliedwithOtherTeam _asprimalcharacter (Variables|Default|GetTargetingTeam)))
    (if (or (and _returnvalue _islocked) (not _islocked))
      (bind _returnvalue_2 (Class|Actor|GetOwnerController _asprimalcharacter))
      (Input|EnableInput _returnvalue_2))))

(event OnComponentEndOverlap(CheckBox)
  (params (OtherActor :type Actor%20Object%20Reference) (OtherComp :type Primitive%20Component%20Object%20Reference) (OtherBodyIndex :type Integer))
  (if (not (Networking|IsDedicatedServer))
    (bind _asprimalcharacter (Utilities|Casting|CastToPrimalCharacter OtherActor))
    (bind _returnvalue (Class|Actor|GetOwnerController _asprimalcharacter))
    (Input|DisableInput _returnvalue)))

(event Input|ActionEvents|InputActionJump
  (bind _returnvalue (Game|GetPlayerController 0))
  (:Pressed
    (if (== self (Components|GetOwner (Class|CharacterMovementComponent|GetMovementBase (Variables|/Script/Engine.Character|GetCharacterMovement (Game|GetPlayerCharacter 0)))))
      (Class|PlayerController|ClientSendNetExecCommandtoServer _returnvalue self "Launch" (Utilities|Struct|MakeBPNetExecParams) true)
      (else
        (Input|DisableInput _returnvalue)))))

(event Input|GamepadEvents|GamepadLeftThumbstick
  (bind _returnvalue (Game|GetPlayerController 0))
  (:Pressed
    (if (== self (Components|GetOwner (Class|CharacterMovementComponent|GetMovementBase (Variables|/Script/Engine.Character|GetCharacterMovement (Game|GetPlayerCharacter 0)))))
      (Class|PlayerController|ClientSendNetExecCommandtoServer _returnvalue self "Launch" (Utilities|Struct|MakeBPNetExecParams) true)
      (else
        (Input|DisableInput _returnvalue)))))

(fn ConstructionScript
  (|CallParentFunction))

(fn BPServerHandleNetExecCommand
  (params (FromPC :type Player%20Controller%20Object%20Reference) (CommandName :type Name :default "None") (ExecParams :type BP%20Net%20Exec%20Params%20Structure%20%28by%20ref%29))
  (bind _islocked (Variables|Default|GetIsLocked))
  (bind _launchparameters (Variables|Default|GetLaunchParameters))
  (Utilities|FlowControl|Sequence
    (:then_0
      (switch name CommandName
        (:Default
          (|CallParentFunction FromPC CommandName ExecParams))
        (:Launch
          (bind _asshooterplayercontroller (Utilities|Casting|CastToShooterPlayerController FromPC))
          (bind _returnvalue (Class|PrimalCharacter|IsAlliedwithOtherTeam (Class|ShooterPlayerController|GetPlayerCharacter _asshooterplayercontroller) (Variables|Default|GetTargetingTeam)))
          (if (or (and _returnvalue _islocked) (not _islocked))
            (Character|LaunchCharacter (select (Utilities|IsValid (Variables|/Script/ShooterGame.ShooterCharacter|GetRidingDino (Class|ShooterPlayerController|GetPlayerCharacter _asshooterplayercontroller))) (Variables|/Script/ShooterGame.ShooterCharacter|GetRidingDino (Class|ShooterPlayerController|GetPlayerCharacter _asshooterplayercontroller)) (Class|ShooterPlayerController|GetPlayerCharacter _asshooterplayercontroller)) (* (Math|Vector|RotateVector (Math|Vector|MakeVector 0.0 0.0 1.0) (Class|KismetMathLibrary|MakeRot (.x _launchparameters) (.yaw (Transformation|GetActorRotation)) (.y _launchparameters))) (* (.z _launchparameters) (Math|Float|SelectFloat 1e+03 5e+02 (== (Math|Float|Floor (.z _launchparameters)) 11)))) true true)))))
    (:then_1
      (return true))))

(fn BPGetMultiUseEntries
  (params (ForPC :type Player%20Controller%20Object%20Reference) (MultiUseEntries :type Array%20of%20Multi%20Use%20Entry%20Structures))
  (bind _tickcolor (CallFunction|GetTickColor))
  (bind _color (CallFunction|SPGetSpecialMenuColor))
  (bind _launchparameters (Variables|Default|GetLaunchParameters))
  (bind _returnvalue (Math|Conversions|ToColor(LinearColor) _tickcolor))
  (bind _returnvalue_2 (Math|Conversions|ToColor(LinearColor) _color))
  (bind _returnvalue_3 (Math|Float|Floor (.z _launchparameters)))
  (bind _returnvalue_4 (|CallParentFunction ForPC MultiUseEntries))
  (Utilities|FlowControl|Sequence
    (:then_0
      (bind _returnvalue_5 (Class|PrimalStructure|AllowStructureAccess ForPC))
      (if _returnvalue_5
        (Utilities|FlowControl|Sequence
          (:then_0
            (Utilities|Array|Add _returnvalue_4 (Utilities|Struct|MakeMultiUseEntry "[Adjust Roll]" 9010 -2000 true true _returnvalue_2))
            (Utilities|Array|Add _returnvalue_4 (Utilities|Struct|MakeMultiUseEntry (Utilities|String|BuildString(Integer) "Current Roll: " "" (Math|Float|Floor (.y _launchparameters))) 9999 2000 true true 1 _returnvalue_2))
            (Utilities|Array|Add _returnvalue_4 (Utilities|Struct|MakeMultiUseEntry "+1" 9014 1999 (>= (.y _launchparameters) 9e+01) true 1))
            (Utilities|Array|Add _returnvalue_4 (Utilities|Struct|MakeMultiUseEntry "+15" 9015 1998 (> (.y _launchparameters) 75.0) true 1))
            (Utilities|Array|Add _returnvalue_4 (Utilities|Struct|MakeMultiUseEntry "BACK" 9013 1997 true 1))
            (Utilities|Array|Add _returnvalue_4 (Utilities|Struct|MakeMultiUseEntry "-15" 9016 1996 (< (.y _launchparameters) -75.0) true 1))
            (Utilities|Array|Add _returnvalue_4 (Utilities|Struct|MakeMultiUseEntry "-1" 9017 1995 (<= (.y _launchparameters) -9e+01) true 1)))
          (:then_1
            (Utilities|Array|Add _returnvalue_4 (Utilities|Struct|MakeMultiUseEntry "[Adjust Pitch]" 9011 -1999 true true _returnvalue_2))
            (Utilities|Array|Add _returnvalue_4 (Utilities|Struct|MakeMultiUseEntry (Utilities|String|BuildString(Integer) "Current Pitch: " "" (Math|Float|Floor (.x _launchparameters))) 9999 2000 true true 2 _returnvalue_2))
            (Utilities|Array|Add _returnvalue_4 (Utilities|Struct|MakeMultiUseEntry "+1" 9018 1999 (>= (.x _launchparameters) 9e+01) true 2))
            (Utilities|Array|Add _returnvalue_4 (Utilities|Struct|MakeMultiUseEntry "+15" 9019 1998 (> (.x _launchparameters) 75.0) true 2))
            (Utilities|Array|Add _returnvalue_4 (Utilities|Struct|MakeMultiUseEntry "BACK" 9013 1997 true 2))
            (Utilities|Array|Add _returnvalue_4 (Utilities|Struct|MakeMultiUseEntry "-15" 9020 1996 (< (.x _launchparameters) -75.0) true 2))
            (Utilities|Array|Add _returnvalue_4 (Utilities|Struct|MakeMultiUseEntry "-1" 9021 1995 (<= (.x _launchparameters) -9e+01) true 2)))
          (:then_2
            (Utilities|Array|Add _returnvalue_4 (Utilities|Struct|MakeMultiUseEntry "[Adjust Strength]" 9012 -1998 true true _returnvalue_2))
            (Variables|Default|SetColorShiftCurrentTime (Math|Float|SelectFloat 0.0 (+ (Variables|Default|GetColorShiftCurrentTime) 1.0) (> (+ (Variables|Default|GetColorShiftCurrentTime) 1.0) (Variables|Default|GetColorShiftTime))))
            (Utilities|Array|Add _returnvalue_4 (Utilities|Struct|MakeMultiUseEntry (Utilities|String|BuildString(Integer) "Current Strength: " "" _returnvalue_3) 9999 2000 true true 3 (select (>= _returnvalue_3 11) _returnvalue _returnvalue_2)))
            (Utilities|Array|Add _returnvalue_4 (Utilities|Struct|MakeMultiUseEntry "+1" 9022 1999 (>= _returnvalue_3 (Variables|Default|GetMaxStrength)) true (== _returnvalue_3 10) 3 _returnvalue))
            (Utilities|Array|Add _returnvalue_4 (Utilities|Struct|MakeMultiUseEntry "BACK" 9013 1997 true 3))
            (Utilities|Array|Add _returnvalue_4 (Utilities|Struct|MakeMultiUseEntry "-1" 9023 1995 (<= _returnvalue_3 1) true 3)))
          (:then_3
            (if (Variables|Default|GetIsArrowVisible)
              (Utilities|Array|Add _returnvalue_4 (Utilities|Struct|MakeMultiUseEntry "Hide Arrow" 9009 5000))))
          (:then_4
            (Utilities|Array|Add _returnvalue_4 (Utilities|Struct|MakeMultiUseEntry (Utilities|String|SelectString "Unlock" "Lock" (Variables|Default|GetIsLocked)) 9024 -1500))))))
    (:then_1
      (return _returnvalue_4))))

(fn BPTryMultiUse
  (params (ForPC :type Player%20Controller%20Object%20Reference) (UseIndex :type Integer))
  (Utilities|FlowControl|Sequence
    (:then_0
      (switch int UseIndex
        (:Default
          (|CallParentFunction ForPC UseIndex))
        (:9009
          (Variables|Default|SetIsArrowVisible false true))
        (:9010
          (Variables|Default|SetIsArrowVisible true true :!label _label))
        (:9011
          (goto _label))
        (:9012
          (goto _label))
        (:9014
          (Variables|Default|SetLaunchParameters (Math|Vector|MakeVector (.x (Variables|Default|GetLaunchParameters)) (+ (.y (Variables|Default|GetLaunchParameters)) 1.0) (.z (Variables|Default|GetLaunchParameters))) true))
        (:9015
          (Variables|Default|SetLaunchParameters (Math|Vector|MakeVector (.x (Variables|Default|GetLaunchParameters)) (+ (.y (Variables|Default|GetLaunchParameters)) 15.0) (.z (Variables|Default|GetLaunchParameters))) true))
        (:9016
          (Variables|Default|SetLaunchParameters (Math|Vector|MakeVector (.x (Variables|Default|GetLaunchParameters)) (- (.y (Variables|Default|GetLaunchParameters)) 15.0) (.z (Variables|Default|GetLaunchParameters))) true))
        (:9017
          (Variables|Default|SetLaunchParameters (Math|Vector|MakeVector (.x (Variables|Default|GetLaunchParameters)) (- (.y (Variables|Default|GetLaunchParameters)) 1.0) (.z (Variables|Default|GetLaunchParameters))) true))
        (:9018
          (Variables|Default|SetLaunchParameters (Math|Vector|MakeVector (+ (.x (Variables|Default|GetLaunchParameters)) 1.0) (.y (Variables|Default|GetLaunchParameters)) (.z (Variables|Default|GetLaunchParameters))) true))
        (:9019
          (Variables|Default|SetLaunchParameters (Math|Vector|MakeVector (+ (.x (Variables|Default|GetLaunchParameters)) 15.0) (.y (Variables|Default|GetLaunchParameters)) (.z (Variables|Default|GetLaunchParameters))) true))
        (:9020
          (Variables|Default|SetLaunchParameters (Math|Vector|MakeVector (- (.x (Variables|Default|GetLaunchParameters)) 15.0) (.y (Variables|Default|GetLaunchParameters)) (.z (Variables|Default|GetLaunchParameters))) true))
        (:9021
          (Variables|Default|SetLaunchParameters (Math|Vector|MakeVector (- (.x (Variables|Default|GetLaunchParameters)) 1.0) (.y (Variables|Default|GetLaunchParameters)) (.z (Variables|Default|GetLaunchParameters))) true))
        (:9022
          (Variables|Default|SetLaunchParameters (Math|Vector|MakeVector (.x (Variables|Default|GetLaunchParameters)) (.y (Variables|Default|GetLaunchParameters)) (+ (.z (Variables|Default|GetLaunchParameters)) 1.0)) true))
        (:9023
          (Variables|Default|SetLaunchParameters (Math|Vector|MakeVector (.x (Variables|Default|GetLaunchParameters)) (.y (Variables|Default|GetLaunchParameters)) (- (.z (Variables|Default|GetLaunchParameters)) 1.0)) true))
        (:9024
          (Variables|Default|SetIsLocked (not (Variables|Default|GetIsLocked)) true))))
    (:then_1
      (return true))))

(fn BPClientDoMultiUse
  (params (ForPC :type Player%20Controller%20Object%20Reference) (ClientUseIndex :type Integer))
  (bind _asshooterplayercontroller (Utilities|Casting|CastToShooterPlayerController ForPC))
  (switch int ClientUseIndex
    (:9010
      (Class|ShooterPlayerController|SetMultiUseWheelCategory _asshooterplayercontroller 1))
    (:9011
      (Class|ShooterPlayerController|SetMultiUseWheelCategory _asshooterplayercontroller 2))
    (:9012
      (Class|ShooterPlayerController|SetMultiUseWheelCategory _asshooterplayercontroller 3))
    (:9013
      (Class|ShooterPlayerController|SetMultiUseWheelCategory _asshooterplayercontroller 0))))

(fn BPPostSetStructureCollisionChannels
  (Collision|SetCollisionProfileName (Variables|Default|GetInteractionMesh) "UsableOnly" :!class /Script/Engine.PrimitiveComponent))

(fn OnRepIsArrowVisible
  (Rendering|SetVisibility (Variables|Default|GetArrow) (Variables|Default|GetIsArrowVisible) false))

(fn ReceiveBeginPlay
  (|CallParentFunction)
  (if (not (Variables|Default|GetbIsPreviewStructure))
    (Networking|SwitchHasAuthority
      (:Authority
        (bind _value (CallFunction|SPGetIntIniOption (Game|GetGameMode) "RepulserMaxStrength" 11 11))
        (Variables|Default|SetMaxStrength (Math|Integer|Max(Integer) _value 1) true)
        (Utilities|SwitchNetAuthority
          (:PlayerServer
            (CallFunction|OnRepIsArrowVisible)
            (CallFunction|OnRepLaunchParameters)))))))

(fn OnRepLaunchParameters
  (bind _launchparameters (Variables|Default|GetLaunchParameters))
  (if (not (Networking|IsDedicatedServer))
    (Transformation|SetRelativeRotation (Variables|Default|GetArrowScene) (Math|Rotator|MakeRotator (.x _launchparameters) 0.0 (.y _launchparameters)) false)))

(fn GetTickColor
  (bind _colorshifttime (Variables|Default|GetColorShiftTime))
  (bind _colorshiftcurrenttime (Variables|Default|GetColorShiftCurrentTime))
  (Utilities|FlowControl|Sequence
    (:then_0
      (if (== _colorshiftcurrenttime 0.0)
        (Variables|Default|SetCurrentColor "(R=1.000000,G=0.000000,B=0.000000,A=1.000000)")
        (Variables|Default|SetTargetColor "(R=0.000000,G=1.000000,B=1.000000,A=1.000000)")
        (elif (>= _colorshifttime 0.5)
          (Variables|Default|SetCurrentColor "(R=0.000000,G=1.000000,B=1.000000,A=1.000000)")
          (Variables|Default|SetTargetColor "(R=1.000000,G=0.000000,B=0.000000,A=1.000000)"))))
    (:then_1
      (return (Class|KismetMathLibrary|CInterpto (Variables|Default|GetCurrentColor) (Variables|Default|GetTargetColor) (/ _colorshiftcurrenttime (/ _colorshifttime 2.0)) 1.0)))))