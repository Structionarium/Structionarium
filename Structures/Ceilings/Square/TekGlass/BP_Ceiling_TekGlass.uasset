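; Square Tek glass ceiling structure with adjustable transparency, exposed through the glass get/set interface.
; Construction gives the mesh separate inside and outside dynamic materials, which the GlassSettings RepNotify updates on non-dedicated instances.
; On begin play the authority reads the minimum glass transparency ini option into MinOpacity, whose RepNotify raises lower opacity to that floor.
; Shared SP helpers build the multi-use menu with glass and pickup entries.
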(event EventIGlassSetModel
  (params (ModelIndex :type Integer)))

(event EventIGlassSetTransparency
  (params (GlassSetting :type SP%20Glass%20Settings%20Structure))
  (Variables|Default|SetGlassSettings GlassSetting true))

(fn ConstructionScript
  (bind _glassmesh (Variables|Default|GetGlassMesh))
  (|CallParentFunction)
  (if (not (or (Variables|Default|GetbIsPreviewStructure) (Networking|IsDedicatedServer)))
    (bind _returnvalue (Rendering|Material|CreateDynamicMaterialInstance "/Game/Mods/StructuresPlusMod/_Materials/GlassMIC.GlassMIC" :!class /Script/Engine.KismetMaterialLibrary))
    (Variables|Default|SetInsideMIC _returnvalue)
    (bind _returnvalue_2 (Rendering|Material|CreateDynamicMaterialInstance "/Game/Mods/StructuresPlusMod/_Materials/GlassMIC.GlassMIC" :!class /Script/Engine.KismetMaterialLibrary))
    (Variables|Default|SetOutsideMIC _returnvalue_2)
    (Rendering|Material|SetMaterial _glassmesh 0 (Variables|Default|GetInsideMIC))
    (Rendering|Material|SetMaterial _glassmesh 1 (Variables|Default|GetOutsideMIC))))

(fn OnRepGlassSettings
  (if (not (Networking|IsDedicatedServer))
    (CallFunction|SPAlterGlassTransparency (Variables|Default|GetGlassSettings) (Variables|Default|GetInsideMIC) (Variables|Default|GetOutsideMIC))))

(fn OnRepMinOpacity
  (bind _minopacity (Variables|Default|GetMinOpacity))
  (Networking|SwitchHasAuthority
    (:Authority
      (if (< (.opacity (Variables|Default|GetGlassSettings)) _minopacity)
        (Variables|Default|SetGlassSettings (Utilities|Struct|MakeSPGlassSettings (.transparencytype (Variables|Default|GetGlassSettings)) _minopacity) true)))))

(fn BPGetMultiUseEntries
  (params (ForPC :type Player%20Controller%20Object%20Reference) (MultiUseEntries :type Array%20of%20Multi%20Use%20Entry%20Structures))
  (bind _entriesout (CallFunction|SPAddMenuEntries MultiUseEntries ForPC self (Variables|Default|GetDisablePickup) (Variables|Default|GetDisablePickupWhenDamaged) true false (Variables|Default|GetDisablePickupAfterTime) (Variables|Default|GetTimeToDisablePickup)))
  (bind _entriesout_2 (CallFunction|SPAddRemoveInternalMenuEntries _entriesout self ForPC))
  (return _entriesout_2))

(fn ReceiveBeginPlay
  (|CallParentFunction)
  (if (not (Variables|Default|GetbIsPreviewStructure))
    (Networking|SwitchHasAuthority
      (:Authority
        (bind _value (CallFunction|SPGetFloatIniOption (Game|GetGameMode) "MinimumGlassTransparency" 0.0 1.0))
        (Variables|Default|SetMinOpacity _value true)
        (Utilities|SwitchNetAuthority
          (:PlayerServer
            (CallFunction|OnRepGlassSettings)))))))

(fn IGlassGetModel
  (return 0 false))

(fn IGlassGetTransparency
  (return (Variables|Default|GetGlassSettings) (Variables|Default|GetMinOpacity)))