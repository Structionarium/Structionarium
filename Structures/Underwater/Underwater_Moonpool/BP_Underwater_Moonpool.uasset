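; Underwater base moonpool structure that shows or hides its top and bottom water-plane meshes according to flooding.
; UpdatedVisuals hides the planes when the moonpool is flooded or the first linked base piece beneath it is dry.
; It reruns on compartment flood changes and on a randomized looping timer, which HandleMoonpool starts once outside save loading.
; Both triggers skip dedicated servers.
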(event Custom|UpdateVisuals
  (CallFunction|UpdatedVisuals))

(fn ConstructionScript
  (|CallParentFunction))

(fn UpdatedVisuals
  (LocalVariables|SetbForceHidden (Variables|Default|GetbIsFlooded))
  (bind _array_element (Utilities|Array|ForEachLoopwithBreak (Variables|Default|GetLinkedStructures) :!label _label)
    (:LoopBody
      (if (> (.z (Transformation|GetActorLocation)) (+ (.z (Transformation|GetActorLocation _array_element)) 5e+01))
        (bind _asprimalstructureunderwaterbase (Utilities|Casting|CastToPrimalStructureUnderwaterBase _array_element))
        (Utilities|IsValid _asprimalstructureunderwaterbase
          (:Is%20Valid
            (Utilities|FlowControl|Sequence
              (:then_0
                (if (not (Variables|/Script/ShooterGame.PrimalStructureUnderwaterBase|GetbIsFlooded _asprimalstructureunderwaterbase))
                  (LocalVariables|SetbForceHidden (not (Variables|Default|GetbIsFlooded)))
                  (if (Variables|Default|GetbIsFlooded)
                    (LocalVariables|SetbForceHidden true))))
              (:then_1
                (goto _label Break)))))))
    (:Completed
      (Rendering|SetVisibility (Variables|Default|GetWaterPlaneTop) (not (LocalVariables|GetbForceHidden)) false))))

(fn ChangedCompartmentFloodState
  (|CallParentFunction)
  (if (not (Networking|IsDedicatedServer))
    (CallFunction|UpdatedVisuals)))

(fn HandleMoonpool
  (if (not (Networking|IsDedicatedServer))
    (bind _returnvalue (Class|VictoryCore|IsLoadingSaveGame))
    (if (and (not _returnvalue) (not (Variables|Default|GetbSetTimer)))
      (Utilities|Time|SetTimerbyFunctionName 0 "UpdateVisuals" (Math|Random|RandomFloatinRange 1.2 2.5) true)
      (Variables|Default|SetbSetTimer true))))