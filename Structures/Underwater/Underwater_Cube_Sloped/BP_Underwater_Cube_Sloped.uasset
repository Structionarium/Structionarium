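; Sloped underwater base compartment for Structures Plus (ARK) that players can flood, drain and build from.
; Multi-use entries toggle flooding and side locks, drain connected compartments and handle portholes, with client-side emitters on flood changes.
; Placement hooks treat snapped structures as foundations, offset certain snaps by roll and optionally destroy above-water placements via server config.
; Server-side logic applies pickup settings and grants a radiation protection buff to overlapping characters.
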(event OnComponentBeginOverlap(RadiationProtectionBox)
  (params (OtherActor :type Actor%20Object%20Reference) (OtherComp :type Primitive%20Component%20Object%20Reference) (OtherBodyIndex :type Integer) (bFromSweep :type Boolean) (SweepResult :type Hit%20Result%20Structure%20%28by%20ref%29))
  (Networking|SwitchHasAuthority
    (:Authority
      (bind _asprimalcharacter (Utilities|Casting|CastToPrimalCharacter OtherActor))
      (bind _returnvalue (Class|PrimalCharacter|HasBuff _asprimalcharacter "/Game/Mods/StructuresPlusMod/_Buffs/Buff_StructuresPlus_RadiationProtection.Buff_StructuresPlus_RadiationProtection_C" true))
      (if (not _returnvalue)
        (Class|PrimalBuff|StaticAddBuff "/Game/Mods/StructuresPlusMod/_Buffs/Buff_StructuresPlus_RadiationProtection.Buff_StructuresPlus_RadiationProtection_C" _asprimalcharacter 0 0 false)))))

(event EventIPickupSetPickupSettings
  (params (DisablePickup :type Boolean) (DisablePickupWhenDamaged :type Boolean) (DisablePickupAfterTime :type Float%20%28single-precision%29) (TimeToDisablePickup :type Float%20%28double-precision%29))
  (Variables|Default|SetDisablePickup DisablePickup true)
  (Variables|Default|SetDisablePickupWhenDamaged DisablePickupWhenDamaged true)
  (Variables|Default|SetDisablePickupAfterTime DisablePickupAfterTime true)
  (Variables|Default|SetTimeToDisablePickup TimeToDisablePickup true))

(fn ConstructionScript
  (|CallParentFunction)
  (if (Variables|Default|GetbIsPreviewStructure)
    (bind _globalactor (CallFunction|SPGetGlobalActor self))
    (Utilities|IsValid _globalactor
      (:Is%20Valid
        (Variables|Default|SetbOnlyAllowPlacementInWater (Variables|/Game/Mods/StructuresPlusMod/SPlusGlobalActor.SPlusGlobalActor_C|GetDisableUnderwaterAboveWater _globalactor))))))

(fn ChangedCompartmentFloodState
  (if (not (Networking|IsDedicatedServer))
    (if (> (Class|VictoryCore|TimeSince (Class|Actor|GetWorld) (Variables|Default|GetCreationTime)) 0.33)
      (Game|SpawnActorfromClass (select (Variables|Default|GetbIsFlooded) "/Game/PrimalEarth/General/UnderwaterBaseFloodedEmitter.UnderwaterBaseFloodedEmitter_C" "/Game/PrimalEarth/General/UnderwaterBaseUnfloodedEmitter.UnderwaterBaseUnfloodedEmitter_C") (Transformation|GetActorTransform) true))))

(fn BPForceConsideredEnemyFoundation
  (params (PC :type Player%20Controller%20Object%20Reference) (ForNewStructure :type Primal%20Structure%20Object%20Reference) (TestAtLocation :type Vector%20%28by%20ref%29 :default "0, 0, 0"))
  (return true))

(fn BPPreventPlacingStructureOntoMe
  (params (PC :type Player%20Controller%20Object%20Reference) (ForNewStructure :type Primal%20Structure%20Object%20Reference) (ForHitResult :type Hit%20Result%20Structure%20%28by%20ref%29))
  (bind (_location _normal _impactpoint _impactnormal _physmat _hitactor _hitcomponent) (Collision|BreakHitResult ForHitResult))
  (bind _requireswall (CallFunction|SPRequiresWallAttachforUnderwater self _location))
  (return (and (not _requireswall) (Math|Boolean|ORBoolean (== _hitcomponent 0) (== _hitcomponent (Variables|Default|GetCollision_Front)) (== _hitcomponent (Variables|Default|GetCollision_Left)) (== _hitcomponent (Variables|Default|GetCollision_Right)) (== _hitcomponent (Variables|Default|GetCollision_Back))))))

(fn BPGetMultiUseEntries
  (params (ForPC :type Player%20Controller%20Object%20Reference) (MultiUseEntries :type Array%20of%20Multi%20Use%20Entry%20Structures))
  (bind _self self)
  (bind _entriesout (CallFunction|SPAddMenuEntries MultiUseEntries ForPC _self (Variables|Default|GetDisablePickup) (Variables|Default|GetDisablePickupWhenDamaged) false false (Variables|Default|GetDisablePickupAfterTime) (Variables|Default|GetTimeToDisablePickup)))
  (bind _entriesout_2 (CallFunction|SPCleanUpPortholeMenuEntries _self _entriesout (Variables|Default|GetLockSides)))
  (Utilities|FlowControl|Sequence
    (:then_0
      (bind _returnvalue (Class|PrimalStructure|AllowStructureAccess ForPC))
      (if _returnvalue
        (Utilities|Array|Add _entriesout_2 (Utilities|Struct|MakeMultiUseEntry (Utilities|String|SelectString "Drain Water" "Flood Compartment" (Variables|Default|GetbIsFlooded)) 9001 -1000 0.25 0.25))
        (Utilities|Array|Add _entriesout_2 (Utilities|Struct|MakeMultiUseEntry "Drain All Connected" 9002 -1000 0.25 0.25))
        (Utilities|Array|Add _entriesout_2 (Utilities|Struct|MakeMultiUseEntry (Utilities|String|SelectString "Unlock Sides" "Lock Sides" (Variables|Default|GetLockSides)) 9003 -1002))))
    (:then_1
      (return _entriesout_2))))

(fn BPTryMultiUse
  (params (ForPC :type Player%20Controller%20Object%20Reference) (UseIndex :type Integer))
  (Utilities|FlowControl|Sequence
    (:then_0
      (switch int UseIndex
        (:Default
          (if (or (and (>= UseIndex 42) (<= UseIndex 47)) (and (>= UseIndex 72) (<= UseIndex 77)))
            (CallFunction|SPNormalizeConnectedPorthole ForPC self UseIndex)))
        (:9001
          (Variables|Default|SetbIsFlooded (not (Variables|Default|GetbIsFlooded)) true))
        (:9002
          (CallFunction|SPDrainAllConnectedCompartments self))
        (:9003
          (Variables|Default|SetLockSides (not (Variables|Default|GetLockSides)) true))))
    (:then_1
      (return true))))

(fn IsValidSnapPointto
  (params (ChildStructure :type Primal%20Structure%20Object%20Reference) (MySnapPointToIndex :type Integer))
  (Variables|/Script/ShooterGame.PrimalStructure|SetbIsFoundation ChildStructure true false)
  (return true))

(fn BPIsAllowedtoBuild
  (params (OutPlacementData :type Placement%20Data%20Structure%20%28by%20ref%29) (CurrentAllowedReason :type Integer))
  (return (Math|Integer|SelectInt 1 CurrentAllowedReason (== CurrentAllowedReason -9))))

(fn BPOverrideSnappedtoTransform
  (params (childStructure :type Primal%20Structure%20Object%20Reference) (ChildSnapFromIndex :type Integer) (ChildSnapFromName :type Name :default "None") (UnsnappedPlacementPos :type Vector :default "0, 0, 0") (UnsnappedPlacementRot :type Rotator :default "0, 0, 0") (SnappedPlacementPos :type Vector :default "0, 0, 0") (SnappedPlacementRot :type Rotator :default "0, 0, 0") (SnapToIndex :type Integer) (SnapToName :type Name :default "None"))
  (return (- SnappedPlacementPos (Math|Vector|SelectVector "0, 0,-60.000000" "0, 0,60.000000" (Math|Float|InRange(Float) (.roll (Transformation|GetActorRotation)) -1.0 1.0))) SnappedPlacementRot 0 (or (== SnapToIndex 43) (== SnapToIndex 44))))

(fn ReceiveBeginPlay
  (bind _returnvalue (Game|GetGameMode))
  (|CallParentFunction)
  (if (not (Variables|Default|GetbIsPreviewStructure))
    (Networking|SwitchHasAuthority
      (:Authority
        (CallFunction|SPSetPickUpSettings _returnvalue self)
        (Utilities|FlowControl|Sequence
          (:then_0
            (bind _asshootergamemode (Utilities|Casting|CastToShooterGameMode _returnvalue))
            (bind _returnvalue_2 (Class|ShooterGameMode|GetBoolOptionIni _asshootergamemode "StructuresPlus" "DisableAbilityToPlaceVacuumCompartmentsAboveWater"))
            (if _returnvalue_2
              (bind _returnvalue_3 (Class|BiomeZoneVolume|IsPointUnderwater (Class|Actor|GetWorld) (Transformation|GetActorLocation) true 0.0 true false))
              (if (not _returnvalue_3)
                (Actor|DestroyActor))))
          (:then_1
            (for _array_element (Variables|Default|GetLinkedStructures)
              (Variables|/Script/ShooterGame.PrimalStructure|SetbIsFoundation _array_element true false))))))))

(fn IPickupGetDisablePickupAfterTime
  (return (Variables|Default|GetDisablePickupAfterTime)))

(fn IPickupGetTimetoDisablePickup
  (return (Variables|Default|GetTimeToDisablePickup)))