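; S+ dynamic gateway structure whose width, height and material tier the player cycles by hotkey during placement, gated by per-material engrams.
; Replicated gateway data drives pillar spacing, stacked mesh visibility and collision; a multi-use wheel handles thickness, crafting, repair, demolition and snap assist.
; Placed gateways show preview materials while crafting and self-destruct at the deadline if unfinished.
; Snapped dynamic gates inherit the gateway's size, scaled per gate material.
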(event Custom|SelfDestructEvent
  (if (Variables|Default|GetIsCrafting)
    (Actor|DestroyActor)))

(event Input|KeyboardEvents|F
  (bind _gatewaydata (Variables|Default|GetGatewayData))
  (bind (_width _height _materialindex) (Utilities|Struct|BreakSP_DynamicGatewayData _gatewaydata))
  (:Pressed
    (if (< _height 12)
      (Utilities|Struct|SetmembersinSP_DynamicGatewayData _gatewaydata (+ _height 1))
      (CallFunction|OnRepGatewayData))))

(event Input|KeyboardEvents|ShiftF
  (bind _gatewaydata (Variables|Default|GetGatewayData))
  (bind (_width _height _materialindex) (Utilities|Struct|BreakSP_DynamicGatewayData _gatewaydata))
  (:Pressed
    (if (> _height 0)
      (Utilities|Struct|SetmembersinSP_DynamicGatewayData _gatewaydata (- _height 1))
      (CallFunction|OnRepGatewayData))))

(event Input|KeyboardEvents|ShiftG
  (bind _gatewaydata (Variables|Default|GetGatewayData))
  (bind (_width _height _materialindex) (Utilities|Struct|BreakSP_DynamicGatewayData _gatewaydata))
  (:Pressed
    (if (> _width 1)
      (Utilities|Struct|SetmembersinSP_DynamicGatewayData _gatewaydata (- _width 1))
      (CallFunction|OnRepGatewayData))))

(event Input|KeyboardEvents|ShiftH
  (bind _gatewaydata (Variables|Default|GetGatewayData))
  (bind (_width _height _materialindex) (Utilities|Struct|BreakSP_DynamicGatewayData _gatewaydata))
  (:Pressed
    (if (> _materialindex 0)
      (Utilities|Struct|SetmembersinSP_DynamicGatewayData _gatewaydata (- _materialindex 1))
      (CallFunction|OnRepGatewayData))))

(event Input|KeyboardEvents|H
  (bind _gatewaydata (Variables|Default|GetGatewayData))
  (bind (_width _height _materialindex) (Utilities|Struct|BreakSP_DynamicGatewayData _gatewaydata))
  (:Pressed
    (if (< _materialindex 4)
      (Utilities|Struct|SetmembersinSP_DynamicGatewayData _gatewaydata (+ _materialindex 1))
      (CallFunction|OnRepGatewayData))))

(event Input|KeyboardEvents|G
  (bind _gatewaydata (Variables|Default|GetGatewayData))
  (bind (_width _height _materialindex) (Utilities|Struct|BreakSP_DynamicGatewayData _gatewaydata))
  (:Pressed
    (if (< _width 12)
      (Utilities|Struct|SetmembersinSP_DynamicGatewayData _gatewaydata (+ _width 1))
      (CallFunction|OnRepGatewayData))))

(fn ConstructionScript
  (|CallParentFunction)
  (if (and (Variables|Default|GetbIsPreviewStructure) (not (Networking|IsDedicatedServer)))
    (Components|StaticMesh|SetStaticMesh (Variables|Default|GetPlacementMesh) "/Game/Mods/StructuresPlusMod/Structures/Gateways/Dynamic/_Models/SM_Gateway_Placement.SM_Gateway_Placement")))

(fn BPIsAllowedtoBuild
  (params (OutPlacementData :type Placement%20Data%20Structure%20%28by%20ref%29) (CurrentAllowedReason :type Integer))
  (bind _gatewaydata (Variables|Default|GetGatewayData))
  (bind _materialindex (Utilities|Struct|BreakSP_DynamicGatewayData _gatewaydata))
  (LocalVariables|SetBuildReason (Math|Integer|SelectInt 1 CurrentAllowedReason (== CurrentAllowedReason -9)))
  (Utilities|FlowControl|Sequence
    (:then_0
      (if (Variables|Default|GetbIsPreviewStructure)
        (bind _returnvalue (Class|Actor|GetOwnerController))
        (bind _asshooterplayercontroller (Utilities|Casting|CastToShooterPlayerController _returnvalue))
        (bind _asshooterplayerstate (Utilities|Casting|CastToShooterPlayerState (Variables|/Script/Engine.Controller|GetPlayerState _asshooterplayercontroller)))
        (if (not (Class|ShooterPlayerState|HasEngram _asshooterplayerstate (Utilities|Select :Index _materialindex :Option%200 "/Game/Mods/StructuresPlusMod/Structures/Gateways/Small/Wood/PrimalItemStructure_Gateway_Wood.PrimalItemStructure_Gateway_Wood_C" :Option%201 "/Game/Mods/StructuresPlusMod/Structures/Gateways/Small/Stone/PrimalItemStructure_Gateway_Stone.PrimalItemStructure_Gateway_Stone_C" :Option%202 "/Game/Mods/StructuresPlusMod/Structures/Gateways/Small/Metal/PrimalItemStructure_Gateway_Metal.PrimalItemStructure_Gateway_Metal_C" :Option%203 "/Game/Mods/StructuresPlusMod/Structures/Gateways/Small/Adobe/PrimalItemStructure_Gateway_Adobe.PrimalItemStructure_Gateway_Adobe_C" :Option%204 "/Game/Mods/StructuresPlusMod/Structures/Gateways/Small/Tek/PrimalItemStructure_Gateway_Tek.PrimalItemStructure_Gateway_Tek_C")))
          (LocalVariables|SetBuildReason (Utilities|Select :Index _materialindex :Option%200 -111 :Option%201 -112 :Option%202 -113 :Option%203 -114 :Option%204 -115)))))
    (:then_1
      (return (LocalVariables|GetBuildReason)))))

(fn BPGetMultiUseEntries
  (params (ForPC :type Player%20Controller%20Object%20Reference) (MultiUseEntries :type Array%20of%20Multi%20Use%20Entry%20Structures))
  (bind _color (CallFunction|SPGetSpecialMenuColor))
  (bind _repaircooldowntime (Variables|Default|GetRepairCooldownTime))
  (bind _pillarthickness (Variables|Default|GetPillarThickness))
  (bind (_canrepair _repairstring) (CallFunction|SPGetRepairMenuEntryData ForPC _repaircooldowntime))
  (bind _returnvalue (Math|Conversions|ToColor(LinearColor) _color))
  (bind _entriesout (CallFunction|CleanMultiuseEntries MultiUseEntries))
  (Utilities|FlowControl|Sequence
    (:then_0
      (bind _returnvalue_2 (Class|PrimalStructure|AllowStructureAccess ForPC))
      (if _returnvalue_2
        (Utilities|Array|Add _entriesout (Utilities|Struct|MakeMultiUseEntry (Utilities|String|SelectString "Enable Snap Assist" "Disable Snap Assist" (Variables|Default|GetIsSnapAssistHidden)) 9006 -2000))
        (Utilities|FlowControl|Sequence
          (:then_0
            (Utilities|Array|Add _entriesout (Utilities|Struct|MakeMultiUseEntry "[Pillar Thickness]" 9000 -1100 true true _returnvalue))
            (Utilities|Array|Add _entriesout (Utilities|Struct|MakeMultiUseEntry (Utilities|String|BuildString(Integer) "Current Thickness: " "" (+ _pillarthickness 1)) 9999 1000 true true 1 _returnvalue))
            (Utilities|Array|Add _entriesout (Utilities|Struct|MakeMultiUseEntry "+1" 9001 0 (>= _pillarthickness 9) true 1))
            (Utilities|Array|Add _entriesout (Utilities|Struct|MakeMultiUseEntry "" 9999 -999 true 1))
            (Utilities|Array|Add _entriesout (Utilities|Struct|MakeMultiUseEntry "-1" 9002 -1000 (<= _pillarthickness 0) true 1)))
          (:then_1
            (Utilities|Array|Add _entriesout (Utilities|Struct|MakeMultiUseEntry "Demolish" 9005 -2500 1.0 1.0))
            (if (Variables|Default|GetIsCrafting)
              (Utilities|Array|Add _entriesout (Utilities|Struct|MakeMultiUseEntry "Finish Crafting" 9003 2500))
              (elif (!= (Math|Float|Floor (Variables|Default|GetHealth)) (Math|Float|Floor (Variables|Default|GetMaxHealth)))
                (Utilities|Array|Add _entriesout (Utilities|Struct|MakeMultiUseEntry _repairstring 9004 2000 (not _canrepair)))))))))
    (:then_1
      (return _entriesout))))

(fn ReceiveBeginPlay
  (|CallParentFunction)
  (if (Variables|Default|GetbIsPreviewStructure)
    (Rendering|SetVisibility (Variables|Default|GetPlacementMesh) true false)
    (bind _returnvalue (Class|Actor|GetOwnerController))
    (Input|EnableInput _returnvalue)
    (bind _globalactor (CallFunction|SPGetGlobalActor self))
    (Utilities|IsValid _globalactor
      (:Is%20Valid
        (Class|PlayerController|ClientSendNetExecCommandtoServer _returnvalue _globalactor "ApplyGatewayBuff" (Utilities|Struct|MakeBPNetExecParams) true))
      (:Is%20Not%20Valid
        (Development|PrintString "Global Actor Not Found")))
    (else
      (Utilities|FlowControl|Sequence
        (:then_0
          (Networking|SwitchHasAuthority
            (:Authority
              (if (Variables|Default|GetIsCrafting)
                (Utilities|Time|SetTimerbyFunctionName 0 "SelfDestructEvent" (Math|Conversions|ToFloat(Integer) (- (Variables|Default|GetDestructionTime) (Utilities|Time|GetGameTimeinSeconds))))))))
        (:then_1
          (if (and (not (Networking|IsDedicatedServer)) (Variables|Default|GetIsCrafting))
            (CallFunction|UpdateMaterials)))
        (:then_2
          (Utilities|SwitchNetAuthority
            (:PlayerServer
              (CallFunction|OnRepGatewayData)
              (CallFunction|OnRepPillarThickness)
              (CallFunction|OnRepIsSnapAssistHidden))))))))

(fn OnRepPillarThickness
  (bind _pillarthickness (Variables|Default|GetPillarThickness))
  (bind _returnvalue (* _pillarthickness 0.15))
  (bind _returnvalue_2 (+ 1.0 _returnvalue))
  (if (not (Networking|IsDedicatedServer))
    (Transformation|SetRelativeScale3D (Variables|Default|GetRightScene) (Math|Vector|MakeVector _returnvalue_2 _returnvalue_2 1.0))))

(fn BPClientDoMultiUse
  (params (ForPC :type Player%20Controller%20Object%20Reference) (ClientUseIndex :type Integer))
  (switch int ClientUseIndex
    (:9000
      (bind _asshooterplayercontroller (Utilities|Casting|CastToShooterPlayerController ForPC))
      (Class|ShooterPlayerController|SetMultiUseWheelCategory _asshooterplayercontroller 1))))

(fn BPTryMultiUse
  (params (ForPC :type Player%20Controller%20Object%20Reference) (UseIndex :type Integer))
  (bind _self self)
  (switch int UseIndex
    (:Default
      _)
    (:9001
      (Variables|Default|SetPillarThickness (+ (Variables|Default|GetPillarThickness) 1) true))
    (:9002
      (Variables|Default|SetPillarThickness (- (Variables|Default|GetPillarThickness) 1) true))
    (:9003
      (CallFunction|SPApplyDynamicCraftingBuff ForPC _self false))
    (:9004
      (CallFunction|SPApplyDynamicCraftingBuff ForPC _self true))
    (:9005
      (CallFunction|SPDemolishDynamicStructure ForPC (select (Variables|Default|GetIsCrafting) (Variables|Default|GetMaterialsStored) (Variables|Default|GetMaterialsRequired)) self))
    (:9006
      (Variables|Default|SetIsSnapAssistHidden (not (Variables|Default|GetIsSnapAssistHidden)) true)))
  (return true))

(fn BPPreInitializeComponents
  (|CallParentFunction)
  (if (not (Variables|Default|GetbIsPreviewStructure))
    (Networking|SwitchHasAuthority
      (:Authority
        (bind _returnvalue (Class|VictoryCore|IsLoadingSaveGame))
        (if (not _returnvalue)
          (CallFunction|SPInitializeDynamicStructure self)
          (Variables|Default|SetIsSnapAssistHidden false true))))))

(fn OnRepGatewayData
  (bind _gatewaydata (Variables|Default|GetGatewayData))
  (bind (_width _height _materialindex) (Utilities|Struct|BreakSP_DynamicGatewayData _gatewaydata))
  (bind _returnvalue (- _width 1))
  (bind _returnvalue_2 (* _returnvalue 149.7))
  (bind _returnvalue_3 (+ _returnvalue_2 149.7))
  (CallFunction|SetCollision)
  (if (not (Networking|IsDedicatedServer))
    (Transformation|SetRelativeLocation (Variables|Default|GetLeftScene) (Math|Vector|MakeVector (* _returnvalue_3 -1.0) 0.0 92.0) false)
    (Transformation|SetRelativeLocation (Variables|Default|GetRightScene) (Math|Vector|MakeVector _returnvalue_3 0.0 92.0) false)
    (Transformation|SetRelativeScale3D (Variables|Default|GetPlacementMesh) (Math|Vector|MakeVector (Math|Conversions|ToFloat(Integer) _width) 1.0 (Math|Conversions|ToFloat(Integer) _height)))
    (for _array_element (Actor|GetComponentsByClass "/Script/Engine.StaticMeshComponent")
      (if (or (>= (Utilities|String|FindSubstring (Utilities|GetDisplayName _array_element) "RightMesh") 0) (>= (Utilities|String|FindSubstring (Utilities|GetDisplayName _array_element) "LeftMesh") 0))
        (bind _asstaticmeshcomponent (Utilities|Casting|CastToStaticMeshComponent _array_element))
        (Components|StaticMesh|SetStaticMesh _asstaticmeshcomponent (Utilities|Select :Index _materialindex :Option%200 "/Game/PrimalEarth/Test_Efecto/Wood_Structure/Pillar/WoodPillar_Model.WoodPillar_Model" :Option%201 "/Game/PrimalEarth/Structures/Stone/Stone_Pillar/SM_Stone_Pillar.SM_Stone_Pillar" :Option%202 "/Game/PrimalEarth/Test_Efecto/Metal_Structures/Pillar/SM_Pillar.SM_Pillar" :Option%203 "/Game/ScorchedEarth/Structures/Adobe/Meshes/SM_AdobePillar.SM_AdobePillar" :Option%204 "/Game/PrimalEarth/TekTier/tek_pillar/tek_Pilar.tek_Pilar"))))
    (Rendering|SetVisibility (Variables|Default|GetLeftMesh2) (>= _height 2) false)
    (Rendering|SetVisibility (Variables|Default|GetLeftMesh3) (>= _height 3) false)
    (Rendering|SetVisibility (Variables|Default|GetRightMesh4) (>= _height 4) false)
    (Rendering|SetVisibility (Variables|Default|GetRightMesh5) (>= _height 5) false)
    (Rendering|SetVisibility (Variables|Default|GetRightMesh6) (>= _height 6) false)
    (Rendering|SetVisibility (Variables|Default|GetRightMesh7) (>= _height 7) false)
    (Rendering|SetVisibility (Variables|Default|GetRightMesh8) (>= _height 8) false)
    (Rendering|SetVisibility (Variables|Default|GetRightMesh9) (>= _height 9) false)
    (Rendering|SetVisibility (Variables|Default|GetRightMesh10) (>= _height 10) false)
    (Rendering|SetVisibility (Variables|Default|GetRightMesh11) (>= _height 11) false)
    (Rendering|SetVisibility (Variables|Default|GetRightMesh12) (>= _height 12) false)))

(fn CleanMultiuseEntries
  (params (EntriesIn :type Array%20of%20Multi%20Use%20Entry%20Structures))
  (bind (_item _index) (Utilities|SPforEachReverse EntriesIn)
    (:Loop
      (if (== (Utilities|Struct|BreakMultiUseEntry _item) 201)
        (Utilities|Array|RemoveIndex EntriesIn _index)
        (elif (== (Utilities|Struct|BreakMultiUseEntry _item) 203)
          (LocalVariables|SetEntry _item)
          (Utilities|Struct|SetmembersinMultiUseEntry (LocalVariables|GetEntry) 0 1.0 1.0)
          (Utilities|Array|SetArrayElem EntriesIn _index (LocalVariables|GetEntry)))))
    (:Completed
      (return EntriesIn))))

(fn OnRepIsCrafting
  (CallFunction|UpdateMaterials))

(fn UpdateMaterials
  (bind _gatewaydata (Variables|Default|GetGatewayData))
  (bind _leftmesh1 (Variables|Default|GetLeftMesh1))
  (bind _materialindex (Utilities|Struct|BreakSP_DynamicGatewayData _gatewaydata))
  (if (not (or (Networking|IsDedicatedServer) (Variables|Default|GetbIsPreviewStructure)))
    (Variables|Default|SetTargetableDamageFXDefaultPhysMaterial (Utilities|Select :Index _materialindex :Option%200 "Wood" :Option%201 "Rock" :Option%202 "Metal" :Option%203 "Rock" :Option%204 "Metal"))
    (if (Variables|Default|GetIsCrafting)
      (Rendering|Material|SetMaterial _leftmesh1 0 "/Game/Mods/StructuresPlusMod/_Materials/PreviewMaterial.PreviewMaterial")
      (else
        (bind _returnvalue (Rendering|Material|CreateDynamicMaterialInstance (Utilities|Select :Index _materialindex :Option%200 "/Game/PrimalEarth/Test_Efecto/Wood_Structure/Pillar/Pillar_Colorize_MIC.Pillar_Colorize_MIC" :Option%201 "/Game/PrimalEarth/Structures/Stone/Stone_Pillar/Stone_Pillar_Colorize_MIC.Stone_Pillar_Colorize_MIC" :Option%202 "/Game/PrimalEarth/Test_Efecto/Metal_Structures/Materials/IndividualPieces/Metal_Pillar_Colorize_MIC.Metal_Pillar_Colorize_MIC" :Option%203 "/Game/ScorchedEarth/Structures/Adobe/Material/MIC_Pillar_Plaster_Colorize.MIC_Pillar_Plaster_Colorize" :Option%204 "/Game/PrimalEarth/TekTier/tek_pillar/Tech_Pilar_Colorize_MIC.Tech_Pilar_Colorize_MIC") :!class /Script/Engine.KismetMaterialLibrary))
        (Rendering|Material|SetMaterial _leftmesh1 0 _returnvalue)))))

(fn SetCollision
  (bind _mystaticmesh (Variables|Default|GetMyStaticMesh))
  (bind _gatewaydata (Variables|Default|GetGatewayData))
  (Components|StaticMesh|SetStaticMesh _mystaticmesh (Utilities|Select :Index (- (Utilities|Struct|BreakSP_DynamicGatewayData _gatewaydata) 1) :Option%200 "/Game/Mods/StructuresPlusMod/Structures/Gateways/Dynamic/_Models/CM_Gateway_1.CM_Gateway_1" :Option%201 "/Game/Mods/StructuresPlusMod/Structures/Gateways/Dynamic/_Models/CM_Gateway_2.CM_Gateway_2" :Option%202 "/Game/Mods/StructuresPlusMod/Structures/Gateways/Dynamic/_Models/CM_Gateway_3.CM_Gateway_3" :Option%203 "/Game/Mods/StructuresPlusMod/Structures/Gateways/Dynamic/_Models/CM_Gateway_4.CM_Gateway_4" :Option%204 "/Game/Mods/StructuresPlusMod/Structures/Gateways/Dynamic/_Models/CM_Gateway_5.CM_Gateway_5" :Option%205 "/Game/Mods/StructuresPlusMod/Structures/Gateways/Dynamic/_Models/CM_Gateway_6.CM_Gateway_6" :Option%206 "/Game/Mods/StructuresPlusMod/Structures/Gateways/Dynamic/_Models/CM_Gateway_7.CM_Gateway_7" :Option%207 "/Game/Mods/StructuresPlusMod/Structures/Gateways/Dynamic/_Models/CM_Gateway_8.CM_Gateway_8" :Option%208 "/Game/Mods/StructuresPlusMod/Structures/Gateways/Dynamic/_Models/CM_Gateway_9.CM_Gateway_9" :Option%209 "/Game/Mods/StructuresPlusMod/Structures/Gateways/Dynamic/_Models/CM_Gateway_10.CM_Gateway_10" :Option%2010 "/Game/Mods/StructuresPlusMod/Structures/Gateways/Dynamic/_Models/CM_Gateway_11.CM_Gateway_11" :Option%2011 "/Game/Mods/StructuresPlusMod/Structures/Gateways/Dynamic/_Models/CM_Gateway_12.CM_Gateway_12"))
  (Transformation|SetRelativeScale3D _mystaticmesh (Math|Vector|MakeVector 1.0 1.0 (Math|Conversions|ToFloat(Integer) (Utilities|Struct|BreakSP_DynamicGatewayData _gatewaydata)))))

(fn BPAllowPickupGiveItem
  (params (ForPC :type Player%20Controller%20Object%20Reference))
  (return (Variables|Default|GetIsCrafting)))

(fn BlueprintDrawHUD
  (params (HUD :type Shooter%20HUD%20Object%20Reference) (CenterX :type Float%20%28single-precision%29) (CenterY :type Float%20%28single-precision%29))
  (if (Variables|Default|GetIsCrafting)
    (CallFunction|SPDrawDestructionTimer HUD CenterX CenterY (Variables|Default|GetDestructionTime))))

(fn BPUnstasis
  (bind _returnvalue (Class|VictoryCore|IsLoadingSaveGame))
  (if (not _returnvalue)
    (Networking|SwitchHasAuthority
      (:Authority
        (CallFunction|SetCollision)
        (if (Variables|Default|GetIsCrafting)
          (Utilities|Time|SetTimerbyFunctionName 0 "SelfDestructEvent" (Math|Conversions|ToFloat(Integer) (- (Variables|Default|GetDestructionTime) (Utilities|Time|GetGameTimeinSeconds)))))))))

(fn BPOverrideSnappedtoTransform
  (params (childStructure :type Primal%20Structure%20Object%20Reference) (ChildSnapFromIndex :type Integer) (UnsnappedPlacementPos :type Vector :default "0, 0, 0") (UnsnappedPlacementRot :type Rotator :default "0, 0, 0") (SnappedPlacementPos :type Vector :default "0, 0, 0") (SnappedPlacementRot :type Rotator :default "0, 0, 0") (SnapToIndex :type Integer))
  (bind _gatewaydata (Variables|Default|GetGatewayData))
  (bind (_width _height) (Utilities|Struct|BreakSP_DynamicGatewayData _gatewaydata))
  (Utilities|FlowControl|Sequence
    (:then_0
      (bind _asbp_gate_dynamic_c (Utilities|Casting|CastToBP_Gate_Dynamic childStructure))
      (if (!= (Variables|/Game/Mods/StructuresPlusMod/Doors/Gates/Dynamic/BP_Gate_Dynamic.BP_Gate_Dynamic_C|GetDoorScale _asbp_gate_dynamic_c) (Math|Vector|MakeVector (* _width (.x (Utilities|Array|Get(acopy) (Variables|Default|GetGateScales) (Utilities|Struct|BreakSP_DynamicGatewayData (Variables|/Game/Mods/StructuresPlusMod/Doors/Gates/Dynamic/BP_Gate_Dynamic.BP_Gate_Dynamic_C|GetGatewayData _asbp_gate_dynamic_c))))) 1.0 (* _height (.z (Utilities|Array|Get(acopy) (Variables|Default|GetGateScales) (Utilities|Struct|BreakSP_DynamicGatewayData (Variables|/Game/Mods/StructuresPlusMod/Doors/Gates/Dynamic/BP_Gate_Dynamic.BP_Gate_Dynamic_C|GetGatewayData _asbp_gate_dynamic_c)))))))
        (Variables|/Game/Mods/StructuresPlusMod/Doors/Gates/Dynamic/BP_Gate_Dynamic.BP_Gate_Dynamic_C|SetDoorScale _asbp_gate_dynamic_c (Math|Vector|MakeVector (* _width (.x (Utilities|Array|Get(acopy) (Variables|Default|GetGateScales) (Utilities|Struct|BreakSP_DynamicGatewayData (Variables|/Game/Mods/StructuresPlusMod/Doors/Gates/Dynamic/BP_Gate_Dynamic.BP_Gate_Dynamic_C|GetGatewayData _asbp_gate_dynamic_c))))) 1.0 (* _height (.z (Utilities|Array|Get(acopy) (Variables|Default|GetGateScales) (Utilities|Struct|BreakSP_DynamicGatewayData (Variables|/Game/Mods/StructuresPlusMod/Doors/Gates/Dynamic/BP_Gate_Dynamic.BP_Gate_Dynamic_C|GetGatewayData _asbp_gate_dynamic_c)))))) false)
        (Utilities|Struct|SetmembersinSP_DynamicGatewayData (Variables|/Game/Mods/StructuresPlusMod/Doors/Gates/Dynamic/BP_Gate_Dynamic.BP_Gate_Dynamic_C|GetGatewayData _asbp_gate_dynamic_c) _width _height)))
    (:then_1
      (return (- SnappedPlacementPos "0, 0,50.000000") SnappedPlacementRot 0 true))))

(fn BPOverrideCantBuildReasonString
  (params (CantBuildReason :type Integer))
  (return (Utilities|String|SelectString (Utilities|String|Append (Utilities|String|Append "You Require the S+ " (Utilities|Select :Index (Math|Integer|Clamp(Integer) (- 4 (+ CantBuildReason 115)) 0 4) :Option%200 "Wood" :Option%201 "Stone" :Option%202 "Metal" :Option%203 "Adobe" :Option%204 "Tek")) " Gateway Engram.") "" (and (<= CantBuildReason -111) (>= CantBuildReason -115)))))

(fn OnRepIsSnapAssistHidden
  (bind _gatesnapmesh (Variables|Default|GetGateSnapMesh))
  (bind _issnapassisthidden (Variables|Default|GetIsSnapAssistHidden))
  (Rendering|SetVisibility _gatesnapmesh (not _issnapassisthidden) false)
  (Collision|SetCollisionProfileName _gatesnapmesh (Utilities|String|StringToName (Utilities|String|SelectString "NoCollision" "BlockAllDynamic" _issnapassisthidden)) :!class /Script/Engine.PrimitiveComponent))

(fn IsValidSnapPointto
  (params (ChildStructure :type Primal%20Structure%20Object%20Reference) (MySnapPointToIndex :type Integer))
  (Utilities|FlowControl|Sequence
    (:then_0
      (if (not (Variables|/Script/ShooterGame.PrimalStructure|GetbIsPreviewStructure ChildStructure))
        (if (not (Variables|Default|GetIsSnapAssistHidden))
          (Variables|Default|SetIsSnapAssistHidden true true))))
    (:then_1
      (return true))))

(fn BPPostSetStructureCollisionChannels
  (Collision|SetCollisionProfileName (Variables|Default|GetGateSnapMesh) (Utilities|String|StringToName (Utilities|String|SelectString "NoCollision" "StructureWall" (Variables|Default|GetIsSnapAssistHidden))) :!class /Script/Engine.PrimitiveComponent))

(fn BPAdjustDamage
  (params (IncomingDamage :type Float%20%28single-precision%29) (TheDamageEvent :type Damage%20Event%20Structure) (EventInstigator :type Controller%20Object%20Reference) (DamageCauser :type Actor%20Object%20Reference) (bIsPointDamage :type Boolean) (PointHitInfo :type Hit%20Result%20Structure))
  (bind _outdamage (CallFunction|SPAdjustDamagetoDynamicStructure TheDamageEvent (Utilities|Struct|BreakSP_DynamicGatewayData (Variables|Default|GetGatewayData))))
  (return _outdamage))

(fn IDynamicGetIsCrafting
  (return (Variables|Default|GetIsCrafting)))

(fn IDynamicGetMaterials
  (return (Variables|Default|GetMaterialsRequired) (Variables|Default|GetMaterialsStored)))

(fn IDynamicGetPerUnitCraftCostArray
  (return (Variables|Default|GetCraftingCosts)))

(fn IDynamicGetStructure
  (return self))

(fn IDynamicSetDestructionTime
  (params (DestructionTime :type Float%20%28double-precision%29))
  (Variables|Default|SetDestructionTime DestructionTime true)
  (return true))

(fn IDynamicSetGatewayData
  (params (GatewayData :type SP%20Dynamic%20Gateway%20Data%20Structure))
  (Variables|Default|SetGatewayData GatewayData true)
  (return true))

(fn IDynamicSetIsCrafting
  (params (IsCrafting :type Boolean))
  (Variables|Default|SetIsCrafting IsCrafting true)
  (return true))

(fn IDynamicSetMaterials
  (params (TotalResources :type Array%20of%20Crafting%20Resource%20Requirement%20Structures) (StoredResources :type Array%20of%20Crafting%20Resource%20Requirement%20Structures))
  (Variables|Default|SetMaterialsRequired TotalResources true)
  (Variables|Default|SetMaterialsStored StoredResources true)
  (return false))

(fn IDynamicSetRepairCooldown
  (params (RepairCooldownTime :type Float%20%28double-precision%29))
  (Variables|Default|SetRepairCooldownTime RepairCooldownTime true)
  (return true))

(fn IDynamicSetStructureSettings
  (params (StructureSettings :type Primal%20Structure%20Settings%20Class%20Reference))
  (Variables|Default|SetStructureSettingsClass StructureSettings)
  (return true))